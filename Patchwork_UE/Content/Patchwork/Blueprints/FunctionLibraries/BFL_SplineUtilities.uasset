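; Blueprint function library of spline helpers for reading points, interpolating values and shaping sagging ropes.
; Lerp helpers remap alpha through an optional float or vector curve, falling back to linear.
; Query helpers gather spline points, segment endpoints and segment structs, and step indices with closed-loop awareness.
; A shared rope calculation derives tangents from distance, gravity direction and sag, feeding setters for spline meshes and two-point splines.
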(fn GetLastSplinePointonComponent
  (params (spline%20component :type Spline%20Component%20Object%20Reference) (CoordinateSpace :type ESplineCoordinateSpace%20Enum :default "Local"))
  (return (Spline|GetSplinePointAt spline%20component (- (Spline|GetNumberOfSplinePoints spline%20component) 1) CoordinateSpace)))

(fn LerpwithOptionalCurve
  (params (start :type Float%20%28double-precision%29) (end :type Float%20%28double-precision%29) (time :type Float%20%28double-precision%29) (obj :type Curve%20Float%20Object%20Reference))
  (if (Utilities|IsValid obj)
    (return (Math|Float|Lerp start end (Math|Curves|GetFloatValue obj time)))
    (else
      (return (Math|Float|Lerp start end time)))))

(fn LerpVectorwithOptionalCurve
  (params (start :type Vector) (end :type Vector) (time :type Float%20%28double-precision%29) (obj :type Curve%20Float%20Object%20Reference))
  (Utilities|IsValid obj
    (:Is%20Valid
      (return (Math|Vector|Lerp(Vector) start end (Math|Curves|GetFloatValue obj time))))
    (:Is%20Not%20Valid
      (return (Math|Vector|Lerp(Vector) start end time)))))

(fn LerpVectorwithOptionalVectorCurve
  (params (start :type Vector) (end :type Vector) (time :type Float%20%28double-precision%29) (obj :type Curve%20Vector%20Object%20Reference))
  (bind (_x _y _z) (Math|Vector|BreakVector end))
  (bind (_x_2 _y_2 _z_2) (Math|Vector|BreakVector start))
  (bind _returnvalue (Math|Curves|GetVectorValue obj time))
  (bind (_x_3 _y_3 _z_3) (Math|Vector|BreakVector _returnvalue))
  (if (Utilities|IsValid obj)
    (return (Math|Vector|MakeVector (Math|Float|Lerp _x_2 _x _x_3) (Math|Float|Lerp _y_2 _y _y_3) (Math|Float|Lerp _z_2 _z _z_3)))
    (else
      (return (Math|Vector|Lerp(Vector) start end time)))))

(fn GetAllSegmentPoints
  (params (component :type Spline%20Component%20Object%20Reference) (CoordinateSpace :type ESplineCoordinateSpace%20Enum :default "Local"))
  (bind _output_get (LocalVariables|Setspline component))
  (Utilities|IsValid _output_get
    (:Is%20Valid
      (LocalVariables|Setcordspace CoordinateSpace)
      (for _index (range 0 (- (Class|SplineComponent|GetNumberOfSplineSegments (LocalVariables|Getspline)) 1))
        (Utilities|FlowControl|Sequence
          (:then_0
            (bind _output_get_2 (LocalVariables|Setcurrent _index))
            (LocalVariables|Setnext (Math|Integer|%(Integer) (+ _output_get_2 1) (Spline|GetNumberOfSplinePoints (LocalVariables|Getspline)))))
          (:then_1
            (Utilities|Array|Add (LocalVariables|Getpts1) (Spline|GetSplinePointAt (LocalVariables|Getspline) (LocalVariables|Getcurrent) (LocalVariables|Getcordspace)))
            (Utilities|Array|Add (LocalVariables|Getpts2) (Spline|GetSplinePointAt (LocalVariables|Getspline) (LocalVariables|Getnext) (LocalVariables|Getcordspace))))))
      (return (LocalVariables|Getpts1) (LocalVariables|Getpts2)))
    (:Is%20Not%20Valid
      (return 0 0))))

(fn GetAllSplinePoints
  (params (component :type Spline%20Component%20Object%20Reference) (CoordinateSpace :type ESplineCoordinateSpace%20Enum :default "Local"))
  (bind _output_get (LocalVariables|Setspline component))
  (Utilities|IsValid _output_get
    (:Is%20Valid
      (LocalVariables|Setcordspace CoordinateSpace)
      (for _index (range 0 (- (Class|SplineComponent|GetNumberOfSplineSegments (LocalVariables|Getspline)) 1))
        (Utilities|FlowControl|Sequence
          (:then_0
            (bind _output_get_2 (LocalVariables|Setcurrent _index))
            (LocalVariables|Setnext (Math|Integer|%(Integer) (+ _output_get_2 1) (Spline|GetNumberOfSplinePoints (LocalVariables|Getspline)))))
          (:then_1
            (Utilities|Array|Add (LocalVariables|Getpts1) (Spline|GetSplinePointAt (LocalVariables|Getspline) (LocalVariables|Getcurrent) (LocalVariables|Getcordspace))))))
      (return (LocalVariables|Getpts1)))
    (:Is%20Not%20Valid
      (return 0))))

(fn GetAllSplineSegments
  (params (component :type Spline%20Component%20Object%20Reference) (CoordinateSpace :type ESplineCoordinateSpace%20Enum :default "Local"))
  (bind (_p0 _p1) (Splines|GetAllSegmentPoints component CoordinateSpace (LocalVariables|Get__WorldContext)))
  (if (> (Utilities|Array|Length _p0) 0)
    (for _array_element _p0
      (Utilities|Array|Add (LocalVariables|Getsegs) (Utilities|Struct|MakeS_SplineSegment _array_element (Utilities|Array|Get(acopy) _p1) (- (.Position (Utilities|Struct|BreakSplinePoint (Utilities|Array|Get(acopy) _p1))) (.Position (Utilities|Struct|BreakSplinePoint _array_element))))))
    (else
      (return 0))))

(fn GetNextSplineIndex
  (params (component :type Spline%20Component%20Object%20Reference) (current%20index :type Integer) (index%20count :type Integer) (increment :type Integer))
  (LocalVariables|Settotal index%20count)
  (LocalVariables|SetnextIndex (+ current%20index increment))
  (Utilities|IsValid component
    (:Is%20Valid
      (if (or (and (>= (LocalVariables|GetnextIndex) (LocalVariables|Gettotal)) (> increment 0)) (and (< (LocalVariables|GetnextIndex) 0) (< increment 0)))
        (return (LocalVariables|GetnextIndex) true)
        (elif (Class|SplineComponent|IsClosedLoop component)
          (return (Math|Integer|%(Integer) (LocalVariables|GetnextIndex) (LocalVariables|Gettotal)) true)
          (else
            (return -1 false)))))
    (:Is%20Not%20Valid
      (return -1 false))))

(fn CalculateRopeTangents
  (params (StartPosition :type Vector) (EndPosition :type Vector) (GravityDirection :type Vector :default "0.000000,0.000000,-1.000000") (Sag :type Float%20%28double-precision%29) (SagLength :type Float%20%28double-precision%29))
  (bind _output_get (LocalVariables|Setdelta (- EndPosition StartPosition)))
  (LocalVariables|SetDist (Math|Vector|VectorLength _output_get))
  (LocalVariables|SetDir (Math|Vector|Normalize (LocalVariables|Getdelta)))
  (return (+ (- (+ (* (LocalVariables|GetDir) (* (LocalVariables|GetDist) SagLength)) (* (* GravityDirection -1.0) (* (LocalVariables|GetDist) Sag))) (* (Math|Vector|DotProduct (+ (* (LocalVariables|GetDir) (* (LocalVariables|GetDist) SagLength)) (* (* GravityDirection -1.0) (* (LocalVariables|GetDist) Sag))) GravityDirection) GravityDirection)) (* (* (Math|Vector|DotProduct (+ (* (LocalVariables|GetDir) (* (LocalVariables|GetDist) SagLength)) (* (* GravityDirection -1.0) (* (LocalVariables|GetDist) Sag))) GravityDirection) GravityDirection) -1.0)) (+ (* (LocalVariables|GetDir) (* (LocalVariables|GetDist) (- 1.0 SagLength))) (* (* GravityDirection -1.0) (* (LocalVariables|GetDist) Sag)))))

(fn SetRopeTangents
  (params (StartPosition :type Vector) (EndPosition :type Vector) (GravityDirection :type Vector :default "0.000000,0.000000,-1.000000") (Sag :type Float%20%28double-precision%29) (offset :type Float%20%28double-precision%29) (SplineMesh :type Spline%20Mesh%20Component%20Object%20Reference))
  (bind (_starttangent _endtangent) (Rope|CalculateRopeTangents StartPosition EndPosition GravityDirection Sag offset (LocalVariables|Get__WorldContext)))
  (SplineMesh|SetStartandEnd SplineMesh StartPosition _starttangent EndPosition _endtangent true :!class /Script/Engine.SplineMeshComponent)
  (return))

(fn SetRopeSpineTangents
  (params (StartPosition :type Vector) (EndPosition :type Vector) (GravityDirection :type Vector :default "0.000000,0.000000,-1.000000") (Sag :type Float%20%28double-precision%29) (SagLength :type Float%20%28double-precision%29) (Spline :type Spline%20Component%20Object%20Reference))
  (Spline|SetLocationatSplinePoint Spline 0 StartPosition "World" false)
  (Spline|SetLocationatSplinePoint Spline 1 EndPosition "World" false)
  (bind (_starttangent _endtangent) (Rope|CalculateRopeTangents StartPosition EndPosition GravityDirection Sag SagLength (LocalVariables|Get__WorldContext)))
  (Spline|SetTangentsatSplinePoint Spline 0 (Math|Vector|NegateVector _starttangent) _starttangent "World" false)
  (Spline|SetTangentsatSplinePoint Spline 1 _endtangent (Math|Vector|NegateVector _endtangent) "World" true))