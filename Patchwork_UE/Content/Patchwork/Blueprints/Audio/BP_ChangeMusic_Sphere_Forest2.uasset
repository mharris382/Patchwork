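; BP_ChangeMusic_Sphere_Forest2 is a spherical music-change trigger, named for a forest area, that inherits its overlap response from a parent class.
; Five seconds after BeginPlay, it finds Paperperson_ledge_grab actors already inside the Sphere and manually runs the parent's ActorBeginOverlap for each.
; The Blueprint's own overlap and Tick events are disabled stubs, and its construction script only calls the parent.
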(event EventBeginPlay
  (|CallParentFunction)
  (Utilities|FlowControl|Delay 5.0)
  (for _array_element (Collision|GetOverlappingActors (Variables|Default|GetSphere) "/Game/Patchwork/Blueprints/Core/Pawns/paperperson_ledge_grab.paperperson_ledge_grab_C" :!class /Script/Engine.PrimitiveComponent)
    (|CallParentFunction _array_element)))

(event Collision|EventActorBeginOverlap
  (params (OtherActor :type Actor%20Object%20Reference))
  (|CallParentFunction OtherActor) ; This node is disabled and will not be called.\nDrag off pins to build functionality.
)

(event EventTick
  (params (DeltaSeconds :type Float%20%28single-precision%29))
  (|CallParentFunction DeltaSeconds) ; This node is disabled and will not be called.\nDrag off pins to build functionality.
)

(fn ConstructionScript
  (|CallParentFunction))