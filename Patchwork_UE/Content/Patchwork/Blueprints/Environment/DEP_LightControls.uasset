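; DEP_LightControls is a switch-driven environment actor that toggles the forest's nighttime lighting state.
; On BeginPlay it caches the referenced sky light's intensity and fog's density.
; SetSwitchValue zeroes both immediately when on; when off, it restores them after a brief delay, only if still off.
; The same event also writes the switch state to GM_ForestGameMode's IsNighttime flag, without waiting for the delay.
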(event EventBeginPlay
  (Variables|Default|SetDefault%20Intensity (Variables|/Script/Engine.LightComponentBase|GetIntensity (Variables|/Script/Engine.SkyLight|GetLightComponent (Variables|Default|GetSkyLightRef))))
  (Variables|Default|SetFog%20Density (Variables|/Script/Engine.ExponentialHeightFogComponent|GetFogDensity (Variables|/Script/Engine.ExponentialHeightFog|GetComponent (Variables|Default|GetFogRef)))))

(event Collision|EventActorBeginOverlap
  (params (OtherActor :type Actor%20Object%20Reference)))

(event EventTick
  (params (DeltaSeconds :type Float%20%28single-precision%29)))

(event EventSetSwitchValue
  (params (is%20On :type Boolean))
  (bind _fogref (Variables|Default|GetFogRef))
  (bind _skylightref (Variables|Default|GetSkyLightRef))
  (bind _lightcomponent (Variables|/Script/Engine.SkyLight|GetLightComponent _skylightref))
  (bind _component (Variables|/Script/Engine.ExponentialHeightFog|GetComponent _fogref))
  (bind _output_get (Variables|Default|SetIs%20On is%20On))
  (Utilities|FlowControl|Sequence
    (:then_0
      (if _output_get
        (Rendering|Components|Light|SetIntensity _lightcomponent 0.0)
        (Class|ExponentialHeightFogComponent|SetFogDensity _component 0.0)
        (else
          (Utilities|FlowControl|Delay 0.1)
          (if (not (Variables|Default|GetIs%20On))
            (Rendering|Components|Light|SetIntensity _lightcomponent (Variables|Default|GetDefault%20Intensity))
            (Class|ExponentialHeightFogComponent|SetFogDensity _component (Variables|Default|GetFog%20Density))))))
    (:then_1
      (bind _asgm_forest_game_mode (Utilities|Casting|CastToGM_ForestGameMode (Game|GetGameMode)))
      (Variables|/Game/Patchwork/Blueprints/Core/Gamemodes/GM_ForestGameMode.GM_ForestGameMode_C|SetIs%20Nighttime _asgm_forest_game_mode (Variables|Default|GetIs%20On)))))

(fn ConstructionScript)