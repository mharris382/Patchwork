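; Spore effect that alters its owning character's gravity while spore toxicity is active.
; Each tick it sets gravity scale from toxicity, either as a constant switch or a curve blend plus summed GravityModifier components.
; It pushes the character along its GravityVector direction, scaling force, falling friction and braking by how vertical that direction is.
; Zero toxicity restores gravity scale and braking; slowdown and lateral steering forces are left unwired.
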(event Custom|Update%20Aerial%20Friction
  (params (LateralAerialFriction :type Float%20%28double-precision%29) (Dt :type Float%20%28double-precision%29))
  (bind _gameplaystatecomponent (Variables|Default|GetGameplayStateComponent)
    (:then
      (Variables|Default|SetTargetAerialFriction LateralAerialFriction)
      (bind _output_get (Variables|Default|SetCurrentAerialFriction (Math|Interpolation|FInterpTo (Variables|Default|GetCurrentAerialFriction) (Variables|Default|GetTargetAerialFriction) Dt 15.0)))
      (if (not (GameplayTags|HasTag (Variables|/Game/Patchwork/Blueprints/Utilities/GameplayObjectState.GameplayObjectState_C|GetGameplayState _gameplaystatecomponent) "(TagName=\"Gameplay.State.Grappling\")"))
        (Class|BPIPlayerPawn|SetPlayerFallingLateralFriction(Message) (Game|Player|GetPlayerPawn 0) _output_get)))
    (:else)))

(event EventBeginPlay
  (|CallParentFunction)
  (bind _ascharacter (Utilities|Casting|CastToCharacter (Components|GetOwner)))
  (bind _output_get (Variables|Default|Setowner%20character _ascharacter))
  (bind _fallinglateralfriction (Class|BPIPlayerPawn|GetPlayerFallingLateralFriction(Message) _output_get))
  (Variables|Default|SetDefaultFallingFriction _fallinglateralfriction)
  (Variables|Default|SetGravityVector (Actor|GetComponentbyClass _output_get "/Game/Patchwork/Blueprints/Core/Pawns/Abilities/System/GravityVector.GravityVector_C"))
  (Variables|Default|SetGameplayStateComponent (Actor|GetComponentbyClass _output_get "/Game/Patchwork/Blueprints/Levels/forest/Utilities/BP_SporeCarrier.BP_SporeCarrier_C"))
  (Utilities|FlowControl|Sequence
    (:then_0
      (Variables|Default|Setnormal%20gravity (Variables|/Script/Engine.CharacterMovementComponent|GetGravityScale (Variables|/Script/Engine.Character|GetCharacterMovement _output_get))))
    (:then_1
      (bind _fallinglateralfriction_2 (Class|BPIPlayerPawn|GetPlayerFallingLateralFriction(Message) (Variables|Default|Getowner%20character)))
      (bind _output_get_2 (Variables|Default|SetNormal%20Falling%20Lateral%20Friction _fallinglateralfriction_2))
      (bind _output_get_3 (Variables|Default|SetCurrentAerialFriction _output_get_2))
      (Variables|Default|SetTargetAerialFriction _output_get_3))
    (:then_2
      (Variables|Default|SetMaxLateralSpeedSqr (Math|Float|Power (Variables|Default|GetMaxLateralSpeed) 2.0)))))

(event EventTick
  (params (DeltaSeconds :type Float%20%28single-precision%29))
  (|CallParentFunction DeltaSeconds)
  (if (> (Variables|Default|GetCurrent%20Toxicity) 0.0)
    (CallFunction|OnToxicityChanged (Variables|Default|GetCurrent%20Toxicity))
    (else
      (Class|BPIPlayerPawn|SetPlayerGravityScale(Message) (Components|GetOwner) (Variables|Default|Getnormal%20gravity))
      (Variables|/Script/Engine.CharacterMovementComponent|SetBrakingFrictionFactor (Variables|/Script/Engine.Character|GetCharacterMovement (Variables|Default|Getowner%20character)) 1.0))))

(fn OnToxicityChanged
  (params (new%20toxicity :type Float%20%28double-precision%29))
  (bind _owner_character (Variables|Default|Getowner%20character))
  (bind _gravityvector (Variables|Default|GetGravityVector))
  (bind _gravitydirection (Variables|/Game/Patchwork/Blueprints/Core/Pawns/Abilities/System/GravityVector.GravityVector_C|GetGravityDirection _gravityvector))
  (bind _returnvalue (Math|Vector|DotProduct _gravitydirection "0.000000,0.000000,1.000000"))
  (bind _returnvalue_2 (Math|Float|Absolute(Float) _returnvalue))
  (bind _output_get (LocalVariables|Settoxicity new%20toxicity))
  (|CallParentFunction _output_get)
  (Utilities|IsValid (Variables|Default|Getowner%20character)
    (:Is%20Valid
      (Utilities|FlowControl|Sequence
        (:then_0
          (LocalVariables|SetTargetGravity (Variables|Default|Getfinal%20gravity)))
        (:then_1
          (if (Variables|Default|GetUseConstantGravity)
            (LocalVariables|SetGravityScale (Math|Float|SelectFloat (LocalVariables|GetTargetGravity) (Variables|Default|Getnormal%20gravity) (> (LocalVariables|Gettoxicity) 0.05)))
            (else
              (bind _total (CallFunction|GetGravityModifier))
              (LocalVariables|SetGravityScale (+ _total (Math|Float|Lerp (Variables|Default|Getnormal%20gravity) (LocalVariables|GetTargetGravity) (Math|Curves|GetFloatValue (Variables|Default|Getgrav%20curve) (LocalVariables|Gettoxicity))))))))
        (:then_3
          (if (> (Variables|Default|GetCurrent%20Toxicity) 0.0)
            (Utilities|FlowControl|Sequence
              (:then_0)
              (:then_1)
              (:then_2
                (Utilities|DebugDirection (* _gravitydirection 255.0) "(R=1.000000,G=0.000000,B=0.621895,A=1.000000)" 0.1)
                (Class|BPIPlayerPawn|AddForce(Message) (Variables|Default|Getowner%20character) (* _gravitydirection (Math|Float|Lerp (Variables|Default|GetActualGravityForceLateral) (Variables|Default|GetActualGravityForceUp) _returnvalue_2) (Variables|/Game/Patchwork/Blueprints/Utilities/BP_GlobalAbilitySettings.BP_GlobalAbilitySettings_C|GetPlayerGravityMultiplier (Variables|Default|GetGlobalAbilitySettings))))
                (Class|BPIPlayerPawn|SetPlayerFallingLateralFriction(Message) _owner_character (Math|Float|Lerp (Variables|Default|GetDefaultFallingFriction) 0.0 _returnvalue_2))
                (Variables|/Script/Engine.CharacterMovementComponent|SetBrakingFrictionFactor (Variables|/Script/Engine.Character|GetCharacterMovement _owner_character) (Math|Float|Lerp 1.0 0.0 _returnvalue_2))))))
        (:then_5
          (Class|BPIPlayerPawn|SetPlayerGravityScale(Message) (Components|GetOwner) (LocalVariables|GetGravityScale)))))))

(fn GetGravityModifier
  (LocalVariables|Setsum 0.0)
  (for _array_element (Actor|GetComponentsByClass (Variables|Default|Getowner%20character) "/Game/Patchwork/Blueprints/Utilities/GravityModifier.GravityModifier_C")
    (LocalVariables|Setsum (+ (Variables|/Game/Patchwork/Blueprints/Utilities/GravityModifier.GravityModifier_C|GetAmount _array_element) (LocalVariables|Getsum))))
  (return (LocalVariables|Getsum)))