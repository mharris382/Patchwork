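; Pooled bouncy mushroom that launches characters, including a player it respawns under, with scale-in/out timelines and removal on player death.
; Bouncing fires a short-lived Chaos field, drives a material parameter collection and rescales force against opposing horizontal velocity.
; A spore carrier component feeds Niagara visuals and attached spore actors, while Iron spores or bounce timing set reported mass.
; It lights up in darkness areas and contains an experimental, uncalled camera quick-turn.
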(event Custom|Despawn
  ;[0.6233 0.6233 0.6233 0.5] Despawn
  (CallFunction|StopBounceCurve)
  (CallFunction|ClearVisuals)
  (Default|ResetSpores (Variables|Default|GetBP_SporeCarrierController))
  (Variables|Default|Setis%20spawned false)
  (Utilities|FlowControl|DoOnce false
    (:Completed
      (bind _scale (Timeline|Despawn%20Timeline Play)
        (:Update
          (Transformation|SetActorScale3D (Math|Conversions|ToVector(Float) _scale)))
        (:Finished
          (Default|CallReturntoPool self))))))

(event Custom|Respawn%20From
  (params (transform :type Transform))
  (Transformation|SetActorTransform transform)
  (Rendering|SetVisibility (Variables|Default|GetStaticMesh) true false)
  ;[0.6233 0.6233 0.6233 0.5] Spawning
  (Utilities|FlowControl|Sequence
    (:then_0
      ;[0.6233 0.6233 0.6233 0.5] Check for Spawned Under Player Pawn
      (bind (_outactors _returnvalue) (Collision|SphereOverlapActors (Transformation|GetActorLocation) 1e+02 (Utilities|Array|MakeArray "ObjectTypeQuery3" "ObjectTypeQuery8") "/Game/Patchwork/Blueprints/Core/Pawns/paperperson.paperperson_C"))
      (if (and _returnvalue (> (Utilities|Array|Length _outactors) 0))
        (CallFunction|SpawnedUnderPlayer)))
    (:then_1
      (Utilities|FlowControl|Sequence
        (:then_0
          (bind _scale (Timeline|Spawn%20Timeline PlayFromStart)
            (:Update
              (Transformation|SetRelativeScale3D (Variables|Default|GetMushroomPivot) (Math|Conversions|ToVector(Float) _scale)))))
        (:then_1
          (CallFunction|OnSpawned))
        (:then_2
          (Utilities|FlowControl|Delay 0.2)
          (Variables|Default|Setis%20spawned true))))))

(event Custom|SpawnedUnderPlayer
  ;[0.6233 0.6233 0.6233 0.5] Spawned Under Player Pawn
  (Utilities|FlowControl|Delay 0.1)
  (CallFunction|BounceCharacter (Game|Player|GetPlayerPawn 0)))

(event Custom|StopBounceCurve
  (Utilities|FlowControl|Sequence
    (:then_0
      (bind (_direction _bounce _bouncetimer) (Timeline|BounceColorVFX Stop)
        (:Update
          (Rendering|Material|SetScalarParameterValue "/Game/Patchwork/Models/Abilities/JumpShroom/MPC_BounceMushroom.MPC_BounceMushroom" "BounceAmount" _bounce :!class /Script/Engine.KismetMaterialLibrary)
          (Variables|Default|SetBounce%20Timer _bouncetimer))))
    (:then_1
      (Rendering|Material|SetScalarParameterValue "/Game/Patchwork/Models/Abilities/JumpShroom/MPC_BounceMushroom.MPC_BounceMushroom" "BounceAmount" 0.0 :!class /Script/Engine.KismetMaterialLibrary)
      (Variables|Default|SetBounce%20Timer 0.0))))

(event Custom|On%20Spawned
  ;[0.6233 0.6233 0.6233 0.5] Despawn
  (Utilities|FlowControl|Sequence
    (:then_0
      (Utilities|FlowControl|DoOnce false) ; enters at Reset
    )
    (:then_1
      (bind _scale (Timeline|Despawn%20Timeline Stop)
        (:Update
          (Transformation|SetActorScale3D (Math|Conversions|ToVector(Float) _scale)))
        (:Finished
          (Default|CallReturntoPool self))))
    (:then_2
      ;[0.6233 0.6233 0.6233 0.5] Darknes Area
      (if (> (Utilities|Array|Length (Collision|GetOverlappingActors "/Game/Patchwork/Blueprints/Environment/DarknessArea.DarknessArea_C" :!class /Script/Engine.Actor)) 0)
        (Class|BPIDarknessListener|SetInsideDarkness(Message) self true)))
    (:then_3
      (CallFunction|SetupVisualsforSpore))))

(event Custom|CustomEvent
  ;[0.6233 0.6233 0.6233 0.5] Begin
  ;;[0.6233 0.6233 0.6233 0.5] Destroy on player long fall
  (Actor|DestroyActor))

(event EventBounceCharacter
  (params (actor :type Actor%20Object%20Reference))
  ;[0.6233 0.6233 0.6233 0.5] Bounce Character
  (|CallParentFunction actor)
  (Utilities|FlowControl|Sequence
    (:then_0
      (if (== actor (Game|Player|GetPlayerPawn 0))
        (Default|CallOnPlayerMushBounced (CallFunction|GetBaseGameMode) self)))
    (:then_1
      (bind _can_bounce (CallFunction|CanBounce actor))
      (if _can_bounce
        (Development|PrintString "Bounced")
        (bind (_direction _bounce _bouncetimer) (Timeline|BounceColorVFX PlayFromStart)
          (:Update
            (Rendering|Material|SetScalarParameterValue "/Game/Patchwork/Models/Abilities/JumpShroom/MPC_BounceMushroom.MPC_BounceMushroom" "BounceAmount" _bounce :!class /Script/Engine.KismetMaterialLibrary)
            (Variables|Default|SetBounce%20Timer _bouncetimer)))))))

(event EventBeginPlay
  ;[0.6233 0.6233 0.6233 0.5] Begin
  (|CallParentFunction)
  (Utilities|FlowControl|Sequence
    (:then_0
      ;[0.6233 0.6233 0.6233 0.5] Cache spore helper
      (Variables|Default|SetSporeHelper (Actor|GetComponentbyClass (Game|GetGameMode) "/Game/Patchwork/Blueprints/Levels/forest/BP_GlobalSporeHelper.BP_GlobalSporeHelper_C")))
    (:then_1
      (|SporeTransportMechanisms))
    (:then_2
      ;;[0.6233 0.6233 0.6233 0.5] Destroy on player long fall
      (EventDispatchers|BindEventtoOnPlayerDeathOccured (CallFunction|GetBaseGameMode) (delegate Custom|CustomEvent)))
    (:then_3
      ;[0.6233 0.6233 0.6233 0.5] Spawning
      (bind _scale (Timeline|Spawn%20Timeline PlayFromStart)
        (:Update
          (Transformation|SetRelativeScale3D (Variables|Default|GetMushroomPivot) (Math|Conversions|ToVector(Float) _scale)))))
    (:then_4
      (CallFunction|ClearVisuals))))

(event EventDestroyed)

(event EventSetInsideDarkness
  (params (is%20inside%20darkness :type Boolean))
  (Rendering|SetVisibility (Variables|Default|GetPointLight) is%20inside%20darkness false))

(event Custom|go%20to%20rotation
  ;[0.6233 0.3134 0 0.5] Experimental - Skill Based Spin Bounce Mechanic
  (if (not (Utilities|Enum|Equal(Enum) (Variables|/Game/Patchwork/Blueprints/Core/Pawns/paperperson.paperperson_C|GetMovement%20Mode (.AsPaperperson (Utilities|Casting|CastTopaperperson (CallFunction|GetBasePlayerPawn)))) "NewEnumerator0"))
    (CallFunction|StopQuickTurn)
    (Utilities|Time|ClearandInvalidateTimerbyHandle (Variables|Default|Getrotation))))

(event Custom|start%20quick%20turn
  (bind _returnvalue (Game|GetPlayerController 0))
  (bind _returnvalue_2 (Pawn|GetControlRotation _returnvalue :!class /Script/Engine.Controller))
  ;[0.6233 0.3134 0 0.5] Experimental - Skill Based Spin Bounce Mechanic
  (Utilities|FlowControl|Sequence
    (:then_0
      (bind _t (Timeline|Timeline PlayFromStart)
        (:Update
          (Pawn|SetControlRotation _returnvalue (Math|Rotator|MakeRotator (.roll _returnvalue_2) (.pitch _returnvalue_2) (Math|Float|Lerp (Variables|Default|GetStart%20Yaw) (Variables|Default|Getdesired%20yaw) _t))))
        (:Finished
          (Utilities|ClearTimer))))
    (:then_1
      (Utilities|ClearTimer)
      (bind _returnvalue_3 (Utilities|Time|SetTimerbyEvent (delegate Custom|go%20to%20rotation) 0.1 true true))
      (Variables|Default|Setrotation _returnvalue_3))))

(event Custom|Stop%20quick%20turn
  (bind _returnvalue (Game|GetPlayerController 0))
  (bind _returnvalue_2 (Pawn|GetControlRotation _returnvalue :!class /Script/Engine.Controller))
  ;[0.6233 0.3134 0 0.5] Experimental - Skill Based Spin Bounce Mechanic
  (Utilities|ClearTimer)
  (bind _t (Timeline|Timeline Stop)
    (:Update
      (Pawn|SetControlRotation _returnvalue (Math|Rotator|MakeRotator (.roll _returnvalue_2) (.pitch _returnvalue_2) (Math|Float|Lerp (Variables|Default|GetStart%20Yaw) (Variables|Default|Getdesired%20yaw) _t))))
    (:Finished
      (Utilities|ClearTimer))))

(event Custom|check%20for%20quick%20turn
  (bind _base_character (CallFunction|GetBasePlayerPawn))
  (bind _launch_direction (Variables|Default|GetLaunch%20Direction))
  (bind _returnvalue (Math|Vector|GetForwardVector _launch_direction))
  (bind _camera (Variables|/Game/Patchwork/Blueprints/Core/Pawns/BP_BaseCharacter.BP_BaseCharacter_C|GetCamera _base_character))
  (bind _returnvalue_2 (Math|Vector|GetForwardVector _camera))
  ;[0.6233 0.3134 0 0.5] Experimental - Skill Based Spin Bounce Mechanic
  (bind _output_get (Variables|Default|Setlaunch%20forward%20direction _returnvalue))
  (if (not (> (Math|Float|Absolute(Float) (Math|Vector|DotProduct _output_get "0.000000,0.000000,1.000000")) 0.1)) ; check if pointing close to up
    (if (< (Math|Vector|DotProduct (Math|Vector|Normalize (* _returnvalue "1.000000,1.000000,0.000000")) (Math|Vector|Normalize (* _returnvalue_2 "1.000000,1.000000,0.000000"))) -0.2) ; looking opposite to bounce direction
      (Variables|Default|SetStart%20Yaw (.yaw (Math|Conversions|RotationFromXVector _returnvalue_2)))
      (Variables|Default|Setdesired%20yaw (.yaw (Math|Conversions|RotationFromXVector _returnvalue)))
      (CallFunction|StartQuickTurn)
      (CallFunction|StartQuickTurn))))

(event Custom|Trigger%20Bounce%20Field
  (bind _mushroompivot (Variables|Default|GetMushroomPivot))
  (bind _returnvalue (Transformation|GetWorldTransform _mushroompivot))
  ;[0.6233 0.6233 0.6233 0.5] Trigger Bounce Chaos Field
  (bind _returnvalue_2 (Game|SpawnActorfromClass "/Game/Patchwork/Blueprints/Core/Pawns/Abilities/MushroomBounceField.MushroomBounceField_C" (Math|Transform|MakeTransform (.location _returnvalue) (.rotation _returnvalue) "4.000000,4.000000,4.000000") "Undefined" "OverrideRootScale" self 0))
  (Default|CETrigger _returnvalue_2)
  (Utilities|FlowControl|Delay 0.2)
  (Actor|DestroyActor _returnvalue_2))

(event EventBounce
  ;[0.6233 0.6233 0.6233 0.5 32] Bounce
  (Utilities|FlowControl|Sequence
    (:then_0
      (|CallParentFunction))
    (:then_1
      (Audio|PlaySoundatLocation "/Game/Patchwork/Audio/Global_SFX/Abilities/BounceShroom/MS_BounceShroom_Jump_Container.MS_BounceShroom_Jump_Container" (Transformation|GetActorLocation) "0, 0, 0" 1.0 1.0 0.0 0 0 0 0))
    (:then_2
      (CallFunction|TriggerBounceField))))

(event Custom|Try%20Spawn%20Temporary%20Spore%20Field
  (bind _bp_sporecarriercontroller (Variables|Default|GetBP_SporeCarrierController))
  (bind _sporecollection (Variables|/Game/Patchwork/Blueprints/Levels/forest/Utilities/BP_SporeCarrier.BP_SporeCarrier_C|GetSporeCollection _bp_sporecarriercontroller))
  (if (> (GameplayTags|GetNumGameplayTagsinContainer _sporecollection) 0)
    (for _array_element (GameplayTags|BreakGameplayTagContainer _sporecollection)
      (bind _returnvalue (Game|SpawnActorfromClass "/Game/Patchwork/Blueprints/Levels/forest/Spores/BP_SporeRegion_Sphere.BP_SporeRegion_Sphere_C" (Math|Transform|MakeTransform (Transformation|GetWorldLocation (Variables|Default|GetMushroomPivot)) "0, 0, 0" "1.000000,1.000000,1.000000") "Undefined" "MultiplyWithRoot" (Game|Player|GetPlayerPawn 0) 0))
      (Variables|/Game/Patchwork/Blueprints/Levels/forest/Spores/BP_SporeRegion.BP_SporeRegion_C|SetSporeTypeTag _returnvalue _array_element)
      (Default|ChangeSporeType _returnvalue (Utilities|Struct|MakeDataTableRowHandle "/Game/Patchwork/Data/Datatables/DT_SporeEffects.DT_SporeEffects" (.SporeName (Default|GetSporeNamefromTag (Variables|Default|GetSporeHelper) _array_element))))
      (Variables|/Game/Patchwork/Blueprints/Levels/forest/Spores/BP_SporeRegion.BP_SporeRegion_C|SetSporeTypeTag _returnvalue _array_element)
      (Actor|SetLifeSpan _returnvalue 5.0))))

(fn ConstructionScript)

(fn GetBounceForce
  (params (direction :type Vector :default "0, 0, 0") (look%20direction :type Vector :default "0, 0, 0") (character%20velocity :type Vector :default "0, 0, 0") (is%20player :type Boolean))
  (bind _returnvalue (Math|Vector|DotProduct direction "0.000000,0.000000,1.000000"))
  (bind _amount (|CallParentFunction direction look%20direction character%20velocity is%20player))
  (bind _returnvalue_2 (Utilities|RemoveZ direction))
  (bind _returnvalue_3 (Utilities|RemoveZ character%20velocity))
  (bind _returnvalue_4 (Math|Vector|DotProduct _returnvalue_2 _returnvalue_3))
  (if (and (< (Math|Float|Absolute(Float) _returnvalue) 0.5) (> _returnvalue 0.0))
    (return _amount)
    (else
      (return (Math|Float|SelectFloat (* _amount (Math|Float|MapRangeClamped (Math|Float|Absolute(Float) _returnvalue_4) 0.0 1.0 1.0 (Variables|Forces|GetBounce%20Force%20Scale%20when%20changing%20direction))) _amount (< _returnvalue_4 0.0))))))

(fn SetupVisualsforSpore
  (bind _ns_bm (Variables|Default|GetNS_BM))
  (bind _bp_sporecarriercontroller (Variables|Default|GetBP_SporeCarrierController))
  (if (Default|HasAnySpores _bp_sporecarriercontroller)
    (Components|Activation|SetActive _ns_bm true true)
    (Rendering|SetVisibility _ns_bm true false)
    (bind _sporehelper (Variables|Default|GetSporeHelper)
      (:then
        _)
      (:else
        (Variables|Default|SetSporeHelper (Actor|GetComponentbyClass (Game|GetGameMode) "/Game/Patchwork/Blueprints/Levels/forest/BP_GlobalSporeHelper.BP_GlobalSporeHelper_C"))))
    (bind _success (Default|ApplySporetoNiagaraSystem _sporehelper (Utilities|Array|Get(acopy) (GameplayTags|BreakGameplayTagContainer (Variables|/Game/Patchwork/Blueprints/Levels/forest/Utilities/BP_SporeCarrier.BP_SporeCarrier_C|GetSporeCollection _bp_sporecarriercontroller))) _ns_bm))
    (if _success
      _)
    (else
      (CallFunction|ClearVisuals))))

(fn ClearVisuals
  (bind _ns_bm (Variables|Default|GetNS_BM))
  (Components|Activation|SetActive _ns_bm false false)
  (Rendering|SetVisibility _ns_bm false false))

(event Custom|gained%20spore
  (params (type :type Name) (source :type BPI%20Spore%20Contagion%20Interface) (instigator :type Actor%20Object%20Reference))
  ;[0.02438 0.6233 0 0.5] Gained Spore
  (Utilities|GetDataTableRow "/Game/Patchwork/Data/Datatables/DT_SporeEffects.DT_SporeEffects" type
    (:then
      (bind _returnvalue (Game|SpawnActorfromClass "/Game/Patchwork/Blueprints/Levels/forest/Spores/BP_Spore_Spawned.BP_Spore_Spawned_C" (Transformation|GetActorTransform) "Undefined" "MultiplyWithRoot" 0 0))
      (Variables|/Game/Patchwork/Blueprints/Levels/forest/Spores/BP_SporeRegion.BP_SporeRegion_C|SetSporeTypeTag _returnvalue (.SporeTag (Default|GetSporeTagfromName (Variables|Default|GetSporeHelper) type)))
      (Utilities|Map|Add (Variables|Default|GetSpawned) type _returnvalue)
      (Transformation|AttachActorToActor _returnvalue self "None" "KeepWorld" "KeepWorld" "KeepWorld" true)
      (Variables|/Game/Patchwork/Blueprints/Levels/forest/Spores/BP_SporeRegion.BP_SporeRegion_C|SetEffect%20Type _returnvalue (Utilities|Struct|MakeDataTableRowHandle "/Game/Patchwork/Data/Datatables/DT_SporeEffects.DT_SporeEffects" type)))))

(event Custom|lost%20spore
  (params (type :type Name))
  (bind _returnvalue (Transformation|GetActorTransform))
  (bind _spawned (Variables|Default|GetSpawned))
  (bind (_value _returnvalue_2) (Utilities|Map|Find _spawned type))
  ;[0.6233 0.02578 0.5693 0.5] Lost Spore
  (if _returnvalue_2
    (Actor|DestroyActor _value)
    (bind _returnvalue_3 (Niagara|SpawnSystematLocation "/Game/Patchwork/Effects/SporeEffects/NS_Spore_Dissapate.NS_Spore_Dissapate" (.location _returnvalue) (.rotation _returnvalue) (.scale _returnvalue) true true "AutoRelease"))
    (CallFunction|ApplySporeTypetoEffect type _returnvalue_3 1.0)))

(fn GetMassforPrimitive
  (params (Primitive :type Primitive%20Component%20Object%20Reference))
  (if (Default|HasSporefromTag (Variables|Default|GetBP_SporeCarrierController) "(TagName=\"SporeEffects.EffectType.IronSpore\")")
    (return 1e+03)
    (else
      (return (Math|Float|Lerp 5e+01 3e+02 (Variables|Default|GetBounce%20Timer))))))