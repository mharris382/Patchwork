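; BP_FireTorch_light is a fire torch prop for the Dark Fantasy Church environment that can be lit or unlit.
; Its construction script applies the Enable variable through SetEnableTorch, toggling visibility of the point light and fire particle system.
; The torch mesh casts shadows only while unlit.
; The event graph holds only disabled placeholder events.
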(event EventBeginPlay)

(event Collision|EventActorBeginOverlap
  (params (OtherActor :type Actor%20Object%20Reference)))

(event EventTick
  (params (DeltaSeconds :type Float%20%28single-precision%29)))

(fn ConstructionScript
  (CallFunction|SetEnableTorch (Variables|Default|GetEnable)))

(fn SetEnableTorch
  (params (Enabled :type Boolean))
  (bind _output_get (Variables|Default|SetEnable Enabled))
  ;[0.459 0.8065 1] Light
  (Rendering|SetVisibility (Variables|Default|GetPointLight) _output_get false)
  ;[1 0.524 0.5406] Particles
  (Rendering|SetVisibility (Variables|Default|GetParticleSystem) _output_get false)
  ;[1 1 1] Cast Shadow Mesh
  (Rendering|SetCastShadow (Variables|Default|GetFire%20Torch%20Big) (not _output_get)))