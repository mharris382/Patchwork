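; Player controller for Patchwork that manages input mapping contexts, interaction and UI for the paperperson pawn.
; Tick finds interactables from the pawn's current target or a camera sphere trace, updating the prompt when target or availability changes.
; Grab state swaps grab and ability contexts.
; It lazily creates pause, anomaly and desk-worker dialogue widgets, pinning the pawn with a looping timer during dialogue, and forwards spore and throw-power UI to the root HUD.
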(event Custom|Show%20Mushroom%20UI
  ;[0.6233 0.6233 0.6233 0.5] Unlock Mushroom Ability
  (CallFunction|MarkPlayerUsingAbility true))

(event Custom|Hide%20mushorom%20UI
  ;[0.6233 0.6233 0.6233 0.5] Unlock Mushroom Ability
  (CallFunction|MarkPlayerUsingAbility false))

(event Custom|Unlock%20Mushroom%20Ability
  (bind _player_pawn (Variables|Default|Getplayer%20pawn))
  (bind _bp_mushroomability (Variables|/Game/Patchwork/Blueprints/Core/Pawns/paperperson_ledge_grab.paperperson_ledge_grab_C|GetBP_MushroomAbility _player_pawn))
  ;[0.6233 0.6233 0.6233 0.5] Unlock Mushroom Ability
  (Utilities|IsValid (Variables|Default|Getplayer%20pawn)
    (:Is%20Valid
      (EventDispatchers|BindEventtoOnAbilityStarted _bp_mushroomability (delegate Custom|Show%20Mushroom%20UI))
      (EventDispatchers|BindEventtoOnAbilityCompleted _bp_mushroomability (delegate Custom|Hide%20mushorom%20UI))
      (bind _returnvalue (UserInterface|CreateWidget "/Game/Patchwork/Blueprints/Widgets/Abilities/UIE_ThrowPowerSlider.UIE_ThrowPowerSlider_C"))
      (Variables|Default|Setmushroom%20throw%20power%20slider _returnvalue))))

(event Input|EnhancedActionEvents|EnhancedInputActionIA_Interact
  (params (ActionValue :type Boolean) (ElapsedSeconds :type Float%20%28double-precision%29) (TriggeredSeconds :type Float%20%28double-precision%29) (InputAction :type Input%20Action%20Object%20Reference :default "/Game/Patchwork/Data/Input/IA_Interact.IA_Interact"))
  (Utilities|CloseAnomalyUIifOpen
    (:UI%20not%20open
      (bind _real_interact_target (Variables|Interacting|GetReal%20Interact%20Target)
        (:then
          (bind _available (Class|BPIInteractible|IsInteractAvailable(Message) _real_interact_target))
          (if _available
            (Class|BPIInteractible|OnInteract(Message) _real_interact_target)))
        (:else)))))

(event EventBeginPlay
  (bind _returnvalue (PlayerController|LocalPlayerSubsystems|GetEnhancedInputLocalPlayerSubsystem))
  ;[0.6233 0.6233 0.6233 0.5] Begin Play
  (Input|AddMappingContext (PlayerController|LocalPlayerSubsystems|GetEnhancedInputLocalPlayerSubsystem) "/Game/Patchwork/Data/Input/IMC_Game.IMC_Game" 0 "(bIgnoreAllPressedKeysUntilRelease=True,bForceImmediately=False,bNotifyUserSettings=False)")
  (Input|AddMappingContext _returnvalue (Variables|InputContexts|GetAbility%20Mapping%20Context) 0 "(bIgnoreAllPressedKeysUntilRelease=True,bForceImmediately=False,bNotifyUserSettings=False)")
  (Input|AddMappingContext _returnvalue (Variables|InputContexts|GetInteract%20Mapping%20Context) 0 "(bIgnoreAllPressedKeysUntilRelease=True,bForceImmediately=False,bNotifyUserSettings=False)")
  (CallFunction|SetEnableAnomalyUIAvailable true))

(event EventTick
  (params (DeltaSeconds :type Float%20%28single-precision%29))
  ;[0.6233 0.6233 0.6233 0.5] Tick
  (|CallParentFunction DeltaSeconds)
  (bind _aspaperperson (Utilities|Casting|CastTopaperperson (Game|Player|GetPlayerPawn 0)))
  (Variables|Default|SetPaperperson _aspaperperson)
  (Utilities|FlowControl|Sequence
    (:then_0
      ;;[0.6233 0.6233 0.6233 0.5] Handle Interaction Tooltips
      (bind (_newlocalvar1 _fopund _realtarget) (Interaction|GetInteractable false))
      (bind _changed (Interaction|CheckInteractChanged _fopund 0 _realtarget))
      (if _changed
        (Interaction|UpdateInteractTargetUI)))))

(event EventPossess
  (params (PossessedPawn :type Pawn%20Object%20Reference))
  ;[0.6233 0.6233 0.6233 0.5] On Possess
  (bind _aspaperperson_ledge_grab (Utilities|Casting|CastTopaperperson_ledge_grab PossessedPawn))
  (bind _output_get (Variables|Default|Setplayer%20pawn _aspaperperson_ledge_grab))
  (EventDispatchers|BindEventtoOnHasGrabbed (Variables|/Game/Patchwork/Blueprints/Core/Pawns/paperperson.paperperson_C|GetPickupHandler _output_get) (EventDispatchers|CreateEvent :!event UpdateInputforGrabbedState))
  (EventDispatchers|BindEventtoOnNotHasGrabbed (Variables|/Game/Patchwork/Blueprints/Core/Pawns/paperperson.paperperson_C|GetPickupHandler _output_get) (EventDispatchers|CreateEvent :!event UpdateInputforNotGrabbedState)))

(event Input|KeyboardEvents|AnyKey
  (params (Key :type Key%20Structure :default "None")))

(event Custom|Add%20Spore%20Indicator
  (params (NewParam :type BP%20Spore%20Effect%20Base%20Object%20Reference))
  (bind _returnvalue (UserInterface|CreateWidget "/Game/Patchwork/Blueprints/Widgets/Spores/SporeIndicator.SporeIndicator_C" self NewParam))
  (Default|AddSporeIndicator (Variables|Default|GetRoot%20Hud) _returnvalue))

(event Custom|Open%20Anomaly%20Window
  ;[0.4769 0.139 0.6233 0.5] Anomaly UI
  (Utilities|CanOpenAnomalyUI
    (:false
      (Variables|Default|Setanomaly%20window%20open true)
      (bind _anomaly_ui (Utilities|GetAnomalyUI)
        (:Is%20Valid
          (Default|UpdateImage _anomaly_ui)
          (UserInterface|Viewport|AddtoViewport _anomaly_ui 3))))))

(event Custom|Assign%20Root%20HUD
  (params (root%20hud :type Game%20HUD%20Root%20Object%20Reference))
  (bind _output_get (Variables|Default|SetRoot%20Hud root%20hud))
  (Default|AddUItoStack _output_get "/Game/Patchwork/UI/GameUI/Parts/AUIE_Main_HUD.AUIE_Main_HUD_C"))

(event Custom|Close%20Anomaly%20Window
  ;[0.4769 0.139 0.6233 0.5] Anomaly UI
  (if (Variables|Default|Getanomaly%20window%20open)
    (Variables|Default|Setanomaly%20window%20open false)
    (bind _anomaly_ui (Utilities|GetAnomalyUI)
      (:Is%20Valid
        (Widget|RemovefromParent _anomaly_ui)))))

(event Custom|Update%20Throw%20Power%20UI
  (params (Normalized%20Throw%20Power :type Float%20%28double-precision%29))
  (Default|UpdateThrowSlider (Variables|Default|GetRoot%20Hud) Normalized%20Throw%20Power))

(event Input|EnhancedActionEvents|EnhancedInputActionIA_Pause
  (params (ActionValue :type Boolean) (ElapsedSeconds :type Float%20%28double-precision%29) (TriggeredSeconds :type Float%20%28double-precision%29) (InputAction :type Input%20Action%20Object%20Reference :default "/Game/Patchwork/Data/Input/IA_Pause.IA_Pause"))
  ;[0.6233 0.6233 0.6233 0.5] Pause Button
  (Utilities|CloseAnomalyUIifOpen
    (:UI%20not%20open
      (if (Game|IsGamePaused)
        (Widgets|HidePauseMenu)
        (else
          (Widgets|ShowPauseMenu))))))

(event Input|EnhancedActionEvents|EnhancedInputActionIA_AnomalyWindow
  (params (ActionValue :type Boolean) (ElapsedSeconds :type Float%20%28double-precision%29) (TriggeredSeconds :type Float%20%28double-precision%29) (InputAction :type Input%20Action%20Object%20Reference :default "/Game/Patchwork/Data/Input/IA_AnomalyWindow.IA_AnomalyWindow"))
  ;[0.4769 0.139 0.6233 0.5] Anomaly UI
)

(fn ConstructionScript)

(fn ShowPauseMenu
  (if (Widgets|CanShowPauseMenu)
    (bind _pause_wb (Utilities|GetPauseUI)
      (:OutputPin
        (CallFunction|AddandActivateWidget _pause_wb)))))

(fn HidePauseMenu
  (Utilities|IsValid (Variables|Default|GetPause%20Wb)
    (:Is%20Valid
      (Widget|RemovefromParent (Variables|Default|GetPause%20Wb))
      (SetMode|SetModetoGame))))

(fn CanShowPauseMenu
  (Utilities|IsValid (Game|Player|GetPlayerPawn 0)
    (:Is%20Valid
      (Utilities|IsValid (Variables|Default|GetPause%20Wb)
        (:Is%20Valid
          (if (Variables|Default|Getis%20desk%20worker%20UI%20open)
            (return false)
            (else
              (return (not (UserInterface|Viewport|IsinViewport (Variables|Default|GetPause%20Wb)))))))
        (:Is%20Not%20Valid
          (return true))))
    (:Is%20Not%20Valid
      (return false))))

(fn SetModetoGame
  (Input|SetInputModeGameOnly self false)
  (Variables|Default|SetbShowMouseCursor false))

(fn SetModetoUI
  (Input|SetInputModeUIOnly self 0 "LockAlways" false)
  (Variables|Default|SetbShowMouseCursor true))

(fn UpdateInteractTargetUI
  (if (Math|Boolean|ANDBoolean (Utilities|IsValid (Variables|Interacting|GetReal%20Interact%20Target)) (Variables|Default|Getinteractable%20valid) (not (Variables|Default|Getgrabbing)))
    (bind _msg (Class|BPIInteractible|GetInteractionMessage(Message) (Variables|Interacting|GetReal%20Interact%20Target)))
    (Default|CallUpdateInteractMessage _msg true)
    (else
      (Default|CallUpdateInteractMessage "" false))))

(fn MarkPlayerUsingAbility
  (params (is%20using%20ability :type Boolean))
  (bind _player_pawn (Variables|Default|Getplayer%20pawn))
  (bind _tags (Variables|/Script/Engine.Actor|GetTags _player_pawn))
  (if is%20using%20ability
    (Utilities|Array|Add _tags "Using Ability")
    (else
      (Utilities|Array|RemoveItem _tags "Using Ability"))))

(fn GetInteractable
  (params (debug :type Boolean))
  (bind _player_pawn (Variables|Default|Getplayer%20pawn)
    (:then
      (Utilities|IsValid (Variables|/Game/Patchwork/Blueprints/Core/Pawns/paperperson.paperperson_C|GetcurrentRealTarget _player_pawn)
        (:Is%20Valid
          (bind _asproxy_pickup (Utilities|Casting|CastToProxyPickup (Variables|/Game/Patchwork/Blueprints/Core/Pawns/paperperson.paperperson_C|GetcurrentRealTarget _player_pawn))
            (:then
              (return 0 true _asproxy_pickup))
            (:CastFailed
              (bind _asproxy_dialogue (Utilities|Casting|CastToProxyDialogue (Variables|/Game/Patchwork/Blueprints/Core/Pawns/paperperson.paperperson_C|GetcurrentRealTarget _player_pawn))
                (:then
                  (return 0 true _asproxy_dialogue))
                (:CastFailed
                  _)))))
        (:Is%20Not%20Valid
          _))
      (bind (_outhits _returnvalue) (Collision|MultiSphereTraceForObjects (+ (Transformation|GetWorldLocation (Variables|/Game/Patchwork/Blueprints/Core/Pawns/BP_BaseCharacter.BP_BaseCharacter_C|GetCamera _player_pawn)) (* (Math|Vector|GetForwardVector (Variables|/Game/Patchwork/Blueprints/Core/Pawns/BP_BaseCharacter.BP_BaseCharacter_C|GetCamera _player_pawn)) 4e+01)) (+ (Transformation|GetWorldLocation (Variables|/Game/Patchwork/Blueprints/Core/Pawns/BP_BaseCharacter.BP_BaseCharacter_C|GetCamera _player_pawn)) (* (Math|Vector|GetForwardVector (Variables|/Game/Patchwork/Blueprints/Core/Pawns/BP_BaseCharacter.BP_BaseCharacter_C|GetCamera _player_pawn)) 1.5e+02)) 4e+01 (Utilities|Array|MakeArray "ObjectTypeQuery1" "ObjectTypeQuery3" "ObjectTypeQuery4" "ObjectTypeQuery2") false 0 (select debug "ForOneFrame" "None")))
      (if _returnvalue
        (bind _array_element (Utilities|Array|ForEachLoopwithBreak _outhits :!label _label)
          (:LoopBody
            (if (Utilities|DoesObjectImplementInterface (.HitActor (Collision|BreakHitResult _array_element)) "/Game/Patchwork/Blueprints/Interfaces/BPI_Interactible.BPI_Interactible_C")
              (LocalVariables|Setresult (.HitActor (Collision|BreakHitResult _array_element)))
              (goto _label Break)))
          (:Completed
            (return 0 (Utilities|IsValid (LocalVariables|Getresult)) (LocalVariables|Getresult))))))
    (:else
      (return 0 false 0))))

(fn CheckInteractChanged
  (params (found%20interact :type Boolean) (Interact%20Target :type Interactible%20Object%20Reference) (RealTarget :type Actor%20Object%20Reference))
  (if found%20interact
    (if (== (Variables|Interacting|GetReal%20Interact%20Target) RealTarget)
      (bind _available (Class|BPIInteractible|IsInteractAvailable(Message) (Variables|Interacting|GetReal%20Interact%20Target)))
      (if (!= (Variables|Default|Getinteractable%20valid) _available)
        (Variables|Default|Setinteractable%20valid _available)
        (return true)
        (else
          (return false)))
      (else
        (bind _output_get (Variables|Interacting|SetReal%20Interact%20Target RealTarget))
        (bind _available_2 (Class|BPIInteractible|IsInteractAvailable(Message) _output_get))
        (Variables|Default|Setinteractable%20valid _available_2)
        (return true)))
    (else
      (Utilities|IsValid (Variables|Interacting|GetReal%20Interact%20Target)
        (:Is%20Valid
          (Variables|Interacting|SetReal%20Interact%20Target 0)
          (return true))
        (:Is%20Not%20Valid
          (return false))))))

(fn SetEnableAnomalyUIAvailable
  (params (is%20available :type Boolean))
  (bind _returnvalue (PlayerController|LocalPlayerSubsystems|GetEnhancedInputLocalPlayerSubsystem))
  (bind _returnvalue_2 (PlayerController|LocalPlayerSubsystems|GetEnhancedInputLocalPlayerSubsystem))
  (if is%20available
    (if (not (.ReturnValue (Class|EnhancedInputSubsystemInterface|HasMappingContext _returnvalue "/Game/Patchwork/Data/Input/IMC_AnomalyUI.IMC_AnomalyUI")))
      (Input|AddMappingContext _returnvalue "/Game/Patchwork/Data/Input/IMC_AnomalyUI.IMC_AnomalyUI" 3 "(bIgnoreAllPressedKeysUntilRelease=True,bForceImmediately=False,bNotifyUserSettings=False)"))
    (elif (.ReturnValue (Class|EnhancedInputSubsystemInterface|HasMappingContext _returnvalue_2 "/Game/Patchwork/Data/Input/IMC_AnomalyUI.IMC_AnomalyUI"))
      (Input|RemoveMappingContext _returnvalue_2 "/Game/Patchwork/Data/Input/IMC_AnomalyUI.IMC_AnomalyUI" "(bIgnoreAllPressedKeysUntilRelease=True,bForceImmediately=False,bNotifyUserSettings=False)"))))

(fn AddandActivateWidget
  (params (widget :type Common%20Activatable%20Widget%20Object%20Reference))
  (UserInterface|Viewport|AddtoViewport widget 5)
  (Class|CommonActivatableWidget|ActivateWidget widget))

(fn RemoveandDeactivateWidget
  (params (widget :type Common%20Activatable%20Widget%20Object%20Reference))
  (Widget|RemovefromParent widget)
  (if (Variables|/Script/CommonUI.CommonActivatableWidget|GetbIsActive widget)
    (Class|CommonActivatableWidget|DeactivateWidget widget)))

(fn UpdateInputforGrabbedState
  (Pickups|SetCanUseGrabInputs true))

(fn SetCanUseGrabInputs
  (params (Has%20Grab%20Inputs :type Boolean))
  (bind _output_get (Variables|Default|Setgrabbing Has%20Grab%20Inputs))
  (CallFunction|SetCanUseInputMappingContext _output_get (Variables|InputContexts|GetGrab%20Mapping%20Context))
  (CallFunction|SetCanUseInputMappingContext (not (Variables|Default|Getgrabbing)) (Variables|InputContexts|GetAbility%20Mapping%20Context)))

(fn UpdateInputforNotGrabbedState
  (Pickups|SetCanUseGrabInputs false))

(fn SetCanUseInteract
  (params (Can%20Interact :type Boolean))
  (if Can%20Interact
    _))

(fn SetMushroomAbilityAvailable
  (params (AbilityIsAvailable :type Boolean))
  (CallFunction|SetCanUseInputMappingContext AbilityIsAvailable (Variables|InputContexts|GetAbility%20Mapping%20Context)))

(fn SetCanUseInputMappingContext
  (params (CanUseContext :type Boolean) (Context :type Input%20Mapping%20Context%20Object%20Reference) (Options :type Modify%20Context%20Options%20Structure%20%28by%20ref%29))
  (bind _returnvalue (PlayerController|LocalPlayerSubsystems|GetEnhancedInputLocalPlayerSubsystem))
  (bind _contextpriorities (Variables|InputContexts|GetcontextPriorities))
  (bind (_value _returnvalue_2) (Utilities|Map|Find _contextpriorities Context))
  (if CanUseContext
    (if (not (.ReturnValue (Class|EnhancedInputSubsystemInterface|HasMappingContext (PlayerController|LocalPlayerSubsystems|GetEnhancedInputLocalPlayerSubsystem) (Variables|InputContexts|GetGrab%20Mapping%20Context))))
      (Input|AddMappingContext _returnvalue Context (Math|Integer|SelectInt _value 0 _returnvalue_2) Options))
    (else
      (Input|RemoveMappingContext _returnvalue Context Options))))

(event Custom|Trigger%20Desk%20Worker%20Dialogue
  (params (dialogue%20component :type Desk%20Worker%20Dialogue%20Object%20Reference))
  (bind _paperperson (Variables|Default|GetPaperperson))
  ;[0.6233 0.6233 0.6233 0.5] Desk Worker Stuff
  (Variables|/Game/Patchwork/Blueprints/Core/Pawns/paperperson.paperperson_C|SetMove%20Value%20Y _paperperson 0.0)
  (Variables|/Game/Patchwork/Blueprints/Core/Pawns/paperperson.paperperson_C|SetMove%20Value%20X _paperperson 0.0)
  (Components|Movement|StopMovementImmediately (Variables|/Script/Engine.Character|GetCharacterMovement (Variables|Default|GetPaperperson)))
  (Variables|Default|Setis%20desk%20worker%20UI%20open true)
  (if (Variables|Default|Getanomaly%20window%20open)
    (CallFunction|CloseAnomalyWindow)
    (Utilities|FlowControl|Delay 0.5))
  (bind _output_get (Utilities|GetDeskWorkerUI)
    (:OutputPin
      (CallFunction|AddandActivateWidget _output_get)
      (Default|StartDialogue _output_get dialogue%20component (Utilities|Struct|MakeDialogueScreenOptionsStruct false false false 0 1.0 false))
      (Variables|Default|Setlocation (Transformation|GetActorLocation (Pawn|GetControlledPawn)))
      (bind _returnvalue (Utilities|Time|SetTimerbyEvent (delegate Custom|CustomEvent) 0.01 true))
      (Variables|Default|SetNewVar _returnvalue))))

(event Custom|Complete%20Desk%20Worker%20Dialogue
  (bind _paperperson (Variables|Default|GetPaperperson))
  ;[0.6233 0.6233 0.6233 0.5] Desk Worker Stuff
  (Variables|Default|Setis%20desk%20worker%20UI%20open false)
  (bind _output_get (Utilities|GetDeskWorkerUI)
    (:OutputPin
      (CallFunction|RemoveandDeactivateWidget _output_get)
      (Variables|/Game/Patchwork/Blueprints/Core/Pawns/paperperson.paperperson_C|SetMove%20Value%20Y _paperperson 0.0)
      (Variables|/Game/Patchwork/Blueprints/Core/Pawns/paperperson.paperperson_C|SetMove%20Value%20X _paperperson 0.0)
      (Variables|Default|SetDesk%20Worker%20UI 0))))

(event Custom|CustomEvent
  ;[0.6233 0.6233 0.6233 0.5] Desk Worker Stuff
  (if (Variables|Default|Getis%20desk%20worker%20UI%20open)
    (Transformation|SetActorLocation (Pawn|GetControlledPawn) (Variables|Default|Getlocation) false false)
    (Variables|/Script/Engine.MovementComponent|SetVelocity (Pawn|GetMovementComponent (Variables|Default|GetPaperperson)) "0, 0, 0")
    (else
      (Utilities|Time|ClearandInvalidateTimerbyHandle (Variables|Default|GetNewVar)))))