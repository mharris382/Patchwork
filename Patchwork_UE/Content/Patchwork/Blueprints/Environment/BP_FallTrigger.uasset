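; Fall trigger volume that respawns the player at their last ground location.
; Overlap by player 0's pawn on the Plane component triggers the respawn; other actors are ignored.
; The construction script sizes Box and Plane from Extents, placing the Plane at negative Z extent plus PlaneOffset.
; PositionAtBottom optionally raises the Box by its Z half-height.
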(event OnComponentBeginOverlap(Plane)
  (params (OverlappedComponent :type Primitive%20Component%20Object%20Reference) (OtherActor :type Actor%20Object%20Reference) (OtherComp :type Primitive%20Component%20Object%20Reference) (OtherBodyIndex :type Integer) (bFromSweep :type Boolean) (SweepResult :type Hit%20Result%20Structure%20%28by%20ref%29))
  (if (== OtherActor (Game|Player|GetPlayerPawn 0))
    (CallFunction|RespawnPlayeratLastGroundLocation)))

(event EventBeginPlay)

(event Collision|EventActorBeginOverlap
  (params (OtherActor :type Actor%20Object%20Reference)))

(event EventTick
  (params (DeltaSeconds :type Float%20%28single-precision%29)))

(fn ConstructionScript
  (bind _plane (Variables|Default|GetPlane))
  (bind _box (Variables|Default|GetBox))
  (bind _extents (Variables|Box|GetExtents))
  (Utilities|FlowControl|Sequence
    (:then_0
      (Transformation|SetRelativeLocation _plane (Math|Vector|MakeVector 0.0 0.0 (+ (* (.z (Variables|Box|GetExtents)) -1.0) (Variables|Plane|GetPlane%20Offset))) false false)
      (Transformation|SetRelativeScale3D _plane (/ (* (Variables|Box|GetExtents) 2.0) 1e+02)))
    (:then_1
      (Components|Box|SetBoxExtent _box _extents true)
      (if (Variables|Box|Getposition%20at%20bottom)
        (Transformation|SetRelativeLocation _box (Math|Vector|MakeVector 0.0 0.0 (.Z (Math|Vector|BreakVector _extents))) false false)))))