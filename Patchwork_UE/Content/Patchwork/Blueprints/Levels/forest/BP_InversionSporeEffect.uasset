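; BP_InversionSporeEffect is a spore effect that shifts its owning character's gravity as toxicity changes.
; On begin play it caches the owner Character and its normal gravity scale.
; Each toxicity change samples GravCurve to blend from normal to FinalGravity, then adds the summed Amount of the character's GravityModifier components.
; The result is written to the movement component's GravityScale, with no tick logic.
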(event EventBeginPlay
  (|CallParentFunction)
  (bind _ascharacter (Utilities|Casting|CastToCharacter (Components|GetOwner)))
  (bind _output_get (Variables|Default|Setowner%20character _ascharacter))
  (Variables|Default|Setnormal%20gravity (Variables|/Script/Engine.CharacterMovementComponent|GetGravityScale (Variables|/Script/Engine.Character|GetCharacterMovement _output_get))))

(event EventTick
  (params (DeltaSeconds :type Float%20%28single-precision%29))
  (|CallParentFunction DeltaSeconds) ; This node is disabled and will not be called.\nDrag off pins to build functionality.
)

(fn OnToxicityChanged
  (params (new%20toxicity :type Float%20%28double-precision%29))
  (bind _output_get (LocalVariables|Settoxicity new%20toxicity))
  (|CallParentFunction _output_get)
  (Utilities|IsValid (Variables|Default|Getowner%20character)
    (:Is%20Valid
      (bind _total (CallFunction|GetGravityModifier))
      (Variables|/Script/Engine.CharacterMovementComponent|SetGravityScale (Variables|/Script/Engine.Character|GetCharacterMovement (Variables|Default|Getowner%20character)) (+ _total (Math|Float|Lerp (Variables|Default|Getnormal%20gravity) (Variables|Default|Getfinal%20gravity) (Math|Curves|GetFloatValue (Variables|Default|Getgrav%20curve) (LocalVariables|Gettoxicity))))))))

(fn GetGravityModifier
  (LocalVariables|Setsum 0.0)
  (for _array_element (Actor|GetComponentsByClass (Variables|Default|Getowner%20character) "/Game/Patchwork/Blueprints/GravityModifier.GravityModifier_C")
    (LocalVariables|Setsum (+ (Variables|/Game/Patchwork/Blueprints/GravityModifier.GravityModifier_C|GetAmount _array_element) (LocalVariables|Getsum))))
  (return (LocalVariables|Getsum)))