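; BP_LightBase is a base light Blueprint in the poolrooms level assets that configures a light component from its variables.
; The construction script fetches the component through GetLight and, if valid, applies intensity, color and indirect lighting intensity.
; GetLight is empty here, so a light is configured only where an override supplies one.
; The event graph has no active logic.
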(event EventBeginPlay)

(event Collision|EventActorBeginOverlap
  (params (OtherActor :type Actor%20Object%20Reference)))

(event EventTick
  (params (DeltaSeconds :type Float%20%28single-precision%29)))

(fn ConstructionScript
  (bind _light (CallFunction|GetLight))
  (bind _output_get (LocalVariables|Setlight _light))
  (Utilities|IsValid _output_get
    (:Is%20Valid
      (Rendering|Components|Light|SetIntensity (LocalVariables|Getlight) (Variables|Light|GetIntensity))
      (Rendering|Components|Light|SetLightColor (LocalVariables|Getlight) (Variables|Light|GetLight%20Color) true)
      (Class|LightComponent|SetIndirectLightingIntensity (LocalVariables|Getlight) (Variables|Light|GetIndirect%20Lighting)))))

(fn GetLight
  (return 0))