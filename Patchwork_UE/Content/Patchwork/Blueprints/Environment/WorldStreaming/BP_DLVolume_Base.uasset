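; Base trigger volume for world streaming that notifies BP_DataLayerManager when the player pawn begins overlapping it.
; It exposes its Activated, Loaded and Unloaded states and a Priority through getters, and passes no data in the trigger call.
; The construction script caches the manager and recolors meshes tagged PriorityVisualizer with the material for the clamped priority, overriding any EditorMaterial applied just before.
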(event EventBeginPlay)

(event Collision|EventActorBeginOverlap
  (params (OtherActor :type Actor%20Object%20Reference))
  (if (== OtherActor (Game|Player|GetPlayerPawn 0))
    (Default|DLStateVolumeTriggered (Variables|Default|GetData%20Layer%20Manager))))

(event EventTick
  (params (DeltaSeconds :type Float%20%28single-precision%29)))

(fn ConstructionScript
  (Utilities|FlowControl|Sequence
    (:then_0
      (bind _returnvalue (Actor|GetActorOfClass "/Game/Patchwork/Blueprints/Environment/WorldStreaming/BP_DataLayerManager.BP_DataLayerManager_C"))
      (Variables|Default|SetData%20Layer%20Manager _returnvalue)
      (bind _editormaterial (Variables|Editor|GetEditorMaterial)
        (:then
          (for _array_element (Actor|GetComponentsbyTag "/Script/Engine.StaticMeshComponent" "PriorityVisualizer")
            (Rendering|Material|SetMaterial _array_element 0 _editormaterial)))
        (:else)))
    (:then_1
      (bind _priority (CallFunction|GetPriority))
      (for _array_element_2 (Actor|GetComponentsbyTag "/Script/Engine.StaticMeshComponent" "PriorityVisualizer")
        (Utilities|IsValid _array_element_2
          (:Is%20Valid
            (Rendering|Material|SetMaterial _array_element_2 0 (Utilities|Array|Get(acopy) (Variables|Default|GetPriorityColors) (Math|Integer|Clamp(Integer) _priority 0 (- (Utilities|Array|Length (Variables|Default|GetPriorityColors)) 1))))))))))

(fn GetStates
  (return (Variables|DataLayers|GetActivated) (Variables|DataLayers|GetLoaded) (Variables|DataLayers|GetUnloaded)))

(fn GetPriority
  (return (Variables|Default|GetPriority)))