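; BlackoutPortal is a paired portal actor that teleports the player to its PartnerPortal on overlap.
; It places the player at an offset along the partner's forward vector and sets control rotation from the negated partner rotation.
; A JustPortaled flag on the partner prevents bouncing back until overlap ends, and an empty OnPlayerPortaled event serves as a hook.
; The construction script sizes the box, fog-blocking plane and thinner trigger box from Size.
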(event Custom|On%20Player%20Portaled
  (params (pp :type Paperperson%20Object%20Reference)))

(event EventBeginPlay)

(event Collision|EventActorBeginOverlap
  (params (OtherActor :type Actor%20Object%20Reference))
  (bind _returnvalue (Game|Player|GetPlayerPawn 0))
  (if (and (== OtherActor (Game|Player|GetPlayerPawn 0)) (not (Variables|Default|GetJust%20Portaled)))
    (bind _partner_portal (Variables|Default|GetPartner%20Portal)
      (:then
        (Variables|BlackoutPortal_C|SetJust%20Portaled _partner_portal true)
        (bind _ascharacter (Utilities|Casting|CastToCharacter _returnvalue))
        (Transformation|SetActorLocation _returnvalue (+ (Transformation|GetActorLocation _partner_portal) (* (Transformation|GetActorForwardVector _partner_portal) (Variables|Default|GetOffset))) false true)
        (Pawn|SetControlRotation (Pawn|GetController _ascharacter) (Class|KismetMathLibrary|NegateRotator (Transformation|GetActorRotation _partner_portal)))
        (CallFunction|OnPlayerPortaled (.AsPaperperson (Utilities|Casting|CastTopaperperson _ascharacter))))
      (:else))))

(event EventTick
  (params (DeltaSeconds :type Float%20%28single-precision%29)))

(event Collision|EventActorEndOverlap
  (params (OtherActor :type Actor%20Object%20Reference))
  (if (== OtherActor (Game|Player|GetPlayerPawn 0))
    (Variables|Default|SetJust%20Portaled false)))

(fn ConstructionScript
  (bind _size (Variables|Default|GetSize))
  (Components|Box|SetBoxExtent (Variables|Default|GetBox) _size true)
  (Transformation|SetRelativeScale3D (Variables|Default|GetFog%20Blocking%20Plane) (/ _size "100.000000,100.000000,100.000000"))
  (Components|Box|SetBoxExtent (Variables|Default|GetTrigger%20Box) (* _size "0.100000,1.000000,1.000000") true))