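; Gravity change ability Blueprint, filed under pawn abilities, that gates its readiness on mana.
; It overrides IsReady to require both the parent's check and CurrentMana at or above the ManaCost in GlobalAbilitySettings.
; The event graph holds only disabled default nodes, and no gravity change logic appears in these graphs.
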(event EventBeginPlay
  (|CallParentFunction) ; This node is disabled and will not be called.\nDrag off pins to build functionality.
)

(event EventTick
  (params (DeltaSeconds :type Float%20%28single-precision%29))
  (|CallParentFunction DeltaSeconds) ; This node is disabled and will not be called.\nDrag off pins to build functionality.
)

(fn IsReady
  (return (and (|CallParentFunction) (>= (Variables|Default|GetCurrentMana) (Variables|/Game/Patchwork/Blueprints/Utilities/BP_GlobalAbilitySettings.BP_GlobalAbilitySettings_C|GetManaCost (Variables|Default|GetGlobalAbilitySettings))))))