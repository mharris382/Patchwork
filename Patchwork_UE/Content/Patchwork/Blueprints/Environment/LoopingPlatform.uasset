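; Looping platform that travels between Position1 and Position2 via InterpToMovement, restarting when the movement resets.
; The construction script derives duration from distance and Speed, sets control points and previews the Time position.
; On reset it releases grabbing or standing players, using Falling mode and a looping teleport timer to hold their location, then optionally snaps the Pivot to start.
; Manual tick-style movement is disconnected, leaving the RestartDelay flag unused.
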(event OnResetDelegate(InterpToMovement)
  (params (ImpactResult :type Hit%20Result%20Structure%20%28by%20ref%29) (Time :type Float%20%28single-precision%29))
  (CallFunction|DoRestart))

(event Custom|Do%20restart
  (Utilities|FlowControl|Sequence
    (:then_0
      (Utilities|FlowControl|Sequence
        (:then_0
          (Utilities|IsPlayerGrabbingPlatform
            (:then
              (Default|ForceExitGrab (Variables|Default|Getpawn)))))
        (:then_1
          (bind _aspaperperson_ledge_grab (Utilities|IsPlayerStandingonPlatform)
            (:true
              (bind _output_get (Variables|Default|Setpawn _aspaperperson_ledge_grab))))))
      (Variables|Default|Setactor%20location (Transformation|GetActorLocation (Variables|Default|Getpawn)))
      (Pawn|Components|CharacterMovement|SetMovementMode (Variables|/Script/Engine.Character|GetCharacterMovement _aspaperperson_ledge_grab) "MOVE_Falling" 0)
      (bind _returnvalue (Utilities|Time|SetTimerbyEvent (delegate Custom|force%20loca) 0.01 true))
      (Variables|Default|Setforce%20location%20timer _returnvalue)
      (Variables|Default|Setend%20force%20location%20timer false)
      (Utilities|FlowControl|Delay 0.1)
      (Variables|Default|Setend%20force%20location%20timer true))
    (:then_2
      ;[0.6233 0.6233 0.6233 0.5] Reset location before delay
      (if (Variables|Default|GetReset%20to%20Start%20Before%20Delay)
        (Transformation|SetRelativeLocation (Variables|Default|GetPivot) (Variables|Default|GetPosition%201) false true)))
    (:then_3
      ;[0.6233 0.6233 0.6233 0.5] Optional delay
      (if (> (Variables|Default|GetRestart%20Delay) 0.0)
        (Variables|Default|Setreseting true)
        (Utilities|FlowControl|Delay (Variables|Default|GetRestart%20Delay))
        (Variables|Default|Setreseting false)))))

(event Custom|force%20loca
  (bind _aspaperperson_ledge_grab (Utilities|IsPlayerStandingonPlatform)
    (:true
      (Transformation|SetActorLocation _aspaperperson_ledge_grab (Variables|Default|Getactor%20location) false true))
    (:false
      (Utilities|Time|ClearandInvalidateTimerbyHandle (Variables|Default|Getforce%20location%20timer)))))

(event EventBeginPlay)

(event Collision|EventActorBeginOverlap
  (params (OtherActor :type Actor%20Object%20Reference)))

(event EventTick
  (params (DeltaSeconds :type Float%20%28single-precision%29)))

(fn ConstructionScript
  (bind _interptomovement (Variables|Default|GetInterpToMovement))
  (Utilities|FlowControl|Sequence
    (:then_0
      (bind _output_get (Variables|Default|Settotal%20time (|(D/(s*100)) (Math|Vector|Distance(Vector) (Variables|Default|GetPosition%201) (Variables|Default|GetPosition%202)) (Math|Float|Max(Float) (Variables|Default|GetSpeed) 0.01))))
      (Variables|Default|SetTime (* _output_get (Variables|Default|GetTime))))
    (:then_1
      (Variables|/Script/Engine.InterpToMovementComponent|SetDuration _interptomovement (Variables|Default|Gettotal%20time))
      (Variables|/Script/Engine.InterpToMovementComponent|SetControlPoints _interptomovement (Utilities|Array|MakeArray (Utilities|Struct|MakeInterpControlPoint (Variables|Default|GetPosition%201) true) (Utilities|Struct|MakeInterpControlPoint (Variables|Default|GetPosition%202) true))))
    (:then_2
      (CallFunction|UpdatePosition (Variables|Default|GetTime)))))

(fn UpdatePosition
  (params (t :type Float%20%28double-precision%29))
  (bind _returnvalue (Math|Float|Max(Float) t 0.01))
  (bind _curve (Variables|Default|GetCurve))
  (bind _position_1 (Variables|Default|GetPosition%201))
  (bind _position_2 (Variables|Default|GetPosition%202))
  (bind _value (CallFunction|LerpVectorwithOptionalCurve _position_1 _position_2 _returnvalue _curve))
  (Utilities|FlowControl|Sequence
    (:then_0
      (if (< (Variables|Default|GetTime) (Variables|Default|Gettotal%20time))
        (LocalVariables|Setsweep (Variables|DynamicPhysics|GetHits%20Obstacles))
        (LocalVariables|Setrestart false)
        (else
          (Variables|Default|SetTime 0.0)
          (LocalVariables|Setsweep false)
          (LocalVariables|Setrestart true))))
    (:then_1
      (Variables|Default|Setvelocity (/ (- _value (Variables|/Script/Engine.SceneComponent|GetRelativeLocation (Variables|Default|GetPivot))) _returnvalue))
      (Transformation|SetRelativeLocation (Variables|Default|GetPivot) _value (LocalVariables|Getsweep) false)
      (return (LocalVariables|Getrestart)))))

(fn GetIsMoving
  (return true))