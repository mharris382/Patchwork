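; Footstep component for a Character owner that plays surface-dependent footstep sounds at the owner's location.
; When set to run automatically, Tick advances a fixed-rate timer while the character moves horizontally, firing PlayFootstep with alternating foot indices on each wrap.
; PlayFootstep requires a blocking floor, asks GM_BaseGameMode for a sound using the tagged floor actor, and plays it with footstep attenuation.
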(event Custom|Play%20Footstep
  (params (foot%20index :type Integer))
  (bind _character_movement (Variables|Default|GetCharacter%20Movement))
  (bind _currentfloor (Variables|/Script/Engine.CharacterMovementComponent|GetCurrentFloor _character_movement))
  (bind (_bblockinghit _binitialoverlap _time _distance _location _impactpoint _normal _impactnormal _physmat _hitactor _hitcomponent) (Collision|BreakHitResult (.hitresult _currentfloor)))
  (Utilities|IsValid _character_movement
    (:Is%20Valid
      (if (.bblockinghit _currentfloor)
        (Utilities|FlowControl|Sequence
          (:then_0
            (bind (_sound _success) (Default|TryGetFootstepSound (Variables|Default|GetGame%20Mode) (select (>= (Utilities|Array|Length (Variables|/Script/Engine.Actor|GetTags _hitactor)) 1) _hitactor 0)))
            (if _success
              (Audio|PlaySoundatLocation _sound (Transformation|GetActorLocation (Components|GetOwner)) "0, 0, 0" (Variables|Default|GetVolume%20Multiplier) 1.0 0.0 "/Game/Defender/Demo/Audio/Attenuations/ATT_Footsteps.ATT_Footsteps" 0 0 0))))))))

(event EventBeginPlay
  (CallFunction|CalculateFootsteps)
  (Utilities|SetCharacterMovement)
  (bind _asgm_base_game_mode (Utilities|Casting|CastToGM_BaseGameMode (Game|GetGameMode)))
  (Variables|Default|SetGame%20Mode _asgm_base_game_mode))

(event EventTick
  (params (DeltaSeconds :type Float%20%28single-precision%29))
  (if (Variables|Default|GetRun%20Automatically)
    (CallFunction|UpdateSteps DeltaSeconds)))

(fn UpdateSteps
  (params (dt :type Float%20%28double-precision%29))
  (bind _footstep_speed (Variables|Default|GetFootstep%20Speed))
  (bind _footstep_time (Variables|Default|Getfootstep%20time))
  (bind _character_movement (Variables|Default|GetCharacter%20Movement))
  (bind _returnvalue (* dt _footstep_speed))
  (bind _velocity (Variables|/Script/Engine.MovementComponent|GetVelocity _character_movement))
  (bind _returnvalue_2 (+ _returnvalue _footstep_time))
  (Utilities|IsValid _character_movement
    (:Is%20Valid
      _)
    (:Is%20Not%20Valid
      (Utilities|SetCharacterMovement)))
  (if (> (+ (Math|Float|Absolute(Float) (.x _velocity)) (Math|Float|Absolute(Float) (.y _velocity))) 0.6)
    (Variables|Default|SetFootstep%20Time (Math|Float|%(Float) _returnvalue_2 1.0))
    (if (> _returnvalue_2 1.0)
      (bind _result (Math|Integer|IncrementInt (Variables|Default|GetFootstep%20Count))
        (:%20%20
          (CallFunction|PlayFootstep (Math|Integer|%(Integer) _result 2)))))))

(fn CalculateFootsteps
  (Variables|Default|SetFootstep%20Speed (/ (Variables|Default|GetFootsteps%20Per%20Second) 1.0)))