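; Actor component that fires a quest step's completion world event when the player pawn overlaps its owning actor.
; It binds to the owner's begin overlap and reads the completion event from the configured quest DataTable row, then invokes it through GM_BaseGameMode.
; When QuestMustBeActive is set, it first requires the step to be among BP_QuestController's current or completed steps.
; Lookup helpers cache the controller and print setup errors.
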(event Custom|On%20Overlap
  (params (OverlappedActor :type Actor%20Object%20Reference) (OtherActor :type Actor%20Object%20Reference))
  (if (== OtherActor (Game|Player|GetPlayerPawn 0))
    (if (Variables|Default|Getquest%20must%20be%20active)
      (bind _row_name (Utilities|GetQuestData)
        (:Row%20Found
          (bind _quest_controller (Utilities|GetQuestController)
            (:Is%20Valid
              (if (or (Utilities|Array|ContainsItem (Variables|/Game/Patchwork/Blueprints/Quests/BP_QuestController.BP_QuestController_C|Getcurrent%20steps _quest_controller) _row_name) (Utilities|Array|ContainsItem (Variables|/Game/Patchwork/Blueprints/Quests/BP_QuestController.BP_QuestController_C|Getcompleted%20steps _quest_controller) _row_name))
                (bind _completion_event (Utilities|GetCompletionEvent :!label _label)
                  (:Row%20Found
                    (Default|InvokeWorldEvent (Variables|Default|GetGame%20Mode) _completion_event))))))))
      (else
        (goto _label)))))

(event EventBeginPlay
  (Collision|BindEventtoOnActorBeginOverlap (Components|GetOwner) (delegate Custom|On%20Overlap))
  (Utilities|GetQuestData
    (:Row%20Found
      (Utilities|GetCompletionEvent
        (:Row%20Found
          (bind _asgm_base_game_mode (Utilities|Casting|CastToGM_BaseGameMode (Game|GetGameMode)))
          (Variables|Default|SetGame%20Mode _asgm_base_game_mode)
          (Utilities|GetQuestController))))))

(event EventTick
  (params (DeltaSeconds :type Float%20%28single-precision%29)))