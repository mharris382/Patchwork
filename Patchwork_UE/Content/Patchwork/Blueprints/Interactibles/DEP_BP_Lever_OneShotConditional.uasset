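; One-shot lever interactible, prefixed DEP, that drives a waterwheel and drawbridge sequence.
; Moving the lever sets HasLeverBeenUsed, which the IsInteractionAvailable override checks alongside the parent result to block reuse.
; BeginPlay casts MainAnimatedItem to the drawbridge and binds OnFinishedMoving.
; When that fires, a DoOnce turns the SecondaryAnimatedItem waterwheel, then calls the drawbridge sequence with IDNum and prints a debug message.
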(event Custom|do%20sequence
  (Utilities|FlowControl|DoOnce false
    (:Completed
      (bind _asbp_water_wheel (Utilities|Casting|CastToBP_WaterWheel (Variables|Sequence|GetSecondaryAnimatedItem)))
      (Default|TurnWaterwheel _asbp_water_wheel)
      (Default|CallSequence (stale EventBeginPlay _asbp_drawbridge) (Variables|Sequence|GetIDNum))
      (Development|PrintString "Call Sequence Function Called" true true "(R=0.000000,G=0.660000,B=1.000000,A=1.000000)" 1e+01))))

(event EventBeginPlay
  (|CallParentFunction)
  (bind _asbp_drawbridge (Utilities|Casting|CastToBP_Drawbridge (Variables|Sequence|GetMainAnimatedItem)))
  (EventDispatchers|BindEventtoOnFinishedMoving (delegate Custom|do%20sequence)))

(event Collision|EventActorBeginOverlap
  (params (OtherActor :type Actor%20Object%20Reference))
  (|CallParentFunction OtherActor))

(event EventTick
  (params (DeltaSeconds :type Float%20%28single-precision%29))
  (|CallParentFunction DeltaSeconds))

(event EventMoveNextPosition
  (Variables|Default|SetHas%20Lever%20Been%20Used true)
  (|CallParentFunction))

(fn ConstructionScript
  (|CallParentFunction))

(fn IsInteractionAvailable
  (if (|CallParentFunction)
    (return (not (Variables|Default|GetHas%20Lever%20Been%20Used)))
    (else
      (return false))))