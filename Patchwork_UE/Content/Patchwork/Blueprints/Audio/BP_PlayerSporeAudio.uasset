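; Player spore audio logic that switches the level's audio bus to match the owner's most toxic spore effect.
; Each tick it finds the highest toxicity above a small threshold among the owner's spore effect components and maps that effect's name to a bus index.
; It sends that index with a trigger to a cached AmbientSound tagged AudioController.
; Clean or unmapped effects use bus zero, with unmapped ones also printing a warning.
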(event EventBeginPlay)

(event EventTick
  (params (DeltaSeconds :type Float%20%28single-precision%29))
  (bind _audio_controller (Utilities|GetAudioController)
    (:Is%20Valid
      (bind (_is_clean _highest_toxicity_effect1) (CallFunction|GetHighestToxicity))
      (if _is_clean
        (CallFunction|UpdateAudioBus _audio_controller :!label _label)
        (elif (.ReturnValue (Utilities|Map|Find (Variables|Default|Geteffect%20to%20trigger%20index%20map) (Variables|/Game/Patchwork/Blueprints/Levels/forest/BP_SporeEffectBase.BP_SporeEffectBase_C|GetSpore%20Effect%20Name _highest_toxicity_effect1)))
          (CallFunction|UpdateAudioBus _audio_controller (.Value (Utilities|Map|Find (Variables|Default|Geteffect%20to%20trigger%20index%20map) (Variables|/Game/Patchwork/Blueprints/Levels/forest/BP_SporeEffectBase.BP_SporeEffectBase_C|GetSpore%20Effect%20Name _highest_toxicity_effect1))))
          (else
            (Development|PrintText (Utilities|Text|FormatText "No Audio Bus implemented for spore effect {0}" (Variables|/Game/Patchwork/Blueprints/Levels/forest/BP_SporeEffectBase.BP_SporeEffectBase_C|GetSpore%20Effect%20Name _highest_toxicity_effect1)))
            (goto _label)))))))

(fn GetHighestToxicity
  (for _array_element (Actor|GetComponentsByClass (Components|GetOwner) "/Game/Patchwork/Blueprints/Levels/forest/BP_PlayerSporeEffectBase.BP_PlayerSporeEffectBase_C")
    (if (> (Variables|/Game/Patchwork/Blueprints/Levels/forest/BP_SporeEffectBase.BP_SporeEffectBase_C|GetCurrent%20Toxicity _array_element) 0.05)
      (if (> (Variables|/Game/Patchwork/Blueprints/Levels/forest/BP_SporeEffectBase.BP_SporeEffectBase_C|GetCurrent%20Toxicity _array_element) (LocalVariables|Gethighest%20toxicity))
        (LocalVariables|Sethighest%20toxicity (Variables|/Game/Patchwork/Blueprints/Levels/forest/BP_SporeEffectBase.BP_SporeEffectBase_C|GetCurrent%20Toxicity _array_element))
        (LocalVariables|Sethighest%20toxicity%20effect _array_element))))
  (return (not (Utilities|IsValid (LocalVariables|Gethighest%20toxicity%20effect))) (LocalVariables|Gethighest%20toxicity%20effect)))

(fn UpdateAudioBus
  (params (InputPin :type Ambient%20Sound%20Object%20Reference) (bus%20index :type Integer))
  (Class|AudioParameterControllerInterface|SetTriggerParameter(Message) InputPin "Trigger_EffectStatus")
  (Effects|Components|ParticleSystem|SetIntParameter InputPin "Bus_Index" bus%20index))