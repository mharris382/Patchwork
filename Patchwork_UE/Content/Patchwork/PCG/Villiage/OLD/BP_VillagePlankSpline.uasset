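; BP_VillagePlankSpline is a village spline Blueprint, filed under an OLD PCG folder, that prepares plank layout parameters.
; Its construction script derives GEN-prefixed values: interior spawning unless a closed loop spawns as a path, grid spawning when either axis exceeds one, and scaled cell size with half-size grid extent.
; It overrides the parent's bounds vertical height with a fixed value and has no active event logic.
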(event EventBeginPlay
  (|CallParentFunction) ; This node is disabled and will not be called.\nDrag off pins to build functionality.
)

(event Collision|EventActorBeginOverlap
  (params (OtherActor :type Actor%20Object%20Reference))
  (|CallParentFunction OtherActor) ; This node is disabled and will not be called.\nDrag off pins to build functionality.
)

(event EventTick
  (params (DeltaSeconds :type Float%20%28single-precision%29))
  (|CallParentFunction DeltaSeconds) ; This node is disabled and will not be called.\nDrag off pins to build functionality.
)

(fn ConstructionScript
  (|CallParentFunction)
  (Utilities|FlowControl|Sequence
    (:then_0
      (Variables|PCGINTERNAL|SetGEN_SpawnInterior (or (not (Variables|Default|GetIsClosedLoop)) (not (Variables|00-Core|GetSpawnAsPath)))))
    (:then_1
      (Variables|PCGINTERNAL|SetGEN_SpawnGrid (or (> (Variables|00-Core|GridSettings|GetGridX) 1) (> (Variables|00-Core|GridSettings|GetGridY) 1))))
    (:then_2
      (bind _output_get (Variables|PCGINTERNAL|SetGEN_CellSize (* (Variables|00-Core|GetCellSize) (Variables|00-Core|GetCellScaleMultiplier))))
      (Variables|PCGINTERNAL|SetGEN_GridExtent (/ (* _output_get (Math|Vector|MakeVector (Math|Conversions|ToFloat(Integer) (Variables|00-Core|GridSettings|GetGridX)) (Math|Conversions|ToFloat(Integer) (Variables|00-Core|GridSettings|GetGridY)) 1.0)) 2.0)))))

(fn GetBoundsVerticalHeight
  (return 1e+02))