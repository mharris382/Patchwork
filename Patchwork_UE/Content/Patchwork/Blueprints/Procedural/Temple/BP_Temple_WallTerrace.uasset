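; Procedural temple wall terrace Blueprint that extends a parent generator, with a PCG-related setup.
; The construction script runs the parent's, derives the scaled generation cell size and preprocesses color variants on its material map.
; Bounds overrides report the wall height and shift the parent's minimum by a Z offset.
; CreateHoles turns hole definitions into PCG points, but its only call, alongside volume sizing and regeneration, sits in disconnected construction logic.
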(event Custom|Print%20Result
  (params (NewParam :type PCG%20Data%20Collection%20Structure))
  (Development|PrintString (Utilities|String|Append "Generated: " (Utilities|GetDisplayName self))))

(event EventBeginPlay)

(event Collision|EventActorBeginOverlap
  (params (OtherActor :type Actor%20Object%20Reference)))

(event EventTick
  (params (DeltaSeconds :type Float%20%28single-precision%29)))

(fn ConstructionScript
  (|CallParentFunction)
  (Utilities|FlowControl|Sequence
    (:then_0
      (Variables|PCGINTERNAL|SetGEN_CellSize (* (Variables|Depricated|GetCell%20Size) (Variables|Depricated|GetConstant%20Scale))))
    (:then_1
      (bind _materialmap_0 (Variables|00-Core|GetMaterialMap_0)
        (:then
          (Default|PreprocessColorVariants _materialmap_0))
        (:else)))))

(fn CreateHoles
  (bind _holes (Variables|Default|GetHoles))
  (if (> (Utilities|Array|Length _holes) 0)
    (Utilities|FlowControl|Sequence
      (:then_0
        (for _array_element _holes
          (Utilities|Array|Add (LocalVariables|Getpcg%20points) (Utilities|Struct|MakePCGPoint (Math|Transform|MakeTransform (.HolePosition (Utilities|Struct|BreakSPCGGridHole _array_element))) 1.0 (* (/ (* (.HoleSize (Utilities|Struct|BreakSPCGGridHole _array_element)) (Variables|Depricated|GetCell%20Size)) 2.0) -1.0) (/ (* (.HoleSize (Utilities|Struct|BreakSPCGGridHole _array_element)) (Variables|Depricated|GetCell%20Size)) 2.0) "(X=1.000000,Y=1.000000,Z=1.000000,W=1.000000)" 0.5 0)))))))

(fn GetBoundsVerticalHeight
  (return (Variables|Depricated|GetWallHeight)))

(fn GetBoundsMinMax
  (bind (_min _max) (|CallParentFunction))
  (return (+ _min (Math|Vector|MakeVector 0.0 0.0 (Variables|00-Core|GetBoundsZOffset))) _max))