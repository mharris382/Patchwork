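; Drawbridge interactible that plays level sequences in response to lever pulls, resetting its rotation and pull count on BeginPlay.
; CallSequence takes a lever ID and increments the count; the first pull picks one of three hint sequences, showing that lever's area water wheel first.
; The second pull plays a fourth sequence, and any later pull plays a fifth.
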(event Custom|Call%20Sequence
  (params (LeverID :type Integer))
  (CallFunction|IncrementPulls)
  ;[0.6233 0.6233 0.6233 0.5] first time we pull any lever we get the game hint
  (if (== (Variables|Default|GetNumOfPulls) 1)
    (CallFunction|DetermineGameHint LeverID LeverID)
    (elif (< (Variables|Default|GetNumOfPulls) 3)
      (Sequencer|Player|Play (Variables|/Script/LevelSequence.LevelSequenceActor|GetSequencePlayer (Variables|Default|GetSequence%204)) :!class /Script/MovieScene.MovieSceneSequencePlayer)
      (else
        (Sequencer|Player|Play (Variables|/Script/LevelSequence.LevelSequenceActor|GetSequencePlayer (Variables|Default|GetSequence%205)) :!class /Script/MovieScene.MovieSceneSequencePlayer)))))

(event EventBeginPlay
  (Transformation|SetActorRotation "-15.000000,0.000000,0.000000")
  (Variables|Default|SetNumOfPulls 0))

(fn ConstructionScript)

(fn IncrementPulls
  (bind _result (Math|Integer|IncrementInt (Variables|Default|GetNumOfPulls))
    (:%20%20
      (Variables|Default|SetNumOfPulls _result))))

(fn DetermineGameHint
  (params (A :type Integer) (A2 :type Integer))
  ;[0.6233 0.6233 0.6233 0.5] If the lever in area 1 was pulled, show the sequence with that water wheel first
  (if (== A2 1)
    (Sequencer|Player|Play (Variables|/Script/LevelSequence.LevelSequenceActor|GetSequencePlayer (Variables|Default|GetSequence%201)) :!class /Script/MovieScene.MovieSceneSequencePlayer)
    (else
      ;[0.6233 0.6233 0.6233 0.5] Area 2 pulled, show that water wheel first
      (if (== A 2)
        (Sequencer|Player|Play (Variables|/Script/LevelSequence.LevelSequenceActor|GetSequencePlayer (Variables|Default|GetSequence%202)) :!class /Script/MovieScene.MovieSceneSequencePlayer)
        (else
          ;[0.6233 0.6233 0.6233 0.5] Otherwise Show the third water wheel first
          (Sequencer|Player|Play (Variables|/Script/LevelSequence.LevelSequenceActor|GetSequencePlayer (Variables|Default|GetSequence%203)) :!class /Script/MovieScene.MovieSceneSequencePlayer))))))