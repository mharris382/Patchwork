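; RandomShelf is a procedural shelf Blueprint that sizes its generation bounds from a shelf mesh and per-axis shelf counts.
; Construction runs SetupGrid before the parent script, enabling the inherited grid mode when any count exceeds one.
; The GetBoundsMinMax override then scales the mesh box by counts and spacing, also setting grid extents and cell size.
; The cell-size divisor swaps the Y and Z counts relative to the extents.
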(event EventBeginPlay
  (|CallParentFunction) ; This node is disabled and will not be called.\nDrag off pins to build functionality.
)

(event Collision|EventActorBeginOverlap
  (params (OtherActor :type Actor%20Object%20Reference))
  (|CallParentFunction OtherActor) ; This node is disabled and will not be called.\nDrag off pins to build functionality.
)

(event EventTick
  (params (DeltaSeconds :type Float%20%28single-precision%29))
  (|CallParentFunction DeltaSeconds) ; This node is disabled and will not be called.\nDrag off pins to build functionality.
)

(fn ConstructionScript
  (PCGINTERNAL|SetupGrid)
  (|CallParentFunction))

(fn GetBoundsMinMax
  (bind _shelfmesh (Variables|Default|GetShelfMesh))
  (bind _shelf_count_x (Variables|Default|GetShelf%20Count%20X))
  (bind _shelf_count_y (Variables|Default|GetShelf%20Count%20Y))
  (bind _shelf_count_z (Variables|Default|GetShelf%20Count%20Z))
  (bind _shelf_spacing (Variables|Default|GetShelf%20Spacing))
  (bind _returnvalue (StaticMesh|GetBoundingBox _shelfmesh))
  (bind _returnvalue_2 (Math|Conversions|ToFloat(Integer) _shelf_count_x))
  (bind _returnvalue_3 (Math|Conversions|ToFloat(Integer) _shelf_count_x))
  (bind _returnvalue_4 (Math|Conversions|ToFloat(Integer) _shelf_count_y))
  (bind _returnvalue_5 (Math|Conversions|ToFloat(Integer) _shelf_count_y))
  (bind _returnvalue_6 (Math|Conversions|ToFloat(Integer) _shelf_count_z))
  (bind _returnvalue_7 (Math|Conversions|ToFloat(Integer) _shelf_count_z))
  (bind _returnvalue_8 (/ _shelf_spacing 2.0))
  (bind (_min _max) (Utilities|Struct|BreakBox _returnvalue))
  (bind _returnvalue_9 (Class|KismetMathLibrary|GetBoxSize _returnvalue))
  (bind _returnvalue_10 (* _returnvalue_8 (Math|Vector|MakeVector _returnvalue_3 _returnvalue_5 _returnvalue_7)))
  (bind _returnvalue_11 (* _returnvalue_9 (Math|Vector|MakeVector _returnvalue_2 _returnvalue_4 _returnvalue_6)))
  (bind _returnvalue_12 (+ _returnvalue_11 _returnvalue_10))
  (|CallParentFunction)
  (if (Variables|PCGINTERNAL|GetGEN_UseGrid)
    (Utilities|FlowControl|Sequence
      (:then_0
        (bind _output_get (Variables|PCGINTERNAL|SetGEN_GridExtents (/ _returnvalue_12 2.0)))
        (Variables|PCGINTERNAL|SetGEN_CellSize (/ _output_get (Math|Vector|MakeVector (Math|Conversions|ToFloat(Integer) (Variables|Default|GetShelf%20Count%20X)) (Math|Conversions|ToFloat(Integer) (Variables|Default|GetShelf%20Count%20Z)) (Math|Conversions|ToFloat(Integer) (Variables|Default|GetShelf%20Count%20Y))))))
      (:then_1
        (return _min (+ _min _returnvalue_12))))
    (else
      (return _min _max))))

(fn SetupGrid
  (bind _shelf_count_x (Variables|Default|GetShelf%20Count%20X))
  (bind _shelf_count_y (Variables|Default|GetShelf%20Count%20Y))
  (bind _shelf_count_z (Variables|Default|GetShelf%20Count%20Z))
  (bind _returnvalue (Math|Integer|Max(Integer) _shelf_count_x _shelf_count_y _shelf_count_z))
  (bind _returnvalue_2 (> _returnvalue 1))
  (Variables|PCGINTERNAL|SetGEN_UseGrid _returnvalue_2)
  (if _returnvalue_2
    _))