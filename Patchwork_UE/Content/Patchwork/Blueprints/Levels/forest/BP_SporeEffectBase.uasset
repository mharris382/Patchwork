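; Base component for spore effects, tracking a 0-1 toxicity on its owner and firing gained, changed and lost events.
; Settings come from DT_SporeEffects by effect name, and player-owned effects register a HUD indicator.
; Each tick, toxicity rises inside matching active spore regions, decays outside, and absorbs instant changes before calling the OnToxicityChanged hook.
; It syncs its gameplay tag with BP_SporeCarrier, clearing toxicity when the tag is missing and the owner is wet.
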(event Custom|Instant%20Change
  (params (Amount :type Float%20%28double-precision%29))
  (Variables|Default|SetInstant%20Toxicity%20Change (/ Amount (.effectduration (Variables|Default|GetSpore%20Effect%20Settings)))))

(event Custom|Update%20Spore%20Effects
  (params (DT :type Float%20%28double-precision%29))
  (bind _effecttag (Variables|Default|GetEffectTag))
  (bind _effecttag_2 (Variables|Default|GetEffectTag))
  (bind _in_spore_region (CallFunction|UpdateSporeZone))
  (Variables|Default|SetInside%20Spore%20Zone _in_spore_region)
  (Utilities|FlowControl|Sequence
    (:then_0
      (Utilities|WillImmediatelyClearSpore
        (:normal
          (if (!= (Variables|Default|GetCurrent%20Toxicity) (Math|Float|Clamp(Float) (+ (/ (CallFunction|GetCurrentContinousRate DT) (.effectduration (Variables|Default|GetSpore%20Effect%20Settings))) (Variables|Default|GetInstant%20Toxicity%20Change) (Variables|Default|GetCurrent%20Toxicity))))
            (CallFunction|CheckforEvents (Variables|Default|GetCurrent%20Toxicity) (Math|Float|Clamp(Float) (+ (/ (CallFunction|GetCurrentContinousRate DT) (.effectduration (Variables|Default|GetSpore%20Effect%20Settings))) (Variables|Default|GetInstant%20Toxicity%20Change) (Variables|Default|GetCurrent%20Toxicity))))
            (bind _output_get (Variables|Default|SetCurrent%20Toxicity (Math|Float|Clamp(Float) (+ (/ (CallFunction|GetCurrentContinousRate DT) (.effectduration (Variables|Default|GetSpore%20Effect%20Settings))) (Variables|Default|GetInstant%20Toxicity%20Change) (Variables|Default|GetCurrent%20Toxicity)))))
            (CallFunction|OnToxicityChanged _output_get)
            (else
              (CallFunction|OnToxicityChanged (Variables|Default|GetCurrent%20Toxicity)))))
        (:cleanse%20spores
          ;[0.6233 0.6233 0.6233 0.5] Cleanse spores (this could happen b/c state is wet so spore effect was lost)
          (if (!= (Variables|Default|GetCurrent%20Toxicity) 0.0)
            (CallFunction|CheckforEvents (Variables|Default|GetCurrent%20Toxicity) 0.0)
            (bind _output_get_2 (Variables|Default|SetCurrent%20Toxicity 0.0))
            (CallFunction|OnToxicityChanged _output_get_2)))))
    (:then_1
      (Variables|Default|SetInstant%20Toxicity%20Change 0.0))
    (:then_2
      (if (> (Variables|Default|GetCurrent%20Toxicity) 0.001)
        (Utilities|FlowControl|DoOnce false :!label _label
          (:Completed
            (Default|CallOnEffectGained)
            (goto _label_2 Reset)))
        (else
          (Utilities|FlowControl|Sequence
            (:then_0
              (Utilities|FlowControl|DoOnce true :!label _label_2
                (:Completed
                  (Default|CallOnEffectLost)
                  (goto _label Reset))))
            (:then_1
              (bind _sporecarrier (Variables|Default|GetSporeCarrier)
                (:then
                  (Utilities|FlowControl|Sequence
                    (:then_0
                      (if (not (Default|HasSporefromTag _sporecarrier _effecttag))
                        (if (GameplayTags|HasTag (Variables|/Game/Patchwork/Blueprints/Utilities/GameplayObjectState.GameplayObjectState_C|GetGameplayState _sporecarrier) _effecttag true)
                          (Development|PrintText "WTF HOW!"))))
                    (:then_1
                      (Default|RemoveSporeTypefromTag _sporecarrier _effecttag_2)
                      (Default|RemoveGameplayTag _sporecarrier _effecttag_2))))
                (:else)))))))))

(event Custom|LoseTag
  (bind _sporecarrier (Variables|Default|GetSporeCarrier)
    (:then
      (Default|RemoveSporeTypefromTag _sporecarrier (Variables|Default|GetEffectTag)))
    (:else)))

(event EventBeginPlay
  (bind _sporehelper_0 (Variables|Default|GetSporeHelper_0))
  (bind _spore_effect_name (Variables|Default|GetSpore%20Effect%20Name))
  (bind _sporenametogameplaytags (Utilities|GetClassDefaults _sporehelper_0))
  (bind (_value _returnvalue) (Utilities|Map|Find _sporenametogameplaytags _spore_effect_name))
  (Utilities|FlowControl|Sequence
    (:then_0
      ;[0.6233 0.6233 0.6233 0.5] Cache Spore Helper
      (Variables|Default|SetSporeHelper (Actor|GetComponentbyClass (Game|GetGameMode) "/Game/Patchwork/Blueprints/Levels/forest/BP_GlobalSporeHelper.BP_GlobalSporeHelper_C")))
    (:then_1
      (bind _returnvalue_2 (Utilities|GetDataTableRow "/Game/Patchwork/Data/Datatables/DT_SporeEffects.DT_SporeEffects" (Variables|Default|GetSpore%20Effect%20Name))
        (:then
          (Utilities|FlowControl|Sequence
            (:then_0
              (Utilities|Array|AddUnique (Variables|Default|GetComponentTags) (Variables|Default|GetSpore%20Effect%20Name)))
            (:then_1
              (Variables|Default|SetSpore%20Effect%20Settings _returnvalue_2)
              (bind _output_get (Variables|Default|SetIs%20Player (== (Game|Player|GetPlayerPawn 0) (Components|GetOwner))))
              (if _output_get
                (bind _aspatchwork_player_controller (Utilities|Casting|CastToPatchworkPlayerController (Game|GetPlayerController 0)))
                (Default|AddSporeIndicator _aspatchwork_player_controller self)))))
        (:RowNotFound
          (Development|PrintText (Utilities|Text|FormatText "the name {0} does not have a valid spore effect name: {1}" (Variables|Default|GetSpore%20Effect%20Name) (Utilities|GetClassDisplayName (Utilities|GetClass self)))))))
    (:then_2
      (if _returnvalue
        (Variables|Default|SetEffectTag _value)
        (else
          (Development|PrintText (Utilities|Text|FormatText "WARNING: Spore Effect Class ({1}) with Spore Type ({0}) has not been upgraded to the Gameplay Tag System.  It may mnot function correctly" (Utilities|GetClassDisplayName (Utilities|GetClass self)) (Variables|Default|GetSpore%20Effect%20Name)) true true "(R=1.000000,G=0.002809,B=0.000000,A=1.000000)" 1.0))))
    (:then_3
      (if (GameplayTags|IsGameplayTagValid (Variables|Default|GetEffectTag))
        (Variables|Default|SetSporeCarrier (Actor|GetComponentbyClass (Components|GetOwner) "/Game/Patchwork/Blueprints/Levels/forest/Utilities/BP_SporeCarrier.BP_SporeCarrier_C"))
        (EventDispatchers|BindEventtoOnEffectLost (delegate Custom|LoseTag))))))

(event EventTick
  (params (DeltaSeconds :type Float%20%28single-precision%29))
  (CallFunction|UpdateSporeEffects DeltaSeconds))

(fn GetCurve
  (bind _spore_effect_settings (Variables|Default|GetSpore%20Effect%20Settings))
  (return (.AsCurve%20Float (Utilities|Casting|CastToCurveFloat (Utilities|SelectObject (.toxicitycurve _spore_effect_settings) (Variables|Default|GetDefault%20Curve) (Utilities|IsValid (.toxicitycurve _spore_effect_settings)))))))

(fn GetCurrentContinousRate
  (params (delta%20time :type Float%20%28double-precision%29))
  (return (* delta%20time (Math|Float|SelectFloat (.gainrate (Variables|Default|GetSpore%20Effect%20Settings)) -1.0 (Variables|Default|GetInside%20Spore%20Zone)))))

(fn OnToxicityChanged
  (params (new%20toxicity :type Float%20%28double-precision%29)))

(fn GetEffect
  (return (Variables|Default|GetSpore%20Effect%20Settings)))

(fn CheckforEvents
  (params (old%20toxicity :type Float%20%28double-precision%29) (new%20toxicity :type Float%20%28double-precision%29))
  (bind _returnvalue (Math|Float|Clamp(Float) old%20toxicity))
  (bind _returnvalue_2 (Math|Float|Clamp(Float) new%20toxicity))
  (Utilities|FlowControl|Sequence
    (:then_0
      (if (!= _returnvalue _returnvalue_2)
        (Default|CallOnEffectChanged _returnvalue _returnvalue_2)))
    (:then_1
      (if (and (<= old%20toxicity 0.0) (> new%20toxicity 0.0))
        (Default|CallOnEffectGained)
        (elif (and (> old%20toxicity 0.0) (<= new%20toxicity 0.0))
          (Default|CallOnEffectLost))))))

(fn VerifyInsideSporeZone
  (if (and (== (Utilities|Array|Length (Collision|GetOverlappingActors (Components|GetOwner) "/Game/Patchwork/Blueprints/Levels/forest/Spores/BP_SporeRegion.BP_SporeRegion_C" :!class /Script/Engine.Actor)) 0) (Variables|Default|GetInside%20Spore%20Zone))
    (Variables|Default|SetInside%20Spore%20Zone false)))

(fn UpdateSporeZone
  (bind _ascharacter (Utilities|Casting|CastToCharacter (Components|GetOwner))
    (:then
      (for _array_element (Collision|GetOverlappingActors (Variables|/Script/Engine.Character|GetCapsuleComponent _ascharacter) "/Game/Patchwork/Blueprints/Levels/forest/Spores/BP_SporeRegion.BP_SporeRegion_C" :!class /Script/Engine.PrimitiveComponent)
        (bind _asbp_spore_region (Utilities|Casting|CastToBP_SporeRegion _array_element))
        (if (and (Default|MatchesSporeType _asbp_spore_region (Variables|Default|GetSpore%20Effect%20Name)) (Variables|/Game/Patchwork/Blueprints/Levels/forest/Spores/BP_SporeRegion.BP_SporeRegion_C|Getis%20active _asbp_spore_region))
          (return true))))
    (:CastFailed
      _))
  (return false))

(fn CleanseSpore)