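; BP_Guard_C is a guard character Blueprint that opens a referenced door and notifies a listener sequence when its dialogue ends.
; OpenDoor forwards the call to the Door reference, printing a warning if it is missing.
; DialogueFinished starts a short looping timer that polls the dialogue component until it leaves dialogue, then informs ListenerSequence and clears the timer.
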(event Custom|Open%20Door
  (bind _door (Variables|Default|GetDoor))
  (Utilities|IsValid _door
    (:Is%20Valid
      (Default|OpenDoor _door))
    (:Is%20Not%20Valid
      (Development|PrintText "Guard is missing door reference"))))

(event Custom|DialogueFinished
  (bind _returnvalue (Utilities|Time|SetTimerbyEvent (delegate Custom|WaitForDialogueToEnd) 0.1 true))
  (Variables|Default|SetWaitHandle _returnvalue))

(event Custom|WaitForDialogueToEnd
  (bind _listenersequence (Variables|Default|GetListenerSequence))
  (if (not (Variables|/Game/Templates/Defender/Blueprints/Components/DialogueComp.DialogueComp_C|GetInDialogue (Variables|Default|GetDialogueComp)))
    (Utilities|FlowControl|Sequence
      (:then_0
        (Utilities|IsValid _listenersequence
          (:Is%20Valid
            (Default|DialogueFinished _listenersequence))))
      (:then_1
        (Utilities|Time|ClearandInvalidateTimerbyHandle (Variables|Default|GetWaitHandle))))))

(event EventBeginPlay
  (|CallParentFunction) ; This node is disabled and will not be called.\nDrag off pins to build functionality.
)

(event Collision|EventActorBeginOverlap
  (params (OtherActor :type Actor%20Object%20Reference))
  (|CallParentFunction OtherActor) ; This node is disabled and will not be called.\nDrag off pins to build functionality.
)

(event EventTick
  (params (DeltaSeconds :type Float%20%28single-precision%29))
  (|CallParentFunction DeltaSeconds))

(fn ConstructionScript
  (|CallParentFunction))