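; Utility Blueprint that hands out shared emissive dynamic material instances keyed by color.
; GetMaterialInstanceForColor looks the color up in the EmissiveMaterialCache map and returns the stored instance if one exists.
; Otherwise it creates an instance from DefaultEmissiveParent, sets its Color vector parameter, caches it and returns it, so each color gets only one instance.
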(event EventBeginPlay)

(event Collision|EventActorBeginOverlap
  (params (OtherActor :type Actor%20Object%20Reference)))

(event EventTick
  (params (DeltaSeconds :type Float%20%28single-precision%29)))

(fn ConstructionScript)

(fn GetMaterialInstanceforColor
  (params (Color :type Linear%20Color%20Structure))
  (bind _emissivematerialcache (Variables|Default|GetEmissiveMaterialCache))
  (bind (_value _returnvalue) (Utilities|Map|Find _emissivematerialcache Color))
  (if _returnvalue
    (return _value)
    (else
      (bind _returnvalue_2 (Rendering|Material|CreateDynamicMaterialInstance (Variables|Default|GetDefaultEmissiveParent) "None" "None" :!class /Script/Engine.KismetMaterialLibrary))
      (Rendering|Material|SetVectorParameterValue _returnvalue_2 "Color" Color :!class /Script/Engine.MaterialInstanceDynamic)
      (Utilities|Map|Add (Variables|Default|GetEmissiveMaterialCache) Color _returnvalue_2)
      (return _returnvalue_2))))