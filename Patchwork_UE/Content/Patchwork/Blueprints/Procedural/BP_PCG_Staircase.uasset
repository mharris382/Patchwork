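; Custom PCG Blueprint element for staircases that levels point rotations so each point stands upright along its original heading.
; It converts spatial data from its first custom input pin to point data, runs a point loop and outputs the results with target actors preserved.
; The loop rebuilds rotation from each point's right vector and world up, keeping location and scale.
; Its node title reads "Curve Remap Density", although it never touches density.
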(fn ExecutewithContext
  (params (InContext :type PCG%20Context%20Structure%20%28by%20ref%29) (Input :type PCG%20Data%20Collection%20Structure%20%28by%20ref%29))
  (bind _result (Utilities|Set|ToArray (PCG|Input&Output|CustomInputLabels self)))
  (bind _returnvalue (Data|GetInputsbyPinLabel Input (Utilities|Array|Get(acopy) _result)))
  (for _array_element _returnvalue
    (bind _aspcgspatial_data (Utilities|Casting|CastToPCGSpatialData (.Data (Utilities|Struct|BreakPCGTaggedData _array_element))))
    (bind _outdata (PCG|FlowControl|PointLoop InContext (SpatialData|ToPointDatawithContext _aspcgspatial_data InContext) 0))
    (Variables|/Script/PCG.PCGSpatialData|SetTargetActor _outdata (Variables|/Script/PCG.PCGSpatialData|GetTargetActor _aspcgspatial_data))
    (Utilities|Array|Add (Variables|Default|GetTagged%20Data) (Utilities|Struct|MakePCGTaggedData _outdata 0 "None")))
  (return (Utilities|Struct|MakePCGDataCollection (Variables|Default|GetTagged%20Data))))

(fn PointLoopBody
  (params (InContext :type PCG%20Context%20Structure%20%28by%20ref%29) (InData :type PCG%20Point%20Data%20Object%20Reference) (InPoint :type PCG%20Point%20Structure%20%28by%20ref%29) (OutMetadata :type PCG%20Metadata%20Object%20Reference) (Iteration :type Integer64))
  (bind _transform (Utilities|Struct|BreakPCGPoint InPoint))
  (bind (_location _rotation _scale) (Math|Transform|BreakTransform _transform))
  (bind _structout (Utilities|Struct|SetmembersinPCGPoint InPoint (Math|Transform|MakeTransform _location (Class|KismetMathLibrary|MakeRotfromYZ (Math|Vector|GetRightVector _rotation) (Math|Vector|VectorUp)) _scale)))
  (return _structout true))

(fn NodeTitleOverride
  (return "Curve Remap Density"))