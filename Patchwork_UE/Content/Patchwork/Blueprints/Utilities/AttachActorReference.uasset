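; Utility component that links a referenced actor to its owner and lets that actor stand in as the controlled actor.
; On BeginPlay, a valid OtherActor is attached to the owner, keeping its world transform.
; Components listed in DestroyIfActorFound are first cleared: static meshes are hidden with collision disabled, others are destroyed.
; GetControlledActor returns OtherActor when valid, otherwise the owner.
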(event EventBeginPlay
  (if (CallFunction|HasControlledActor)
    (CallFunction|DestroyonFound)
    (Transformation|AttachActorToActor (Variables|Default|GetOtherActor) (Components|GetOwner) "None" "KeepWorld" "KeepWorld" "KeepWorld" true)))

(event EventTick
  (params (DeltaSeconds :type Float%20%28single-precision%29)))

(fn GetControlledActor
  (bind _otheractor (Variables|Default|GetOtherActor))
  (return (select (Utilities|IsValid _otheractor) _otheractor (Components|GetOwner))))

(fn HasControlledActor
  (return (Utilities|IsValid (Variables|Default|GetOtherActor))))

(fn DestroyonFound
  (for _array_element (Variables|Default|GetDestroyIfActorFound)
    (Utilities|IsValid _array_element
      (:Is%20Valid
        (bind _asstatic_mesh_component (Utilities|Casting|CastToStaticMeshComponent _array_element)
          (:then
            (Rendering|SetVisibility _asstatic_mesh_component false false)
            (Collision|SetCollisionEnabled _asstatic_mesh_component "NoCollision"))
          (:CastFailed
            (Components|DestroyComponent _array_element)))))))