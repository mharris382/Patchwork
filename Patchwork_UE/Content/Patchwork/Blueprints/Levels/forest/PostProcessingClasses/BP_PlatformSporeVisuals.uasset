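; BP_PlatformSporeVisuals attaches a spore particle effect to the player's paperperson pawn, filed under the forest level's post-processing classes.
; On BeginPlay it runs the parent logic, spawns NS_PlatformSpawnSporeVisuals on the player's mesh, stores it as SporeVisualSystem and zeroes its Spore Toxicity parameter.
; The UpdateBlend event is empty, so this Blueprint never changes the toxicity afterwards.
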(event EventBeginPlay
  (|CallParentFunction)
  (bind _aspaperperson (Utilities|Casting|CastTopaperperson (Game|Player|GetPlayerPawn 0)))
  (bind _returnvalue (Niagara|SpawnSystemAttached "/Game/Patchwork/Effects/Platforms/NS_PlatformSpawnSporeVisuals.NS_PlatformSpawnSporeVisuals" (Variables|/Script/Engine.Character|GetMesh _aspaperperson) "None" "0, 0, 0" "0, 0, 0" "KeepRelativeOffset" false))
  (bind _output_get (Variables|Default|SetSpore%20Visual%20System _returnvalue))
  (Effects|Components|ParticleSystem|SetFloatParameter _output_get "Spore Toxicity" 0.0))

(event Collision|EventActorBeginOverlap
  (params (OtherActor :type Actor%20Object%20Reference))
  (|CallParentFunction OtherActor) ; This node is disabled and will not be called.\nDrag off pins to build functionality.
)

(event EventTick
  (params (DeltaSeconds :type Float%20%28single-precision%29))
  (|CallParentFunction DeltaSeconds) ; This node is disabled and will not be called.\nDrag off pins to build functionality.
)

(event EventUpdateBlend
  (params (blend :type Float%20%28double-precision%29)))

(fn ConstructionScript
  (|CallParentFunction))