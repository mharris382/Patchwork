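; BP_Candle_3 is a three-candle prop with a holder for the Dark Fantasy Church set, switchable through an Enabled flag.
; The construction script passes that flag to SetEnableCandle, which stores it and sets the visibility of the three particle systems.
; The same function sets shadow casting on the candle and holder meshes to the inverse, so they cast no shadows while enabled.
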(fn ConstructionScript
  ;[1 1 1] Activar Function Enable Cande
  (CallFunction|SetEnableCandle (Variables|Default|GetEnabled)))

(fn SetEnableCandle
  (params (Enabled :type Boolean))
  ;[1 1 1] Setear Enabled Bool
  (bind _output_get (Variables|Default|SetEnabled Enabled))
  ;[1 0.524 0.5406] Particles
  (Rendering|SetVisibility (Variables|Default|GetParticleSystem) _output_get false)
  ;[1 1 1] Cast Shadow Mesh
  (Rendering|SetCastShadow (Variables|Default|GetCandle) (not _output_get)))