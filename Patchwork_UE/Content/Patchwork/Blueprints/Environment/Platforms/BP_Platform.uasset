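; Moving platform that oscillates between two local positions and can drop under physics or rise back to its hover point.
; Tick advances a sine-driven lerp of the hover point, carrying the mesh and any AttachActorReference-controlled actor while hovering.
; Optional pressure plate events ease the speed multiplier between pressed and depressed rates.
; Rising uses a randomly delayed timeline with quaternion slerp, and construction-time setup mode previews both endpoints with temporary meshes.
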(event Custom|Rise%20To%20Hover%20Point
  (bind _platform_mesh (Variables|Default|GetPlatform%20Mesh))
  ;[1 1 1] add random delay to rise animation
  (Variables|Default|Setrising true)
  (Utilities|FlowControl|Delay (Math|Random|RandomFloatinRange 0.0 (Variables|DynamicPhysics|Getrise%20delay)))
  (if (Variables|Default|Getrising) ; check not released after delay
    ;[1 1 1] Cache start loc and rotation before starting animtion
    (Variables|Default|Setstart%20position (Transformation|GetWorldLocation _platform_mesh))
    (Variables|Default|Setstart%20rotation (Transformation|GetWorldRotation _platform_mesh))
    (CallFunction|SetSimulatePhysics false)
    (bind _rise (Timeline|Rise PlayFromStart)
      (:Update
        ;[1 1 1] Lerp from start points to hover position
        (Transformation|SetWorldLocationAndRotation (Variables|Default|GetPlatform%20Mesh) (Math|Vector|Lerp(Vector) (Variables|Default|Getstart%20position) (Transformation|GetWorldLocation (Variables|Default|GetHover%20Position)) _rise) (Class|KismetMathLibrary|QuatRotator (Class|KismetMathLibrary|QuatSlerp (Math|Conversions|ToQuaternion(Rotator) (Variables|Default|Getstart%20rotation)) (Math|Conversions|ToQuaternion(Rotator) (Transformation|GetWorldRotation (Variables|Default|GetHover%20Position))) _rise)) false false))
      (:Finished
        (Variables|Default|SetIs%20Hovering true)))))

(event Custom|Release%20from%20Hover%20Point
  (Variables|Default|Setrising false)
  (Variables|Default|SetIs%20Hovering false)
  (CallFunction|SetSimulatePhysics true)
  (bind _rise (Timeline|Rise Stop)
    (:Update
      ;[1 1 1] Lerp from start points to hover position
      (Transformation|SetWorldLocationAndRotation (Variables|Default|GetPlatform%20Mesh) (Math|Vector|Lerp(Vector) (Variables|Default|Getstart%20position) (Transformation|GetWorldLocation (Variables|Default|GetHover%20Position)) _rise) (Class|KismetMathLibrary|QuatRotator (Class|KismetMathLibrary|QuatSlerp (Math|Conversions|ToQuaternion(Rotator) (Variables|Default|Getstart%20rotation)) (Math|Conversions|ToQuaternion(Rotator) (Transformation|GetWorldRotation (Variables|Default|GetHover%20Position))) _rise)) false false))
    (:Finished
      (Variables|Default|SetIs%20Hovering true))))

(event Custom|SetDepressed)

(event Custom|Set%20Pressed)

(event EventBeginPlay
  (Utilities|FlowControl|Sequence
    (:then_0
      (CallFunction|SetSetupModeEnabled false))
    (:then_1
      ;[0.6233 0.6233 0.6233 0.5] Hover Stuff
      (if (Variables|DynamicPhysics|Getrelease%20on%20start)
        (CallFunction|ReleasefromHoverPoint)
        (else
          (Variables|Default|SetIs%20Hovering true)
          (CallFunction|SetSimulatePhysics false))))
    (:then_2
      (Utilities|IsPressurePlateListener
        (:then
          (Variables|Mechanism|SetSpeedMultiplier 0.0))
        (:false
          (Variables|Mechanism|SetSpeedMultiplier 1.0))))))

(event EventOnPlateDepressed
  (Utilities|IsPressurePlateListener
    (:then
      (Variables|Mechanism|SetIsPressed false)
      (CallFunction|SetDepressed))))

(event EventTick
  (params (DeltaSeconds :type Float%20%28single-precision%29))
  (CallFunction|UpdatePressed DeltaSeconds)
  ;[1 1 1] update hover point position
  (bind _output_get (Variables|Movement|Sett (+ (* DeltaSeconds (Variables|Movement|GetSpeed) (Variables|Mechanism|GetSpeedMultiplier)) (Variables|Movement|Gett))))
  (CallFunction|UpdatePosition _output_get false))

(event EventOnPlatePressed
  (Utilities|IsPressurePlateListener
    (:then
      (Variables|Mechanism|SetIsPressed true)
      (CallFunction|SetPressed))))

(fn ConstructionScript
  (Utilities|FlowControl|Sequence
    (:then_0
      (Utilities|IsValid (Variables|Mesh|GetStatic%20Mesh%20Asset)
        (:Is%20Valid
          (Components|StaticMesh|SetStaticMesh (Variables|Default|GetPlatform%20Mesh) (Variables|Mesh|GetStatic%20Mesh%20Asset)))
        (:Is%20Not%20Valid
          _))
      (CallFunction|UpdatePosition (* (Variables|Movement|Gett) (Variables|Movement|GetSpeed)) false)
      (Transformation|SetWorldLocation (Variables|Default|GetPlatform%20Mesh) (Transformation|GetWorldLocation (Variables|Default|GetHover%20Position)) false false))
    (:then_1
      (CallFunction|SetSetupModeEnabled (Variables|Movement|GetSetup%20Mode)))
    (:then_2
      (Utilities|Array|Add (Variables|/Game/Patchwork/Blueprints/Utilities/AttachActorReference.AttachActorReference_C|GetDestroyIfActorFound (Variables|Default|GetAttachActorReference)) (Variables|Default|GetPlatform%20Mesh)))))

(fn UpdatePosition
  (params (t :type Float%20%28double-precision%29) (sweep :type Boolean))
  (bind _hover_position (Variables|Default|GetHover%20Position))
  (bind _attachactorreference (Variables|Default|GetAttachActorReference))
  (bind _returnvalue (Transformation|GetWorldLocation _hover_position))
  (bind _controlled_actor (Default|GetControlledActor _attachactorreference))
  (Transformation|SetRelativeLocation (Variables|Default|GetHover%20Position) (CallFunction|GePositionfromInterpTime (CallFunction|GetMoveInterpTime t)) false false)
  ;[1 1 1] if hovering update platform position
  (if (Variables|Default|GetIs%20Hovering)
    (Transformation|SetWorldLocation (Variables|Default|GetPlatform%20Mesh) _returnvalue false false)
    (if (and (Default|HasControlledActor _attachactorreference) (Utilities|IsValid _controlled_actor))
      (Transformation|SetActorLocation _controlled_actor _returnvalue false false))))

(fn SetSimulatePhysics
  (params (bSimulate :type Boolean))
  (Physics|SetSimulatePhysics (Variables|Default|GetPlatform%20Mesh) bSimulate))

(fn SetSetupModeEnabled
  (params (enabled :type Boolean))
  (if enabled
    (Utilities|FlowControl|Sequence
      (:then_0
        (Utilities|DestroySetupChildren))
      (:then_1
        (Utilities|AddSetupMesh (Variables|Movement|GetPosition%201))
        (Utilities|AddSetupMesh (Variables|Movement|GetPosition%202))))
    (else
      (Utilities|DestroySetupChildren)
      (Rendering|SetVisibility (Variables|Default|GetPlatform%20Mesh) true false))))

(fn UpdatePressed
  (params (dt :type Float%20%28double-precision%29))
  (Utilities|IsPressurePlateListener
    (:then
      (Utilities|FlowControl|Sequence
        (:then_0
          (LocalVariables|Settarget (Math|Float|SelectFloat (Variables|Mechanism|Speed|GetPressedSpeedMultiplier) (Variables|Mechanism|Speed|GetDepressedSpeedMultiplier) (Variables|Mechanism|GetIsPressed)))
          (LocalVariables|Setrate (Math|Float|SelectFloat (Variables|Mechanism|Speed|GetStartMovingAccelerationRate) (Variables|Mechanism|Speed|GetStopMovingSlowdownRate) (Variables|Mechanism|GetIsPressed))))
        (:then_1
          (Variables|Mechanism|SetSpeedMultiplier (Math|Interpolation|FInterpTo (Variables|Mechanism|GetSpeedMultiplier) (LocalVariables|Gettarget) dt (LocalVariables|Getrate))))))
    (:false
      (Variables|Mechanism|SetSpeedMultiplier 1.0))))

(fn GetMoveInterpTime
  (params (A :type Float%20%28double-precision%29))
  (return (Math|Float|MapRangeClamped (Math|Trig|Sin(Radians) A) -1.0 1.0 0.0 1.0)))

(fn GePositionfromInterpTime
  (params (percent :type Float%20%28single-precision%29))
  (return (Math|Vector|Lerp(Vector) (Variables|Movement|GetPosition%201) (Variables|Movement|GetPosition%202) percent)))