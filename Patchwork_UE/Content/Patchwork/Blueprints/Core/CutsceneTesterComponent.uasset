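; CutsceneTesterComponent is an actor component for testing cutscenes, meant to sit on a Level Sequence Actor.
; When its Test flag is on, BeginPlay waits a configurable delay, then plays the owner's sequence either once or looping indefinitely.
; It can then move the first player's pawn to the location of a referenced position actor, if teleporting is enabled and that actor is valid.
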(event EventBeginPlay
  (bind _returnvalue (Components|GetOwner))
  (bind _aslevel_sequence_actor (Utilities|Casting|CastToLevelSequenceActor _returnvalue))
  (bind _sequenceplayer (Variables|/Script/LevelSequence.LevelSequenceActor|GetSequencePlayer _aslevel_sequence_actor))
  (if (Variables|Default|GetTest)
    (Utilities|FlowControl|Delay (Variables|Default|GetDelay))
    (Utilities|FlowControl|Sequence
      (:then_0
        (if (Variables|Default|GetLooping)
          (Class|MovieSceneSequencePlayer|PlayLooping _sequenceplayer -1)
          (else
            (Sequencer|Player|Play _sequenceplayer :!class /Script/MovieScene.MovieSceneSequencePlayer))))
      (:then_1
        (if (Variables|Default|GetTeleportPlayer)
          (bind _teleportplayerposition (Variables|Default|GetTeleportPlayerPosition)
            (:then
              (Transformation|SetActorLocation (Game|Player|GetPlayerPawn 0) (Transformation|GetActorLocation _teleportplayerposition) false false))
            (:else)))))))