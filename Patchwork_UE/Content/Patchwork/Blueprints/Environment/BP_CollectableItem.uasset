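; BP_CollectableItem is a collectable item actor that spins in the world and takes its appearance from a data table row.
; The construction script looks up the Item row handle and applies that row's mesh to the static mesh, which Tick rotates around yaw at SpinRate.
; It overrides the parent's collectable functions, hiding the mesh when collected and returning the row name as its collectable ID.
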(event EventBeginPlay
  (|CallParentFunction) ; This node is disabled and will not be called.\nDrag off pins to build functionality.
)

(event Collision|EventActorBeginOverlap
  (params (OtherActor :type Actor%20Object%20Reference))
  (|CallParentFunction OtherActor) ; This node is disabled and will not be called.\nDrag off pins to build functionality.
)

(event EventTick
  (params (DeltaSeconds :type Float%20%28single-precision%29))
  (Transformation|AddRelativeRotation (Variables|Default|GetStaticMesh) (Math|Rotator|MakeRotator 0.0 0.0 (* DeltaSeconds (Variables|Default|GetSpin%20Rate))) false false))

(fn ConstructionScript
  (bind _item (Variables|Default|GetItem))
  (|CallParentFunction)
  (bind _returnvalue (Utilities|GetDataTableRow (.datatable _item) (.rowname _item))
    (:then
      (Components|StaticMesh|SetStaticMesh (Variables|Default|GetStaticMesh) (.Mesh (Utilities|Struct|BreakS_CollectableItemData _returnvalue))))))

(fn SetCollected
  (params (collected :type Boolean))
  (|CallParentFunction collected)
  (Rendering|SetVisibility (Variables|Default|GetStaticMesh) (not collected) false))

(fn GetCollectableID
  (return (.rowname (Variables|Default|GetItem))))