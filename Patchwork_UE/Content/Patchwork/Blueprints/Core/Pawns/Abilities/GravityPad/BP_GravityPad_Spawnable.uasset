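; A spawnable gravity pad from the player abilities that bounces the player along the pad's up axis.
; On BeginPlay it sizes its box collision from the gravity well radius and height in GlobalAbilitySettings and offsets it by half that height along the actor's up vector.
; When the player character begins overlapping, it sends a bounce force message scaled by the player impulse multiplier, with no XY or Z override.
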(event EventBeginPlay
  (bind _globalabilitysettings (Variables|Default|GetGlobalAbilitySettings))
  (bind _gravitywellradius (Variables|/Game/Patchwork/Blueprints/Utilities/BP_GlobalAbilitySettings.BP_GlobalAbilitySettings_C|GetGravityWellRadius _globalabilitysettings))
  (Components|Box|SetBoxExtent (Variables|Default|GetBoxCollision) (Math|Vector|MakeVector _gravitywellradius _gravitywellradius (/ (Variables|/Game/Patchwork/Blueprints/Utilities/BP_GlobalAbilitySettings.BP_GlobalAbilitySettings_C|GetGravityWellHeight _globalabilitysettings) 2.0)) true)
  (Transformation|SetRelativeLocation (Variables|Default|GetBoxCollision) (* (Transformation|GetActorUpVector) (/ (Variables|/Game/Patchwork/Blueprints/Utilities/BP_GlobalAbilitySettings.BP_GlobalAbilitySettings_C|GetGravityWellHeight (Variables|Default|GetGlobalAbilitySettings)) 2.0)) false false))

(event Collision|EventActorBeginOverlap
  (params (OtherActor :type Actor%20Object%20Reference))
  (bind _returnvalue (Game|GetPlayerCharacter 0))
  (if (== OtherActor _returnvalue)
    (Class|BPIPlayerPawn|ApplyBounceForce(Message) _returnvalue (* (Transformation|GetActorUpVector) (Variables|/Game/Patchwork/Blueprints/Utilities/BP_GlobalAbilitySettings.BP_GlobalAbilitySettings_C|GetPlayerImpulseMultiplier (Variables|Default|GetGlobalAbilitySettings))) false false)))

(event EventTick
  (params (DeltaSeconds :type Float%20%28single-precision%29)))

(fn ConstructionScript)