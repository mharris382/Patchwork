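; One-shot lever interactible that can be used only once and plays a level sequence when it finishes moving.
; It extends a parent lever, flagging itself used on its first move and reporting interaction unavailable afterwards.
; A DoOnce plays OneshotSequence, optionally blocking player input until it ends.
; The move and look stop flags are cross-wired, each ignoring the other input type.
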(event Custom|do%20sequence
  (bind _oneshot_sequence (Variables|Sequence|GetOneshot%20Sequence))
  (bind _sequenceplayer (Variables|/Script/LevelSequence.LevelSequenceActor|GetSequencePlayer _oneshot_sequence))
  (Utilities|FlowControl|DoOnce false
    (:Completed
      (Utilities|IsValid _oneshot_sequence
        (:Is%20Valid
          (Utilities|FlowControl|Sequence
            (:then_0
              (if (or (Variables|Sequence|Getstop%20move%20input%20for%20sequence) (Variables|Sequence|Getstop%20look%20input%20for%20sequence))
                (EventDispatchers|BindEventtoOnFinished _sequenceplayer (delegate Custom|on%20finished))
                (Utilities|FlowControl|Sequence
                  (:then_0
                    (if (Variables|Sequence|Getstop%20move%20input%20for%20sequence)
                      (Input|SetIgnoreLookInput (Game|GetPlayerController 0) true)))
                  (:then_1
                    (if (Variables|Sequence|Getstop%20look%20input%20for%20sequence)
                      (Input|SetIgnoreMoveInput (Game|GetPlayerController 0) true))))))
            (:then_1
              (Sequencer|Player|Play _sequenceplayer :!class /Script/MovieScene.MovieSceneSequencePlayer))))))))

(event Custom|on%20finished
  (Class|Controller|ResetIgnoreInputFlags (Game|GetPlayerController 0)))

(event EventBeginPlay
  (|CallParentFunction)
  (EventDispatchers|BindEventtoOnFinishedMoving (delegate Custom|do%20sequence)))

(event Collision|EventActorBeginOverlap
  (params (OtherActor :type Actor%20Object%20Reference))
  (|CallParentFunction OtherActor))

(event EventTick
  (params (DeltaSeconds :type Float%20%28single-precision%29))
  (|CallParentFunction DeltaSeconds))

(event EventMoveNextPosition
  (Variables|Default|SetHas%20Lever%20Been%20Used true)
  (|CallParentFunction))

(fn ConstructionScript
  (|CallParentFunction))

(fn IsInteractionAvailable
  (if (|CallParentFunction)
    (return (not (Variables|Default|GetHas%20Lever%20Been%20Used)))
    (else
      (return false))))