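; BP_ToF_TutorialBox is a trigger volume that shows a tutorial control tip when a BP_BaseCharacter enters its Box.
; A DoOnce gates creation of a WBP_ToF_ControlTip widget carrying the configured text, and resets if another kind of actor triggered it.
; Any end overlap removes the valid widget without checking the actor, re-arming the DoOnce only when CanReplay is set.
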(event OnComponentBeginOverlap(Box)
  (params (OverlappedComponent :type Primitive%20Component%20Object%20Reference) (OtherActor :type Actor%20Object%20Reference) (OtherComp :type Primitive%20Component%20Object%20Reference) (OtherBodyIndex :type Integer) (bFromSweep :type Boolean) (SweepResult :type Hit%20Result%20Structure%20%28by%20ref%29))
  (Utilities|FlowControl|DoOnce false
    (:Completed
      (Utilities|Casting|CastToBP_BaseCharacter OtherActor
        (:then
          (bind _returnvalue (UserInterface|CreateWidget "/Game/Patchwork/Blueprints/Widgets/ControlTip/WBP_ToF_ControlTip.WBP_ToF_ControlTip_C" 0 (Variables|Default|GetText%20Control%20Tip)))
          (bind _output_get (Variables|Default|SetWBPControlTipRef _returnvalue))
          (UserInterface|Viewport|AddtoViewport _output_get 0))
        (:CastFailed
          (CallFunction|Reset))))))

(event OnComponentEndOverlap(Box)
  (params (OverlappedComponent :type Primitive%20Component%20Object%20Reference) (OtherActor :type Actor%20Object%20Reference) (OtherComp :type Primitive%20Component%20Object%20Reference) (OtherBodyIndex :type Integer))
  (bind _wbpcontroltipref (Variables|Default|GetWBPControlTipRef))
  (Utilities|IsValid _wbpcontroltipref
    (:Is%20Valid
      (Default|RemoveWidget _wbpcontroltipref)
      (if (Variables|Default|GetCanReplay?)
        (CallFunction|Reset)))))

(event Custom|Reset
  (Utilities|FlowControl|DoOnce false) ; enters at Reset
)

(event EventBeginPlay)

(event Collision|EventActorBeginOverlap
  (params (OtherActor :type Actor%20Object%20Reference)))

(event EventTick
  (params (DeltaSeconds :type Float%20%28single-precision%29)))

(fn ConstructionScript)