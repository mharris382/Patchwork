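; BP_Anomoly is an interactable glowing anomaly that advances through stages, spawning fragments and notifying BPI_AnomalyEventListener actors.
; Stage changes can drive its sphere along one of two splines via a timeline that modulates VFX and flags the player as interacting.
; It tracks fragment collection through game mode world events keyed by data table rows, with helpers that validate that data.
; Interaction requires the player camera to be close and facing the sphere.
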(event Custom|Events
  (params (World%20Event :type Name))
  (bind _fragments (Variables|Default|Getfragments))
  ;[0.6233 0.6233 0.6233 0.5] React to Fragment Collection (TODO: move to controller?)
  (if (Utilities|Map|Contains _fragments World%20Event)
    (Utilities|Map|Add _fragments World%20Event true)))

(event Custom|Set%20Interact%20Enabled
  (params (enabled :type Boolean))
  ;[0.2378 0.2378 0.2378 0.504 32] Interact
  (bind _output_get (Variables|Default|Setinteraction%20enabled enabled))
  (Collision|SetCollisionEnabled (Variables|Default|GetStaticMesh) (select _output_get "NoCollision" "QueryAndPhysics")))

(event Custom|Do%20Transition
  (bind _returnvalue (Game|Player|GetPlayerPawn 0))
  (bind _asbp_base_character (Utilities|Casting|CastToBP_BaseCharacter _returnvalue))
  ;[0.6233 0.6233 0.6233 0.5] Move Along Spline
  (Variables|Transitions|Setin%20transition true)
  (Variables|/Game/Patchwork/Blueprints/Core/Pawns/BP_BaseCharacter.BP_BaseCharacter_C|Setdialogue%20target _asbp_base_character self)
  (Variables|/Game/Patchwork/Blueprints/Core/Pawns/BP_BaseCharacter.BP_BaseCharacter_C|Setis%20Interacting%20With%20Anomaly _asbp_base_character true)
  (bind (_direction _spline_position _fx_radius _fx_rate) (Timeline|Transition PlayFromStart)
    (:Update
      (CallFunction|SetSpherePositiononSpline _spline_position)
      (FX|SetVFXSpawnRadiusMultiplier _fx_radius)
      (FX|SetVFXSpawnRateMultiplier _fx_rate))
    (:Finished
      (CallFunction|CompletePlayerInteraction))))

(event Custom|Touch%20Anomaly)

(event Custom|Untouch%20Anomaly)

(event Custom|update%20fx)

(event EventBeginPlay
  (bind _returnvalue (Game|GetGameMode))
  (bind _asgm_base_game_mode (Utilities|Casting|CastToGM_BaseGameMode _returnvalue))
  (|CallParentFunction)
  ;[0.6233 0.6233 0.6233 0.5] React to Fragment Collection (TODO: move to controller?)
  (bind _outrownames (DataTable|GetDataTableRowNames (.fragmentdatatable (Variables|Settings|GetAnomolyData))))
  (Utilities|Map|Clear (Variables|Default|Getfragments))
  (for _array_element _outrownames
    (bind _event_occured (Default|HasWorldEventOccured _asgm_base_game_mode _array_element))
    (Utilities|Map|Add (Variables|Default|Getfragments) _array_element _event_occured))
  (EventDispatchers|BindEventtoWorldEventOccured _asgm_base_game_mode (delegate Custom|Events)))

(event Collision|EventActorBeginOverlap
  (params (OtherActor :type Actor%20Object%20Reference))
  (bind _update_fx_handle (Variables|Visuals|Getupdate%20fx%20handle))
  (|CallParentFunction 0)
  (if (== OtherActor (Game|Player|GetPlayerPawn 0))
    (Variables|Visuals|Setis%20player%20near%20anomaly false)
    (if (Utilities|Time|IsValidTimerHandle _update_fx_handle)
      (Utilities|Time|ClearandInvalidateTimerbyHandle _update_fx_handle))))

(event EventTick
  (params (DeltaSeconds :type Float%20%28single-precision%29))
  (|CallParentFunction DeltaSeconds))

(event EventOnInteract
  ;[0.2378 0.2378 0.2378 0.504 32] Interact
  (if (Variables|Default|Getinteraction%20enabled)
    (Default|CallOnPlayerInteracted)))

(event EventLoadEvent
  (params (occured :type Boolean))
  ;[1 1 1] On Load
  (bind _output_get (Variables|Default|Sethas%20player%20interacted occured))
  (if _output_get
    (Default|CallOnAnomolyLoaded)))

(event Collision|EventActorEndOverlap
  (params (OtherActor :type Actor%20Object%20Reference))
  (if (== OtherActor (Game|Player|GetPlayerPawn 0))
    (Variables|Visuals|Setis%20player%20near%20anomaly true)
    (bind _returnvalue (Utilities|Time|SetTimerbyEvent (delegate Custom|update%20fx) 0.0 true))
    (Variables|Visuals|Setupdate%20fx%20handle _returnvalue)))

(event Custom|Move%20Along%20Spline
  (params (spline :type Spline%20Component%20Object%20Reference) (delay :type Float%20%28double-precision%29))
  (bind _output_get (Variables|Transitions|SetCurrent%20Spline spline))
  (Utilities|IsValid _output_get
    (:Is%20Valid
      (Variables|Transitions|Setin%20transition true)
      (Utilities|FlowControl|Delay delay)
      (CallFunction|DoTransition))))

(fn ConstructionScript
  (bind _color (Variables|Visuals|GetColor))
  (bind _radius (Variables|Settings|Getradius))
  (|CallParentFunction)
  (Utilities|FlowControl|Sequence
    (:then_0
      (Transformation|SetRelativeLocation (Variables|Default|GetSpline_To_Stage_2) (.position (CallFunction|GetLastSplinePointonComponent (Variables|Default|GetSpline_To_Stage_1) "Local")) false false))
    (:then_1
      (Rendering|Components|Light|SetLightColor (Variables|Default|GetPointLight) _color true)
      (Effects|Components|ParticleSystem|SetColorParameter (Variables|Default|GetVFX%20System) "Color" (* _color (Variables|Visuals|GetEmissive%20Intensity))))
    (:then_2
      (Rendering|Lighting|SetAttenuationRadius (Variables|Default|GetPointLight) _radius)
      (Components|Sphere|SetSphereRadius (Variables|Default|GetAnomaly%20Sphere) _radius true))
    (:then_3
      (Rendering|SetVisibility (Variables|Default|GetSpline_To_Stage_2) (not (Variables|Default|GetHide%20Splines)) false))))

(fn GetActionVerb
  (return "Touch"))

(fn GetInteractVerb
  (return ""))

(fn IsAnomolyValid
  (bind _anomolydata (Variables|Settings|GetAnomolyData))
  (bind _returnvalue (Utilities|String|Len (.word1 _anomolydata)))
  (bind _returnvalue_2 (Utilities|String|Len (.word2 _anomolydata)))
  (if (!= (.anomolyuniquename _anomolydata) "")
    (if (and (== _returnvalue _returnvalue_2) (> _returnvalue 0))
      (if (Utilities|IsValid (.fullimage _anomolydata))
        (if (Utilities|IsValid (.fragmentdatatable _anomolydata))
          (return true)
          (else
            (Development|PrintText "fragment database not assigned" true true "(R=1.000000,G=0.000000,B=0.055256,A=1.000000)" 1e+01)
            (return false) ; fragment data is not assigned
          ))
        (else
          (Development|PrintText "final image not assigned" true true "(R=1.000000,G=0.000000,B=0.055256,A=1.000000)" 1e+01)
          (return false) ; final image not assigned
        ))
      (else
        (Development|PrintText (Utilities|Text|FormatText "words are not same length or empty (word 1 = {0}, len({1}) word 2 = {2}, len({3})" (.word1 _anomolydata) _returnvalue (.word2 _anomolydata) _returnvalue_2) true true "(R=1.000000,G=0.000000,B=0.055256,A=1.000000)" 1e+01)
        (return false) ; words are not same length or empty
      ))
    (else
      (Development|PrintText "anomoly missing unique ID" true true "(R=1.000000,G=0.000000,B=0.055256,A=1.000000)" 1e+01)
      (return false) ; missing unique ID
    )))

(fn IsFragmentDatabaseValid
  (bind _anomolydata (Variables|Settings|GetAnomolyData))
  (bind _returnvalue (Utilities|GetDisplayName (.fragmentdatatable _anomolydata)))
  (if (Interaction|IsAnomolyValid)
    (bind _outrownames (DataTable|GetDataTableRowNames (.fragmentdatatable _anomolydata)))
    (for _array_element _outrownames
      (bind _returnvalue_2 (Utilities|GetDataTableRow (.fragmentdatatable _anomolydata) _array_element)
        (:then
          (if (== (Utilities|String|Len (.word1 _anomolydata)) (Utilities|String|Len (.word1unlocks (Utilities|Struct|BreakS_Fragment _returnvalue_2))))
            (if (== (Utilities|String|Len (.word2 _anomolydata)) (Utilities|String|Len (.word2unlocks (Utilities|Struct|BreakS_Fragment _returnvalue_2))))
              (Utilities|IsValid (.fragmentimage (Utilities|Struct|BreakS_Fragment _returnvalue_2))
                (:Is%20Not%20Valid
                  (Development|PrintText (Utilities|Text|FormatText "Database Error (DB={1}, row={0}) no image assigned" 0) true true "(R=1.000000,G=0.000000,B=0.055256,A=1.000000)" 1e+01)
                  (return false) ; row has missing image assignment
                ))
              (else
                (Development|PrintText (Utilities|Text|FormatText "Database Error (DB={1}, row={0})  word 2 length != anomoly word 1 length (anomoly word = {2}, row word = {3})" _array_element _returnvalue (.word2 _anomolydata) (.word2unlocks (Utilities|Struct|BreakS_Fragment _returnvalue_2))) true true "(R=1.000000,G=0.000000,B=0.055256,A=1.000000)" 1e+01)))
            (else
              (Development|PrintText (Utilities|Text|FormatText "Database Error (DB={1}, row={0})  word 1 length != anomoly word 1 length (anomoly word = {2}, row word = {3})" _array_element _returnvalue (.word1 _anomolydata) (.word1unlocks (Utilities|Struct|BreakS_Fragment _returnvalue_2))) true true "(R=1.000000,G=0.000000,B=0.055256,A=1.000000)" 1e+01)))
          (return false) ; row has word missmatch
        )))
    (return true)
    (else
      (return false) ; can only be valid if main data is valid
    )))

(fn MoveAnomalytoNextStage
  (params (fragments%20to%20spawn :type Array%20of%20BP%20Fragment%20Object%20References))
  (LocalVariables|Setfrags fragments%20to%20spawn)
  (Utilities|FlowControl|Sequence
    (:then_0
      (Math|Integer|IncrementInt (Variables|Default|Getanomaly%20state)))
    (:then_1
      (Utilities|FlowControl|Sequence
        (:then_0
          (switch int (- (Variables|Default|Getanomaly%20state) 1)
            (:0
              (CallFunction|CompletePlayerInteraction))
            (:1
              (CallFunction|MoveAlongSpline (Variables|Default|GetSpline_To_Stage_1) 0.0))
            (:2
              (CallFunction|MoveAlongSpline (Variables|Default|GetSpline_To_Stage_2) 0.0))
            (:3
              (CallFunction|CompletePlayerInteraction))
            (:4
              (CallFunction|CompletePlayerInteraction))))
        (:then_1
          (for _array_element (LocalVariables|Getfrags)
            (Default|SpawnFragment _array_element (Transformation|GetWorldLocation (Variables|Default|GetAnomaly%20Sphere)))))
        (:then_2
          (bind _outactors (Actor|GetAllActorswithInterface "/Game/Patchwork/Blueprints/Interfaces/BPI_AnomalyEventListener.BPI_AnomalyEventListener_C"))
          (for _array_element_2 _outactors
            (Class|BPIAnomalyEventListener|OnAnomalyStageChanged(Message) _array_element_2 (Variables|Default|Getanomaly%20state))))))))

(fn UnlockFragment
  (params (fragment :type BP%20Fragment%20Object%20Reference)))

(fn UpdateRadius
  (params (new%20radius :type Float%20%28double-precision%29))
  (Variables|Settings|Setradius new%20radius)
  (Rendering|Lighting|SetAttenuationRadius (Variables|Default|GetPointLight) (Variables|Settings|Getradius))
  (Components|Sphere|SetSphereRadius (Variables|Default|GetAnomaly%20Sphere) (Variables|Settings|Getradius) true)
  (Effects|Components|ParticleSystem|SetFloatParameter (Variables|Default|GetVFX%20System) "Max Radius" (Variables|Settings|Getradius)))

(fn SetVFXSpawnRateMultiplier
  (params (rate%20multiplier :type Float%20%28double-precision%29))
  (Niagara|SetNiagaraVariable(Float) (Variables|Default|GetVFX%20System) "rate multiplier" rate%20multiplier))

(fn SetVFXSpawnVelocityMultiplier
  (params (rate%20multiplier :type Float%20%28double-precision%29))
  (Niagara|SetNiagaraVariable(Float) (Variables|Default|GetVFX%20System) "rate multiplier" rate%20multiplier))

(fn SetVFXSpawnRadiusMultiplier
  (params (rate%20multiplier :type Float%20%28double-precision%29))
  (Niagara|SetNiagaraVariable(Float) (Variables|Default|GetVFX%20System) "velocity multiplier" rate%20multiplier))

(fn SetSpherePositiononSpline
  (params (normalized%20position :type Float%20%28double-precision%29))
  (bind _current_spline (Variables|Transitions|GetCurrent%20Spline))
  (Utilities|IsValid (Variables|Transitions|GetCurrent%20Spline)
    (:Is%20Valid
      (Transformation|SetWorldTransform (Variables|Default|GetAnomaly%20Sphere) (Spline|GetTransformatDistanceAlongSpline _current_spline (* normalized%20position (Spline|GetSplineLength _current_spline)) "World" false) false false))))

(fn CompletePlayerInteraction
  (bind _returnvalue (Game|Player|GetPlayerPawn 0))
  (bind _asbp_base_character (Utilities|Casting|CastToBP_BaseCharacter _returnvalue))
  (Variables|Transitions|Setin%20transition false)
  (Variables|/Game/Patchwork/Blueprints/Core/Pawns/BP_BaseCharacter.BP_BaseCharacter_C|Setdialogue%20target _asbp_base_character 0)
  (Input|EnableInput _asbp_base_character (Game|GetPlayerController 0))
  (Variables|/Game/Patchwork/Blueprints/Core/Pawns/BP_BaseCharacter.BP_BaseCharacter_C|Setis%20Interacting%20With%20Anomaly _asbp_base_character false))

(fn GetAnomalyLocationinStage(enum)
  (params (stage :type EAnomalyStage%20Enum :default "NewEnumerator8"))
  (bind _returnvalue (Transformation|GetActorLocation))
  (bind _spline_to_stage_2 (Variables|Default|GetSpline_To_Stage_2))
  (bind _spline_to_stage_1 (Variables|Default|GetSpline_To_Stage_1))
  (return (Utilities|Select :Index stage :NewEnumerator8 _returnvalue :NewEnumerator7 _returnvalue :NewEnumerator0 (Spline|GetLocationatSplinePoint _spline_to_stage_1 (- (Spline|GetNumberOfSplinePoints _spline_to_stage_1) 1) "World") :NewEnumerator2 (Spline|GetLocationatSplinePoint _spline_to_stage_2 (- (Spline|GetNumberOfSplinePoints _spline_to_stage_2) 1) "World") :NewEnumerator3 (Math|Transform|TransformLocation (Transformation|GetActorTransform) (Variables|Default|GetClimax%20Teleport%20Location)) :NewEnumerator4 "0, 0, 0")))

(fn GetAnomalyLocationinStage(int)
  (params (stage :type EAnomalyStage%20Enum :default "NewEnumerator8") (NewParam :type Integer))
  (return (Stages|GetAnomalyLocationinStage(enum) (Stages|StageInttoEnum NewParam))))

(fn StageInttoEnum
  (params (stage%20int :type Integer))
  (return (Utilities|Select :Index (Math|Integer|Clamp(Integer) stage%20int 0 5) :Option%200 "NewEnumerator8" :Option%201 "NewEnumerator7" :Option%202 "NewEnumerator0" :Option%203 "NewEnumerator2" :Option%204 "NewEnumerator3" :Option%205 "NewEnumerator4")))

(fn GetMovementSplineforStageCompletion
  (params (stage%20started :type EAnomalyStage%20Enum :default "NewEnumerator8"))
  (return (Utilities|Select :Index stage%20started :NewEnumerator8 0 :NewEnumerator7 0 :NewEnumerator0 (Variables|Default|GetSpline_To_Stage_1) :NewEnumerator2 (Variables|Default|GetSpline_To_Stage_2) :NewEnumerator3 0 :NewEnumerator4 0)))

(fn IsInteractionAvailable
  (bind _base_character (CallFunction|GetBasePlayerPawn))
  (bind _anomaly_sphere (Variables|Default|GetAnomaly%20Sphere))
  (bind _returnvalue (Transformation|GetWorldLocation _anomaly_sphere))
  (bind _camera (Variables|/Game/Patchwork/Blueprints/Core/Pawns/BP_BaseCharacter.BP_BaseCharacter_C|GetCamera _base_character))
  (bind _returnvalue_2 (Transformation|GetWorldLocation _camera))
  (return (Math|Boolean|ANDBoolean (|CallParentFunction) (not (Variables|/Game/Patchwork/Blueprints/Core/Pawns/BP_BaseCharacter.BP_BaseCharacter_C|Getis%20Interacting%20With%20Anomaly _base_character)) (< (Class|KismetMathLibrary|DegAcos (Math|Vector|DotProduct (Math|Vector|GetForwardVector _camera) (Math|Vector|Normalize (- _returnvalue _returnvalue_2)))) 2e+01) (< (Class|KismetMathLibrary|VectorDistanceSquared _returnvalue_2 _returnvalue) (Math|Float|Power 2.5e+02 2.0)))))

(fn GetEventName
  (return (.anomolyuniquename (Variables|Settings|GetAnomolyData))))

(fn GetFPLookatLocationWS
  (return (Transformation|GetWorldLocation (Variables|Default|GetAnomaly%20Sphere))))