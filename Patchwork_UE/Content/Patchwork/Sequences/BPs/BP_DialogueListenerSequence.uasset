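; BP_DialogueListenerSequence is a dialogue listener that plays a Level Sequence when a dialogue finishes.
; Its DialogueFinished event runs only once, waits a configurable delay, then calls EventTrigger on the SequenceTrigger if valid and starts the sequence player.
; An optional PlayFromBeginning flag jumps the playback position before playing.
; An invalid sequence only prints a placeholder debug string.
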(event Custom|DialogueFinished
  (params (SequenceTrigger :type BP%20Sequence%20Trigger%20Object%20Reference))
  (bind _levelsequence (Variables|LevelSequence|GetLevelSequence))
  (bind _sequenceplayer (Variables|/Script/LevelSequence.LevelSequenceActor|GetSequencePlayer _levelsequence))
  (Utilities|FlowControl|DoOnce false
    (:Completed
      (Utilities|IsValid (Variables|LevelSequence|GetLevelSequence)
        (:Is%20Valid
          (Utilities|FlowControl|Delay (Variables|LevelSequence|GetDelay))
          (Utilities|FlowControl|Sequence
            (:then_0
              (Utilities|IsValid (Variables|LevelSequence|GetSequenceTrigger)
                (:Is%20Valid
                  (Default|EventTrigger (Variables|LevelSequence|GetSequenceTrigger)))))
            (:then_1
              (if (Variables|LevelSequence|GetPlayFromBeginning)
                (Components|Timeline|SetPlaybackPosition _sequenceplayer (Utilities|Struct|MakeMovieSceneSequencePlaybackParams "(FrameNumber=(Value=0),SubFrame=0.000000)" 0.0 "" "(Hours=0,Minutes=0,Seconds=0,Frames=0,Subframe=0.000000,bDropFrameFormat=False)" "Frame" "Jump" false)))
              (Sequencer|Player|Play _sequenceplayer :!class /Script/MovieScene.MovieSceneSequencePlayer))))
        (:Is%20Not%20Valid
          (Development|PrintString "Hello"))))))

(fn ConstructionScript)