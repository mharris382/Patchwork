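; Base actor for custom world logic tied to a quest step, referenced through a StepInfo data table row handle.
; Its construction script finds the BP_QuestController and, if StepInfo points to a different table, switches it to the controller's Questline, selecting the first row or None if empty.
; IsStepCompleted is a stub that always returns false, and the event graph has no active logic.
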(event EventBeginPlay)

(event Collision|EventActorBeginOverlap
  (params (OtherActor :type Actor%20Object%20Reference)))

(event EventTick
  (params (DeltaSeconds :type Float%20%28single-precision%29)))

(fn ConstructionScript
  (bind _returnvalue (Actor|GetActorOfClass "/Game/Patchwork/Blueprints/Quests/BP_QuestController.BP_QuestController_C"))
  (Utilities|IsValid _returnvalue
    (:Is%20Valid
      (Utilities|IsValid (Variables|/Game/Patchwork/Blueprints/Quests/BP_QuestController.BP_QuestController_C|GetQuestline _returnvalue)
        (:Is%20Valid
          (if (!= (.datatable (Variables|Default|GetStep%20Info)) (Variables|/Game/Patchwork/Blueprints/Quests/BP_QuestController.BP_QuestController_C|GetQuestline _returnvalue))
            (bind _outrownames (DataTable|GetDataTableRowNames (Variables|/Game/Patchwork/Blueprints/Quests/BP_QuestController.BP_QuestController_C|GetQuestline _returnvalue)))
            (if (> (Utilities|Array|Length _outrownames) 0)
              (Variables|Default|SetStep%20Info (Utilities|Struct|MakeDataTableRowHandle (Variables|/Game/Patchwork/Blueprints/Quests/BP_QuestController.BP_QuestController_C|GetQuestline _returnvalue) (Utilities|Array|Get(acopy) _outrownames)))
              (else
                (Variables|Default|SetStep%20Info (Utilities|Struct|MakeDataTableRowHandle (Variables|/Game/Patchwork/Blueprints/Quests/BP_QuestController.BP_QuestController_C|GetQuestline _returnvalue) "None"))))))))))

(fn IsStepCompleted
  (return false))