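; BP_Mushroom_Projectile is an ability projectile that plants a bouncy mushroom where it hits.
; On a valid hit it respawns its assigned pooled mushroom, or spawns one if none is valid, aligned to the surface normal.
; It attaches the mushroom to the hit component, fires OnMushroomSpawned and destroys itself.
; Characters and anything tagged "No Mush" instead destroy the projectile with an invalid-spawn Niagara effect.
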(event OnProjectileBounce(ProjectileMovement)
  (params (ImpactResult :type Hit%20Result%20Structure%20%28by%20ref%29) (ImpactVelocity :type Vector%20%28by%20ref%29 :default "0, 0, 0")))

(event Custom|Handle%20Invalid%20Hit
  (params (hit :type Hit%20Result%20Structure))
  (bind (_bblockinghit _binitialoverlap _time _distance _location _impactpoint _normal) (Collision|BreakHitResult hit))
  (Actor|DestroyActor)
  (Niagara|SpawnSystematLocation "/Game/Patchwork/Blueprints/Pawns/Abilities/Effects/NS_Invalid_Spawn.NS_Invalid_Spawn" _location (Math|Conversions|RotationFromXVector _normal)))

(event Custom|Assign%20Pooled%20Bouncer
  (params (pooled%20mushroom :type BP%20Bouncy%20Mushroom%20Object%20Reference))
  (Variables|Default|SetPooled%20Mushroom pooled%20mushroom))

(event EventBeginPlay)

(event Collision|EventActorBeginOverlap
  (params (OtherActor :type Actor%20Object%20Reference)))

(event EventTick
  (params (DeltaSeconds :type Float%20%28single-precision%29)))

(event Collision|EventHit
  (params (MyComp :type Primitive%20Component%20Object%20Reference) (Other :type Actor%20Object%20Reference) (OtherComp :type Primitive%20Component%20Object%20Reference) (bSelfMoved :type Boolean) (HitLocation :type Vector :default "0, 0, 0") (HitNormal :type Vector :default "0, 0, 0") (NormalImpulse :type Vector :default "0, 0, 0") (Hit :type Hit%20Result%20Structure%20%28by%20ref%29))
  (bind (_bblockinghit _binitialoverlap _time _distance _location _impactpoint _normal _impactnormal _physmat _hitactor _hitcomponent) (Collision|BreakHitResult Hit))
  (Utilities|Casting|CastToCharacter Other
    (:then
      (CallFunction|HandleInvalidHit Hit :!label _label))
    (:CastFailed
      (if (not (or (Actor|ActorHasTag Other "No Mush") (Components|ComponentHasTag OtherComp "No Mush")))
        (Development|PrintText "HIT OCCURRED 
")
        (bind _returnvalue (CallFunction|GetorSpawnMushroom (Math|Transform|MakeTransform _location (Math|Rotator|MakeRotfromZ _normal))))
        (Transformation|AttachComponentToComponent _returnvalue _hitcomponent "None" "KeepWorld" "KeepWorld" "KeepWorld" true)
        (Default|CallOnMushroomSpawned _returnvalue)
        (Actor|DestroyActor)
        (else
          (goto _label))))))

(fn ConstructionScript)

(fn GetorSpawnMushroom
  (params (SpawnTransform :type Transform))
  (bind _pooled_mushroom (Variables|Default|GetPooled%20Mushroom))
  (Utilities|IsValid _pooled_mushroom
    (:Is%20Valid
      (Default|Respawnfrom _pooled_mushroom SpawnTransform)
      (return _pooled_mushroom))
    (:Is%20Not%20Valid
      (bind _returnvalue (Game|SpawnActorfromClass "/Game/Patchwork/Blueprints/Pawns/Abilities/BP_Bouncy_Mushroom.BP_Bouncy_Mushroom_C" SpawnTransform "Undefined" "MultiplyWithRoot" 0 0))
      (return _returnvalue))))