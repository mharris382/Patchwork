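; Shrinking platform environment actor that scales a pivot between sizes, apparently unfinished.
; Tick, unless waiting, advances a clamped alpha through a curve to lerp the pivot's scale, toggling a shrinking flag via a counter while at full alpha.
; Player overlaps only start delays, with exit then calling an empty Grow event; other target and growth events are stubs.
; Construction sets the mesh and previews scale between shrink and grow values.
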(event Custom|Next%20Growth
  (bind _result (Math|Integer|IncrementInt (Variables|Default|Getcnt))
    (:%20%20
      (Variables|Default|Setcnt (Math|Integer|%(Integer) _result 2))
      (Variables|Default|Setis%20shrinking (== (Math|Integer|%(Integer) _result 2) 0)))))

(event Custom|Return%20to%20Growth%20Size
  (Utilities|FlowControl|Delay (Variables|Default|GetGrow%20Wait%20Time)))

(event Custom|Grow)

(event Custom|Start%20Growing)

(event Custom|Set%20Target
  (params (delay :type Float%20%28double-precision%29) (end%20scale :type Vector)))

(event EventBeginPlay)

(event Collision|EventActorBeginOverlap
  (params (OtherActor :type Actor%20Object%20Reference))
  (if (== OtherActor (Game|Player|GetPlayerPawn 0))
    (Utilities|FlowControl|Delay 0.2)))

(event EventTick
  (params (DeltaSeconds :type Float%20%28single-precision%29))
  (if (not (Variables|Default|Getis%20waiting))
    (Variables|Default|Sett (Math|Float|Clamp(Float) (+ (* DeltaSeconds (Variables|Default|Gettarget%20time)) (Variables|Default|Gett))))
    (Transformation|SetRelativeScale3D (Variables|Default|GetScale%20Pivot) (Math|Vector|Lerp(Vector) (Variables|Default|Getstart%20scale) (Variables|Default|Gettarget%20scale) (Math|Curves|GetFloatValue (Variables|Default|Gettarget%20curve) (Variables|Default|Gett))))
    (if (>= (Variables|Default|Gett) 1.0)
      (CallFunction|NextGrowth))))

(event Collision|EventActorEndOverlap
  (params (OtherActor :type Actor%20Object%20Reference))
  (if (== OtherActor (Game|Player|GetPlayerPawn 0))
    (Utilities|FlowControl|Delay (Variables|Default|GetGrow%20Wait%20Time))
    (CallFunction|Grow)))

(fn ConstructionScript
  (Components|StaticMesh|SetStaticMesh (Variables|Default|GetStaticMesh1) (Variables|Default|GetMesh))
  (Transformation|SetRelativeScale3D (Variables|Default|GetScale%20Pivot) (Math|Vector|Lerp(Vector) (Variables|Default|GetShrink%20Scale) (Variables|Default|GetGrow%20Scale) (Variables|Default|Gett))))