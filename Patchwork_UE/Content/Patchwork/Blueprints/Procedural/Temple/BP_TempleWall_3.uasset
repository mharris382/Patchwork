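; BP_TempleWall_3 is a procedural temple wall Blueprint that extends a parent generator and supports PCG.
; Its construction script runs the parent's logic and derives GENCellSize from the scaled cell size, leaving volume sizing, hole creation and regeneration disconnected.
; The unwired CreateHoles function converts hole definitions into cell-scaled PCG points.
; It overrides the vertical bounds height with WallHeight, and a PrintResult event prints the generated actor's name.
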(event Custom|Print%20Result
  (params (NewParam :type PCG%20Data%20Collection%20Structure))
  (Development|PrintString (Utilities|String|Append "Generated: " (Utilities|GetDisplayName self))))

(event EventBeginPlay)

(event Collision|EventActorBeginOverlap
  (params (OtherActor :type Actor%20Object%20Reference)))

(event EventTick
  (params (DeltaSeconds :type Float%20%28single-precision%29)))

(fn ConstructionScript
  (|CallParentFunction)
  (Variables|PCGINTERNAL|SetGEN_CellSize (* (Variables|01-Wall|Dep|GetCell%20Size) (Variables|01-Wall|Dep|GetConstant%20Scale))))

(fn CreateHoles
  (bind _holes (Variables|Default|GetHoles))
  (if (> (Utilities|Array|Length _holes) 0)
    (Utilities|FlowControl|Sequence
      (:then_0
        (for _array_element _holes
          (Utilities|Array|Add (LocalVariables|Getpcg%20points) (Utilities|Struct|MakePCGPoint (Math|Transform|MakeTransform (.HolePosition (Utilities|Struct|BreakSPCGGridHole _array_element))) 1.0 (* (/ (* (.HoleSize (Utilities|Struct|BreakSPCGGridHole _array_element)) (Variables|01-Wall|Dep|GetCell%20Size)) 2.0) -1.0) (/ (* (.HoleSize (Utilities|Struct|BreakSPCGGridHole _array_element)) (Variables|01-Wall|Dep|GetCell%20Size)) 2.0) "(X=1.000000,Y=1.000000,Z=1.000000,W=1.000000)" 0.5 0)))))))

(fn GetBoundsVerticalHeight
  (return (Variables|01-Wall|GetWallHeight)))