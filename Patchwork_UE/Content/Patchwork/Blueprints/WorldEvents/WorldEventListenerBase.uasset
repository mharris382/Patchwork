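; Base actor that listens for world events broadcast by the game mode and reacts to the one matching its configured event name.
; On BeginPlay it casts the game mode to GM_BaseGameMode and binds to its world event dispatcher.
; A matching event fires a received event, whose default here prints the event name and the listener's display name.
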(event Custom|On%20World%20Event%20Occured
  (params (World%20Event :type Name))
  (if (== World%20Event (Variables|Default|GetEvent%20Name))
    (CallFunction|EventRecieved)))

(event Custom|Event%20Recieved
  (Development|PrintText (Utilities|Text|FormatText "{0} (listener {1})" (Variables|Default|GetEvent%20Name) (Utilities|GetDisplayName self))))

(event EventBeginPlay
  (bind _asgm_base_game_mode (Utilities|Casting|CastToGM_BaseGameMode (Game|GetGameMode)))
  (EventDispatchers|BindEventtoWorldEventOccured _asgm_base_game_mode (delegate Custom|On%20World%20Event%20Occured)))

(event Collision|EventActorBeginOverlap
  (params (OtherActor :type Actor%20Object%20Reference)))

(event EventTick
  (params (DeltaSeconds :type Float%20%28single-precision%29)))

(fn ConstructionScript)