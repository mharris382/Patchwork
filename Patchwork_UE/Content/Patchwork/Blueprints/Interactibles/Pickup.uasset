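; Interactable physics pickup that the player's paperperson pawn can grab and drop.
; On interact it turns its PaperSprite toward the player camera, passes itself to GrabPickup and enables physics on the static mesh.
; Pickup and drop events swap the mesh collision profile so it ignores pawns while held.
; Query functions supply the action verb, name and grab target, with stub defaults for use, configuration and forced release.
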(event EventBeginPlay
  (|CallParentFunction)
  (Collision|SetCollisionProfileName (Variables|Default|GetStaticMesh) "PhysicsActor" true :!class /Script/Engine.PrimitiveComponent))

(event Collision|EventActorBeginOverlap
  (params (OtherActor :type Actor%20Object%20Reference))
  (|CallParentFunction OtherActor) ; This node is disabled and will not be called.\nDrag off pins to build functionality.
)

(event EventTick
  (params (DeltaSeconds :type Float%20%28single-precision%29))
  (|CallParentFunction DeltaSeconds) ; This node is disabled and will not be called.\nDrag off pins to build functionality.
)

(event EventOnPickedUp
  (params (owner :type Actor%20Object%20Reference) (handler :type Pickup%20Handler%20Object%20Reference))
  (CallFunction|SetGrabbed true))

(event EventOnInteract
  (bind _papersprite (Variables|Default|GetPaperSprite))
  (bind _aspaperperson (Utilities|Casting|CastTopaperperson (Game|Player|GetPlayerPawn 0)))
  (Transformation|SetWorldRotation _papersprite (Math|Rotator|FindLookatRotation (Transformation|GetWorldLocation _papersprite) (Transformation|GetWorldLocation (Variables|/Game/Patchwork/Blueprints/Core/Pawns/BP_BaseCharacter.BP_BaseCharacter_C|GetCamera _aspaperperson))) false false)
  (Default|GrabPickup _aspaperperson self)
  (Physics|SetSimulatePhysics (Variables|Default|GetStaticMesh) true))

(event EventOnDropped
  (CallFunction|SetGrabbed false))

(fn ConstructionScript
  (|CallParentFunction))

(fn SetGrabbed
  (params (is%20grabbed :type Boolean))
  (if is%20grabbed
    (Collision|SetCollisionProfileName (Variables|Default|GetStaticMesh) "IgnoreOnlyPawn" false :!class /Script/Engine.PrimitiveComponent)
    (else
      (Collision|SetCollisionProfileName (Variables|Default|GetStaticMesh) "PhysicsActor" false :!class /Script/Engine.PrimitiveComponent))))

(fn GetActionVerb
  (return (select (Variables|Default|Getuse%20pickup%20name) (Utilities|Text|FormatText "pickup {0}" (Variables|Default|Getpickup%20name)) "pickup")))

(fn CanUsePickup
  (return false))

(fn GetGrabPhysicsTarget
  (return (Variables|Default|GetStaticMesh)))

(fn GetPickupName
  (return (Utilities|Text|ToText(Name) (Variables|Default|Getpickup%20name))))

(fn GetPickupConfiguration
  (return ""))

(fn ShouldForceablyRelease
  (return false))