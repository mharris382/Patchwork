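; Procedural puzzle floor tile tied to a PuzzleArea, apparently a work in progress.
; Applies an optional override material on construction, and binds to the area's tile-update event at BeginPlay.
; UpdateUV samples the area's render target at the tile's U/V on construction, BeginPlay and each update.
; The sampled color is currently unused: transform lerping, interpolation and carrier-follow binding are all disconnected.
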(event Custom|OnCarriersChanged
  (params (Carriers :type Array%20of%20BP%20Spore%20Carrier%20Object%20References))
  (Actor|Tick|SetActorTickEnabled (> (Utilities|Array|Length Carriers) 0))
  (Variables|Default|SetFollower (Components|GetOwner (Utilities|Array|Get(acopy) Carriers))))

(event Custom|Test
  (CallFunction|UpdateUV))

(event EventBeginPlay
  (bind _puzzlearea (Variables|Default|GetPuzzleArea)
    (:then
      (EventDispatchers|BindEventtoUpdateTiles _puzzlearea (delegate Custom|Test))
      (CallFunction|UpdateUV))
    (:else)))

(event Collision|EventActorBeginOverlap
  (params (OtherActor :type Actor%20Object%20Reference)))

(event EventTick
  (params (DeltaSeconds :type Float%20%28single-precision%29)))

(fn ConstructionScript
  (Utilities|FlowControl|Sequence
    (:then_0
      (bind _overridematerial (Variables|Default|GetOverrideMaterial)
        (:then
          (Rendering|Material|SetMaterial (Variables|Debug|GetStaticMeshComponent) 0 _overridematerial))
        (:else)))
    (:then_1
      (CallFunction|UpdateUV))))

(fn UpdateUV
  (bind _returnvalue (Class|KismetRenderingLibrary|ReadRenderTargetUV (Variables|/Game/Patchwork/Blueprints/Procedural/Effects/BP_PuzzleFloor.BP_PuzzleFloor_C|GetRT (Variables|Default|GetPuzzleArea)) (Variables|Default|GetU) (Variables|Default|GetV))))