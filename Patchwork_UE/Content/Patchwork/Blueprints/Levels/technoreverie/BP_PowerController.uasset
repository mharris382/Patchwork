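; Power controller for the technoreverie level that switches and dims registered lights in three groups.
; AddTRLight assigns each light to a group by location and applies that group's stored power state.
; UpdatePowerForQuadrent stores a new on/off state and amount, then pushes both to every light in that group.
; As written, the location test yields group 2 at zero X/Y and group 0 elsewhere, never group 1.
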(event EventBeginPlay
  (Variables|Default|Setpowered (Utilities|Array|MakeArray true true true))
  (Variables|Default|Setpower%20levels (Utilities|Array|MakeArray 1.0 1.0 1.0)))

(event Collision|EventActorBeginOverlap
  (params (OtherActor :type Actor%20Object%20Reference)))

(event EventTick
  (params (DeltaSeconds :type Float%20%28single-precision%29)))

(fn ConstructionScript)

(fn GetGroupfromLocation
  (params (location :type Vector))
  (bind (_x _y) (Math|Vector|BreakVector location))
  (bind _returnvalue (Math|Float|Sign(Float) _x))
  (bind _returnvalue_2 (Math|Float|Sign(Float) _y))
  (bind _returnvalue_3 (Math|Float|Absolute(Float) _returnvalue))
  (bind _returnvalue_4 (Math|Float|Absolute(Float) _returnvalue_2))
  (bind _returnvalue_5 (+ _returnvalue_3 _returnvalue_4))
  (if (== _returnvalue_5 0.0)
    (return 2)
    (elif (> _returnvalue_5 0.0)
      (return 0)
      (else
        (return 1)))))

(fn GetGroup
  (params (index :type Integer))
  (return (Utilities|Select :Index index :Option%200 (Variables|Default|GetGroup%201) :Option%201 (Variables|Default|GetGroup%202) :Option%202 (Variables|Default|GetGroup%203))))

(fn AddTRLight
  (params (light :type BPI%20Techno%20Reverie%20Light%20Interface))
  (bind _location (Default|GetLocation light))
  (bind _group_index (CallFunction|GetGroupfromLocation _location))
  (Utilities|Array|AddUnique (CallFunction|GetGroup _group_index) light)
  (Default|SetLightPowered light (Utilities|Array|Get(acopy) (Variables|Default|Getpowered) _group_index) (Utilities|Array|Get(acopy) (Variables|Default|Getpower%20levels) _group_index)))

(fn UpdatePowerforQuadrent
  (params (quadrent :type Integer) (on :type Boolean) (amount :type Float%20%28double-precision%29))
  (Utilities|Array|SetArrayElem (Variables|Default|Getpowered) quadrent on)
  (Utilities|Array|SetArrayElem (Variables|Default|Getpower%20levels) quadrent amount)
  (for _array_element (CallFunction|GetGroup quadrent)
    (Default|SetLightPowered _array_element on amount)))