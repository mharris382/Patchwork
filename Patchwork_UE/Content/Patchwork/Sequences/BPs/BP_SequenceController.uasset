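; Sequence controller Blueprint that starts, pauses and resumes playback of a referenced sequence actor.
; On BeginPlay it can autoplay the sequence after a configurable delay.
; PauseSequence and ResumeSequence check the actor is valid before calling its SequencePlayer, while Pause_Event pauses through a passed-in controller without that check.
; Both pause events print on-screen debug messages.
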(event Custom|PauseSequence
  (Development|PrintString "Paused triggered in controller" true true "(R=0.700191,G=1.000000,B=0.000000,A=1.000000)" 5.0)
  (bind _sequenceactor (Variables|Default|GetSequenceActor)
    (:then
      (Sequencer|Player|Pause (Variables|/Script/LevelSequence.LevelSequenceActor|GetSequencePlayer _sequenceactor))
      (Development|PrintString "Pause called" true true "(R=1.000000,G=0.261811,B=0.000000,A=1.000000)" 5.0))
    (:else)))

(event Custom|ResumeSequence
  (bind _sequenceactor (Variables|Default|GetSequenceActor)
    (:then
      (Sequencer|Player|Play (Variables|/Script/LevelSequence.LevelSequenceActor|GetSequencePlayer _sequenceactor) :!class /Script/MovieScene.MovieSceneSequencePlayer))
    (:else)))

(event Custom|Pause_Event
  (params (Sequence%20Controller :type BP%20Sequence%20Controller%20Object%20Reference))
  (Development|PrintString "Paused triggered in controller" true true "(R=0.700191,G=1.000000,B=0.000000,A=1.000000)" 5.0)
  (Sequencer|Player|Pause (Variables|/Script/LevelSequence.LevelSequenceActor|GetSequencePlayer (Variables|BP_SequenceController_C|GetSequenceActor Sequence%20Controller)))
  (Development|PrintString "Pause called" true true "(R=1.000000,G=0.261811,B=0.000000,A=1.000000)" 5.0))

(event EventBeginPlay
  (if (Variables|Default|GetAutoplay)
    (Utilities|FlowControl|Delay (Variables|Default|GetDelay))
    (Sequencer|Player|Play (Variables|/Script/LevelSequence.LevelSequenceActor|GetSequencePlayer (Variables|Default|GetSequenceActor)) :!class /Script/MovieScene.MovieSceneSequencePlayer)))

(event EventTick
  (params (DeltaSeconds :type Float%20%28single-precision%29)))

(fn ConstructionScript)