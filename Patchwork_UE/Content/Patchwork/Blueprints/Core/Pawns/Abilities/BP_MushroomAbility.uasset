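; Player ability that throws a projectile to place a bouncy mushroom, with throw speed scaled by how long the input is held.
; One mushroom, pre-spawned out of sight at BeginPlay, is despawned on each throw and handed to the new projectile for reuse.
; The projectile's hit event records the placement, and affected actors receive spawn and despawn messages.
; Throwing while falling launches the player opposite the projectile's direction.
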(event Custom|Throw%20Mushroom
  (bind _current_spawned_mushroom (Variables|Default|Getcurrent%20spawned%20mushroom))
  (bind _current_spawned_mushroom_2 (Variables|Default|Getcurrent%20spawned%20mushroom))
  (bind _last_attached_component (Variables|Default|Getlast%20attached%20component))
  (bind _returnvalue (Transformation|GetActorLocation _current_spawned_mushroom_2))
  (Utilities|FlowControl|Sequence
    (:then_0
      ;[0.2396 0.2396 0.2396] Cleanup previous projectiles and mushrooms
      (Utilities|IsValid (Variables|Default|Getlast%20projectile)
        (:Is%20Valid
          ;;[0.6233 0.6233 0.6233 0.5] Probably not necessary since projectile currently destroys itself after
          (EventDispatchers|UnbindallEventsfromOnSuccefullHit (Variables|Default|Getlast%20projectile))
          (Actor|DestroyActor (Variables|Default|Getlast%20projectile))
          (Variables|Default|Setlast%20projectile 0))))
    (:then_1
      ;[0.6233 0.6233 0.6233 0.5] Despawn previous Mushroom
      (Utilities|IsValid _current_spawned_mushroom_2
        (:Is%20Valid
          (Utilities|FlowControl|Sequence
            (:then_0
              (Utilities|IsValid _last_attached_component
                (:Is%20Valid
                  (Class|BPIMushroomListener|OnMushroomDespawned(Message) _last_attached_component _returnvalue)
                  (Class|BPIMushroomListener|OnMushroomDespawned(Message) (Components|GetOwner _last_attached_component) _returnvalue))))
            (:then_1
              (Default|Despawn _current_spawned_mushroom_2))))))
    (:then_2
      (Utilities|FlowControl|Sequence
        (:then_0
          ;[1 1 1] Throw new projectile
          (bind _returnvalue_2 (CallFunction|GetProjectilefromPool (CallFunction|GetProjectileSpawnTransform)))
          (bind _output_get (Variables|Default|Setlast%20projectile _returnvalue_2))
          (Utilities|FlowControl|Sequence
            (:then_0
              (Utilities|IsValid _current_spawned_mushroom
                (:Is%20Valid
                  (Default|AssignPooledBouncer (Variables|Default|Getlast%20projectile) _current_spawned_mushroom))))
            (:then_1
              (EventDispatchers|BindEventtoOnSuccefullHit _output_get (delegate Custom|CustomEvent_0))
              (Variables|/Script/Engine.ProjectileMovementComponent|SetInitialSpeed (Variables|/Game/Patchwork/Blueprints/Core/Pawns/Abilities/BP_Mushroom_Projectile.BP_Mushroom_Projectile_C|GetProjectileMovement _output_get) (CallFunction|GetThrowVelocity)))))
        (:then_1
          (CallFunction|CheckforAerialThrowForce))))))

(event Custom|CustomEvent_0
  (params (mushroom :type BP%20Bouncy%20Mushroom%20Object%20Reference) (attached%20component :type Primitive%20Component%20Object%20Reference) (location :type Vector) (impact%20normal :type Vector) (Hit :type Hit%20Result%20Structure))
  (bind _output_get (Variables|Default|Setcurrent%20spawned%20mushroom mushroom))
  (Variables|Default|Setlast%20attached%20component attached%20component)
  (Class|BPIMushroomListener|OnMushroomSpawned(Message) (.HitActor (Collision|BreakHitResult Hit)) _output_get 0 location impact%20normal Hit))

(event Input|EnhancedActionEvents|EnhancedInputActionIA_Ability_1
  (params (ActionValue :type Boolean) (ElapsedSeconds :type Float%20%28double-precision%29) (TriggeredSeconds :type Float%20%28double-precision%29) (InputAction :type Input%20Action%20Object%20Reference :default "/Game/Patchwork/Data/Input/IA_Ability_1.IA_Ability_1"))
  ;[0.6233 0.6233 0.6233 0.5] Input Listener
  (:Started
    (bind _success (CallFunction|UseAbility))
    (if _success
      (Variables|Default|Sethold%20time 0.0)
      (Variables|Default|Setis%20holding true)
      (Default|CallOnAbilityStarted)))
  (:Ongoing
    (if (Variables|Default|Getis%20holding)
      (Variables|Default|Sethold%20time (Math|Float|Min(Float) ElapsedSeconds (Variables|Default|Getmax%20hold%20time)))))
  (:Canceled
    (if (Variables|Default|Getis%20holding) :!label _label
      (Variables|Default|Setis%20holding false)
      (Default|CallOnAbilityCompleted false)
      (CallFunction|ThrowMushroom)))
  (:Completed
    (goto _label)))

(event EventBeginPlay
  (|CallParentFunction)
  (bind _returnvalue (Game|SpawnActorfromClass "/Game/Patchwork/Blueprints/Core/Pawns/Abilities/BP_Bouncy_Mushroom.BP_Bouncy_Mushroom_C" (Math|Transform|MakeTransform "0.000000,0.000000,-10000000.000000") "Undefined" "MultiplyWithRoot" 0 0))
  (Variables|Default|Setcurrent%20spawned%20mushroom _returnvalue))

(event EventTick
  (params (DeltaSeconds :type Float%20%28single-precision%29)))

(fn GetThrowPowerPercent
  (return (/ (Variables|Default|Gethold%20time) (Variables|Default|Getmax%20hold%20time))))

(fn GetThrowVelocity
  (return (Math|Float|Lerp (Variables|Default|Getmin%20throw%20velocity) (Variables|Default|Getmax%20throw%20velocity) (CallFunction|GetThrowPowerPercent))))

(fn CheckforAerialThrowForce
  (bind _last_projectile (Variables|Default|Getlast%20projectile))
  (bind _asbp_base_character (Utilities|Casting|CastToBP_BaseCharacter (Game|Player|GetPlayerPawn 0)))
  (if (Utilities|Enum|Equal(Enum) (Variables|/Script/Engine.CharacterMovementComponent|GetMovementMode (Variables|/Script/Engine.Character|GetCharacterMovement _asbp_base_character)) "MOVE_Falling")
    (Utilities|IsValid _last_projectile
      (:Is%20Valid
        (Character|LaunchCharacter _asbp_base_character (* (Transformation|GetActorForwardVector _last_projectile) -1.0 (Variables|Default|Getmax%20repulsion%20force)) false false)))))

(fn GetProjectileSpawnTransform
  (bind _returnvalue (Components|GetOwner))
  (bind _asbp_base_character (Utilities|Casting|CastToBP_BaseCharacter _returnvalue))
  (return (select (Default|IsCameraFP _asbp_base_character) (Transformation|GetWorldTransform) (Transformation|GetWorldTransform (Variables|/Game/Patchwork/Blueprints/Core/Pawns/BP_BaseCharacter.BP_BaseCharacter_C|GetThrow%20Point _asbp_base_character)))))

(fn GetProjectilefromPool
  (params (SpawnTransform :type Transform))
  (bind _projectilepool (Variables|Default|GetProjectilePool))
  (bind _projectilepool_2 (Variables|Default|GetProjectilePool))
  (bind _returnvalue (Utilities|Array|Length _projectilepool_2))
  (if (> _returnvalue 0)
    (Utilities|Array|RemoveItem _projectilepool (Utilities|Array|Get(acopy) _projectilepool (- _returnvalue 1)))
    (return 0)
    (else
      (bind _returnvalue_2 (Game|SpawnActorfromClass "/Game/Patchwork/Blueprints/Core/Pawns/Abilities/BP_Mushroom_Projectile.BP_Mushroom_Projectile_C" SpawnTransform "Undefined" "MultiplyWithRoot" (Components|GetOwner) (Game|Player|GetPlayerPawn 0)))
      (return _returnvalue_2))))