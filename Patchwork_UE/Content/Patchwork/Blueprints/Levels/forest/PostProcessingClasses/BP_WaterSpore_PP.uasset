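; BP_WaterSpore_PP is a forest level post-processing Blueprint, named for a water spore effect, that extends a parent class providing blend updates.
; Its UpdateBlend event runs the parent logic, then writes the blend value to a named scalar in a Material Parameter Collection, exposing it to materials.
; BeginPlay, overlap and Tick are disabled stubs, and the construction script only calls its parent.
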(event EventBeginPlay
  (|CallParentFunction) ; This node is disabled and will not be called.\nDrag off pins to build functionality.
)

(event Collision|EventActorBeginOverlap
  (params (OtherActor :type Actor%20Object%20Reference))
  (|CallParentFunction OtherActor) ; This node is disabled and will not be called.\nDrag off pins to build functionality.
)

(event EventTick
  (params (DeltaSeconds :type Float%20%28single-precision%29))
  (|CallParentFunction DeltaSeconds) ; This node is disabled and will not be called.\nDrag off pins to build functionality.
)

(event EventUpdateBlend
  (params (blend :type Float%20%28double-precision%29))
  (|CallParentFunction blend)
  (Rendering|Material|SetScalarParameterValue (Variables|Default|GetParam%20Collection) (Variables|Default|Get%20Name) blend :!class /Script/Engine.KismetMaterialLibrary))

(fn ConstructionScript
  (|CallParentFunction))