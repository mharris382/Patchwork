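; Geyser water prop that holds a platform at MaxHeight above a Niagara spout, using a physics constraint.
; Construction script sizes the effect, places the platform and sets a limited Z constraint with a position drive targeting MaxHeight.
; Tick reapplies height and zeroes platform rotation every frame, but frees the Z limit, targets zero and adds velocity drive with tunable strength and force limit.
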(event EventBeginPlay)

(event Collision|EventActorBeginOverlap
  (params (OtherActor :type Actor%20Object%20Reference)))

(event EventTick
  (params (DeltaSeconds :type Float%20%28single-precision%29))
  (bind _physicsconstraint (Variables|Default|GetPhysicsConstraint))
  (Effects|Components|ParticleSystem|SetFloatParameter (Variables|Default|GetNS_Geyser) "GyeserHeight" (Variables|Default|GetMaxHeight))
  (Transformation|SetRelativeLocation (Variables|Default|GetPlatform) (Math|Vector|MakeVector 0.0 0.0 (Variables|Default|GetMaxHeight)) false false)
  (Class|PhysicsConstraintComponent|SetLinearZLimit (Variables|Default|GetPhysicsConstraint) "LCM_Free" (+ (Variables|Default|GetMaxHeight) (Variables|Default|GetDistanceLimitOffset)))
  (Class|PhysicsConstraintComponent|SetLinearPositionTarget (Variables|Default|GetPhysicsConstraint) (Math|Vector|MakeVector 0.0 0.0 0.0))
  (Class|PhysicsConstraintComponent|SetLinearPositionDrive _physicsconstraint false false true)
  (Class|PhysicsConstraintComponent|SetLinearDriveParams _physicsconstraint (Variables|Default|GetMaxLinearPositionStrength) (Variables|Default|GetMaxLinearVelocityStrength) (Variables|Default|GetMaxForceLimit))
  (Class|PhysicsConstraintComponent|SetLinearVelocityDrive _physicsconstraint true true true)
  (Transformation|SetRelativeRotation (Variables|Default|GetPlatform) "0, 0, 0" false false))

(fn ConstructionScript
  (bind _physicsconstraint (Variables|Default|GetPhysicsConstraint))
  (Effects|Components|ParticleSystem|SetFloatParameter (Variables|Default|GetNS_Geyser) "GyeserHeight" (Variables|Default|GetMaxHeight))
  (Transformation|SetRelativeLocation (Variables|Default|GetPlatform) (Math|Vector|MakeVector 0.0 0.0 (Variables|Default|GetMaxHeight)) false false)
  (Class|PhysicsConstraintComponent|SetLinearZLimit (Variables|Default|GetPhysicsConstraint) "LCM_Limited" (+ (Variables|Default|GetMaxHeight) (Variables|Default|GetDistanceLimitOffset)))
  (Class|PhysicsConstraintComponent|SetLinearPositionTarget (Variables|Default|GetPhysicsConstraint) (Math|Vector|MakeVector 0.0 0.0 (Variables|Default|GetMaxHeight)))
  (Class|PhysicsConstraintComponent|SetLinearPositionDrive _physicsconstraint false false true)
  (Class|PhysicsConstraintComponent|SetLinearDriveParams _physicsconstraint (Variables|Default|GetMaxLinearPositionStrength) 0.0 0.0))