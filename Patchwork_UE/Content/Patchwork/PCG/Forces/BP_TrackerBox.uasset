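; BP_TrackerBox is an actor that tracks when actors from a supplied list are inside its overlap volume.
; Init sets the list, then overlap events store each tracked actor's entry game time in a map and remove it on exit.
; IsActorInBox reports presence from that map, returning the raw entry timestamp as DurationInBox rather than elapsed time.
; Tick prints all overlapping actor names for debugging.
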(event Custom|Init
  (params (TrackedActors :type Array%20of%20Actor%20Object%20References))
  (Variables|Default|SetTracked%20Actors TrackedActors)
  (Variables|Default|SetInited true)
  (Development|PrintString "Inited"))

(event EventBeginPlay)

(event Collision|EventActorBeginOverlap
  (params (OtherActor :type Actor%20Object%20Reference))
  (if (Math|Boolean|ANDBoolean (Utilities|IsValid OtherActor) (Variables|Default|GetInited) (Utilities|Array|ContainsItem (Variables|Default|GetTracked%20Actors) OtherActor))
    (Utilities|Map|Add (Variables|Default|GetActorEnterTimestamps) OtherActor (Utilities|Time|GetGameTimeinSeconds))))

(event EventTick
  (params (DeltaSeconds :type Float%20%28single-precision%29))
  (bind _overlappingactors (Collision|GetOverlappingActors "/Script/Engine.Actor" :!class /Script/Engine.Actor))
  (bind _returnvalue (Utilities|Array|Length _overlappingactors))
  (if (Variables|Default|GetInited)
    (if (> _returnvalue 0)
      (Variables|Default|Setactors (Utilities|String|Append (Utilities|GetDisplayName self) ":" (Utilities|String|Append "(" (Utilities|String|ToString(Integer) _returnvalue) ")") "-"))
      (for _array_element _overlappingactors
        (Utilities|IsValid _array_element
          (:Is%20Valid
            (Variables|Default|Setactors (Utilities|String|Append (Variables|Default|Getactors) ", " (Utilities|GetDisplayName _array_element))))))
      (Development|PrintString (Variables|Default|Getactors)))))

(event Collision|EventActorEndOverlap
  (params (OtherActor :type Actor%20Object%20Reference))
  (Utilities|IsActorTracked OtherActor
    (:then
      (Utilities|Map|Remove (Variables|Default|GetActorEnterTimestamps) OtherActor))))

(fn ConstructionScript)

(fn IsActorinBox
  (params (Actor :type Actor%20Object%20Reference))
  (bind _actorentertimestamps (Variables|Default|GetActorEnterTimestamps))
  (bind (_value _returnvalue) (Utilities|Map|Find _actorentertimestamps Actor))
  (Utilities|IsValid Actor
    (:Is%20Valid
      (Utilities|IsActorTracked Actor
        (:then
          (return _returnvalue _value))
        (:false
          (Development|PrintText (Utilities|Text|FormatText "Actor {0} is not tracked" 0)))))
    (:Is%20Not%20Valid
      (return false 0.0))))