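; A placeable trigger volume that invokes a named world event when the player pawn overlaps it, if overlap invoking is enabled.
; Overlap first requires every prerequisite event to have occurred, as checked through GM_BaseGameMode.
; InvokeEvent then asks that game mode to fire the event and prints success or failure.
; The construction script copies the event name to the EventInvoker and sizes the box from exposed variables.
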(event Collision|EventActorBeginOverlap
  (params (OtherActor :type Actor%20Object%20Reference))
  (bind _all_met (CallFunction|AllPrerequisitsMet))
  (if _all_met
    (if (and (== OtherActor (Game|Player|GetPlayerPawn 0)) (Variables|Default|GetInvoke%20On%20Player%20Overlapped))
      (CallFunction|InvokeEvent))))

(fn ConstructionScript
  (Variables|/Game/Patchwork/Blueprints/WorldEvents/EventInvoker.EventInvoker_C|SetEvent%20Name (Variables|Default|GetEventInvoker) (Variables|Default|GetWorld%20Event%20Name))
  (Components|Box|SetBoxExtent (Variables|Default|GetBox) (Variables|Default|GetBox%20Size) true))

(fn InvokeEvent
  (bind _self self)
  (bind _returnvalue (Utilities|GetDisplayName _self))
  (bind _asgm_base_game_mode (Utilities|Casting|CastToGM_BaseGameMode (Game|GetGameMode)))
  (bind _invoked (Default|InvokeWorldEvent _asgm_base_game_mode (Variables|Default|GetWorld%20Event%20Name)))
  (if _invoked
    (Development|PrintText (Utilities|Text|FormatText "{0} invoked {1}" _returnvalue (Variables|Default|GetWorld%20Event%20Name)))
    (else
      (Development|PrintText (Utilities|Text|FormatText "{0} failed to invoke {1}" _returnvalue (Variables|Default|GetWorld%20Event%20Name))))))

(fn AllPrerequisitsMet
  (LocalVariables|Setmet true)
  (bind _asgm_base_game_mode (Utilities|Casting|CastToGM_BaseGameMode (Game|GetGameMode))
    (:then
      (LocalVariables|Setgmode _asgm_base_game_mode)
      (bind _array_element (Utilities|Array|ForEachLoopwithBreak (Variables|Default|GetPrerequisite%20Events) :!label _label)
        (:LoopBody
          (bind _event_occured (Default|HasWorldEventOccured (LocalVariables|Getgmode) _array_element))
          (if (not _event_occured)
            (LocalVariables|Setmet false)
            (goto _label Break)))
        (:Completed
          (return (LocalVariables|Getmet)))))
    (:CastFailed
      (return false))))