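; Quest logic Blueprint for the desert key collection quest that determines whether the quest is complete.
; IsQuestCompleted asks the GameMode whether each world event in the EventNames array has occurred, failing on the first missing one and passing only when all have.
; The event graph holds only disabled BeginPlay and Tick stubs, so completion is evaluated whenever the function is called.
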(event EventBeginPlay
  (|CallParentFunction) ; This node is disabled and will not be called.\nDrag off pins to build functionality.
)

(event EventTick
  (params (DeltaSeconds :type Float%20%28single-precision%29))
  (|CallParentFunction DeltaSeconds) ; This node is disabled and will not be called.\nDrag off pins to build functionality.
)

(fn IsQuestCompleted
  (for _array_element (Variables|Default|Getevent%20names)
    (bind _event_occured (Default|HasWorldEventOccured (Variables|Default|GetGame%20Mode) _array_element))
    (if (not _event_occured)
      (return false)))
  (return true))