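; BP_Lever_Reality is a lever interactible that can only be used while the player carries a Reality spore.
; It overrides IsInteractAvailable, keeping the parent check and then querying the player pawn's BP_SporeCarrier for the RealitySpore effect tag.
; All other behavior comes from the parent lever class, as its own event graph holds only disabled default events.
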(event EventBeginPlay
  (|CallParentFunction) ; This node is disabled and will not be called.\nDrag off pins to build functionality.
)

(event Collision|EventActorBeginOverlap
  (params (OtherActor :type Actor%20Object%20Reference))
  (|CallParentFunction OtherActor) ; This node is disabled and will not be called.\nDrag off pins to build functionality.
)

(event EventTick
  (params (DeltaSeconds :type Float%20%28single-precision%29))
  (|CallParentFunction DeltaSeconds) ; This node is disabled and will not be called.\nDrag off pins to build functionality.
)

(fn ConstructionScript
  (|CallParentFunction))

(fn IsInteractAvailable
  (bind _available (|CallParentFunction))
  (if _available
    (return (Default|HasSporefromTag (Actor|GetComponentbyClass (Game|Player|GetPlayerPawn 0) "/Game/Patchwork/Blueprints/Levels/forest/Utilities/BP_SporeCarrier.BP_SporeCarrier_C") "(TagName=\"SporeEffects.EffectType.RealitySpore\")"))
    (else
      (return false))))