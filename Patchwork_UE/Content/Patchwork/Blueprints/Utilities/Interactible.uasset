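; Base Interactible actor Blueprint that exposes an interaction event, prompt text and availability for in-world interactions.
; OnInteract is empty, and availability returns the CanInteract flag, which is set true on BeginPlay.
; The prompt is just the action verb, "Interact" here, exposed through wrapper getters with near-duplicate names.
; GetInteractKey picks a key label from the CommonInput input type, but the formatted "Press key to verb" message is left unused.
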(event EventBeginPlay
  (Variables|Default|Setcan%20interact true))

(event Collision|EventActorBeginOverlap
  (params (OtherActor :type Actor%20Object%20Reference)))

(event EventTick
  (params (DeltaSeconds :type Float%20%28single-precision%29)))

(event EventOnInteract)

(fn ConstructionScript)

(fn GetInteractMessage
  (return (Interaction|GetActionVerb)))

(fn GetActionVerb
  (return "Interact"))

(fn GetInteractKey
  (bind _returnvalue (PlayerController|LocalPlayerSubsystems|GetCommonInputSubsystem))
  (Utilities|IsValid _returnvalue
    (:Is%20Valid
      (switch Utilities|FlowControl|Switch|SwitchonECommonInputType (Class|CommonInputSubsystem|GetCurrentInputType _returnvalue)
        (:MouseAndKeyboard
          _)
        (:Gamepad
          (return "X"))
        (:Touch
          (return "?"))
        (:Count
          (return "?"))))
    (:Is%20Not%20Valid
      _))
  (return "e"))

(fn IsInteractionAvailable
  (return (Variables|Default|Getcan%20interact)))

(fn GetInteractionMessage
  (return (Interaction|GetInteractMessage)))

(fn GetInteractVerb
  (return (Interaction|GetActionVerb)))

(fn IsInteractAvailable
  (return (CallFunction|IsInteractionAvailable)))