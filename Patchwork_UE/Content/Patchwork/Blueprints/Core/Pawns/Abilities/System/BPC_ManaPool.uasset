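; BPC_ManaPool is an ability-system component that stores the player's current mana against a maximum tied to GlobalPlayerAbilitySettings.
; AddMana clamps at the maximum, RemoveMana refuses amounts exceeding the pool, and InstantRefill either fills it or delegates to AddMana.
; Dispatchers report changes, insufficient mana and, through AddMana only, reaching maximum.
; A cached flag blocks additions when full, while the IsAtMaximum getter actually returns true below maximum.
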(event Custom|AddMana
  (params (Amount :type Float%20%28double-precision%29))
  ;[0.6233 0.6233 0.6233 0.5] Try to add mana to the pool
  (if (not (Variables|Default|GetIsManaAtMaximum))
    (if (>= (+ Amount (Variables|Default|GetCurrentMana)) (Utilities|PlayerMaxMana))
      (Variables|Default|SetCurrentMana (Utilities|PlayerMaxMana))
      (Variables|Default|SetIsManaAtMaximum true)
      (Default|CallMaximumManaReached)
      (Default|CallManaChanged (Variables|Default|GetCurrentMana) true)
      (else
        (bind _output_get (Variables|Default|SetCurrentMana (+ Amount (Variables|Default|GetCurrentMana))))
        (Default|CallManaChanged _output_get true)))))

(event Custom|RemoveMana
  (params (Amount :type Float%20%28double-precision%29))
  ;[0.6233 0.6233 0.6233 0.5] Try to remove mana from the pool
  (if (> Amount (Variables|Default|GetCurrentMana))
    (Default|CallNotEnoughMana)
    (Variables|Default|SetIsManaAtMaximum false)
    (else
      (bind _output_get (Variables|Default|SetCurrentMana (- (Variables|Default|GetCurrentMana) Amount)))
      (Default|CallManaChanged _output_get false)
      (Variables|Default|SetIsManaAtMaximum false))))

(event Custom|InstantRefill
  (params (FillToMax :type Boolean) (Amount :type Float%20%28double-precision%29))
  ;[0.6233 0.6233 0.6233 0.5] Instantly set the mana to the maximum
  (if FillToMax
    (bind _output_get (Variables|Default|SetCurrentMana (Utilities|PlayerMaxMana)))
    (Variables|Default|SetIsManaAtMaximum true)
    (Default|CallManaChanged _output_get true)
    (else
      (CallFunction|AddMana Amount))))

(event EventBeginPlay
  (if (< (Variables|Default|GetCurrentMana) 0.0)
    (Development|PrintText "Invalid mana data" true true "(R=1.000000,G=0.000000,B=0.000000,A=1.000000)")
    (else
      (Variables|Default|SetIsManaAtMaximum (== (Variables|Default|GetCurrentMana) (Variables|/Game/Patchwork/Blueprints/Utilities/BP_GlobalAbilitySettings.BP_GlobalAbilitySettings_C|GetPlayerMaxMana (Variables|Default|GetGlobalPlayerAbilitySettings)))))))

(event EventTick
  (params (DeltaSeconds :type Float%20%28single-precision%29)))

(fn GetMana
  (return (Variables|Default|GetCurrentMana)))

(fn GetMaximum
  (return (Utilities|PlayerMaxMana)))

(fn IsatMaximum
  (return (< (Variables|Default|GetCurrentMana) (Utilities|PlayerMaxMana))))