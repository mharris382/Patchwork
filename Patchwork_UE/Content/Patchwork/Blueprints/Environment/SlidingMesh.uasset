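; Environment actor that slides a Pivot back and forth along a spline, with MoveToStart and MoveToEnd setting the travel direction.
; Tick eases the actual direction toward the target by an acceleration factor, accumulates time, and converts it to a clamped, normalized spline position.
; UpdatePosition places the Pivot there, optionally matching spline rotation.
; The construction script applies the configured position in-editor and seeds the current time from it.
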(event EventBeginPlay)

(event Collision|EventActorBeginOverlap
  (params (OtherActor :type Actor%20Object%20Reference)))

(event EventTick
  (params (DeltaSeconds :type Float%20%28single-precision%29))
  (bind _total_time_on_spline (Variables|Default|Gettotal%20time%20on%20spline))
  (Variables|Default|Setactual%20direction (Math|Float|Lerp (Variables|Default|Getactual%20direction) (Variables|Default|Getdirection) (Math|Float|Clamp(Float) (* DeltaSeconds (Variables|Default|Getacceleration)))))
  (bind _output_get (Variables|Default|Setcurrent%20time (+ (* DeltaSeconds (Variables|Default|Getactual%20direction)) (Variables|Default|Getcurrent%20time))))
  (Variables|Default|Setposition%20on%20spline (/ (Math|Float|Clamp(Float) _output_get 0.0 _total_time_on_spline) _total_time_on_spline))
  (CallFunction|UpdatePosition))

(fn ConstructionScript
  (Utilities|FlowControl|Sequence
    (:then_0
      (CallFunction|UpdatePosition))
    (:then_1
      (if (not (Variables|Default|Getignore%20rotation))
        (Transformation|SetRelativeRotation (Variables|Default|Getpivot) (Class|SplineComponent|GetRotationatTime (Variables|Default|GetSpline) (Variables|Default|Getposition%20on%20spline) "Local" false) false false)))
    (:then_2
      (Variables|Default|Setcurrent%20time (* (Variables|Default|Getposition%20on%20spline) (Variables|Default|Gettotal%20time%20on%20spline))))))

(fn MovetoStart
  (Variables|Default|Setdirection -1.0))

(fn MovetoEnd
  (Variables|Default|Setdirection 1.0))

(fn UpdatePosition
  (Transformation|SetRelativeLocation (Variables|Default|Getpivot) (Spline|GetLocationatTime (Variables|Default|GetSpline) (Variables|Default|Getposition%20on%20spline) "Local" false) false false)
  (if (not (Variables|Default|Getignore%20rotation))
    (Transformation|SetRelativeRotation (Variables|Default|Getpivot) (Class|SplineComponent|GetRotationatTime (Variables|Default|GetSpline) (Variables|Default|Getposition%20on%20spline) "Local" false) false false)))