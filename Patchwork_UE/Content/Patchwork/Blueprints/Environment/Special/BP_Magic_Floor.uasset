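; BP_Magic_Floor is a resizable special environment floor made of a plane and a Niagara effect.
; The construction script passes Size to the effect's "Box Size" parameter and scales the plane in X and Y from Size plus CollisionPadding, keeping Z at 1.
; The mushroom spawned and despawned events are empty, so the graphs add no runtime logic.
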(event EventBeginPlay)

(event EventTick
  (params (DeltaSeconds :type Float%20%28single-precision%29)))

(event EventOnMushroomDespawned
  (params (despawned%20location :type Vector :default "0, 0, 0")))

(event EventOnMushroomSpawned
  (params (mushroom :type BP%20Bouncy%20Mushroom%20Object%20Reference) (hit%20component :type Shape%20Component%20Object%20Reference) (hit%20point :type Vector :default "0, 0, 0") (hit%20normal :type Vector :default "0, 0, 0")))

(fn ConstructionScript
  (bind _size (Variables|Default|GetSize))
  (bind _collision_padding (Variables|Default|GetCollision%20Padding))
  (bind _returnvalue (/ _size "100.000000,100.000000,100.000000"))
  (bind _returnvalue_2 (+ _returnvalue _collision_padding))
  (bind (_x _y) (Math|Vector|BreakVector _returnvalue_2))
  (Utilities|FlowControl|Sequence
    (:then_0
      (Effects|Components|ParticleSystem|SetVectorParameter (Variables|NiagaraActor|GetNiagaraComponent) "Box Size" (Variables|Default|GetSize)))
    (:then_1
      (Transformation|SetRelativeScale3D (Variables|Default|GetPlane) (Math|Vector|MakeVector _x _y 1.0)))))