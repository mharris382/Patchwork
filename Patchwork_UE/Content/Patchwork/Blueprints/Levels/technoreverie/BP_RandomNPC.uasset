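; Random NPC for the technoreverie level, assembled from Paper2D sprites with no active runtime logic.
; The construction script picks random body, head and gear sprites from their lists, so the look re-rolls whenever the script runs.
; Head and gear each copy their sprite to a matching back component.
; Body, head and gear each draw their own random material from a shared list, with each front and back pair matching.
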(event EventBeginPlay)

(event Collision|EventActorBeginOverlap
  (params (OtherActor :type Actor%20Object%20Reference)))

(event EventTick
  (params (DeltaSeconds :type Float%20%28single-precision%29)))

(fn ConstructionScript
  (Rendering|Components|Sprite|SetSprite (Variables|Default|GetBody) (.OutItem (Utilities|Array|Random (Variables|Default|GetBodyList))))
  (bind _output_get (LocalVariables|Setselected%20face (.OutItem (Utilities|Array|Random (Variables|Default|GetHeadList)))))
  (Rendering|Components|Sprite|SetSprite (Variables|Default|GetHead) _output_get)
  (Rendering|Components|Sprite|SetSprite (Variables|Default|GetHead%20Back) _output_get)
  (bind _output_get_2 (LocalVariables|Setselected%20gear (.OutItem (Utilities|Array|Random (Variables|Default|GetGearList)))))
  (Rendering|Components|Sprite|SetSprite (Variables|Default|GetGear) _output_get_2)
  (Rendering|Components|Sprite|SetSprite (Variables|Default|GetGear%20Back) _output_get_2)
  (bind _output_get_3 (LocalVariables|Setselected%20material (.OutItem (Utilities|Array|Random (Variables|Default|GetMaterials)))))
  (Rendering|Material|SetMaterial (Variables|Default|GetGear) 0 _output_get_3)
  (Rendering|Material|SetMaterial (Variables|Default|GetGear%20Back) 0 _output_get_3)
  (bind _output_get_4 (LocalVariables|Setselected%20material (.OutItem (Utilities|Array|Random (Variables|Default|GetMaterials)))))
  (Rendering|Material|SetMaterial (Variables|Default|GetHead) 0 _output_get_4)
  (Rendering|Material|SetMaterial (Variables|Default|GetHead%20Back) 0 _output_get_4)
  (Rendering|Material|SetMaterial (Variables|Default|GetBody) 0 (.OutItem (Utilities|Array|Random (Variables|Default|GetMaterials)))))