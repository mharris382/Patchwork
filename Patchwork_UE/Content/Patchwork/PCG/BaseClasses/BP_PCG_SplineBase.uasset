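; Base actor for spline-driven PCG tools, holding a Spline and a PCG component.
; After running the parent construction script, it forces Looping on when SpawnOnInterior is set, then applies Looping as the spline's closed-loop state without an immediate spline update.
; Nodes to set the PCG graph and generate are present but never run, and the event graph is empty.
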(event EventBeginPlay)

(event Collision|EventActorBeginOverlap
  (params (OtherActor :type Actor%20Object%20Reference)))

(event EventTick
  (params (DeltaSeconds :type Float%20%28single-precision%29)))

(fn ConstructionScript
  (|CallParentFunction)
  (Utilities|FlowControl|Sequence
    (:then_0
      (if (Variables|Spline|GetSpawn%20on%20Interior)
        (Variables|Spline|SetLooping true)))
    (:then_1
      (Spline|SetClosedLoop (Variables|Default|GetSpline) (Variables|Spline|GetLooping) false))))