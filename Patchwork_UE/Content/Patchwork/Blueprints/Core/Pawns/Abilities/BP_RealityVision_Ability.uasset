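; BP_RealityVision_Ability is the player's toggleable Reality Vision ability, which drives the tripping spore effect while draining mana.
; On BeginPlay it caches the player pawn's mana pool and finds or adds the tripping effect component.
; Input toggles it on when the parent check and mana allow.
; Tick drains mana, ends the ability when mana runs short, and interpolates the effect's toxicity toward the on/off state.
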(event Input|EnhancedActionEvents|EnhancedInputActionIA_Ability_RealityVision
  (params (ActionValue :type Boolean) (ElapsedSeconds :type Float%20%28double-precision%29) (TriggeredSeconds :type Float%20%28double-precision%29) (InputAction :type Input%20Action%20Object%20Reference :default "/Game/Patchwork/Data/Input/IA_Ability_RealityVision.IA_Ability_RealityVision"))
  (bind _state (CallFunction|TryToggleAbility))
  (Variables|Default|SetState _state))

(event EventBeginPlay
  (bind _returnvalue (Game|Player|GetPlayerPawn 0))
  (bind _returnvalue_2 (Actor|GetComponentbyClass _returnvalue "/Game/Patchwork/Blueprints/Levels/forest/Effects/BP_PlayerTrippingSporeEffect.BP_PlayerTrippingSporeEffect_C"))
  (|CallParentFunction)
  (Variables|Default|SetManaPool (Actor|GetComponentbyClass _returnvalue "/Game/Patchwork/Blueprints/Core/Pawns/Abilities/System/BPC_ManaPool.BPC_ManaPool_C"))
  (Utilities|IsValid _returnvalue_2
    (:Is%20Valid
      (Variables|Default|SetTrippingEffectComponent _returnvalue_2))
    (:Is%20Not%20Valid
      (Development|PrintString "Tripping Effect Component Invalid" true true "(R=1.000000,G=0.009730,B=0.000000,A=1.000000)")
      (bind _returnvalue_3 (Game|AddComponentbyClass _returnvalue "/Game/Patchwork/Blueprints/Levels/forest/Effects/BP_PlayerTrippingSporeEffect.BP_PlayerTrippingSporeEffect_C"))
      (Variables|Default|SetTrippingEffectComponent _returnvalue_3))))

(event EventTick
  (params (DeltaSeconds :type Float%20%28single-precision%29))
  (bind _trippingeffectcomponent (Variables|Default|GetTrippingEffectComponent))
  (bind _manapool (Variables|Default|GetManaPool))
  (bind _manarequirement (Variables|Default|GetManaRequirement))
  (bind _returnvalue (* _manarequirement DeltaSeconds))
  (|CallParentFunction DeltaSeconds)
  (if (Variables|Default|GetState)
    (Default|RemoveMana _manapool _returnvalue)
    (if (< (Default|GetMana _manapool) _returnvalue)
      (CallFunction|CompleteAbility false)
      (Variables|Default|SetState false)))
  (Variables|/Game/Patchwork/Blueprints/Levels/forest/BP_SporeEffectBase.BP_SporeEffectBase_C|SetCurrent%20Toxicity _trippingeffectcomponent (Math|Interpolation|FInterpTo (Variables|/Game/Patchwork/Blueprints/Levels/forest/BP_SporeEffectBase.BP_SporeEffectBase_C|GetCurrent%20Toxicity _trippingeffectcomponent) (Math|Float|SelectFloat 1.0 0.0 (Variables|Default|GetState)) DeltaSeconds (Variables|Default|GetInterp%20Speed))))

(fn TryToggleAbility
  (if (Variables|Default|GetInUse)
    (Variables|Default|SetInUse false)
    (Default|CallOnAbilityCompleted true)
    (return false)
    (elif (CallFunction|IsReady)
      (Variables|Default|SetInUse true)
      (Default|CallOnAbilityStarted)
      (return true)
      (else
        (return false)))))

(fn IsReady
  (return (and (|CallParentFunction) (>= (Default|GetMana (Variables|Default|GetManaPool)) (Variables|Default|GetManaRequirement)))))