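; BP_PlatformTriggerGroup links a BP_Lever to a set of BP_Platforms, raising or releasing them together.
; On BeginPlay it collects unique platforms overlapping the GatherAreas' primitive components and binds to the lever, printing a warning if none is set.
; Lever position changes send every platform up to its hover point or release it.
; The construction script falls back to a parent actor lever; its box component loop has no effect.
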(event Custom|Level%20Position%20Changed
  (params (position :type Integer))
  (switch int position
    (:0
      (for _array_element (Variables|Default|GetPlatforms)
        (Default|ReleasefromHoverPoint _array_element)))
    (:1
      (for _array_element_2 (Variables|Default|GetPlatforms)
        (Default|RisetoHoverPoint _array_element_2)))))

(event EventBeginPlay
  (Utilities|IsValid (Variables|Default|GetLever)
    (:Is%20Valid
      (for _array_element (Variables|Default|GetGather%20Areas)
        (for _array_element_2 (Actor|GetComponentsByClass _array_element "/Script/Engine.PrimitiveComponent")
          (for _array_element_3 (Collision|GetOverlappingActors _array_element_2 "/Game/Patchwork/Blueprints/Environment/BP_Platform.BP_Platform_C" :!class /Script/Engine.PrimitiveComponent)
            (bind _asbp_platform (Utilities|Casting|CastToBP_Platform _array_element_3))
            (Utilities|Array|AddUnique (Variables|Default|GetPlatforms) _asbp_platform))))
      (EventDispatchers|BindEventtoOnPositionChanged (Variables|Default|GetLever) (delegate Custom|Level%20Position%20Changed)))
    (:Is%20Not%20Valid
      (Development|PrintText (Utilities|Text|FormatText "Platform Trigger Group ({0}) is missing a lever and will not function" (Utilities|GetDisplayName self))))))

(fn ConstructionScript
  (bind _returnvalue (Actor|GetParentActor))
  (Utilities|IsValid (Variables|Default|GetLever)
    (:Is%20Not%20Valid
      (Utilities|IsValid _returnvalue
        (:Is%20Valid
          (bind _asbp_lever (Utilities|Casting|CastToBP_Lever _returnvalue))
          (Variables|Default|SetLever _asbp_lever)
          (for _array_element (Components|GetChildrenComponents (Variables|Default|GetDefaultSceneRoot) true)
            (Utilities|Casting|CastToBoxComponent _array_element)))))))