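; BP_Teleport is an actor that moves the player pawn to a linked destination when the pawn overlaps it.
; On overlap, it checks that TargetLocation is valid and that the overlapping actor is player 0's pawn, then teleports it to the target's TeleportArrive component.
; On success it sets the player controller's control rotation to match that component, and on failure it prints a message.
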(event EventBeginPlay)

(event Collision|EventActorBeginOverlap
  (params (OtherActor :type Actor%20Object%20Reference))
  (bind _targetlocation (Variables|Default|GetTargetLocation))
  (bind _teleportarrive (Variables|BP_Teleport_C|GetTeleportArrive _targetlocation))
  (Utilities|IsValid (Variables|Default|GetTargetLocation)
    (:Is%20Valid
      (if (== OtherActor (Game|Player|GetPlayerPawn 0))
        (bind _returnvalue (Transformation|Teleport OtherActor (Transformation|GetWorldLocation _teleportarrive) "0, 0, 0"))
        (if _returnvalue
          (Pawn|SetControlRotation (Game|GetPlayerController 0) (Transformation|GetWorldRotation _teleportarrive))
          (else
            (Development|PrintText "Teleportation failed" true true "(R=1.000000,G=0.000000,B=0.014042,A=1.000000)")))))))

(event EventTick
  (params (DeltaSeconds :type Float%20%28single-precision%29)))

(fn ConstructionScript)