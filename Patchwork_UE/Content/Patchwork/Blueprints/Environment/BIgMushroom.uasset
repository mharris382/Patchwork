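; BigMushroom is a configurable environment mushroom Blueprint built from Stem and Cap components, with no active gameplay logic in its event graph.
; The construction script sets each part's world scale from a constant multiplied by its scale variable, and rotates the cap in world or relative space according to AbsoluteRotation.
; When valid, a single material is applied to both parts' first slot and an override mesh replaces the stem's.
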(event EventBeginPlay)

(event Collision|EventActorBeginOverlap
  (params (OtherActor :type Actor%20Object%20Reference)))

(event EventTick
  (params (DeltaSeconds :type Float%20%28single-precision%29)))

(fn ConstructionScript
  (bind _cap (Variables|Default|GetCap))
  (bind _cap_rotation (Variables|Default|GetCap%20Rotation))
  (Utilities|FlowControl|Sequence
    (:then_0
      (Transformation|SetWorldScale3D (Variables|Default|GetStem) (* (Variables|Default|GetStem%20Constant%20Scale) (Variables|Default|GetStem%20Scale))))
    (:then_1
      (Transformation|SetWorldScale3D (Variables|Default|GetCap) (* (Variables|Default|GetCap%20Constant%20Scale) (Variables|Default|GetCap%20Scale)))
      (if (Variables|Default|GetAbsolute%20Rotation)
        (Transformation|SetWorldRotation _cap _cap_rotation false false)
        (else
          (Transformation|SetRelativeRotation _cap _cap_rotation false false))))
    (:then_2
      (bind _material (Variables|Default|GetMaterial)
        (:then
          (Rendering|Material|SetMaterial (Variables|Default|GetStem) 0 _material)
          (Rendering|Material|SetMaterial (Variables|Default|GetCap) 0 _material))
        (:else)))
    (:then_3
      (bind _stem_mesh (Variables|Default|GetStem%20Mesh)
        (:then
          (Components|StaticMesh|SetStaticMesh (Variables|Default|GetStem) _stem_mesh))
        (:else)))))