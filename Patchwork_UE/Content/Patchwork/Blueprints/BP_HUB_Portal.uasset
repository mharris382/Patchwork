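; BP_HUB_Portal is a portal actor that sends the player back to the HUB level.
; It inherits from a parent Blueprint, calling the parent logic and opening its doorway on BeginPlay.
; When the first player's pawn overlaps it, it waits through a short delay and then opens the HUB level by name.
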(event EventBeginPlay
  (|CallParentFunction)
  (CallFunction|OpenDoorway))

(event Collision|EventActorBeginOverlap
  (params (OtherActor :type Actor%20Object%20Reference))
  (|CallParentFunction 0)
  (if (== OtherActor (Game|Player|GetPlayerPawn 0))
    (Utilities|FlowControl|Delay 1.0)
    (Game|OpenLevel(byName) "HUB")))

(event EventTick
  (params (DeltaSeconds :type Float%20%28single-precision%29))
  (|CallParentFunction DeltaSeconds) ; This node is disabled and will not be called.\nDrag off pins to build functionality.
)

(fn ConstructionScript
  (|CallParentFunction))