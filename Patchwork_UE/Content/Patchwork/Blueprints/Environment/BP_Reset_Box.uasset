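; BP_Reset_Box is an environment trigger that moves the player back to a reset point when overlapped.
; On actor overlap, it checks that ResetPoint is valid and the other actor is player 0's pawn, then sets that pawn's location to the ResetPoint actor's location without sweeping.
; At BeginPlay it prints a warning if no reset point is assigned.
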(event EventBeginPlay
  (Utilities|IsValid (Variables|Default|GetReset%20Point)
    (:Is%20Not%20Valid
      (Development|PrintText "Warning Reset Box Missing Reset Point"))))

(event Collision|EventActorBeginOverlap
  (params (OtherActor :type Actor%20Object%20Reference))
  (bind _returnvalue (Game|Player|GetPlayerPawn 0))
  (bind _reset_point (Variables|Default|GetReset%20Point))
  (Utilities|IsValid _reset_point
    (:Is%20Valid
      (if (== OtherActor _returnvalue)
        (Transformation|SetActorLocation _returnvalue (Transformation|GetActorLocation _reset_point) false false)))))

(event EventTick
  (params (DeltaSeconds :type Float%20%28single-precision%29)))

(fn ConstructionScript)