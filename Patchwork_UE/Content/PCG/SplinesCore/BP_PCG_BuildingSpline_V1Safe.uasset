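; Spline-driven building actor that defines a footprint for PCG generation, with its closed-loop state set in the construction script.
; ResetOriginToBuilding shifts spline points so the first sits at the local XY origin, flattens Z, then calls UpdateBounds and triggers PCGMain generation.
; UpdateBounds fits the bounding box to the footprint, with height from CellSize.Z times ZCount.
; A separate cell-grid snapping function exists but is disconnected from the reset flow.
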(event Custom|SnapPointsToGrid)

(event EventBeginPlay
  (|CallParentFunction) ; This node is disabled and will not be called.\nDrag off pins to build functionality.
)

(event Collision|EventActorBeginOverlap
  (params (OtherActor :type Actor%20Object%20Reference))
  (|CallParentFunction OtherActor) ; This node is disabled and will not be called.\nDrag off pins to build functionality.
)

(event EventTick
  (params (DeltaSeconds :type Float%20%28single-precision%29))
  (|CallParentFunction DeltaSeconds) ; This node is disabled and will not be called.\nDrag off pins to build functionality.
)

(fn ConstructionScript
  (bind _returnvalue (Actor|GetComponentbyClass "/Script/Engine.SplineComponent"))
  (|CallParentFunction)
  (Utilities|FlowControl|Sequence
    (:then_0
      (Utilities|IsValid _returnvalue
        (:Is%20Valid
          (Spline|SetClosedLoop _returnvalue (Variables|00-Core|GetIsClosedLoop) false))))))

(fn ResetOrigintoBuilding
  (bind _spline (Variables|Default|GetSpline))
  (bind _returnvalue (Spline|GetSplinePointAt _spline 0 "Local"))
  (bind _position (Utilities|Struct|BreakSplinePoint _returnvalue))
  (bind _returnvalue_2 (* _position -1.0))
  (Utilities|FlowControl|Sequence
    (:then_0
      (Transformation|SetRelativeLocation _spline "0, 0, 0" false false)
      (LocalVariables|SetLS%20Offset (Math|Vector|MakeVector (.x _returnvalue_2) (.y _returnvalue_2) 0.0))
      (LocalVariables|SetLS%20Z 0.0)
      (for _index (range 0 (- (Spline|GetNumberOfSplinePoints (Variables|Default|GetSpline)) 1))
        (Spline|SetLocationatSplinePoint (Variables|Default|GetSpline) _index (Math|Vector|MakeVector (.x (+ (Spline|GetLocationatSplinePoint (Variables|Default|GetSpline) _index "Local") (LocalVariables|GetLS%20Offset))) (.y (+ (Spline|GetLocationatSplinePoint (Variables|Default|GetSpline) _index "Local") (LocalVariables|GetLS%20Offset))) (LocalVariables|GetLS%20Z)) "Local" false))
      (Spline|UpdateSpline (Variables|Default|GetSpline))
      (00-Core|UpdateBounds))
    (:then_1
      (PCG|Generate (Variables|Default|GetPCG_Main) false))))

(fn SnapPointstoGrid
  (bind _returnvalue (Transformation|GetActorTransform))
  (bind _spline (Variables|Default|GetSpline))
  (bind _cell_size (Variables|00-Core|GetCell%20Size))
  (bind _location (Math|Transform|BreakTransform _returnvalue))
  (bind (_x _y _z) (Math|Vector|BreakVector _location))
  (for _index (range 0 (- (Spline|GetNumberOfSplinePoints _spline) 1))
    (Spline|SetLocationatSplinePoint (Variables|Default|GetSpline) _index (Math|Vector|MakeVector (Utilities|SnaptoGrid (.X (Math|Vector|BreakVector (.Position (Utilities|Struct|BreakSplinePoint (Spline|GetSplinePointAt _spline _index "Local"))))) _x (.x _cell_size)) (Utilities|SnaptoGrid (.Y (Math|Vector|BreakVector (.Position (Utilities|Struct|BreakSplinePoint (Spline|GetSplinePointAt _spline _index "Local"))))) _y (.y _cell_size)) (Utilities|SnaptoGrid (.Z (Math|Vector|BreakVector (.Position (Utilities|Struct|BreakSplinePoint (Spline|GetSplinePointAt _spline _index "Local"))))) _z (.z _cell_size))) "Local" false))
  (Spline|UpdateSpline (Variables|Default|GetSpline)))

(fn UpdateBounds
  (bind _spline (Variables|Default|GetSpline))
  (bind _boundingbox (Variables|Default|GetBoundingBox))
  (bind _returnvalue (Spline|GetNumberOfSplinePoints _spline))
  (bind _returnvalue_2 (Spline|GetLocationatSplinePoint _spline 0 "Local"))
  (LocalVariables|Setvertical%20offset (Math|Vector|MakeVector 0.0 0.0 (* (.z (Variables|00-Core|GetCell%20Size)) (Variables|01-Walls|GetZ%20Count))))
  (LocalVariables|Setmin _returnvalue_2)
  (LocalVariables|Setmax (+ _returnvalue_2 (LocalVariables|Getvertical%20offset)))
  (if (> _returnvalue 2)
    (for _index (range 1 (- _returnvalue 1))
      (LocalVariables|Setmin (Math|Vector|MakeVector (Math|Float|SelectFloat (.X (Math|Vector|BreakVector (Spline|GetLocationatSplinePoint (Variables|Default|GetSpline) _index "Local"))) (.x (LocalVariables|Getmin)) (< (.X (Math|Vector|BreakVector (Spline|GetLocationatSplinePoint (Variables|Default|GetSpline) _index "Local"))) (.x (LocalVariables|Getmin)))) (Math|Float|SelectFloat (.Y (Math|Vector|BreakVector (Spline|GetLocationatSplinePoint (Variables|Default|GetSpline) _index "Local"))) (.y (LocalVariables|Getmin)) (< (.Y (Math|Vector|BreakVector (Spline|GetLocationatSplinePoint (Variables|Default|GetSpline) _index "Local"))) (.y (LocalVariables|Getmin)))) (.z (LocalVariables|Getmin))))
      (LocalVariables|Setmax (Math|Vector|MakeVector (Math|Float|SelectFloat (.x (+ (Spline|GetLocationatSplinePoint (Variables|Default|GetSpline) _index "Local") (LocalVariables|Getvertical%20offset))) (.x (LocalVariables|Getmax)) (> (.x (+ (Spline|GetLocationatSplinePoint (Variables|Default|GetSpline) _index "Local") (LocalVariables|Getvertical%20offset))) (.x (LocalVariables|Getmax)))) (Math|Float|SelectFloat (.y (+ (Spline|GetLocationatSplinePoint (Variables|Default|GetSpline) _index "Local") (LocalVariables|Getvertical%20offset))) (.y (LocalVariables|Getmax)) (> (.y (+ (Spline|GetLocationatSplinePoint (Variables|Default|GetSpline) _index "Local") (LocalVariables|Getvertical%20offset))) (.y (LocalVariables|Getmax)))) (.z (LocalVariables|Getmax)))))
    (Components|Box|SetBoxExtent _boundingbox (/ (- (LocalVariables|Getmax) (LocalVariables|Getmin)) 2.0) true)
    (Transformation|SetRelativeLocation _boundingbox (Math|Vector|Lerp(Vector) (LocalVariables|Getmax) (LocalVariables|Getmin) 0.5) false false)))