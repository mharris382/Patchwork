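; A poolable box trigger that tracks whether one assigned actor is inside its area.
; Overlap events and an initial check on assignment update the inside state, record enter and exit times, and fire entered or exited notifications.
; The inside query also requires the actor, or an optional reference location, to be within a squared minimum distance of the box.
; Returning to the pool disables collision and moves it far below the world.
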(event EventBeginPlay
  (bind _mindistance (Variables|Default|GetMinDistance))
  (Variables|Default|SetMinDistanceSqr (* _mindistance _mindistance)))

(event Collision|EventActorBeginOverlap
  (params (OtherActor :type Actor%20Object%20Reference))
  (if (== OtherActor (Variables|Default|GetTrackedActor))
    (CallFunction|SetTrackedActorInside true)))

(event EventTick
  (params (DeltaSeconds :type Float%20%28single-precision%29)))

(event Collision|EventActorEndOverlap
  (params (OtherActor :type Actor%20Object%20Reference))
  (if (== OtherActor (Variables|Default|GetTrackedActor))
    (CallFunction|SetTrackedActorInside false)))

(event EventRetrievedfromPool
  (params (World%20Location :type Transform))
  (bind (_location _rotation _scale) (Math|Transform|BreakTransform World%20Location))
  (Collision|SetActorEnableCollision true)
  (Transformation|SetActorLocationAndRotation _location _rotation)
  (Transformation|SetActorScale3D _scale))

(event EventReturnedtoPool
  (Collision|SetActorEnableCollision false)
  (Transformation|SetActorLocation "0.000000,0.000000,-10000000.000000" false false))

(fn ConstructionScript
  (bind _box (Variables|Default|GetBox))
  (Components|Box|SetBoxExtent _box (/ (Variables|Default|GetSize) 2.0) true)
  (Transformation|SetRelativeLocation _box (Variables|Default|GetOffset) false false))

(fn SetTrackedActorInside
  (params (IsInsideArea :type Boolean))
  (if (Utilities|HasActorBeenInside)
    (if (not (!= IsInsideArea (Variables|Default|GetIsActorInsideArea)))
      (bind _output_get (Variables|Default|SetIsActorInsideArea IsInsideArea :!label _label))
      (if _output_get
        (Variables|Default|SetLastEnterTime (Utilities|Time|GetGameTimeinSeconds))
        (Default|CallOnTrackedActorEntered (Variables|Default|GetTrackedActor))
        (else
          (Variables|Default|SetLastExitTime (Utilities|Time|GetGameTimeinSeconds))
          (Default|CallOnTrackedActorExited (Variables|Default|GetTrackedActor)))))
    (else
      (goto _label))))

(fn AssignTrackedActor
  (params (Actor%20to%20Track :type Actor%20Object%20Reference))
  (Utilities|IsValid Actor%20to%20Track
    (:Is%20Valid
      (Variables|Default|SetTrackedActor Actor%20to%20Track)
      (Variables|Default|SetLastEnterTime -1e+02)
      (Variables|Default|SetLastExitTime -1e+02)
      (CallFunction|SetTrackedActorInside (Utilities|Array|ContainsItem (Collision|GetOverlappingActors (Variables|Default|GetBox) "/Script/Engine.Actor" :!class /Script/Engine.PrimitiveComponent) (Variables|Default|GetTrackedActor))))))

(fn IsTrackedActorInside
  (Variables|Default|GetTrackedActor
    (:then
      (if (Variables|Default|GetIsActorInsideArea)
        (return (<= (Class|KismetMathLibrary|VectorDistanceSquared (Math|Vector|SelectVector (Variables|Default|GetRefLocation) (Transformation|GetActorLocation (Variables|Default|GetTrackedActor)) (Variables|Default|GetuseRefLocaiton)) (Transformation|GetWorldLocation (Variables|Default|GetBox))) (Variables|Default|GetMinDistanceSqr)))
        (else
          _)))
    (:else
      _))
  (return false))