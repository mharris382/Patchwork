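; BP_GlitchPortal is a level actor marking a glitch portal linked to a destination GlitchActor.
; GetGlitchLocation returns that actor's transform as the destination.
; On BeginPlay it prints a warning if the destination is missing; with DrawPortal on, a looping timer draws a red debug arrow from the portal to the target.
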(event Custom|Debug%20Portal
  (CallFunction|Debug))

(event EventBeginPlay
  (Utilities|IsValid (Variables|Default|GetGlitch%20Actor)
    (:Is%20Valid
      (if (Variables|Default|GetDraw%20Portal)
        (bind _returnvalue (Utilities|Time|SetTimerbyEvent (delegate Custom|Debug%20Portal) 1.0 true))
        (Variables|Default|Setdebug%20timer _returnvalue)))
    (:Is%20Not%20Valid
      (Development|PrintText "Glitch portal missing destination"))))

(event Collision|EventActorBeginOverlap
  (params (OtherActor :type Actor%20Object%20Reference)))

(event EventTick
  (params (DeltaSeconds :type Float%20%28single-precision%29)))

(fn ConstructionScript)

(fn GetGlitchLocation
  (return (Transformation|GetActorTransform (Variables|Default|GetGlitch%20Actor))))

(fn Debug
  (Rendering|Debug|DrawDebugArrow (Transformation|GetActorLocation) (Transformation|GetActorLocation (Variables|Default|GetGlitch%20Actor)) 0.0 "(R=1.000000,G=0.000000,B=0.113821,A=1.000000)" 1.0 0.0))