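; Wormhole actor that drives a see-through portal effect between two ends, A and B, using two scene captures.
; Each Tick copies the player camera's FOV to both captures and mirrors its transform, relative to each wormhole, as that capture's relative transform.
; Viewport size changes trigger a resize of both render targets to half resolution, though a note says this is disconnected because new textures never update.
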(event Custom|UpdateRenderTargets
  (bind _returnvalue (Viewport|GetViewportSize))
  (bind _returnvalue_2 (* (.y _returnvalue) 0.5))
  (bind _returnvalue_3 (* (.x _returnvalue) 0.5))
  (bind _returnvalue_4 (Math|Float|Truncate _returnvalue_3))
  (bind _returnvalue_5 (Math|Float|Truncate _returnvalue_2))
  ;[1 1 1] Build and assign new render targets
  (Rendering|ResizeRenderTarget2D (Variables|Default|GetRenderTargetA) _returnvalue_4 _returnvalue_5)
  (Rendering|ResizeRenderTarget2D (Variables|Default|GetRenderTargetB) _returnvalue_4 _returnvalue_5))

(event EventBeginPlay)

(event EventTick
  (params (DeltaSeconds :type Float%20%28single-precision%29))
  (bind _returnvalue (Viewport|GetViewportSize))
  (bind _scenecapturea (Variables|Default|GetSceneCaptureA))
  (bind _scenecaptureb (Variables|Default|GetSceneCaptureB))
  (bind _wormholea (Variables|Default|GetWormholeA))
  (bind _wormholeb (Variables|Default|GetWormholeB))
  (bind _returnvalue_2 (Transformation|GetWorldTransform _wormholeb))
  (bind _returnvalue_3 (Transformation|GetWorldTransform _wormholea))
  (Utilities|FlowControl|Sequence
    (:then_0
      ;[1 1 1] Check for changes in viewport size, rebuild render targets if changed
      (if (Utilities|Operators|NotEqual(!=) _returnvalue (Variables|Default|GetviewportSize) 0.01)
        (CallFunction|UpdateRenderTargets))
      (Variables|Default|SetviewportSize _returnvalue))
    (:then_1
      (bind _asbp_base_character (Utilities|Casting|CastToBP_BaseCharacter (Game|Player|GetPlayerPawn 0)))
      (bind _output_get (Variables|/Script/Engine.SceneCaptureComponent2D|SetFOVAngle _scenecapturea (Variables|/Script/Engine.CameraComponent|GetFieldOfView (Variables|/Game/Patchwork/Blueprints/Pawns/BP_BaseCharacter.BP_BaseCharacter_C|GetCamera _asbp_base_character))))
      (Variables|/Script/Engine.SceneCaptureComponent2D|SetFOVAngle _scenecaptureb _output_get)
      (Transformation|SetRelativeLocation _scenecapturea (Math|Transform|InverseTransformLocation _returnvalue_3 (.location (Transformation|GetWorldTransform (Variables|/Game/Patchwork/Blueprints/Pawns/BP_BaseCharacter.BP_BaseCharacter_C|GetCamera _asbp_base_character)))) false false)
      (Transformation|SetRelativeRotation _scenecapturea (Math|Transform|InverseTransformRotation _returnvalue_3 (.rotation (Transformation|GetWorldTransform (Variables|/Game/Patchwork/Blueprints/Pawns/BP_BaseCharacter.BP_BaseCharacter_C|GetCamera _asbp_base_character)))) false false)
      (Transformation|SetRelativeLocation _scenecaptureb (Math|Transform|InverseTransformLocation _returnvalue_2 (.location (Transformation|GetWorldTransform (Variables|/Game/Patchwork/Blueprints/Pawns/BP_BaseCharacter.BP_BaseCharacter_C|GetCamera _asbp_base_character)))) false false)
      (Transformation|SetRelativeRotation _scenecaptureb (Math|Transform|InverseTransformRotation _returnvalue_2 (.rotation (Transformation|GetWorldTransform (Variables|/Game/Patchwork/Blueprints/Pawns/BP_BaseCharacter.BP_BaseCharacter_C|GetCamera _asbp_base_character)))) false false))))

(fn ConstructionScript)