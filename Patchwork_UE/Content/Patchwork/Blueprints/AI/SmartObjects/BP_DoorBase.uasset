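; Base door smart object that players or other callers can toggle, open, close, lock and unlock, with interaction prompts.
; Timelines blend the Pivot between closed and open transforms or jiggle it when locked, while a NotAnimating macro blocks overlapping requests.
; Gameplay tags select impact sounds played at the pivot.
; Opened and closed dispatchers report success and feed a combined state-change-completed event.
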(event Custom|ToggleDoorState
  ;[0.6233 0.6233 0.6233 0.5 35] Play Door Animation
  (Utilities|NotAnimating
    (:then
      (Variables|Default|SetIsOpen (not (Variables|Default|GetIsOpen)))
      (Utilities|FlowControl|Sequence
        (:then_0
          (Variables|Default|SetIsAnimating true)
          (if (Variables|Default|GetIsOpen)
            (bind _t (Timeline|OpenDoor Reverse)
              (:Update
                (CallFunction|SetDoorAnimationPosition _t))
              (:Finished
                (Variables|Default|SetIsAnimating false)
                (Utilities|FlowControl|Sequence
                  (:then_0
                    ;;[0.6233 0.6233 0.6233 0.5] Check if locked state will change
                    (if (Variables|Default|GetWillLockChange)
                      (Variables|Default|SetWillLockChange false)
                      (bind _output_get (Variables|Default|SetLocked (not (Variables|Default|GetIsOpen))))
                      ;;;[0.6233 0.6233 0.6233 0.5] Play Lock SFX after animation
                      (if _output_get
                        (Utilities|PlayImpact (Variables|SFX|Locked|GetDoorLocked)))))
                  (:then_1
                    ;;[0.6233 0.6233 0.6233 0.5] Send Succes Events
                    (if (Variables|Default|GetIsOpen)
                      (Default|CallOnDoorOpened true)
                      (else
                        (Default|CallOnDoorClosed true)))))))
            (elif (Variables|Default|GetLocked)
              ;;[0.6233 0.6233 0.6233 0.5] Play open door failed
              (bind _t_2 (Timeline|JiggleLocked PlayFromStart)
                (:Update
                  (CallFunction|SetDoorAnimationPosition (Math|Float|Clamp(Float) _t_2))
                  (Default|CallOnDoorOpened false))
                (:Finished
                  (Variables|Default|SetIsAnimating false)))
              (else
                (Timeline|OpenDoor Play)))))
        (:then_1
          ;;[0.6233 0.6233 0.6233 0.5] Play Door SFX
          (Utilities|PlayImpact (select (Variables|Default|GetIsOpen) (select (Variables|Default|GetLocked) (Variables|SFX|Locked|GetDoorOpenFailedBecauseLocked) (Variables|SFX|GetDoorOpenStartedFeedback)) (Variables|SFX|GetDoorCloseStartedFeedback))))))))

(event Custom|CloseAndLock
  ;[0.6233 0.6233 0.6233 0.5] Close And Lock
  (if (Variables|Default|GetIsOpen)
    (Variables|Default|SetWillLockChange true)
    (Utilities|NotAnimating
      (:then
        (CallFunction|ToggleDoorState))
      (:animating
        (Default|CallOnDoorClosed false)))
    (else
      (CallFunction|SetDoorLockState true true)
      (Default|CallOnDoorClosed true))))

(event Custom|OpenAndUnlock
  ;[0.6233 0.6233 0.6233 0.5] Open And Unlock
  (if (not (Variables|Default|GetIsOpen))
    (Variables|Default|SetWillLockChange true)
    (Utilities|NotAnimating
      (:then
        (Variables|Default|SetIsAnimating true)
        ;;[0.6233 0.6233 0.6233 0.5] Play Unlock SFX before animation
        (Utilities|PlayImpact (Variables|SFX|Locked|GetDoorUnLocked))
        (Utilities|FlowControl|Delay (Variables|Default|GetDoorUnlockExtraDelay))
        (CallFunction|ToggleDoorState))
      (:animating
        (Default|CallOnDoorOpened false)))
    (else
      (CallFunction|SetDoorLockState false true)
      (Default|CallOnDoorOpened true))))

(event Custom|DoOpenDoor
  ;[0.6233 0.6233 0.6233 0.5] Open Door
  (if (not (Variables|Default|GetIsOpen))
    (Utilities|NotAnimating
      (:then
        (CallFunction|ToggleDoorState))
      (:animating
        (Default|CallOnDoorOpened false)))
    (else
      (Default|CallOnDoorOpened true))))

(event Custom|CloseDoor
  ;[0.6233 0.6233 0.6233 0.5] Close Door
  (if (Variables|Default|GetIsOpen)
    (Utilities|NotAnimating
      (:then
        (CallFunction|ToggleDoorState))
      (:animating
        (Default|CallOnDoorClosed false)))
    (else
      (Default|CallOnDoorClosed true))))

(event Custom|onclose
  (params (Successful :type Boolean))
  ;[0.6233 0.6233 0.6233 0.5] Bind to both events to call combined event (for convience)
  (Default|CallOnDoorStateChangeCompleted (Variables|Default|GetIsOpen) Successful))

(event Custom|onopen
  (params (Successful :type Boolean))
  ;[0.6233 0.6233 0.6233 0.5] Bind to both events to call combined event (for convience)
  (Default|CallOnDoorStateChangeCompleted (Variables|Default|GetIsOpen) Successful))

(event EventBeginPlay
  ;[0.6233 0.6233 0.6233 0.5] On Begin
  (Utilities|FlowControl|Sequence
    (:then_0
      ;[0.6233 0.6233 0.6233 0.5 35] Play Door Animation
      (bind _t (Timeline|OpenDoor SetNewTime)
        (:Update
          (CallFunction|SetDoorAnimationPosition _t))
        (:Finished
          (Variables|Default|SetIsAnimating false)
          (Utilities|FlowControl|Sequence
            (:then_0
              ;;[0.6233 0.6233 0.6233 0.5] Check if locked state will change
              (if (Variables|Default|GetWillLockChange)
                (Variables|Default|SetWillLockChange false)
                (bind _output_get (Variables|Default|SetLocked (not (Variables|Default|GetIsOpen))))
                ;;;[0.6233 0.6233 0.6233 0.5] Play Lock SFX after animation
                (if _output_get
                  (Utilities|PlayImpact (Variables|SFX|Locked|GetDoorLocked)))))
            (:then_1
              ;;[0.6233 0.6233 0.6233 0.5] Send Succes Events
              (if (Variables|Default|GetIsOpen)
                (Default|CallOnDoorOpened true)
                (else
                  (Default|CallOnDoorClosed true))))))))
    (:then_1
      ;[0.6233 0.6233 0.6233 0.5] Bind to both events to call combined event (for convience)
      (EventDispatchers|BindEventtoOnDoorClosed (delegate Custom|onclose))
      (EventDispatchers|BindEventtoOnDoorOpened (delegate Custom|onopen)))))

(event Collision|EventActorBeginOverlap
  (params (OtherActor :type Actor%20Object%20Reference)))

(event EventTick
  (params (DeltaSeconds :type Float%20%28single-precision%29)))

(event EventOnInteract
  (CallFunction|ToggleDoorState))

(fn ConstructionScript
  (Transformation|SetRelativeTransform (Variables|Default|GetPivot) (Math|Transform|SelectTransform (Variables|Default|GetTransformOpen) (Variables|Default|GetTransformClosed) (Variables|Default|GetIsOpen)) false false))

(fn SetDoorAnimationPosition
  (params (Alpha :type Float%20%28single-precision%29))
  (Transformation|SetRelativeTransform (Variables|Default|GetPivot) (Math|Transform|Lerp(Transform) (Variables|Default|GetTransformClosed) (Variables|Default|GetTransformOpen) Alpha) false false))

(fn SetDoorLockState
  (params (Locked :type Boolean) (WithSFX :type Boolean))
  (if (!= Locked (Variables|Default|GetLocked))
    (bind _output_get (Variables|Default|SetLocked Locked))
    (if WithSFX
      (Utilities|PlayImpact (select _output_get (Variables|SFX|Locked|GetDoorLocked) (Variables|SFX|Locked|GetDoorUnLocked))))))

(fn GetInteractionMessage
  (return (Utilities|String|SelectText "Close Door" "Open Door" (Variables|Default|GetIsOpen))))

(fn GetInteractVerb
  (return (Utilities|String|SelectText "Open" "Close" (Variables|Default|GetIsOpen))))

(fn IsInteractAvailable
  (return (not (Variables|Default|GetIsAnimating))))