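; BP_TorchMount is a torch holder for the paper desert level that can be placed with or without a torch.
; The construction script reads HasTorch and shows or hides its built-in BPPaperTorch component through two helper functions.
; Despite their names, these functions only toggle visibility, as their older spawn, socket-attach and destroy logic is left disconnected.
; The event graph is empty.
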(event EventBeginPlay)

(event Collision|EventActorBeginOverlap
  (params (OtherActor :type Actor%20Object%20Reference)))

(event EventTick
  (params (DeltaSeconds :type Float%20%28single-precision%29)))

(fn ConstructionScript
  (if (Variables|Default|GetHas%20Torch)
    (CallFunction|CreateandAttachTorch)
    (else
      (CallFunction|RemoveandDestroyTorch))))

(fn CreateandAttachTorch
  (Rendering|SetVisibility (Variables|Default|GetBP_PaperTorch) true false))

(fn RemoveandDestroyTorch
  (Rendering|SetVisibility (Variables|Default|GetBP_PaperTorch) false false))