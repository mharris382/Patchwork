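; Spore projectile ability component that fires a projectile on input release to plant an inversion spore where it lands.
; Firing requires parent readiness and enough mana, deactivates the current spore, and spawns from the component or character throw point depending on camera mode.
; A successful hit replaces the spore, aligns it to the surface, sets its type tag and spends mana; invalid hits only play feedback.
; Projectile pooling helpers exist but the live firing path bypasses them.
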(event Custom|InvalidHit
  (params (Hit :type Hit%20Result%20Structure))
  (CallFunction|PlayImpactfromHit "(TagName=\"Feedbacks.Abilities.GravPad.InvalidHit\")" Hit))

(event Custom|SpawnSpore
  (params (Hit :type Hit%20Result%20Structure) (Spore :type Gameplay%20Tag%20Structure))
  (CallFunction|ActivateSpore Hit Spore)
  (Default|RemoveMana (Variables|Default|GetManaPool) (Math|Conversions|ToFloat(Integer) (Variables|/Game/Patchwork/Blueprints/Utilities/BP_GlobalAbilitySettings.BP_GlobalAbilitySettings_C|GetManaCost (Variables|Default|GetGlobalAbilitySettings))))
  (CallFunction|PlayImpactfromHit "(TagName=\"Feedbacks.Abilities.GravPad.Hit\")" Hit))

(event Input|EnhancedActionEvents|EnhancedInputActionIA_Ability_SporeProjectile
  (params (ActionValue :type Boolean) (ElapsedSeconds :type Float%20%28double-precision%29) (TriggeredSeconds :type Float%20%28double-precision%29) (InputAction :type Input%20Action%20Object%20Reference :default "/Game/Patchwork/Data/Input/IA_Ability_SporeProjectile.IA_Ability_SporeProjectile"))
  (bind _spawntransform (CallFunction|GetProjectileSpawnTransform))
  (:Completed
    (if (CallFunction|IsReady)
      (Utilities|FlowControl|Sequence
        (:then_0
          (CallFunction|DeactivateSpore))
        (:then_1
          (bind _returnvalue (Game|SpawnActorfromClass "/Game/Patchwork/Blueprints/Core/Pawns/Abilities/BP_SporeProjectile.BP_SporeProjectile_C" _spawntransform "Undefined" "MultiplyWithRoot" 0 0))
          (Utilities|FlowControl|Sequence
            (:then_0
              (EventDispatchers|BindEventtoOnSuccessfulHit _returnvalue (delegate Custom|SpawnSpore))
              (EventDispatchers|BindEventtoOnInvalidHit _returnvalue (delegate Custom|InvalidHit)))
            (:then_1
              (bind _success (CallFunction|PlayImpactatTransform "(TagName=\"Feedbacks.Abilities.GravPad.Launched\")" _spawntransform))
              (if (not _success)
                (Development|PrintText "Failed")))))))))

(event EventBeginPlay
  (|CallParentFunction)
  (Variables|Default|SetManaPool (Actor|GetComponentbyClass (Game|Player|GetPlayerPawn 0) "/Game/Patchwork/Blueprints/Core/Pawns/Abilities/System/BPC_ManaPool.BPC_ManaPool_C")))

(event EventTick
  (params (DeltaSeconds :type Float%20%28single-precision%29))
  (|CallParentFunction DeltaSeconds) ; This node is disabled and will not be called.\nDrag off pins to build functionality.
)

(fn DeactivateSpore
  (if (Variables|Spore|GetIsSporeActive)
    (Default|SetActive (Variables|Spore|GetSpore) false)
    (Variables|Spore|SetIsSporeActive false)
    (return)))

(fn ActivateSpore01
  (params (Location :type Vector) (Normal :type Vector))
  (Game|SpawnActorfromClass (Utilities|GetClass (Variables|Spore|GetSpore)) (Math|Transform|MakeTransform Location (Math|Conversions|RotationFromXVector Normal)) "Undefined" "MultiplyWithRoot" 0 0)
  (if (not (Variables|Spore|GetIsSporeActive))
    (Default|SetActive (Variables|Spore|GetSpore) true)
    (Variables|Spore|SetIsSporeActive true)
    (Development|PrintString "Spore activated")))

(fn ActivateProjectile
  (if (not (Variables|Projectile|GetIsProjectileActive))
    (Utilities|IsValid (Variables|Projectile|GetCurrentProjectile)
      (:Is%20Valid
        (Default|SetActive (Variables|Projectile|GetCurrentProjectile) true)
        (Variables|Projectile|SetIsProjectileActive true)))))

(fn DeactivateProjectile
  (if (Variables|Projectile|GetIsProjectileActive)
    (Default|SetActive (Variables|Projectile|GetCurrentProjectile) false)
    (Variables|Projectile|SetIsProjectileActive false)))

(fn SendProjectiletoPool
  (params (Projectile :type BP%20Spore%20Projectile%20Object%20Reference))
  (Utilities|IsValid Projectile
    (:Is%20Valid
      (Default|SetActive Projectile false)
      (if (< (Utilities|Array|Length (Variables|Projectile|GetProjectilePool)) (Variables|Projectile|GetProjectilePoolSize))
        (Utilities|Array|Add (Variables|Projectile|GetProjectilePool) Projectile)
        (return true)
        (else
          (return false))))
    (:Is%20Not%20Valid
      (return false))))

(fn RemoveProjectilefromPool
  (bind _currentprojectile (Variables|Projectile|GetCurrentProjectile))
  (if (Utilities|Array|IsEmpty (Variables|Projectile|GetProjectilePool))
    (Utilities|IsValid _currentprojectile
      (:Is%20Valid
        (return _currentprojectile))
      (:Is%20Not%20Valid
        (bind _returnvalue (Game|SpawnActorfromClass "/Game/Patchwork/Blueprints/Core/Pawns/Abilities/BP_SporeProjectile.BP_SporeProjectile_C" (Transformation|GetActorTransform (Game|GetPlayerController 0)) "DontSpawnIfColliding" "MultiplyWithRoot" 0 0))
        (Utilities|Array|Add (Variables|Projectile|GetProjectilePool) _returnvalue)
        (return _returnvalue)))
    (else
      (return (Utilities|Array|Get(acopy) (Variables|Projectile|GetProjectilePool))))))

(fn GetProjectileSpawnTransform
  (bind _returnvalue (Components|GetOwner))
  (bind _asbp_base_character (Utilities|Casting|CastToBP_BaseCharacter _returnvalue))
  (return (select (Default|IsCameraFP _asbp_base_character) (Transformation|GetWorldTransform) (Transformation|GetWorldTransform (Variables|/Game/Patchwork/Blueprints/Core/Pawns/BP_BaseCharacter.BP_BaseCharacter_C|GetThrow%20Point _asbp_base_character)))))

(fn ActivateSpore
  (params (Hit :type Hit%20Result%20Structure) (GameplayTag :type Gameplay%20Tag%20Structure))
  (bind (_bblockinghit _binitialoverlap _time _distance _location _impactpoint _normal) (Collision|BreakHitResult Hit))
  (Utilities|IsValid (Variables|Spore|GetSpore)
    (:Is%20Valid
      (Actor|DestroyActor (Variables|Spore|GetSpore)))
    (:Is%20Not%20Valid
      _))
  (bind _returnvalue (Game|SpawnActorfromClass "/Game/Patchwork/Blueprints/Levels/forest/Spores/BP_InversionAbilitySpore.BP_InversionAbilitySpore_C" (Math|Transform|MakeTransform _location (Math|Rotator|MakeRotfromZ _normal)) "AlwaysSpawn" "MultiplyWithRoot" 0 0))
  (bind _output_get (Variables|Spore|SetSpore _returnvalue))
  (Default|SetSporeType _output_get GameplayTag))

(fn IsReady
  (return (and (|CallParentFunction) (>= (Default|GetMana (Variables|Default|GetManaPool)) (Variables|/Game/Patchwork/Blueprints/Utilities/BP_GlobalAbilitySettings.BP_GlobalAbilitySettings_C|GetManaCost (Variables|Default|GetGlobalAbilitySettings))))))