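; Gravity zone actor that changes the player character's gravity while it overlaps the zone.
; On begin overlap, it sets player 0's CharacterMovement gravity scale to the zone's GravityScale variable.
; On end overlap, it resets the scale to the default of one rather than restoring the previous value.
; Both events check Enabled, so disabling the zone while the player is inside skips the reset on exit.
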(event Collision|EventActorBeginOverlap
  (params (OtherActor :type Actor%20Object%20Reference))
  (bind _returnvalue (Game|GetPlayerCharacter 0))
  (if (Variables|Default|Getenabled)
    (if (== OtherActor _returnvalue)
      (Variables|/Script/Engine.CharacterMovementComponent|SetGravityScale (Variables|/Script/Engine.Character|GetCharacterMovement _returnvalue) (Variables|Default|GetgravityScale)))))

(event Collision|EventActorEndOverlap
  (params (OtherActor :type Actor%20Object%20Reference))
  (bind _returnvalue (Game|GetPlayerCharacter 0))
  (if (Variables|Default|Getenabled)
    (if (== OtherActor _returnvalue)
      (Variables|/Script/Engine.CharacterMovementComponent|SetGravityScale (Variables|/Script/Engine.Character|GetCharacterMovement _returnvalue) 1.0))))

(fn ConstructionScript)