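; BP_LightBase is a base light Blueprint that applies shared light settings in its construction script, with no active runtime logic.
; It sets intensity, color and indirect lighting on the light from GetLight, an empty stub here, if valid.
; It also sets color, shadow casting and volumetric scattering on secondary spot and point lights.
; AddSecondarySpotLight toggles visibility of both secondary lights, including the point light.
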(event EventBeginPlay)

(event Collision|EventActorBeginOverlap
  (params (OtherActor :type Actor%20Object%20Reference)))

(event EventTick
  (params (DeltaSeconds :type Float%20%28single-precision%29)))

(fn ConstructionScript
  (bind _secondarypointlight (Variables|Default|GetSecondaryPointLight))
  (bind _secondaryspotlight (Variables|Default|GetSecondarySpotLight))
  (Utilities|FlowControl|Sequence
    (:then_0
      (bind _light (CallFunction|GetLight))
      (bind _output_get (LocalVariables|Setlight _light))
      (Utilities|IsValid _output_get
        (:Is%20Valid
          (Rendering|Components|Light|SetIntensity (LocalVariables|Getlight) (Variables|Light|GetIntensity))
          (Rendering|Components|Light|SetLightColor (LocalVariables|Getlight) (Variables|Light|GetLight%20Color) true)
          (Class|LightComponent|SetIndirectLightingIntensity (LocalVariables|Getlight) (Variables|Light|GetIndirect%20Lighting)))))
    (:then_1
      (Rendering|SetVisibility _secondaryspotlight (Variables|SpotLight|GetAdd%20Secondary%20Spot%20Light) false)
      (LocalVariables|Setlight _secondaryspotlight)
      (Rendering|Components|Light|SetLightColor (LocalVariables|Getlight) (Variables|Light|GetLight%20Color) true)
      (Rendering|Components|Light|SetCastShadows (LocalVariables|Getlight) (Variables|SpotLight|GetSecondary%20Spot%20Light%20Cast%20Shadows))
      (Class|LightComponent|SetVolumetricScatteringIntensity (LocalVariables|Getlight) (Variables|SpotLight|GetSecondary%20Spot%20Volumentric%20Intensity)))
    (:then_2
      (Rendering|SetVisibility _secondarypointlight (Variables|SpotLight|GetAdd%20Secondary%20Spot%20Light) false)
      (LocalVariables|Setlight _secondarypointlight)
      (Rendering|Components|Light|SetLightColor (LocalVariables|Getlight) (Variables|Light|GetLight%20Color) true)
      (Rendering|Components|Light|SetCastShadows (LocalVariables|Getlight) (Variables|PointLight|GetSecondary%20Point%20Light%20Cast%20Shadows))
      (Class|LightComponent|SetVolumetricScatteringIntensity (LocalVariables|Getlight) (Variables|PointLight|GetSecondary%20Point%20Volumentric%20Intensity)))))

(fn GetLight
  (return 0))

(fn GetLights
  (return 0))