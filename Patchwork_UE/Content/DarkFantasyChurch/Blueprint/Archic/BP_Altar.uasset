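; BP_Altar is an altar prop from the DarkFantasyChurch content with fire and lighting that can be switched on or off.
; The construction script passes the Enabled variable to SetEnabled, which stores it and sets the visibility of three point lights and two fire components to match.
; The event graph holds only disabled stub events, so the Blueprint runs no gameplay logic of its own.
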(event EventBeginPlay)

(event Collision|EventActorBeginOverlap
  (params (OtherActor :type Actor%20Object%20Reference)))

(event EventTick
  (params (DeltaSeconds :type Float%20%28single-precision%29)))

(fn ConstructionScript
  (CallFunction|SetEnabled (Variables|Default|GetEnabled)))

(fn SetEnabled
  (params (Enabled :type Boolean))
  (bind _output_get (Variables|Default|SetEnabled Enabled))
  (Rendering|SetVisibility (Variables|Default|GetPointLight4) _output_get false)
  (Rendering|SetVisibility (Variables|Default|GetFire) _output_get false))