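; BP_Lever_Switch is an interactable lever that acts as a two-position on/off switch for other actors.
; On BeginPlay it syncs the initial state from CurrentPosition, then binds to OnPositionChanged, mapping position 1 to on and 0 to off.
; SetSwitch pushes that state to every entry in Listeners through the BPI_OnOffSwitch_Listener interface, printing a message for any entry that does not implement it.
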(event Custom|Position%20Changed
  (params (position :type Integer))
  (switch int position
    (:0
      (CallFunction|SetSwitch false))
    (:1
      (CallFunction|SetSwitch true))))

(event EventBeginPlay
  (|CallParentFunction)
  (CallFunction|SetSwitch (== (Variables|Default|Getcurrent%20position) 1))
  (EventDispatchers|BindEventtoOnPositionChanged (delegate Custom|Position%20Changed)))

(event Collision|EventActorBeginOverlap
  (params (OtherActor :type Actor%20Object%20Reference))
  (|CallParentFunction OtherActor) ; This node is disabled and will not be called.\nDrag off pins to build functionality.
)

(event EventTick
  (params (DeltaSeconds :type Float%20%28single-precision%29))
  (|CallParentFunction DeltaSeconds) ; This node is disabled and will not be called.\nDrag off pins to build functionality.
)

(fn ConstructionScript
  (|CallParentFunction))

(fn SetSwitch
  (params (is%20on :type Boolean))
  (for _array_element (Variables|Default|GetListeners)
    (bind _asbpi_on_off_switch_listener (Utilities|Casting|CastToBPI_OnOffSwitch_Listener _array_element)
      (:then
        (Default|SetSwitchValue _asbpi_on_off_switch_listener is%20on))
      (:CastFailed
        (Development|PrintText (Utilities|Text|FormatText "{0} is not a BPI switch" (Utilities|GetDisplayName _array_element)))))))