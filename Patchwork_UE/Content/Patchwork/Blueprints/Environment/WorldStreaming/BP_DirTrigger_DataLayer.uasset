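; Directional world-streaming trigger that switches Data Layer runtime states as the player crosses between sides A and B.
; When the player pawn leaves TriggerB it applies the A-to-B layer lists, and leaving TriggerA applies the B-to-A lists.
; Each direction has unloaded, loaded and activated lists, applied through SetDataLayerStates via the Data Layer Manager, non-recursively, followed by a debug print.
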(event EventBeginPlay)

(event Collision|EventActorBeginOverlap
  (params (OtherActor :type Actor%20Object%20Reference)))

(event EventTick
  (params (DeltaSeconds :type Float%20%28single-precision%29)))

(event OnComponentEndOverlap(TriggerB)
  (params (OverlappedComponent :type Primitive%20Component%20Object%20Reference) (OtherActor :type Actor%20Object%20Reference) (OtherComp :type Primitive%20Component%20Object%20Reference) (OtherBodyIndex :type Integer))
  (if (== OtherActor (Game|Player|GetPlayerPawn 0))
    (bind _returnvalue (WorldPartition|GetDataLayerManager))
    (Utilities|IsValid _returnvalue
      (:Is%20Valid
        (CallFunction|SetDataLayerStates _returnvalue (Variables|AtoB|GetAB%20Unloaded) "Unloaded" false)
        (CallFunction|SetDataLayerStates _returnvalue (Variables|AtoB|GetAB%20Loaded) "Loaded" false)
        (CallFunction|SetDataLayerStates _returnvalue (Variables|AtoB|GetAB%20Activated) "Activated" false)
        (Development|PrintString "A to B completed")))))

(event OnComponentEndOverlap(TriggerA)
  (params (OverlappedComponent :type Primitive%20Component%20Object%20Reference) (OtherActor :type Actor%20Object%20Reference) (OtherComp :type Primitive%20Component%20Object%20Reference) (OtherBodyIndex :type Integer))
  (if (== OtherActor (Game|Player|GetPlayerPawn 0))
    (bind _returnvalue (WorldPartition|GetDataLayerManager))
    (Utilities|IsValid _returnvalue
      (:Is%20Valid
        (CallFunction|SetDataLayerStates _returnvalue (Variables|BtoA|GetBA%20Unloaded) "Unloaded" false)
        (CallFunction|SetDataLayerStates _returnvalue (Variables|BtoA|GetBA%20Loaded) "Loaded" false)
        (CallFunction|SetDataLayerStates _returnvalue (Variables|BtoA|GetBA%20Activated) "Activated" false)
        (Development|PrintString "B to A completed")))))

(fn ConstructionScript)

(fn SetDataLayerStates
  (params (DL%20manager :type Data%20Layer%20Manager%20Object%20Reference) (Layers :type Array%20of%20Data%20Layer%20Asset%20Object%20References) (Target%20State :type EDataLayerRuntimeState%20Enum :default "Unloaded") (bInIsRecursive :type Boolean))
  (LocalVariables|Setstate Target%20State)
  (for _array_element Layers
    (Utilities|IsValid _array_element
      (:Is%20Valid
        (DataLayers|SetDataLayerRuntimeState DL%20manager _array_element (LocalVariables|Getstate) false :!class /Script/Engine.DataLayerManager)))))