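; Memory Shard quest logic that tracks how many shards are collected in the forest game mode.
; On BeginPlay it casts to GM_ForestGameMode, copies the current count and binds to count changes, printing a warning if the cast fails.
; The IsQuestCompleted override has an unconnected body, so its parent call and check for more than ten shards never run.
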(event Custom|On%20Shard%20Collected
  (params (count :type Integer))
  (Variables|Default|SetShards%20Collected count))

(event EventBeginPlay
  (|CallParentFunction)
  (bind _asgm_forest_game_mode (Utilities|Casting|CastToGM_ForestGameMode (Game|GetGameMode))
    (:then
      (bind _output_get (Variables|Default|SetForest%20Game%20Mode _asgm_forest_game_mode))
      (EventDispatchers|BindEventtoCollectedCountChanged _output_get (delegate Custom|On%20Shard%20Collected))
      (bind _count (Default|GetCollectedCount (Variables|Default|GetForest%20Game%20Mode)))
      (Variables|Default|SetShards%20Collected _count))
    (:CastFailed
      (Development|PrintText "Memory Shard Quest is not used with forest game mode"))))

(fn IsQuestCompleted)