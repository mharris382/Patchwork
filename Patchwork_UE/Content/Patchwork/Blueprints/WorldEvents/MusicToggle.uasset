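; World event Blueprint that toggles music between daytime and nighttime through a switch value.
; It plays its MetaSound on BeginPlay, and SetSwitchValue stores the night state, then sends the matching trigger parameter to it.
; The same trigger goes to an AmbientSound tagged AudioController, found and cached by a macro.
; An older two-component volume crossfade using timelines remains unconnected.
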(event EventBeginPlay
  (Audio|Components|Audio|Play (Variables|Default|Getmetasound%20audio) 0.0))

(event Collision|EventActorBeginOverlap
  (params (OtherActor :type Actor%20Object%20Reference)))

(event EventTick
  (params (DeltaSeconds :type Float%20%28single-precision%29)))

(event EventSetSwitchValue
  (params (is%20On :type Boolean))
  (bind _output_get (Variables|Default|SetIs%20Nighttime is%20On))
  (if _output_get
    (Utilities|FlowControl|Sequence
      (:then_0
        (Class|AudioParameterControllerInterface|SetTriggerParameter(Message) (Variables|Default|Getmetasound%20audio) "Nightime_Music"))
      (:then_1
        (bind _audio_controller (Utilities|GetAudioController)
          (:OutputPin
            (Class|AudioParameterControllerInterface|SetTriggerParameter(Message) _audio_controller "Nightime_Music")))))
    (else
      (Utilities|FlowControl|Sequence
        (:then_0
          (Class|AudioParameterControllerInterface|SetTriggerParameter(Message) (Variables|Default|Getmetasound%20audio) "Daytime_music"))
        (:then_1
          (bind _audio_controller_2 (Utilities|GetAudioController)
            (:OutputPin
              (Class|AudioParameterControllerInterface|SetTriggerParameter(Message) _audio_controller_2 "Daytime_music"))
            (:missing%20controller
              (Development|PrintText "Hello"))))))))

(fn ConstructionScript)