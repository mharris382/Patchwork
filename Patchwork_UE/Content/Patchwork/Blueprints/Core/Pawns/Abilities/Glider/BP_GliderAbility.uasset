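; Player ability component that spawns a BP_Glider for the player to ride, toggled with the Ability 3 input.
; Starting it spawns the glider at its own transform, changes the owner's move state and adds the Gliding gameplay tag.
; A glider impact or second press completes the ability, destroying the glider and restoring the player's state.
; Jump exits riding with an impulse along the glider's up vector, without despawning it.
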(event Input|EnhancedActionEvents|EnhancedInputActionIA_Ability_3
  (params (ActionValue :type Boolean) (ElapsedSeconds :type Float%20%28double-precision%29) (TriggeredSeconds :type Float%20%28double-precision%29) (InputAction :type Input%20Action%20Object%20Reference :default "/Game/Patchwork/Data/Input/IA_Ability_3.IA_Ability_3"))
  (:Started
    (if (CallFunction|IsAbilityinUse)
      (CallFunction|CompleteAbility true)
      (else
        (bind _started (CallFunction|StartAbility))
        (if _started
          _)))))

(event Input|EnhancedActionEvents|EnhancedInputActionIA_Jump
  (params (ActionValue :type Boolean) (ElapsedSeconds :type Float%20%28double-precision%29) (TriggeredSeconds :type Float%20%28double-precision%29) (InputAction :type Input%20Action%20Object%20Reference :default "/Game/Patchwork/Data/Input/IA_Jump.IA_Jump"))
  (CallFunction|JumpfromGlider))

(event EventBeginPlay
  (|CallParentFunction)
  (Variables|Default|SetGameplayState (Actor|GetComponentbyClass (Components|GetOwner) "/Game/Patchwork/Blueprints/Utilities/GameplayObjectState.GameplayObjectState_C")))

(event EventTick
  (params (DeltaSeconds :type Float%20%28single-precision%29))
  (|CallParentFunction DeltaSeconds) ; This node is disabled and will not be called.\nDrag off pins to build functionality.
)

(fn Spawn
  (Utilities|FlowControl|Sequence
    (:then_0
      (Variables|Default|GetCurrentGlider
        (:then
          (Glider|Despawn))
        (:else)))
    (:then_1
      (bind _returnvalue (Game|SpawnActorfromClass "/Game/Patchwork/Blueprints/Core/Pawns/Abilities/Glider/BP_Glider.BP_Glider_C" (Transformation|GetWorldTransform) "Undefined" "MultiplyWithRoot" 0 0))
      (bind _output_get (Variables|Default|SetCurrentGlider _returnvalue))
      (EventDispatchers|BindEventtoOnImpact _output_get (EventDispatchers|CreateEvent :!event OnGliderHit)))))

(fn Despawn
  (bind _currentglider (Variables|Default|GetCurrentGlider)
    (:then
      (Actor|DestroyActor _currentglider))
    (:else)))

(fn OnGliderHit
  (params (Hit :type Hit%20Result%20Structure))
  (CallFunction|CompleteAbility true))

(fn CompleteAbility
  (params (Success :type Boolean))
  (|CallParentFunction Success)
  (Glider|Despawn)
  (CallFunction|SetPlayerRidingGlider false))

(fn StartAbility
  (bind (_started _start_vfx) (|CallParentFunction))
  (Utilities|FlowControl|Sequence
    (:then_0
      (if _started
        (Glider|Spawn)
        (CallFunction|SetPlayerRidingGlider true)))
    (:then_1
      (return _started _start_vfx))))

(fn SetPlayerRidingGlider
  (params (Riding%20Glider :type Boolean))
  (bind _output_get (Variables|Default|SetIsRidingGlider Riding%20Glider))
  (if _output_get
    (Class|BPIPlayerPawn|SetPlayerMoveState(Message) (Components|GetOwner) "NewEnumerator7")
    (Default|AddGameplayTag (Variables|Default|GetGameplayState) "(TagName=\"Gameplay.State.Gliding\")")
    (else
      (Default|RemoveGameplayTag (Variables|Default|GetGameplayState) "(TagName=\"Gameplay.State.Gliding\")")
      (Class|BPIPlayerPawn|SetPlayerMoveState(Message) (Components|GetOwner) "NewEnumerator0"))))

(fn JumpfromGlider
  (if (Variables|Default|GetIsRidingGlider)
    (CallFunction|SetPlayerRidingGlider false)
    (Class|BPIPlayerPawn|AddImpulse(Message) (Components|GetOwner) (* (Transformation|GetActorUpVector (Variables|Default|GetCurrentGlider)) (Variables|/Game/Patchwork/Blueprints/Utilities/BP_GlobalAbilitySettings.BP_GlobalAbilitySettings_C|GetJumpFromGliderImpulse (Variables|Default|GetGlobalSettings))) false)))