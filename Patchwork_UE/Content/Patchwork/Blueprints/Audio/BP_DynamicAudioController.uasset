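; BP_DynamicAudioController plays a MetaSound source for dynamic music and switches its tracks at runtime.
; On BeginPlay it assigns the MetaSound to its DynamicAudio component and starts playback.
; Two near-identical functions, ChangeMusicTrack and ChangeMusTrack, clamp a track index to four slots and fire the matching MetaSound trigger parameter, each from its own name array.
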(event EventBeginPlay
  (bind _dynamic_audio (Variables|Default|GetDynamic%20Audio))
  (Audio|Components|Audio|SetSound _dynamic_audio (Variables|Default|GetMetasound%20Source))
  (Audio|Components|Audio|Play _dynamic_audio 0.0))

(fn ConstructionScript)

(fn ChangeMusicTrack
  (params (music%20track :type Integer))
  (Class|AudioParameterControllerInterface|SetTriggerParameter(Message) (Variables|Default|GetDynamic%20Audio) (Utilities|Array|Get(acopy) (Variables|Default|Getmusic%20track%20trigger%20names) (Math|Integer|Clamp(Integer) music%20track 0 3))))

(fn ChangeMusTrack
  (params (music%20track :type Integer))
  (Class|AudioParameterControllerInterface|SetTriggerParameter(Message) (Variables|Default|GetDynamic%20Audio) (Utilities|Array|Get(acopy) (Variables|Default|GetMusic%20track%20trigger%20names2) (Math|Integer|Clamp(Integer) music%20track 0 3))))