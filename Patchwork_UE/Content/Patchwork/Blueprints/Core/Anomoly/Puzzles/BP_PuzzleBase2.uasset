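; Base puzzle actor that renders a picture of collected fragments into a render target.
; Construction pairs child meshes with FragmentData rows by index, applies each row's texture, sizes meshes to their images, and configures a show-only scene capture over them and an optional base image.
; BeginPlay rebuilds the name-to-mesh map and hides the meshes.
; Update events make collected pieces visible in scene capture only, then recapture.
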(event Custom|Update%20Fragments
  (params (collected%20fragments :type Array%20of%20Names))
  (bind _keys (Utilities|Map|Keys (Variables|Default|Getmeshes)))
  (for _array_element _keys
    (if (Utilities|Array|ContainsItem collected%20fragments _array_element)
      (if (.ReturnValue (Utilities|Map|Find (Variables|Default|Getmeshes) _array_element))
        (Class|PrimitiveComponent|SetVisibleinSceneCaptureOnly (.Value (Utilities|Map|Find (Variables|Default|Getmeshes) _array_element)) true)
        (Rendering|SetVisibility (.Value (Utilities|Map|Find (Variables|Default|Getmeshes) _array_element)) true false)
        (else
          (Development|PrintText (Utilities|Text|FormatText "couldn't find piece for {0} may not be enought meshes" (stale _array_element)))))))
  (Rendering|SceneCapture|CaptureScene (Variables|Default|GetSceneCaptureComponent2D) :!class /Script/Engine.SceneCaptureComponent2D))

(event Custom|Update%20Fragment
  (params (fragment :type Name))
  (bind _meshes (Variables|Default|Getmeshes))
  (bind (_value _returnvalue) (Utilities|Map|Find _meshes fragment))
  (if _returnvalue
    (Class|PrimitiveComponent|SetVisibleinSceneCaptureOnly _value true)
    (Rendering|SceneCapture|CaptureScene (Variables|Default|GetSceneCaptureComponent2D) :!class /Script/Engine.SceneCaptureComponent2D)
    (else
      (Development|PrintText (Utilities|Text|FormatText "couldn't find piece for {0} may not be enought meshes" 0)))))

(event EventBeginPlay
  (CallFunction|SetupMeshMap))

(fn ConstructionScript
  (bind _fragment_data (Variables|Default|GetFragment%20Data))
  (bind _scenecapturecomponent2d (Variables|Default|GetSceneCaptureComponent2D))
  (bind _scenecapturecomponent2d_2 (Variables|Default|GetSceneCaptureComponent2D))
  (bind _base (Variables|Default|GetBase))
  (bind _base_image (Variables|Default|GetBase%20Image))
  (bind _show_base_image (Variables|Default|Getshow%20base%20image))
  (bind _texture_target (Variables|Default|GetTexture%20Target))
  (bind _relativelocation (Variables|/Script/Engine.SceneComponent|GetRelativeLocation _base))
  (Utilities|FlowControl|Sequence
    (:then_0
      (Rendering|SceneCapture|ClearShowOnlyComponents (Variables|Default|GetSceneCaptureComponent2D)))
    (:then_1
      (Utilities|IsValid _fragment_data
        (:Is%20Valid
          (bind _outrownames (DataTable|GetDataTableRowNames _fragment_data))
          (LocalVariables|Setdatat%20table%20rows _outrownames)
          (for (_array_element _array_index) (Components|GetChildrenComponents (Variables|Default|GetFragments) false)
            (if (< _array_index (Utilities|Array|Length (LocalVariables|Getdatat%20table%20rows)))
              (bind _returnvalue (Utilities|GetDataTableRow (Variables|Default|GetFragment%20Data) (Utilities|Array|Get(acopy) (LocalVariables|Getdatat%20table%20rows) _array_index))
                (:then
                  (bind _asstatic_mesh_component (Utilities|Casting|CastToStaticMeshComponent _array_element))
                  (Utilities|Map|Add (Variables|Default|Getmeshes) (Utilities|Array|Get(acopy) (LocalVariables|Getdatat%20table%20rows) _array_index) _asstatic_mesh_component)
                  (bind _returnvalue_2 (Rendering|Material|CreateDynamicMaterialInstance _asstatic_mesh_component 0 "/Game/Patchwork/Blueprints/Core/Anomoly/Materials/M_FragmentUnllit_Inst.M_FragmentUnllit_Inst" "None" :!class /Script/Engine.PrimitiveComponent))
                  (Rendering|Material|SetTextureParameterValue _returnvalue_2 "Fragment Texture" (.fragmentimage (Utilities|Struct|BreakS_Fragment _returnvalue)))
                  (Transformation|SetRelativeScale3D _asstatic_mesh_component (Math|Vector|MakeVector (Math|Conversions|ToFloat(Integer) (Class|Texture2D|BlueprintGetSizeX (.fragmentimage (Utilities|Struct|BreakS_Fragment _returnvalue)))) (Math|Conversions|ToFloat(Integer) (Class|Texture2D|BlueprintGetSizeY (.fragmentimage (Utilities|Struct|BreakS_Fragment _returnvalue)))) 1.0))
                  (Rendering|SceneCapture|ShowOnlyComponent (Variables|Default|GetSceneCaptureComponent2D) _asstatic_mesh_component))))))))
    (:then_2
      (Utilities|IsValid (Variables|Default|GetBase%20Image)
        (:Is%20Valid
          (bind _returnvalue_3 (Rendering|Material|CreateDynamicMaterialInstance _base 0 "/Game/Patchwork/Blueprints/Core/Anomoly/Materials/M_FragmentUnllit_Inst.M_FragmentUnllit_Inst" "None" :!class /Script/Engine.PrimitiveComponent))
          (Rendering|Material|SetTextureParameterValue _returnvalue_3 "Fragment Texture" _base_image)
          (Transformation|SetRelativeScale3D _base (Math|Vector|MakeVector (Math|Conversions|ToFloat(Integer) (Class|Texture2D|BlueprintGetSizeX _base_image)) (Math|Conversions|ToFloat(Integer) (Class|Texture2D|BlueprintGetSizeY _base_image)) 0.0))
          (Rendering|SetVisibility _base _show_base_image true)
          (if _show_base_image
            (Rendering|SceneCapture|ShowOnlyComponent (Variables|Default|GetSceneCaptureComponent2D) _base)))))
    (:then_3
      (Utilities|IsValid _texture_target
        (:Is%20Valid
          (bind _astexture_render_target_2d (Utilities|Casting|CastToTextureRenderTarget2D _texture_target))
          (Variables|/Script/Engine.SceneCaptureComponent2D|SetTextureTarget _scenecapturecomponent2d _astexture_render_target_2d)
          (Variables|/Script/Engine.SceneCaptureComponent2D|SetOrthoWidth _scenecapturecomponent2d (* (.x (.BoxExtent (Collision|GetActorBounds false false))) 2.0))
          (Transformation|SetRelativeRotation _scenecapturecomponent2d_2 (Math|Rotator|MakeRotator -9e+01 -9e+01 0.0) false false)
          (Rendering|SceneCapture|CaptureScene _scenecapturecomponent2d_2 :!class /Script/Engine.SceneCaptureComponent2D)
          (Transformation|SetRelativeLocation _scenecapturecomponent2d_2 (Math|Vector|MakeVector (.x _relativelocation) (.y _relativelocation) 3.93e+04) false false))))))

(fn SetupMeshMap
  (bind _fragment_data (Variables|Default|GetFragment%20Data))
  (Utilities|FlowControl|Sequence
    (:then_0
      (Utilities|Map|Clear (Variables|Default|Getmeshes))
      (Utilities|IsValid _fragment_data
        (:Is%20Valid
          (bind _outrownames (DataTable|GetDataTableRowNames _fragment_data))
          (LocalVariables|SetFragment%20Names _outrownames)
          (for (_array_element _array_index) (Components|GetChildrenComponents (Variables|Default|GetFragments) false)
            (bind _asstatic_mesh_component (Utilities|Casting|CastToStaticMeshComponent _array_element))
            (Utilities|Map|Add (Variables|Default|Getmeshes) (Utilities|Array|Get(acopy) (LocalVariables|GetFragment%20Names) _array_index) _asstatic_mesh_component)
            (Rendering|SetVisibility _asstatic_mesh_component false false)))))
    (:then_1
      (Rendering|SetVisibility (Variables|Default|GetBase) false false))))

(fn GetNumberOfFragments
  (return (Class|SceneComponent|GetNumChildrenComponents (Variables|Default|GetFragments))))