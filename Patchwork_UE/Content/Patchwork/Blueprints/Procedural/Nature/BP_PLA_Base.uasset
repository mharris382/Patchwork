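; Base Blueprint for procedural nature actors that picks one PLA variant from the PLAs array.
; The construction script either uses SpecificPLAIndex, clamped to the array and written back, or picks a random entry.
; It stores the choice in GENPLA before calling the parent construction script, so inherited logic runs with the selection already set.
; The event graph holds no active logic.
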(event EventBeginPlay
  (|CallParentFunction) ; This node is disabled and will not be called.\nDrag off pins to build functionality.
)

(event Collision|EventActorBeginOverlap
  (params (OtherActor :type Actor%20Object%20Reference))
  (|CallParentFunction OtherActor) ; This node is disabled and will not be called.\nDrag off pins to build functionality.
)

(event EventTick
  (params (DeltaSeconds :type Float%20%28single-precision%29))
  (|CallParentFunction DeltaSeconds) ; This node is disabled and will not be called.\nDrag off pins to build functionality.
)

(fn ConstructionScript
  (bind _plas (Variables|Default|GetPLAs))
  (bind _returnvalue (Utilities|Array|Length _plas))
  (bind _returnvalue_2 (- _returnvalue 1))
  (Utilities|FlowControl|Sequence
    (:then_0
      (if (Variables|Default|GetUseSpecificPLA)
        (Variables|PCGINTERNAL|SetGEN_PLA (Utilities|Array|Get(acopy) (Variables|Default|GetPLAs) (Math|Integer|Clamp(Integer) (Variables|Default|GetSpecificPLAIndex) 0 _returnvalue_2)))
        (Variables|Default|SetSpecificPLAIndex (Math|Integer|Clamp(Integer) (Variables|Default|GetSpecificPLAIndex) 0 _returnvalue_2))
        (else
          (Variables|PCGINTERNAL|SetGEN_PLA (Utilities|Array|Get(acopy) _plas (Math|Random|RandomIntegerinRange 0 _returnvalue_2))))))
    (:then_1
      (|CallParentFunction))))