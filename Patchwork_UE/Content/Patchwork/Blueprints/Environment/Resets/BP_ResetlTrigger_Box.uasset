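; Box-shaped reset trigger for level environments, leaving overlap behavior to its parent class and returning its Box through GetComponentShape.
; The construction script sizes the box from BoxExtents and can raise it by its half-height so the origin sits at the bottom.
; An optional plane is scaled to the box footprint and placed relative to its lower face with a Z offset, or destroyed when disabled.
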(event EventBeginPlay
  (|CallParentFunction))

(event Collision|EventActorBeginOverlap
  (params (OtherActor :type Actor%20Object%20Reference))
  (|CallParentFunction OtherActor))

(event EventTick
  (params (DeltaSeconds :type Float%20%28single-precision%29))
  (|CallParentFunction DeltaSeconds) ; This node is disabled and will not be called.\nDrag off pins to build functionality.
)

(fn ConstructionScript
  (bind _plane (Variables|Default|GetPlane))
  (bind _box (Variables|Default|GetBox))
  (bind _box_extents (Variables|Default|GetBox%20Extents))
  (|CallParentFunction)
  (Utilities|FlowControl|Sequence
    (:then_0
      (Components|Box|SetBoxExtent _box _box_extents true)
      (if (Variables|Default|GetAt%20Bottom)
        (Transformation|SetRelativeLocation _box (Math|Vector|MakeVector 0.0 0.0 (.Z (Math|Vector|BreakVector _box_extents))) false false)))
    (:then_1
      (if (Variables|Plane|GetAdd%20Plane)
        (Transformation|SetRelativeLocation _plane (Math|Vector|MakeVector 0.0 0.0 (+ (* (.z (Variables|Default|GetBox%20Extents)) -1.0) (Variables|Plane|GetPlane%20Z%20Offset))) false false)
        (Transformation|SetRelativeScale3D _plane (/ (* (Variables|Default|GetBox%20Extents) 2.0) 1e+02))
        (else
          (Components|DestroyComponent (Variables|Default|GetPlane)))))))

(fn GetComponentShape
  (return (Variables|Default|GetBox)))