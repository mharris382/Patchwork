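; BP_Streetlight is a streetlight whose secondary point light is switched on or off through SetLightPowered.
; On BeginPlay it finds the BP_PowerController in the level and adds itself to it as a light.
; If no controller is found, it prints a warning and retries every Tick, disabling Tick once registered.
; The construction script applies the AttenuationRadius variable to that point light.
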(event EventBeginPlay
  (|CallParentFunction)
  (Utilities|TryRegisterLightwithController))

(event Collision|EventActorBeginOverlap
  (params (OtherActor :type Actor%20Object%20Reference))
  (|CallParentFunction OtherActor) ; This node is disabled and will not be called.\nDrag off pins to build functionality.
)

(event EventTick
  (params (DeltaSeconds :type Float%20%28single-precision%29))
  (|CallParentFunction DeltaSeconds)
  (if (not (Variables|Default|Getadded))
    (Utilities|TryRegisterLightwithController)))

(event EventSetLightPowered
  (params (powered :type Boolean) (power :type Float%20%28double-precision%29))
  (Rendering|SetVisibility (Variables|Default|GetSecondaryPointLight) powered false))

(fn ConstructionScript
  (|CallParentFunction)
  (Rendering|Lighting|SetAttenuationRadius (Variables|Default|GetSecondaryPointLight) (Variables|Light|GetAttenuation%20Radius)))

(fn GetLocation
  (return (Transformation|GetActorLocation)))