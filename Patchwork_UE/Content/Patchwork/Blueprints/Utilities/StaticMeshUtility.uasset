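; A utility component that gathers the static mesh components on its owner as targets, with a hook for overriding their materials.
; On BeginPlay it loops over those targets, though the loop body is empty.
; UpdateTarget queries GetOverrideMaterial, which always declines the override here, and takes no action on the result.
; The functions read as a base scaffold, with no material change implemented in this asset.
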(event EventBeginPlay
  (|CallParentFunction)
  (for _array_element (CallFunction|GetTargets)
    _))

(fn GetOverrideMaterial
  (params (target :type Primitive%20Component%20Object%20Reference))
  (return false 0))

(fn GetTargets
  (return (Actor|GetComponentsByClass (Components|GetOwner) "/Script/Engine.StaticMeshComponent")))

(fn UpdateTarget
  (params (target :type Primitive%20Component%20Object%20Reference))
  (bind _output_get (LocalVariables|Set_target target))
  (bind _apply_override (CallFunction|GetOverrideMaterial _output_get))
  (if _apply_override
    _))