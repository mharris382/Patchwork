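; Base Blueprint for a player spore effect that drives post-processing from toxicity.
; On BeginPlay it spawns the post-processing actor class defined by its effect, keeps it as a BP_SporePostProcessing reference and zeroes its blend.
; Toxicity changes pass the new value straight to that actor's UpdateBlend, after calling the parent handler.
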(event EventBeginPlay
  (|CallParentFunction)
  (bind _returnvalue (Game|SpawnActorfromClass (.PostProcessingClass (Utilities|Struct|BreakS_SporeEffectData (CallFunction|GetEffect))) (Math|Transform|MakeTransform "0, 0, 0") "Undefined" "MultiplyWithRoot" 0 0))
  (bind _asbp_spore_post_processing (Utilities|Casting|CastToBP_SporePostProcessing _returnvalue))
  (bind _output_get (Variables|Default|SetSpore%20Post%20Processing _asbp_spore_post_processing))
  (Default|UpdateBlend _output_get 0.0))

(event EventTick
  (params (DeltaSeconds :type Float%20%28single-precision%29))
  (|CallParentFunction DeltaSeconds))

(fn OnToxicityChanged
  (params (new%20toxicity :type Float%20%28double-precision%29))
  (|CallParentFunction new%20toxicity)
  (Default|UpdateBlend (Variables|Default|GetSpore%20Post%20Processing) new%20toxicity))