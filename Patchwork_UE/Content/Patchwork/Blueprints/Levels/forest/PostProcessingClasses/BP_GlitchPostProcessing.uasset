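; Post-processing Blueprint that plays a glitch effect on demand and broadcasts when the glitch hits.
; TriggerGlitchEffect restarts the PlayGlitch timeline, which writes its GlitchIntensity curve into a Material Parameter Collection scalar on every update.
; The timeline's Glitch event track calls the OnGlitch dispatcher so other objects can react in sync.
; UpdateBlend and the construction script only forward to the parent class.
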(event Custom|Trigger%20Glitch%20Effect
  (bind _glitch_intensity (Timeline|Play%20Glitch PlayFromStart)
    (:Update
      (Rendering|Material|SetScalarParameterValue (Variables|Default|GetMaterial%20Collection) (Variables|Default|GetGlitch%20Intensity%20Name) _glitch_intensity :!class /Script/Engine.KismetMaterialLibrary))
    (:Glitch
      (Default|CallOnGlitch))))

(event EventBeginPlay
  (|CallParentFunction) ; This node is disabled and will not be called.\nDrag off pins to build functionality.
)

(event Collision|EventActorBeginOverlap
  (params (OtherActor :type Actor%20Object%20Reference))
  (|CallParentFunction OtherActor) ; This node is disabled and will not be called.\nDrag off pins to build functionality.
)

(event EventTick
  (params (DeltaSeconds :type Float%20%28single-precision%29))
  (|CallParentFunction DeltaSeconds) ; This node is disabled and will not be called.\nDrag off pins to build functionality.
)

(event EventUpdateBlend
  (params (blend :type Float%20%28double-precision%29))
  (|CallParentFunction blend))

(fn ConstructionScript
  (|CallParentFunction))