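; Inversion ability spore: a child spore that creates a gravity well, turning the gravity of overlapping GravityVector actors toward its up axis.
; Construction strips the mushroom meshes; construction and BeginPlay size the box and Niagara effect from GlobalSettings.
; Overlap also launches player 0 toward the closest point on the well's axis, computed from the overlapping actor, with debug drawing.
; If that actor is the player, it bounces them along the axis.
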(event EventBeginPlay
  (|CallParentFunction)
  (CallFunction|SetupGravityWellSize))

(event Collision|EventActorBeginOverlap
  (params (OtherActor :type Actor%20Object%20Reference))
  (bind _returnvalue (Actor|GetComponentbyClass OtherActor "/Game/Patchwork/Blueprints/Core/Pawns/Abilities/System/GravityVector.GravityVector_C"))
  (bind _returnvalue_2 (Transformation|GetActorLocation OtherActor))
  (Utilities|FlowControl|Sequence
    (:then_0
      (|CallParentFunction OtherActor))
    (:then_1
      (Utilities|IsValid _returnvalue
        (:Is%20Valid
          (Default|SetGravityDirection _returnvalue (Transformation|GetActorUpVector))
          (bind (_segment_start _segment_end_) (CallFunction|GetSegmentData))
          (Rendering|Debug|DrawDebugLine _segment_start _segment_end_ "(R=1.000000,G=0.337796,B=0.000000,A=1.000000)" 1e+01 5.0)
          (Rendering|Debug|DrawDebugPoint (Math|Vector|FindClosestPointonSegment _returnvalue_2 _segment_start _segment_end_) 8.0 "(R=1.000000,G=0.051641,B=0.000000,A=1.000000)" 5.0)
          (Character|LaunchCharacter (Game|GetPlayerCharacter 0) (* (Math|Vector|GetUnitDirection(Vector) _returnvalue_2 (Math|Vector|FindClosestPointonSegment _returnvalue_2 _segment_start _segment_end_)) 3e+01) false false)
          (CallFunction|BouncePlayer OtherActor false false))))))

(event EventTick
  (params (DeltaSeconds :type Float%20%28single-precision%29))
  (|CallParentFunction DeltaSeconds) ; This node is disabled and will not be called.\nDrag off pins to build functionality.
)

(fn ConstructionScript
  (bind _main_mush (Variables|Default|GetMain%20Mush))
  (|CallParentFunction)
  (Utilities|FlowControl|Sequence
    (:then_0
      (Components|DestroyComponent (Variables|Default|GetSmall%20Mush))
      (Rendering|SetVisibility _main_mush false false)
      (Collision|SetCollisionEnabled _main_mush "NoCollision"))
    (:then_1
      (CallFunction|SetupGravityWellSize))))

(fn SetupGravityWellSize
  (bind _globalsettings (Variables|Default|GetGlobalSettings))
  (bind _niagara_box (Variables|Default|GetNiagara-Box))
  (bind _gravitywellradius (Variables|/Game/Patchwork/Blueprints/Utilities/BP_GlobalAbilitySettings.BP_GlobalAbilitySettings_C|GetGravityWellRadius _globalsettings))
  (bind _gravitywellheight (Variables|/Game/Patchwork/Blueprints/Utilities/BP_GlobalAbilitySettings.BP_GlobalAbilitySettings_C|GetGravityWellHeight _globalsettings))
  (bind _returnvalue (Math|Vector|MakeVector _gravitywellradius _gravitywellradius _gravitywellheight))
  (Utilities|FlowControl|Sequence
    (:then_0
      (Components|Box|SetBoxExtent (Variables|Default|GetBox) _returnvalue true)
      (Niagara|SetNiagaraVariable(Vector3) _niagara_box "Box Size" _returnvalue)
      (Niagara|SetNiagaraVariable(Float) _niagara_box "WellRadius" _gravitywellradius))
    (:then_1
      (Transformation|SetRelativeLocation (Variables|Default|GetNiagara-Box) (Math|Vector|MakeVector 0.0 0.0 (* _gravitywellheight 0.0)) false false))))

(fn BouncePlayer
  (params (Other%20Actor :type Actor%20Object%20Reference) (XYOverride :type Boolean) (ZOverride :type Boolean))
  (bind _returnvalue (Game|GetPlayerCharacter 0))
  (if (== _returnvalue Other%20Actor)
    (bind _success (Class|BPIPlayerPawn|ApplyBounceForce(Message) _returnvalue (* (Transformation|GetActorUpVector) (Variables|/Game/Patchwork/Blueprints/Utilities/BP_GlobalAbilitySettings.BP_GlobalAbilitySettings_C|GetPlayerImpulseMultiplier (Variables|Default|GetGlobalSettings))) XYOverride ZOverride))
    (return _success)))

(fn GetSegmentData
  (bind _returnvalue (Transformation|GetActorUpVector))
  (bind _returnvalue_2 (Transformation|GetActorLocation))
  (bind _globalsettings (Variables|Default|GetGlobalSettings))
  (bind (_x _y _z) (Math|Vector|BreakVector _returnvalue_2))
  (bind _gravitywellheight (Variables|/Game/Patchwork/Blueprints/Utilities/BP_GlobalAbilitySettings.BP_GlobalAbilitySettings_C|GetGravityWellHeight _globalsettings))
  (bind _returnvalue_3 (* _returnvalue _gravitywellheight))
  (bind (_x_2 _y_2 _z_2) (Math|Vector|BreakVector _returnvalue_3))
  (return _returnvalue_2 (Math|Vector|MakeVector (+ _x _x_2) (+ _y _y_2) (+ _z _z_2))))