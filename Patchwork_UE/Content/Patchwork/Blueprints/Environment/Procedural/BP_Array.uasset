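; BP_Array is a procedural environment actor that repeats a static mesh in a 3D grid sized by XCount, YCount and ZCount.
; The construction script resolves Mesh and Material, falling back to the StaticMesh component's own, and applies them to it as the origin cell.
; Cell spacing is the mesh's local bounds plus Offset.
; SpawnMeshAt adds a separate StaticMeshComponent per remaining cell; its instanced-mesh node never runs.
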(event EventBeginPlay)

(event Collision|EventActorBeginOverlap
  (params (OtherActor :type Actor%20Object%20Reference)))

(event EventTick
  (params (DeltaSeconds :type Float%20%28single-precision%29)))

(fn ConstructionScript
  (bind _material (Variables|Default|GetMaterial))
  (bind _mesh (Variables|Default|GetMesh))
  (bind _staticmesh (Variables|Default|GetStaticMesh))
  (bind _staticmesh_2 (Variables|Default|GetStaticMesh))
  (bind (_min _max) (Components|StaticMesh|GetLocalBounds _staticmesh_2))
  (Utilities|FlowControl|Sequence
    (:then_0
      (LocalVariables|Setmat (.AsMaterial%20Interface (Utilities|Casting|CastToMaterialInterface (Utilities|SelectObject _material (Rendering|Material|GetMaterial (Variables|Default|GetStaticMesh) 0) (Utilities|IsValid _material)))))
      (LocalVariables|Set_mesh (.AsStatic%20Mesh (Utilities|Casting|CastToStaticMesh (Utilities|SelectObject _mesh (Variables|/Script/Engine.StaticMeshComponent|GetStaticMesh (Variables|Default|GetStaticMesh)) (Utilities|IsValid _mesh))))))
    (:then_1
      (Components|StaticMesh|SetStaticMesh _staticmesh (LocalVariables|Get_mesh))
      (Rendering|Material|SetMaterial _staticmesh 0 (LocalVariables|Getmat))
      (LocalVariables|Set_bounds (+ (- _max _min) (Variables|Default|GetOffset))))
    (:then_2
      (for _index (range 0 (- (Variables|Default|GetX%20Count) 1))
        (for _index_2 (range 0 (- (Variables|Default|GetY%20Count) 1))
          (for _index_3 (range 0 (- (Variables|Default|GetZ%20Count) 1))
            (if (not (Math|Boolean|ANDBoolean (== _index 0) (== _index_2 0) (== _index_3 0)))
              (CallFunction|SpawnMeshat (LocalVariables|Get_bounds) _index _index_2 _index_3 (LocalVariables|Get_mesh) (LocalVariables|Getmat)))))))))

(fn SpawnMeshat
  (params (increment :type Vector) (x :type Integer) (y :type Integer) (z :type Integer) (mesh :type Static%20Mesh%20Object%20Reference) (material :type Material%20Interface%20Object%20Reference))
  (bind (_x _y _z) (Math|Vector|BreakVector increment))
  (bind _returnvalue (Game|AddComponentbyClass "/Script/Engine.StaticMeshComponent" false (Math|Transform|MakeTransform (Math|Vector|MakeVector (* _x x) (* _y y) (* _z z)))))
  (Components|StaticMesh|SetStaticMesh _returnvalue mesh)
  (Rendering|Material|SetMaterial (stale _returnvalue) 0 material))