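; Spore projectile actor that reports whether what it hit can take a spore.
; On a collider hit, it checks the hit actor for the NoSpore tag, fires the invalid or successful hit dispatcher with the hit result, then destroys itself.
; SetActive shows or hides the projectile and switches collider collision between the stored active setting and none.
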(event OnComponentHit(Collider)
  (params (HitComponent :type Primitive%20Component%20Object%20Reference) (OtherActor :type Actor%20Object%20Reference) (OtherComp :type Primitive%20Component%20Object%20Reference) (NormalImpulse :type Vector :default "0, 0, 0") (Hit :type Hit%20Result%20Structure%20%28by%20ref%29))
  (bind _returnvalue (Collision|MakeHitResult (.bblockinghit Hit) (.binitialoverlap Hit) (.time Hit) (.distance Hit) (.location Hit) (.impactpoint Hit) (.normal Hit) (.impactnormal Hit) (.physmat Hit) (.hitactor Hit) (.hitcomponent Hit) (.hitbonename Hit) (.bonename Hit) (.hititem Hit) (.elementindex Hit) (.faceindex Hit) (.tracestart Hit) (.traceend Hit)))
  (if (Actor|ActorHasTag (.hitactor Hit) "NoSpore")
    (Default|CallOnInvalidHit _returnvalue)
    (else
      (Default|CallOnSuccessfulHit _returnvalue)))
  (Actor|DestroyActor))

(event EventBeginPlay)

(event Collision|EventActorBeginOverlap
  (params (OtherActor :type Actor%20Object%20Reference)))

(event EventTick
  (params (DeltaSeconds :type Float%20%28single-precision%29)))

(fn ConstructionScript)

(fn SetActive
  (params (NewState :type Boolean))
  (bind _collider (Variables|Default|GetCollider))
  (Rendering|SetActorHiddenInGame (not NewState))
  (if NewState
    (Collision|SetCollisionEnabled _collider (Variables|Default|GetActiveCollision))
    (else
      (Collision|SetCollisionEnabled _collider "NoCollision"))))