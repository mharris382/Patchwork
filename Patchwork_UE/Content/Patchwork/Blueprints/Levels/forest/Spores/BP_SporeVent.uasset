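; BP_SporeVent is a forest level spore vent whose glow material and Niagara effects reflect its spore type and active state.
; It extends parent type and activation logic, refreshing visuals through UpdateSporeVisuals on changes and at construction.
; Construction sizes the box and Niagara volume from BoxSize, while an optional BoxCenter actor positions the box.
; The trace-based auto-fit in ResizeBox is disconnected and never runs.
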(event EventBeginPlay
  (|CallParentFunction) ; This node is disabled and will not be called.\nDrag off pins to build functionality.
)

(event Collision|EventActorBeginOverlap
  (params (OtherActor :type Actor%20Object%20Reference))
  (|CallParentFunction OtherActor) ; This node is disabled and will not be called.\nDrag off pins to build functionality.
)

(event EventTick
  (params (DeltaSeconds :type Float%20%28single-precision%29))
  (|CallParentFunction DeltaSeconds) ; This node is disabled and will not be called.\nDrag off pins to build functionality.
)

(event EventChangeSporeType
  (params (spore%20type :type Data%20Table%20Row%20Handle%20Structure))
  (|CallParentFunction spore%20type)
  (CallFunction|UpdateSporeVisuals))

(event EventSetActive
  (params (active :type Boolean))
  (|CallParentFunction active)
  (CallFunction|SetVisualsActive active)
  (CallFunction|UpdateSporeVisuals))

(fn ConstructionScript
  (bind _box_size (Variables|Default|GetBox%20Size))
  (bind _box_size_2 (Variables|Default|GetBox%20Size))
  (|CallParentFunction)
  (CallFunction|UpdateSporeVisuals)
  (if (Math|Boolean|ANDBoolean (> (.x _box_size) 0.1) (> (.y _box_size) 0.1) (> (.z _box_size) 0.1))
    (Components|Box|SetBoxExtent (Variables|Default|GetBox) _box_size_2 true)
    (Niagara|SetNiagaraVariable(Vector3) (Variables|Default|GetNiagara) "Box Size" _box_size_2)))

(fn ResizeBox)

(fn UpdateSporeVisuals
  (bind _ns_vent (Variables|Default|GetNS_Vent))
  (bind _overridematieral (Variables|Default|GetOverrideMatieral))
  (bind _box_center (Variables|Default|GetBox%20Center))
  (bind _vent (Variables|Default|Getvent))
  (Utilities|FlowControl|Sequence
    (:then_0
      (if (Variables|Default|Getis%20active)
        (bind _mat (CallFunction|GetGlowMaterial (Variables|Default|GetEffect) false))
        (Rendering|Material|SetMaterial _vent 2 _mat)
        (CallFunction|ApplySporeTypetoEffect (.rowname (Variables|Default|GetEffect)) _ns_vent 1.0 false)
        (Rendering|SetVisibility _ns_vent true false)
        (else
          (Rendering|Material|SetMaterial _vent 2 "/Game/Patchwork/Materials/Levels/M_Spore_Inert.M_Spore_Inert")
          (Rendering|SetVisibility _ns_vent false false))))
    (:then_1
      (CallFunction|ResizeBox)
      (Utilities|IsValid _box_center
        (:Is%20Valid
          (Transformation|SetWorldLocationAndRotation (Variables|Default|GetBox) (Transformation|GetActorLocation _box_center) (Transformation|GetActorRotation _box_center) false false))))
    (:then_2
      (Utilities|IsValid _overridematieral
        (:Is%20Valid
          (Rendering|Material|SetMaterial (Variables|Default|Getvent) 1 _overridematieral))))))

(fn SetVisualsActive
  (params (active :type Boolean))
  (Rendering|SetVisibility (Variables|Default|GetNS_Vent) active false)
  (if active
    (CallFunction|UpdateSporeVisuals)
    (else
      (bind _mat (CallFunction|GetGlowMaterial))
      (Rendering|Material|SetMaterial (Variables|Default|Getvent) 2 _mat)
      (Rendering|SetVisibility (Variables|Default|GetNS_Vent) false false))))