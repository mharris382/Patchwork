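; GameData is a save-data Blueprint that tracks recorded world events, lever positions and per-level player transforms.
; World events are checked by membership in a recorded collection, with None always reading as not occurred.
; Lever positions are keyed by SwitchID, stored only when non-zero or already saved, and levers without an ID print a warning.
; Player transforms are keyed by level name, and saving skips the HUB level.
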(fn HasEventOccured
  (params (world%20event :type Name))
  (if (== world%20event "None")
    (return false)
    (else
      (return (Utilities|Array|ContainsItem (Variables|Default|Getrecorded%20world%20events) world%20event)))))

(fn TryLoadLever
  (params (lever :type BP%20Lever%20Object%20Reference))
  (bind _switch_id (Variables|/Game/Patchwork/Blueprints/Interactibles/BP_Lever.BP_Lever_C|Getswitch%20ID lever))
  (Utilities|IsValid lever
    (:Is%20Valid
      (if (== _switch_id "")
        (Development|PrintText 0 (Utilities|Text|FormatText "{0} Lever has no switch ID, it cannot be saved" (Utilities|GetDisplayName lever)))
        (elif (Utilities|Map|Contains (Variables|Default|Getswitch%20save%20data) _switch_id)
          (Default|SetPosition lever (.Value (Utilities|Map|Find (Variables|Default|Getswitch%20save%20data) _switch_id))))))))

(fn TrySaveLever
  (params (lever :type BP%20Lever%20Object%20Reference))
  (bind _switch_id (Variables|/Game/Patchwork/Blueprints/Interactibles/BP_Lever.BP_Lever_C|Getswitch%20ID lever))
  (bind _current_position (Variables|/Game/Patchwork/Blueprints/Interactibles/BP_Lever.BP_Lever_C|Getcurrent%20position lever))
  (Utilities|IsValid lever
    (:Is%20Valid
      (if (== _switch_id "")
        (Development|PrintText 0 (Utilities|Text|FormatText "{0} Lever has no switch ID, it cannot be saved" (Utilities|GetDisplayName lever)))
        (elif (or (!= _current_position 0) (Utilities|Map|Contains (Variables|Default|Getswitch%20save%20data) _switch_id))
          (Utilities|Map|Add (Variables|Default|Getswitch%20save%20data) _switch_id _current_position))))))

(fn TryGetPlayerSaveLocation
  (params (level%20name :type Name))
  (bind _player_transform_per_level (Variables|Default|Getplayer_transform_per_level))
  (bind (_value _returnvalue) (Utilities|Map|Find _player_transform_per_level level%20name))
  (return _value _returnvalue))

(fn SavePlayerLocation
  (params (level%20name :type Name) (transform :type Transform))
  (if (!= level%20name "HUB")
    (Utilities|Map|Add (Variables|Default|Getplayer_transform_per_level) level%20name transform)))