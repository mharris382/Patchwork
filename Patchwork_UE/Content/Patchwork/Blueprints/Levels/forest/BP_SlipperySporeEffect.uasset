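; Spore effect attached to a character in the forest level that makes movement slippery and faster as toxicity rises.
; Each tick above a small toxicity threshold, it blends braking friction toward a configured factor along a square-root curve.
; For paperperson characters it also overrides max walk speed, easing toward up to double the desired speed.
; Below the threshold it resets braking friction and restores desired speed.
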(event EventBeginPlay
  (|CallParentFunction)
  (bind _ascharacter (Utilities|Casting|CastToCharacter (Components|GetOwner)))
  (bind _output_get (Variables|Default|SetCharacter _ascharacter))
  (Variables|Default|SetCharacter%20Movement (Variables|/Script/Engine.Character|GetCharacterMovement _output_get))
  (bind _aspaperperson (Utilities|Casting|CastTopaperperson _ascharacter))
  (Variables|Default|SetAs%20Paperperson _aspaperperson))

(event EventTick
  (params (DeltaSeconds :type Float%20%28single-precision%29))
  (bind _current_toxicity (Variables|Default|GetCurrent%20Toxicity))
  (bind _as_paperperson (Variables|Default|GetAs%20Paperperson))
  (bind _as_paperperson_2 (Variables|Default|GetAs%20Paperperson))
  (bind _character_movement (Variables|Default|GetCharacter%20Movement))
  (|CallParentFunction DeltaSeconds)
  (Utilities|IsValid (Variables|Default|GetCharacter%20Movement)
    (:Is%20Valid
      (if (> _current_toxicity 0.1)
        (Variables|/Script/Engine.CharacterMovementComponent|SetBrakingFrictionFactor _character_movement (Math|Float|Lerp 1.0 (Variables|Default|Getbraking%20friction%20factor) (Math|Float|Power _current_toxicity 0.5)))
        (Utilities|IsValid _as_paperperson_2
          (:Is%20Valid
            (Variables|/Game/Patchwork/Blueprints/Core/Pawns/paperperson.paperperson_C|Setis%20max%20speed%20overridden _as_paperperson_2 true)
            (bind _max_walk_speed (Default|GetDesiredSpeed _as_paperperson_2))
            (Variables|Default|Setnew%20desired%20speed (Math|Float|Lerp _max_walk_speed (* _max_walk_speed 2.0) _current_toxicity))
            (Variables|/Script/Engine.CharacterMovementComponent|SetMaxWalkSpeed _character_movement (Math|Float|Lerp (Variables|/Script/Engine.CharacterMovementComponent|GetMaxWalkSpeed _character_movement) (Variables|Default|Getnew%20desired%20speed) (* DeltaSeconds 3.0)))))
        (else
          (Variables|/Script/Engine.CharacterMovementComponent|SetBrakingFrictionFactor (Variables|Default|GetCharacter%20Movement) 1.0)
          (Utilities|IsValid _as_paperperson
            (:Is%20Valid
              (Variables|/Game/Patchwork/Blueprints/Core/Pawns/paperperson.paperperson_C|Setis%20max%20speed%20overridden _as_paperperson false)
              (bind _max_walk_speed_2 (Default|GetDesiredSpeed _as_paperperson))
              (Variables|/Script/Engine.CharacterMovementComponent|SetMaxWalkSpeed (Variables|Default|GetCharacter%20Movement) _max_walk_speed_2))))))))

(fn OnToxicityChanged
  (params (new%20toxicity :type Float%20%28double-precision%29))
  (|CallParentFunction new%20toxicity))