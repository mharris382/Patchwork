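; BP_CooridorLightConfig holds corridor light settings for procedural temple generation.
; Its Validate function reorders the IllumHeight pair into min/max order.
; When UseSourceEmissive is on and the source material is valid, it creates and caches a dynamic material instance tinted by LightColor and scaled by emissive intensity.
; It returns that generated material, clearing it when source emissive is disabled.
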(fn Validate
  (params (WorldContextObject :type Object%20Object%20Reference))
  (Utilities|FlowControl|Sequence
    (:then_0
      (Variables|Sizing|SetIllumHeight (Math|Vector2D|MakeVector2D (Math|Float|Min(Float) (.x (Variables|Sizing|GetIllumHeight)) (.y (Variables|Sizing|GetIllumHeight))) (Math|Float|Max(Float) (.x (Variables|Sizing|GetIllumHeight)) (.y (Variables|Sizing|GetIllumHeight))))))
    (:then_1
      (if (Variables|Source|GetUseSourceEmissive)
        (bind _sourceemissivematerial (Variables|Source|GetSourceEmissiveMaterial)
          (:then
            (bind _returnvalue (Rendering|Material|CreateDynamicMaterialInstance WorldContextObject _sourceemissivematerial "None" :!class /Script/Engine.KismetMaterialLibrary))
            (bind _output_get (Variables|Source|SetGEN_SourceEmissiveMaterial _returnvalue))
            (Rendering|Material|SetVectorParameterValue _output_get (Variables|Source|GetColorParameterName) (Variables|LightSettings|GetLightColor) :!class /Script/Engine.MaterialInstanceDynamic)
            (Rendering|Material|SetScalarParameterValue _output_get (Variables|Source|GetIntensityParameterName) (Variables|Source|GetSourceEmissiveIntensityScalar) :!class /Script/Engine.MaterialInstanceDynamic))
          (:else))
        (else
          (Variables|Source|SetGEN_SourceEmissiveMaterial 0))))
    (:then_2
      (return (Variables|Source|GetGEN_SourceEmissiveMaterial)))))