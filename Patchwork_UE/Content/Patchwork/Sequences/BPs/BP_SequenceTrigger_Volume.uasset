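; BP_SequenceTrigger_Volume is a trigger volume that resumes a sequence through its SequenceController reference when an actor overlaps it.
; The overlap event calls ResumeSequence on the controller behind an always-true branch, with no filter on the overlapping actor.
; It also exposes ResumeSequence and PauseSequence functions that simply forward to the controller.
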(event EventBeginPlay)

(event Collision|EventActorBeginOverlap
  (params (OtherActor :type Actor%20Object%20Reference))
  (if true
    (Default|ResumeSequence (Variables|Default|GetSequence%20Controller))))

(event EventTick
  (params (DeltaSeconds :type Float%20%28single-precision%29)))

(fn ConstructionScript)

(fn ResumeSequence
  (Default|ResumeSequence (Variables|Default|GetSequence%20Controller))
  (return))

(fn PauseSequence
  (Default|PauseSequence (Variables|Default|GetSequence%20Controller))
  (return))