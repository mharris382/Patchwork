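; BP_Spore_Spawned_Temporary is a spore actor variant that keeps its effect without the mushroom body.
; On BeginPlay it runs the parent logic, then destroys MainMush and all of its child components.
; Its construction script runs the parent's, then passes EffectDuration to the NiagaraBox "Loop Duration" parameter, so the particle loop matches the effect length.
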(event EventBeginPlay
  (bind _main_mush (Variables|Default|GetMain%20Mush))
  (|CallParentFunction)
  (for _array_element (Components|GetChildrenComponents _main_mush true)
    (Components|DestroyComponent _array_element))
  (Components|DestroyComponent _main_mush))

(event Collision|EventActorBeginOverlap
  (params (OtherActor :type Actor%20Object%20Reference))
  (|CallParentFunction OtherActor) ; This node is disabled and will not be called.\nDrag off pins to build functionality.
)

(event EventTick
  (params (DeltaSeconds :type Float%20%28single-precision%29))
  (|CallParentFunction DeltaSeconds) ; This node is disabled and will not be called.\nDrag off pins to build functionality.
)

(fn ConstructionScript
  (|CallParentFunction)
  (Effects|Components|ParticleSystem|SetFloatParameter (Variables|Default|GetNiagara-Box) "Loop Duration" (Variables|Default|GetEffectDuration)))