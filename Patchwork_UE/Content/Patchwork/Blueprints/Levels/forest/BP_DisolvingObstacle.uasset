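; BP_DisolvingObstacle is a forest level obstacle that loses collision while the player is under the tripping spore effect.
; Each tick it reads CurrentToxicity from the player pawn's BP_PlayerTrippingSporeEffect component and disables mesh collision when that value is above a tiny threshold.
; Collision stays on when the component is missing.
; The construction script applies a configurable mesh and material; the Blueprint itself changes only collision, not visuals, at runtime.
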(event EventBeginPlay)

(event Collision|EventActorBeginOverlap
  (params (OtherActor :type Actor%20Object%20Reference)))

(event EventTick
  (params (DeltaSeconds :type Float%20%28single-precision%29))
  (bind _returnvalue (Utilities|GetPlayerTrippingComponent)
    (:Is%20Valid
      (CallFunction|SetCollisionsEnabled (not (> (Variables|/Game/Patchwork/Blueprints/Levels/forest/BP_SporeEffectBase.BP_SporeEffectBase_C|GetCurrent%20Toxicity _returnvalue) 0.01))))
    (:Is%20Not%20Valid
      (CallFunction|SetCollisionsEnabled true))))

(fn ConstructionScript
  (bind _staticmesh (Variables|Default|GetStaticMesh))
  (Components|StaticMesh|SetStaticMesh _staticmesh (Variables|Default|GetMesh))
  (Rendering|Material|SetMaterial _staticmesh 0 (Variables|Default|GetMaterial%20Instance)))

(fn SetCollisionsEnabled
  (params (enable%20collisions :type Boolean))
  (if enable%20collisions
    (Collision|SetCollisionEnabled (Variables|Default|GetStaticMesh) "QueryAndPhysics")
    (else
      (Collision|SetCollisionEnabled (Variables|Default|GetStaticMesh) "NoCollision"))))