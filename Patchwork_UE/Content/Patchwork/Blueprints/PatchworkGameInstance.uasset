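; Game instance for Patchwork that owns persistent settings and game saves, plus global pause and a shared confirm dialog.
; Init loads or creates both save slots, applies master volume through a sound mix and creates the settings menu.
; SaveGame records the level, NPC data, per-level player ground positions and game mode world events; LoadGame reopens the saved level or delegates to the game mode.
; Settings functions sync graphics, display and colorblind options with GameUserSettings.
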(event Custom|PauseGame
  (bind _returnvalue (Game|GetPlayerController 0))
  ;[1 1 1] attempts to pause game
  (if (not (Variables|Default|GetPaused))
    (bind _returnvalue_2 (UserInterface|CreateWidget "/Game/Patchwork/Blueprints/Widgets/PauseMenu.PauseMenu_C" (Game|GetPlayerController 0)))
    (UserInterface|Viewport|AddtoViewport _returnvalue_2 0)
    (Input|SetInputModeGameandUI _returnvalue _returnvalue_2 "DoNotLock" true false)
    (Variables|/Script/Engine.PlayerController|SetbShowMouseCursor _returnvalue true)
    (Input|DisableInput (Game|Player|GetPlayerPawn 0) _returnvalue)
    (Variables|Default|SetPaused true)
    (Utilities|Time|SetGlobalTimeDilation 0.0)))

(event Custom|OnCurrentSettingsChanged
  (bind _returnvalue (Actor|GetActorOfClass "/Game/Patchwork/Blueprints/Pawns/BP_BaseCharacter.BP_BaseCharacter_C"))
  (Utilities|IsValid _returnvalue
    (:Is%20Valid
      (Default|OnCurrentSettingsChanged _returnvalue (Variables|Default|GetCurrentSettings)))))

(event Custom|UnpauseGame
  ;[1 1 1] attempts to unpause game
  (if (Variables|Default|GetPaused)
    (Variables|Default|SetPaused false)
    (Utilities|Time|SetGlobalTimeDilation 1.0)))

(event Custom|SaveGame
  (params (overwrite%20level :type Boolean))
  (bind _returnvalue (Game|Player|GetPlayerPawn 0))
  (bind _currentgamedata (Variables|Default|GetCurrentGameData))
  (bind _currentgamedata_2 (Variables|Default|GetCurrentGameData))
  (bind _recorded_world_events (Variables|/Game/Patchwork/Blueprints/SaveData/GameData.GameData_C|Getrecorded%20world%20events _currentgamedata_2))
  ;[1 1 1 0.309 64] Save Game
  ;;[1 1 1] Check that we are able to save
  (Default|CallGameWillSave)
  (Utilities|IsValid (Variables|Default|GetCurrentGameData)
    (:Is%20Valid
      (if overwrite%20level
        (bind _returnvalue_2 (Game|GetCurrentLevelName true))
        (if (!= (Utilities|String|StringToName _returnvalue_2) "MainMenu")
          ;;[1 1 1] Save Current Level Name
          (Variables|/Game/Patchwork/Blueprints/SaveData/GameData.GameData_C|Setlevelname (Variables|Default|GetCurrentGameData) _returnvalue_2)
          (Utilities|FlowControl|Sequence :!label _label
            (:then_0
              ;;[1 1 1] Save NPC Data
              (bind _npc_save_data (CallFunction|GetNPCSaveData))
              (for _array_element _npc_save_data
                (Utilities|Map|Add (Variables|/Game/Patchwork/Blueprints/SaveData/GameData.GameData_C|Getnpc%20save%20data (Variables|Default|GetCurrentGameData)) (.ActorName (Utilities|Struct|BreakS_NPC_SaveData _array_element)) _array_element)))
            (:then_1
              ;;[1 1 1] Save Player Data
              (bind _asbp_base_character (Utilities|Casting|CastToBP_BaseCharacter _returnvalue)
                (:then
                  (if (Variables|/Game/Patchwork/Blueprints/Pawns/BP_BaseCharacter.BP_BaseCharacter_C|Gethas%20last%20location _asbp_base_character)
                    (Utilities|Map|Add (Variables|/Game/Patchwork/Blueprints/SaveData/GameData.GameData_C|Getplayer_transform_per_level _currentgamedata) (Utilities|String|StringToName (Variables|/Game/Patchwork/Blueprints/SaveData/GameData.GameData_C|Getlevelname _currentgamedata)) (Math|Transform|MakeTransform (Variables|/Game/Patchwork/Blueprints/Pawns/BP_BaseCharacter.BP_BaseCharacter_C|Getlast%20ground%20location _asbp_base_character) (Variables|/Game/Patchwork/Blueprints/Pawns/BP_BaseCharacter.BP_BaseCharacter_C|Getlast%20ground%20rotation _asbp_base_character)))
                    (else
                      (Development|PrintText "Cannot save location because player does not have last ground location"))))
                (:CastFailed
                  (Variables|/Game/Patchwork/Blueprints/SaveData/GameData.GameData_C|Setplayer_transform (Variables|Default|GetCurrentGameData) (Transformation|GetActorTransform _returnvalue)))))
            (:then_2
              ;;[1 1 1] Save World Events
              (bind _asgm_base_game_mode (Utilities|Casting|CastToGM_BaseGameMode (Game|GetGameMode)))
              (Utilities|Array|Clear _recorded_world_events)
              (for _array_element_2 (Variables|/Game/Patchwork/Blueprints/Gamemodes/GM_BaseGameMode.GM_BaseGameMode_C|Getworld%20events _asgm_base_game_mode)
                (Utilities|Array|Add _recorded_world_events _array_element_2)))
            (:then_3
              ;;[1 1 1] Save Game Data
              (SaveGame|SaveGametoSlot (Variables|Default|GetCurrentGameData) "game"))
            (:then_4
              (Variables|Default|Sethas%20last%20save true)
              (Variables|Default|Setlast%20save%20time (Math|DateTime|UTCNow)))))
        (else
          (goto _label))))))

(event Custom|LoadGame
  (params (force%20level%20reload :type Boolean))
  (bind _currentgamedata (Variables|Default|GetCurrentGameData))
  (bind _currentgamedata_2 (Variables|Default|GetCurrentGameData))
  (bind _levelname (Variables|/Game/Patchwork/Blueprints/SaveData/GameData.GameData_C|Getlevelname _currentgamedata_2))
  (bind _returnvalue (Utilities|String|StringToName _levelname))
  (CallFunction|LoadSaveData)
  ;[1 1 1] Check if has valid save data
  (Utilities|IsValid _currentgamedata
    (:Is%20Valid
      (if (not (Utilities|Array|IsEmpty (Variables|/Game/Patchwork/Blueprints/SaveData/GameData.GameData_C|Getlevelname _currentgamedata)))
        ;[1 1 1] Check if correct level is already open
        (bind _returnvalue_2 (Game|GetCurrentLevelName true))
        (if (!= (Utilities|String|StringToName _returnvalue_2) _returnvalue)
          ;[1 1 1] Level not loaded so flag for world load then open level
          (Variables|Default|SetJust%20Loaded%20Game true :!label _label)
          (Game|OpenLevel(byName) _returnvalue)
          (Development|PrintText "Is Level Open")
          (elif force%20level%20reload
            (goto _label)
            (else
              (bind _asgm_base_game_mode (Utilities|Casting|CastToGM_BaseGameMode (Game|GetGameMode)))
              (Default|LoadGame _asgm_base_game_mode))))))))

(event Custom|Load%20Into%20Level
  (params (level%20name :type Name))
  (CallFunction|LoadSaveData)
  (if (Utilities|Map|Contains (Variables|/Game/Patchwork/Blueprints/SaveData/GameData.GameData_C|Getplayer_transform_per_level (Variables|Default|GetCurrentGameData)) level%20name) ; check if player has been to level before
    (Variables|/Game/Patchwork/Blueprints/SaveData/GameData.GameData_C|Setlevelname (Variables|Default|GetCurrentGameData) (Utilities|String|ToString(Name) level%20name))
    (SaveGame|SaveGametoSlot (Variables|Default|GetCurrentGameData) "game")
    (CallFunction|LoadGame true)
    (else
      (Game|OpenLevel(byName) level%20name)
      (Variables|Default|Setload%20to%20level level%20name))))

(event Custom|check%20level%20loaded
  (bind _returnvalue (Game|GetCurrentLevelName true))
  (if (== (Utilities|String|StringToName _returnvalue) (Variables|Default|Getload%20to%20level))
    (Utilities|Time|ClearandInvalidateTimerbyHandle (Variables|Default|Getload%20timer%20handle))))

(event EventInit
  (Utilities|FlowControl|Sequence
    (:then_0
      ;[1 1 1] Load settings from disk to memory, or create new settings save if no disk save exists
      (bind _returnvalue (SaveGame|DoesSaveGameExist "settings"))
      (if _returnvalue
        (bind _returnvalue_2 (SaveGame|LoadGamefromSlot "settings"))
        (bind _asplayer_settings (Utilities|Casting|CastToPlayerSettings _returnvalue_2))
        (Variables|Default|SetCurrentSettings _asplayer_settings)
        (else
          (bind _returnvalue_3 (SaveGame|CreateSaveGameObject "/Game/Patchwork/Blueprints/SaveData/PlayerSettings.PlayerSettings_C"))
          (SaveGame|SaveGametoSlot _returnvalue_3 "settings")
          (Variables|Default|SetCurrentSettings _returnvalue_3)))
      ;[1 1 1] Copy current video settings values
      (bind _returnvalue_4 (Settings|GetGameUserSettings))
      (Utilities|FlowControl|Sequence
        (:then_0
          (Utilities|FlowControl|Sequence
            (:then_0
              (Variables|/Game/Patchwork/Blueprints/SaveData/PlayerSettings.PlayerSettings_C|SetVSync (Variables|Default|GetCurrentSettings) (Class|GameUserSettings|IsVSyncEnabled _returnvalue_4)))
            (:then_1
              (Variables|/Game/Patchwork/Blueprints/SaveData/PlayerSettings.PlayerSettings_C|SetScreenMode (Variables|Default|GetCurrentSettings) (Utilities|String|EnumtoString (Class|GameUserSettings|GetFullscreenMode _returnvalue_4))))))
        (:then_1
          (SaveGame|SaveGametoSlot (Variables|Default|GetCurrentSettings) "settings"))))
    (:then_1
      ;[1 1 1] init audio settings
      (Utilities|FlowControl|Delay 0.2)
      (Audio|SetSoundMixClassOverride "/Game/Patchwork/Profiles/Audio/PatchworkDefaultSoundMix.PatchworkDefaultSoundMix" "/Engine/EngineSounds/Master.Master" (Variables|/Game/Patchwork/Blueprints/SaveData/PlayerSettings.PlayerSettings_C|Getvolume_master (Variables|Default|GetCurrentSettings)) 1.0 0.0 true)
      (Audio|PushSoundMixModifier "/Game/Patchwork/Profiles/Audio/PatchworkDefaultSoundMix.PatchworkDefaultSoundMix"))
    (:then_2
      ;[1 1 1] create settings menu
      (bind _returnvalue_5 (UserInterface|CreateWidget "/Game/Patchwork/Blueprints/Widgets/SettingsMenu.SettingsMenu_C"))
      (Variables|Default|SetSettingsMenuRef _returnvalue_5))
    (:then_3
      ;[1 1 1] Load settings from disk to memory, or create new settings save if no disk save exists
      (bind _returnvalue_6 (SaveGame|DoesSaveGameExist "game"))
      (if _returnvalue_6
        (bind _returnvalue_7 (SaveGame|LoadGamefromSlot "game"))
        (bind _asgame_data (Utilities|Casting|CastToGameData _returnvalue_7))
        (Variables|Default|SetCurrentGameData _asgame_data)
        (else
          (bind _returnvalue_8 (SaveGame|CreateSaveGameObject "/Game/Patchwork/Blueprints/SaveData/GameData.GameData_C"))
          (SaveGame|SaveGametoSlot _returnvalue_8 "game")
          (Variables|Default|SetCurrentGameData _returnvalue_8))))
    (:then_4
      ;[1 1 1] Create HUD
      (Utilities|FlowControl|Delay 0.1))))

(fn RevertSettingstoSave
  (bind _returnvalue (SaveGame|LoadGamefromSlot "settings"))
  (bind _asplayer_settings (Utilities|Casting|CastToPlayerSettings _returnvalue))
  (Variables|Default|SetCurrentSettings _asplayer_settings)
  (Utilities|FlowControl|Sequence
    (:then_0
      (CallFunction|OnCurrentSettingsChanged))
    (:then_1
      (bind _returnvalue_2 (Settings|GetGameUserSettings))
      (Class|GameUserSettings|SetTextureQuality _returnvalue_2 (Variables|/Game/Patchwork/Blueprints/SaveData/PlayerSettings.PlayerSettings_C|Gettex%20quality (Variables|Default|GetCurrentSettings)))
      (Class|GameUserSettings|SetGlobalIlluminationQuality _returnvalue_2 (Variables|/Game/Patchwork/Blueprints/SaveData/PlayerSettings.PlayerSettings_C|Getlight%20quality (Variables|Default|GetCurrentSettings)))
      (Class|GameUserSettings|SetShadowQuality _returnvalue_2 (Variables|/Game/Patchwork/Blueprints/SaveData/PlayerSettings.PlayerSettings_C|Getshadow%20quality (Variables|Default|GetCurrentSettings)))
      (Class|GameUserSettings|SetReflectionQuality _returnvalue_2 (Variables|/Game/Patchwork/Blueprints/SaveData/PlayerSettings.PlayerSettings_C|Getreflection%20quality (Variables|Default|GetCurrentSettings)))
      (Class|GameUserSettings|SetFoliageQuality _returnvalue_2 (Variables|/Game/Patchwork/Blueprints/SaveData/PlayerSettings.PlayerSettings_C|Getfoliage%20quality (Variables|Default|GetCurrentSettings)))
      (Class|GameUserSettings|SetPostProcessingQuality _returnvalue_2 (Variables|/Game/Patchwork/Blueprints/SaveData/PlayerSettings.PlayerSettings_C|Getpost%20process%20quality (Variables|Default|GetCurrentSettings)))
      (Class|GameUserSettings|SetVisualEffectQuality _returnvalue_2 (Variables|/Game/Patchwork/Blueprints/SaveData/PlayerSettings.PlayerSettings_C|Getfx%20quality (Variables|Default|GetCurrentSettings)))
      (Class|GameUserSettings|SetViewDistanceQuality _returnvalue_2 (Variables|/Game/Patchwork/Blueprints/SaveData/PlayerSettings.PlayerSettings_C|Getview%20distance%20quality (Variables|Default|GetCurrentSettings)))
      (Class|GameUserSettings|ApplySettings _returnvalue_2 true))))

(fn SaveCurrentSettings
  (bind _currentsettings (Variables|Default|GetCurrentSettings))
  (bind _currentsettings_2 (Variables|Default|GetCurrentSettings))
  ;[1 1 1 0.134 36] Apply settings
  (bind _returnvalue (Settings|GetGameUserSettings))
  (Utilities|FlowControl|Sequence
    (:then_0
      ;;[1 1 1 1 36] Save Graphics Settings
      (Class|GameUserSettings|ApplySettings _returnvalue true)
      (Variables|/Game/Patchwork/Blueprints/SaveData/PlayerSettings.PlayerSettings_C|Settex%20quality _currentsettings_2 (Class|GameUserSettings|GetTextureQuality _returnvalue))
      (Variables|/Game/Patchwork/Blueprints/SaveData/PlayerSettings.PlayerSettings_C|Setlight%20quality _currentsettings_2 (Settings|GetGlobalIlluminationQuality _returnvalue))
      (Variables|/Game/Patchwork/Blueprints/SaveData/PlayerSettings.PlayerSettings_C|Setshadow%20quality _currentsettings_2 (Settings|GetShadowQuality _returnvalue))
      (Variables|/Game/Patchwork/Blueprints/SaveData/PlayerSettings.PlayerSettings_C|Setreflection%20quality _currentsettings_2 (Settings|GetReflectionQuality _returnvalue))
      (Variables|/Game/Patchwork/Blueprints/SaveData/PlayerSettings.PlayerSettings_C|Setfoliage%20quality _currentsettings_2 (Class|GameUserSettings|GetFoliageQuality _returnvalue))
      (Variables|/Game/Patchwork/Blueprints/SaveData/PlayerSettings.PlayerSettings_C|Setpost%20process%20quality _currentsettings_2 (Class|GameUserSettings|GetPostProcessingQuality _returnvalue))
      (Variables|/Game/Patchwork/Blueprints/SaveData/PlayerSettings.PlayerSettings_C|Setfx%20quality _currentsettings_2 (Settings|GetVisualEffectQuality _returnvalue))
      (Variables|/Game/Patchwork/Blueprints/SaveData/PlayerSettings.PlayerSettings_C|Setview%20distance%20quality _currentsettings_2 (Class|GameUserSettings|GetViewDistanceQuality _returnvalue))
      (Variables|/Game/Patchwork/Blueprints/SaveData/PlayerSettings.PlayerSettings_C|Setaa%20quality _currentsettings_2 (Class|GameUserSettings|GetAntiAliasingQuality _returnvalue)))
    (:then_1
      ;;[1 1 1 1 36] Apply Display Settings
      (Utilities|FlowControl|Sequence
        (:then_0
          (Class|GameUserSettings|SetVSyncEnabled _returnvalue (Variables|/Game/Patchwork/Blueprints/SaveData/PlayerSettings.PlayerSettings_C|GetVSync (Variables|Default|GetCurrentSettings))))
        (:then_1
          (switch string (Variables|/Game/Patchwork/Blueprints/SaveData/PlayerSettings.PlayerSettings_C|GetScreenMode (Variables|Default|GetCurrentSettings))
            (:Fullscreen
              (Class|GameUserSettings|SetFullscreenMode _returnvalue "Fullscreen"))
            (:Windowed%20Fullscreen
              (Class|GameUserSettings|SetFullscreenMode _returnvalue "WindowedFullscreen"))
            (:Windowed
              (Class|GameUserSettings|SetFullscreenMode _returnvalue "Windowed"))))))
    (:then_2
      ;;[1 1 1 1 25] Apply Accessibility Settings
      (Class|WidgetBlueprintLibrary|SetColorVisionDeficiencyType (Utilities|Enum|ByteToEnumEColorVisionDeficiency (Math|Conversions|ToByte(Integer) (Variables|/Game/Patchwork/Blueprints/SaveData/PlayerSettings.PlayerSettings_C|Getcolor%20mode _currentsettings))) (Variables|/Game/Patchwork/Blueprints/SaveData/PlayerSettings.PlayerSettings_C|Getcolor%20mode%20intensity _currentsettings) false))
    (:then_3
      ;;[1 1 1 1 36] Save Current Settings
      (SaveGame|SaveGametoSlot (Variables|Default|GetCurrentSettings) "settings"))))

(fn GetNPCSaveData
  (bind _outactors (Actor|GetAllActorsOfClass "/Game/Patchwork/Blueprints/Character/BP_DialogueNPC.BP_DialogueNPC_C"))
  (for _array_element _outactors
    (Utilities|Array|Add (LocalVariables|Getsave%20data) (Default|GetNPCSaveData _array_element)))
  (return (LocalVariables|Getsave%20data)))

(fn HasSaveGame
  (bind _returnvalue (SaveGame|DoesSaveGameExist "game"))
  (return _returnvalue))

(fn GetSaveGameData
  (Utilities|IsValid (Variables|Default|GetCurrentGameData)
    (:Is%20Valid
      (return (Variables|Default|GetCurrentGameData)))
    (:Is%20Not%20Valid
      (SaveGame|CreateSaveGameObject "/Game/Patchwork/Blueprints/SaveData/GameData.GameData_C"))))

(fn LoadSaveData
  (bind _returnvalue (SaveGame|DoesSaveGameExist "game"))
  (if _returnvalue
    (bind _returnvalue_2 (SaveGame|LoadGamefromSlot "game"))
    (bind _asgame_data (Utilities|Casting|CastToGameData _returnvalue_2))
    (Variables|Default|SetCurrentGameData _asgame_data)
    (else
      (bind _returnvalue_3 (SaveGame|CreateSaveGameObject "/Game/Patchwork/Blueprints/SaveData/GameData.GameData_C"))
      (SaveGame|SaveGametoSlot _returnvalue_3 "game")
      (Variables|Default|SetCurrentGameData _returnvalue_3))))

(fn ShouldAsktoSave
  (return (or (not (Variables|Default|Gethas%20last%20save)) (>= (- (Math|DateTime|UTCNow) (Variables|Default|Getlast%20save%20time)) (Math|Timespan|MakeTimespan 0 0 3)))))

(fn ShowConfirm
  (params (Confirm%20Text :type Text) (ZOrder :type Integer) (Widget%20Called%20From :type User%20Widget%20Object%20Reference))
  (LocalVariables|Setin%20confirm%20text Confirm%20Text)
  (LocalVariables|Setin%20zorder ZOrder)
  (LocalVariables|Setin%20widget%20called%20from Widget%20Called%20From)
  (Utilities|IsValid (CallFunction|GetConfirmWidget)
    (:Is%20Valid
      (if (UserInterface|Viewport|IsinViewport (Variables|Default|GetConfirm%20Wb))
        (Widget|RemovefromParent (Variables|Default|GetConfirm%20Wb)))
      (Default|SetConfirmText (Variables|Default|GetConfirm%20Wb) (LocalVariables|Getin%20confirm%20text))
      (Variables|/Game/Patchwork/Blueprints/Widgets/Parts/WB_PWConfirm.WB_PWConfirm_C|SetWidgetCalledFrom (Variables|Default|GetConfirm%20Wb) (LocalVariables|Getin%20widget%20called%20from))
      (UserInterface|Viewport|AddtoViewport (Variables|Default|GetConfirm%20Wb) (LocalVariables|Getin%20zorder))
      (Utilities|FlowControl|Sequence
        (:then_0
          (Utilities|IsValid (LocalVariables|Getin%20widget%20called%20from)
            (:Is%20Valid
              (bind _ascommon_activatable_widget (Utilities|Casting|CastToCommonActivatableWidget (LocalVariables|Getin%20widget%20called%20from)))
              (Class|CommonActivatableWidget|DeactivateWidget _ascommon_activatable_widget))))
        (:then_1
          (return (Variables|Default|GetConfirm%20Wb)))))
    (:Is%20Not%20Valid
      (return 0))))

(fn GetConfirmWidget
  (Utilities|IsValid (Variables|Default|GetConfirm%20Wb)
    (:Is%20Valid
      _)
    (:Is%20Not%20Valid
      (bind _returnvalue (UserInterface|CreateWidget "/Game/Patchwork/Blueprints/Widgets/Parts/WB_PWConfirm.WB_PWConfirm_C"))
      (Variables|Default|SetConfirm%20Wb _returnvalue)))
  (return (Variables|Default|GetConfirm%20Wb)))