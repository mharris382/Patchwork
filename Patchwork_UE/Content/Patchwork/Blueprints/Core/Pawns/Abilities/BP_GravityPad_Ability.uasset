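; Gravity Pad ability Blueprint for a pawn, triggered by the IA_Ability_GravityPad input action.
; IsReady extends the parent check by also requiring current mana to cover the ManaCost from GlobalAbilitySettings.
; Completing the input runs that readiness check, but nothing is wired after it, so no pad behavior is implemented here.
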(event Input|EnhancedActionEvents|EnhancedInputActionIA_Ability_GravityPad
  (params (ActionValue :type Boolean) (ElapsedSeconds :type Float%20%28double-precision%29) (TriggeredSeconds :type Float%20%28double-precision%29) (InputAction :type Input%20Action%20Object%20Reference :default "/Game/Patchwork/Data/Input/IA_Ability_GravityPad.IA_Ability_GravityPad"))
  (:Completed
    (if (CallFunction|IsReady)
      _)))

(event EventBeginPlay
  (|CallParentFunction) ; This node is disabled and will not be called.\nDrag off pins to build functionality.
)

(event EventTick
  (params (DeltaSeconds :type Float%20%28single-precision%29))
  (|CallParentFunction DeltaSeconds) ; This node is disabled and will not be called.\nDrag off pins to build functionality.
)

(fn IsReady
  (return (and (|CallParentFunction) (>= (Variables|Default|GetCurrentMana) (Variables|/Game/Patchwork/Blueprints/Utilities/BP_GlobalAbilitySettings.BP_GlobalAbilitySettings_C|GetManaCost (Variables|Default|GetGlobalAbilitySettings))))))