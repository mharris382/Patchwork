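; Lever interactible that links a set of BP_Platform actors to a child BP_PlatformTriggerGroup; the DEP prefix suggests it is deprecated.
; The construction script can optionally fill the Platforms list with every BP_Platform matching PlatformGroupTag.
; It then passes that list and a reference to itself to the trigger group child actor.
; The event graph only calls parent events, apart from an unreachable debug print.
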(event EventBeginPlay
  (|CallParentFunction))

(event Collision|EventActorBeginOverlap
  (params (OtherActor :type Actor%20Object%20Reference))
  (|CallParentFunction OtherActor))

(event EventTick
  (params (DeltaSeconds :type Float%20%28single-precision%29))
  (|CallParentFunction DeltaSeconds))

(fn ConstructionScript
  (bind _bp_platformtriggergroup (Variables|Default|GetBP_PlatformTriggerGroup))
  (bind _childactor (Variables|/Script/Engine.ChildActorComponent|GetChildActor _bp_platformtriggergroup))
  (bind _asbp_platform_trigger_group (Utilities|Casting|CastToBP_PlatformTriggerGroup _childactor))
  (|CallParentFunction)
  (Utilities|FlowControl|Sequence
    (:then_0
      (if (and (Variables|Default|Getget%20all%20platforms%20with%20tag) (!= (Variables|Default|Getplatform%20group%20tag) ""))
        (bind _outactors (Actor|GetAllActorsOfClasswithTag "/Game/Patchwork/Blueprints/Environment/Platforms/BP_Platform.BP_Platform_C" (Variables|Default|Getplatform%20group%20tag)))
        (Variables|Default|SetPlatforms _outactors)))
    (:then_1
      (Variables|/Game/Patchwork/Blueprints/Interactibles/BP_PlatformTriggerGroup.BP_PlatformTriggerGroup_C|SetPlatforms _asbp_platform_trigger_group (Variables|Default|GetPlatforms))
      (Variables|/Game/Patchwork/Blueprints/Interactibles/BP_PlatformTriggerGroup.BP_PlatformTriggerGroup_C|SetLever _asbp_platform_trigger_group self))))