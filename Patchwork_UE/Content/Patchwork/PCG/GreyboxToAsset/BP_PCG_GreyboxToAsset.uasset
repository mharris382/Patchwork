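; PCG helper actor that records tagged greybox static mesh actors as data, as its name suggests for replacing greybox with assets.
; The Construction Script clears the Data array, then gathers every actor with TargetTag.
; Each one that casts to StaticMeshActor adds a struct holding its transform and static mesh.
; The event graph is unused, and no PCG or replacement logic appears in this Blueprint.
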(event EventBeginPlay
  (|CallParentFunction) ; This node is disabled and will not be called.\nDrag off pins to build functionality.
)

(event Collision|EventActorBeginOverlap
  (params (OtherActor :type Actor%20Object%20Reference))
  (|CallParentFunction OtherActor) ; This node is disabled and will not be called.\nDrag off pins to build functionality.
)

(event EventTick
  (params (DeltaSeconds :type Float%20%28single-precision%29))
  (|CallParentFunction DeltaSeconds) ; This node is disabled and will not be called.\nDrag off pins to build functionality.
)

(fn ConstructionScript
  (|CallParentFunction)
  (Utilities|Array|Clear (Variables|Default|GetData))
  (bind _outactors (Actor|GetAllActorswithTag (Variables|Default|GetTargetTag)))
  (for _array_element _outactors
    (bind _asstatic_mesh_actor (Utilities|Casting|CastToStaticMeshActor _array_element))
    (Utilities|Array|Add (Variables|Default|GetData) (Utilities|Struct|MakeS_GreyboxToAssetStruct (Transformation|GetActorTransform _array_element) (Variables|/Script/Engine.StaticMeshComponent|GetStaticMesh (Variables|/Script/Engine.StaticMeshActor|GetStaticMeshComponent _asstatic_mesh_actor))))))