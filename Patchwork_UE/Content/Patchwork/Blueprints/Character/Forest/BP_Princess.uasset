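; BP_Princess is a forest character Blueprint for the princess, displayed as a Paper2D sprite.
; HoodOn and HoodOff events switch the PaperSprite between two princess sprites to change her hood state.
; It has no other active logic: BeginPlay, overlap and Tick are disabled stubs, and the construction script only calls its parent.
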(event Custom|Hood%20On
  (Rendering|Components|Sprite|SetSprite (Variables|Default|GetPaperSprite) "/Game/Patchwork/Textures/Sprites/Forest/T_princess_Sprite.T_princess_Sprite"))

(event Custom|Hood%20Off
  (Rendering|Components|Sprite|SetSprite (Variables|Default|GetPaperSprite) "/Game/Patchwork/Textures/Sprites/Forest/T_princess_2_Sprite.T_princess_2_Sprite"))

(event EventBeginPlay
  (|CallParentFunction) ; This node is disabled and will not be called.\nDrag off pins to build functionality.
)

(event Collision|EventActorBeginOverlap
  (params (OtherActor :type Actor%20Object%20Reference))
  (|CallParentFunction OtherActor) ; This node is disabled and will not be called.\nDrag off pins to build functionality.
)

(event EventTick
  (params (DeltaSeconds :type Float%20%28single-precision%29))
  (|CallParentFunction DeltaSeconds) ; This node is disabled and will not be called.\nDrag off pins to build functionality.
)

(fn ConstructionScript
  (|CallParentFunction))