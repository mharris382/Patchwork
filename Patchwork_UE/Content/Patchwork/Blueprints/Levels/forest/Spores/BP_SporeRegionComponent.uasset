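; Actor component for spore regions in the forest level, holding a data table row reference for a spore effect.
; GetEffectData looks up that row and returns it with a success flag.
; BeginPlay binds to the owner's begin and end overlap events, but both handlers are empty.
; Disconnected leftover logic would track overlapping actors, find or add their matching effect component, and initialise a new one's toxicity to zero.
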(event Custom|On%20Overlap%20Begin
  (params (OverlappedActor :type Actor%20Object%20Reference) (OtherActor :type Actor%20Object%20Reference)))

(event Custom|On%20Overlap%20End
  (params (OverlappedActor :type Actor%20Object%20Reference) (OtherActor :type Actor%20Object%20Reference)))

(event EventBeginPlay
  (bind _returnvalue (Components|GetOwner))
  (Collision|BindEventtoOnActorBeginOverlap _returnvalue (delegate Custom|On%20Overlap%20Begin))
  (Collision|BindEventtoOnActorEndOverlap _returnvalue (delegate Custom|On%20Overlap%20End)))

(event EventTick
  (params (DeltaSeconds :type Float%20%28single-precision%29)))

(fn GetEffectData
  (bind _sporeeffect (Variables|Default|GetSporeEffect))
  (bind _returnvalue (Utilities|GetDataTableRow (.datatable _sporeeffect) (.rowname _sporeeffect))
    (:then
      (return _returnvalue true))
    (:RowNotFound
      (return "" false))))