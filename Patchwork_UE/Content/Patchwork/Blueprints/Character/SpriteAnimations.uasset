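; An actor component that feeds the owning character's movement into its Paper2D sprite material, so the shader can animate the sprite.
; On BeginPlay it caches the movement component and gets or creates a dynamic material instance on the sprite.
; Each tick it remaps speed to a Movement value, smoothed with separate rise and fall rates.
; It writes that value and the negated velocity direction to the Movement and Direction material parameters.
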(event EventBeginPlay
  (bind _returnvalue (Components|GetOwner))
  (bind _returnvalue_2 (Actor|GetComponentbyClass _returnvalue "/Script/Paper2D.PaperSpriteComponent"))
  (bind _returnvalue_3 (Rendering|Material|GetMaterial _returnvalue_2 0))
  (Variables|Default|SetCharacterMovement (Actor|GetComponentbyClass _returnvalue "/Script/Engine.CharacterMovementComponent"))
  (Utilities|IsValid _returnvalue_2
    (:Is%20Valid
      (bind _asmaterial_instance_dynamic (Utilities|Casting|CastToMaterialInstanceDynamic _returnvalue_3)
        (:then
          (Variables|Default|SetDynamicMaterialInstance _asmaterial_instance_dynamic))
        (:CastFailed
          (bind _returnvalue_4 (Rendering|Material|CreateDynamicMaterialInstance _returnvalue_2 0 _returnvalue_3 "None" :!class /Script/Engine.PrimitiveComponent))
          (Variables|Default|SetDynamicMaterialInstance _returnvalue_4))))))

(event EventTick
  (params (DeltaSeconds :type Float%20%28single-precision%29))
  (bind _remapspeedrange (Variables|Default|GetRemapSpeedRange))
  (bind _charactermovement (Variables|Default|GetCharacterMovement))
  (bind _velocity (Variables|/Script/Engine.MovementComponent|GetVelocity _charactermovement))
  (bind _returnvalue (Math|Vector|VectorLength _velocity))
  (bind _returnvalue_2 (Math|Float|MapRangeClamped _returnvalue (.x _remapspeedrange) (.y _remapspeedrange) (.z _remapspeedrange) (.w _remapspeedrange)))
  (bind _dynamicmaterialinstance (Variables|Default|GetDynamicMaterialInstance)
    (:then
      (bind _output_get (Variables|Default|SetCurrentMovement (Math|Interpolation|FInterpTo (Variables|Default|GetCurrentMovement) _returnvalue_2 DeltaSeconds (Math|Float|SelectFloat (Variables|Default|GetMovementInterpSpeedDown) (Variables|Default|GetMovementInterpSpeedUp) (> (Variables|Default|GetCurrentMovement) _returnvalue_2)))))
      (Rendering|Material|SetScalarParameterValue _dynamicmaterialinstance "Movement" _output_get :!class /Script/Engine.MaterialInstanceDynamic)
      (Rendering|Material|SetVectorParameterValue _dynamicmaterialinstance "Direction" (Math|Conversions|ToLinearColor(Vector) (Math|Vector|NegateVector (Math|Vector|Normalize _velocity))) :!class /Script/Engine.MaterialInstanceDynamic))
    (:else)))