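; Base procedural tower spawner that prepares level sizes, grammar and extrude vector from a stack of level spawners in its construction script.
; Fixed levels subtract from tower height, weighted fill levels share the remainder, and accumulated offsets go into a generated level array.
; Repeated flexible levels get numbered symbols, which form the automatic grammar unless a manual one is used.
; Helpers adjust bounds for inverted towers, randomize debug colors and destroy all "Spawned"-tagged actors.
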(event EventBeginPlay
  (|CallParentFunction) ; This node is disabled and will not be called.\nDrag off pins to build functionality.
)

(event Collision|EventActorBeginOverlap
  (params (OtherActor :type Actor%20Object%20Reference))
  (|CallParentFunction OtherActor) ; This node is disabled and will not be called.\nDrag off pins to build functionality.
)

(event EventTick
  (params (DeltaSeconds :type Float%20%28single-precision%29))
  (|CallParentFunction DeltaSeconds) ; This node is disabled and will not be called.\nDrag off pins to build functionality.
)

(fn ConstructionScript
  (Utilities|FlowControl|Sequence
    (:then_0
      (|CallParentFunction))
    (:then_1
      (CallFunction|ProcessTowerLevels))
    (:then_2
      (CallFunction|ComputeAutoGrammar))
    (:then_3
      (CallFunction|SetupExtrudeVector))))

(fn ProcessTowerLevels
  (LocalVariables|SetRemainingSize (Variables|Default|GetTowerHeight))
  (Utilities|FlowControl|Sequence
    (:then_0
      (for (_array_element _array_index) (Variables|Default|GetTowerLevels)
        (Utilities|IsValid (.TowerLevelSpawner (Utilities|Struct|BreakS_TowerLevelUserData _array_element))
          (:Is%20Valid
            (LocalVariables|Setcur (.TowerLevelSpawner (Utilities|Struct|BreakS_TowerLevelUserData _array_element)))
            (Default|FromConstructor (.TowerLevelSpawner (Utilities|Struct|BreakS_TowerLevelUserData _array_element)))
            (Utilities|FlowControl|Sequence
              (:then_0
                ;[0.6233 0.6233 0.6233 0.5] Handle Multiple Flexible Levels
                (if (Utilities|Enum|Equal(Enum) (Variables|/Game/Patchwork/Blueprints/Procedural/Tower/Data/TowerLevelSpawner.TowerLevelSpawner_C|GetSizeMode (LocalVariables|Getcur)) "NewEnumerator2")
                  (if (Utilities|Map|Contains (LocalVariables|GetNewLocalVar_2) (LocalVariables|Getcur))
                    (Utilities|FlowControl|Sequence
                      (:then_0
                        (Utilities|Struct|SetmembersinS_TowerLevelUserData (Utilities|Array|Get(acopy) (Variables|Default|GetTowerLevels) _array_index) (Utilities|String|Append (Variables|/Game/Patchwork/Blueprints/Procedural/Tower/Data/TowerLevelSpawner.TowerLevelSpawner_C|GetSymbol (LocalVariables|Getcur)) (Utilities|String|ToString(Integer) (.Value (Utilities|Map|Find (LocalVariables|GetNewLocalVar_2) (LocalVariables|Getcur)))))))
                      (:then_1
                        (Utilities|Map|Add (LocalVariables|GetNewLocalVar_2) (LocalVariables|Getcur) (+ (.Value (Utilities|Map|Find (LocalVariables|GetNewLocalVar_2) (LocalVariables|Getcur))) 1))))
                    (else
                      (Utilities|FlowControl|Sequence
                        (:then_0
                          (Utilities|Struct|SetmembersinS_TowerLevelUserData (Utilities|Array|Get(acopy) (Variables|Default|GetTowerLevels) _array_index) (Variables|/Game/Patchwork/Blueprints/Procedural/Tower/Data/TowerLevelSpawner.TowerLevelSpawner_C|GetSymbol (LocalVariables|Getcur)) :!label _label))
                        (:then_1
                          (Utilities|Map|Add (LocalVariables|GetNewLocalVar_2) (LocalVariables|Getcur) 1)))))
                  (else
                    (goto _label))))
              (:then_1
                (bind (_sizeout _fillweight _isfill) (Default|RWLevelUserDataSize (.TowerLevelSpawner (Utilities|Struct|BreakS_TowerLevelUserData _array_element)) (.Size (Utilities|Struct|BreakS_TowerLevelUserData _array_element))))
                (if _isfill
                  (LocalVariables|SetTotalWeight (+ (LocalVariables|GetTotalWeight) _fillweight))
                  (Utilities|Array|Add (LocalVariables|GetWeights) _fillweight)
                  (Utilities|Array|Add (LocalVariables|GetIndexes) _array_index)
                  (else
                    (bind _structout (Utilities|Struct|SetmembersinS_TowerLevelUserData _array_element _sizeout))
                    (Utilities|Array|SetArrayElem (Variables|Default|GetTowerLevels) _array_index _structout)
                    (LocalVariables|SetRemainingSize (- (LocalVariables|GetRemainingSize) _sizeout))))))))))
    (:then_1
      (if (and (Utilities|Array|IsNotEmpty (LocalVariables|GetIndexes)) (> (LocalVariables|GetRemainingSize) 0.0))
        (for (_array_element_2 _array_index_2) (LocalVariables|GetIndexes)
          (bind _structout_2 (Utilities|Struct|SetmembersinS_TowerLevelUserData (Utilities|Array|Get(acopy) (Variables|Default|GetTowerLevels) _array_element_2) (- (|(totalSize*(w/totalW)) (LocalVariables|GetRemainingSize) (Utilities|Array|Get(acopy) (LocalVariables|GetWeights) _array_index_2) (LocalVariables|GetTotalWeight)) 1.0)))
          (Utilities|Array|SetArrayElem (Variables|Default|GetTowerLevels) _array_element_2 _structout_2))))
    (:then_2
      (Utilities|Array|Clear (Variables|PCGINTERNAL|GetGEN_TowerLevels))
      (for (_array_element_3 _array_index_3) (Variables|Default|GetTowerLevels)
        (bind _output_get (LocalVariables|SetCurrentOffset (+ (Variables|/Game/Patchwork/Blueprints/Procedural/Tower/Data/TowerLevelSpawner.TowerLevelSpawner_C|GetSpawnerOffset (.TowerLevelSpawner (Utilities|Struct|BreakS_TowerLevelUserData _array_element_3))) (.SplineOffset (Utilities|Struct|BreakS_TowerLevelUserData _array_element_3)) (LocalVariables|GetCurrentOffset))))
        (bind _structout_3 (Utilities|Struct|SetmembersinS_TowerLevelUserData _array_element_3 _output_get))
        (Utilities|Array|SetArrayElem (Variables|PCGINTERNAL|GetGEN_TowerLevels) _array_index_3 _structout_3 true)))))

(fn GetBoundsVerticalHeight
  (return (Variables|Default|GetTowerHeight)))

(fn ComputeAutoGrammar
  (bind _towerlevels (Variables|Default|GetTowerLevels))
  (if (Variables|Grammar|GetAutomaticGrammar)
    (for (_array_element _array_index) _towerlevels
      (if (== _array_index (- (Utilities|Array|Length _towerlevels) 1))
        (LocalVariables|Settmp (Utilities|String|Append (LocalVariables|Gettmp) (.Symbol (Utilities|Struct|BreakS_TowerLevelUserData _array_element))))
        (else
          (LocalVariables|Settmp (Utilities|String|Append (Utilities|String|Append (LocalVariables|Gettmp) (.Symbol (Utilities|Struct|BreakS_TowerLevelUserData _array_element))) ",")))))
    (Variables|Grammar|SetGrammar (Utilities|String|Append "[" (LocalVariables|Gettmp) "]"))
    (else
      (Variables|Grammar|SetGrammar (Variables|Grammar|GetManualGrammar)))))

(fn GetGrammarOptions
  (for _array_element (Variables|Default|GetTowerLevels)
    (Utilities|Array|Add (LocalVariables|GetNewLocalVar) (.Symbol (Utilities|Struct|BreakS_TowerLevelUserData _array_element))))
  (return (LocalVariables|GetNewLocalVar)))

(fn RandomDebugColors
  (bind _returnvalue (Math|Random|RandomFloat))
  (bind _towerlevels (Variables|Default|GetTowerLevels))
  (for (_ _array_index) _towerlevels
    (bind _output_get (LocalVariables|SetNewLocalVar_1 (Utilities|Struct|MakeLinearColor _returnvalue _returnvalue _returnvalue 1.0)))
    (Class|KismetMathLibrary|LinearColorSetRandomHue _output_get)
    (Utilities|Struct|SetmembersinS_TowerLevelUserData (Utilities|Array|Get(acopy) _towerlevels _array_index) _output_get)))

(fn SetupExtrudeVector
  (bind _returnvalue (Transformation|GetActorUpVector))
  (bind _towerheight (Variables|Default|GetTowerHeight))
  (bind _returnvalue_2 (* _returnvalue _towerheight))
  (if (Variables|Default|GetInvertTowerDirection)
    (Variables|PCGINTERNAL|SetGEN_ExtrudeVector (Math|Vector|NegateVector _returnvalue_2))
    (else
      (Variables|PCGINTERNAL|SetGEN_ExtrudeVector _returnvalue_2))))

(fn GetBoundsMinMax
  (bind _towerheight (Variables|Default|GetTowerHeight))
  (if (Variables|Default|GetInvertTowerDirection)
    (bind (_min _max) (|CallParentFunction))
    (return (Math|Vector|MakeVector (.x _min) (.y _min) (- (.z _min) _towerheight)) (Math|Vector|MakeVector (.x _max) (.y _max) (- (.z _max) _towerheight)))
    (else
      (bind (_min_2 _max_2) (|CallParentFunction))
      (return _min_2 _max_2))))

(fn CleanupSpawnedActors
  (bind _outactors (Actor|GetAllActorswithTag "Spawned"))
  (for _array_element _outactors
    (Actor|DestroyActor _array_element)))