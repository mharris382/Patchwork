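; Actor component that tracks which spore types its owner carries, broadcasting events when spores are gained or lost.
; Spores are added directly or caught through BPI_SporeContagion on optional overlaps, which query OverlappedActor (the owner) rather than OtherActor.
; Catching either accumulates types or swaps to the source's first, per CanCarryMultipleSpores.
; Deactivation clears all spores without blocking new ones; effect data for carried types comes from DT_SporeEffects.
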(event Custom|begin%20overlap
  (params (OverlappedActor :type Actor%20Object%20Reference) (OtherActor :type Actor%20Object%20Reference))
  (bind _asbpi_spore_contagion (Utilities|Casting|CastToBPI_SporeContagion OverlappedActor))
  (CallFunction|Catchfrom _asbpi_spore_contagion OverlappedActor))

(event Custom|Reset%20Spores
  (for _array_element (Variables|Default|GetCarried%20Spores)
    (Default|CallOnSporeLost _array_element))
  (Utilities|Array|Clear (Variables|Default|GetCarried%20Spores)))

(event EventBeginPlay
  (if (Variables|Default|GetCatch%20from%20Overlaps)
    (Collision|BindEventtoOnActorBeginOverlap (Components|GetOwner) (delegate Custom|begin%20overlap))))

(fn AddSpore)

(fn Catchfrom
  (params (containgion :type BPI%20Spore%20Contagion%20Interface) (instigator :type Actor%20Object%20Reference))
  (bind _carried_spores (Default|GetCarriedSporeTypes containgion))
  (if (> (Utilities|Array|Length _carried_spores) 0)
    (if (Variables|Default|Getcan%20carry%20multiple%20spores)
      (for _array_element _carried_spores
        (if (not (Utilities|Array|ContainsItem (Variables|Default|GetCarried%20Spores) _array_element))
          (Utilities|Array|AddUnique (Variables|Default|GetCarried%20Spores) _array_element)
          (Default|CallOnSporeGained _array_element containgion instigator)))
      (elif (> (Utilities|Array|Length (Variables|Default|GetCarried%20Spores)) 0)
        (if (!= (Utilities|Array|Get(acopy) _carried_spores) (Utilities|Array|Get(acopy) (Variables|Default|GetCarried%20Spores))) ; false do nothing because we already carry that spore
          (CallFunction|ResetSpores)
          (Utilities|Array|AddUnique (Variables|Default|GetCarried%20Spores) (Utilities|Array|Get(acopy) _carried_spores) :!label _label)
          (Default|CallOnSporeGained (Utilities|Array|Get(acopy) _carried_spores) containgion instigator))
        (else
          (goto _label))))))

(fn SetCarrierActive
  (params (active :type Boolean))
  (bind _output_get (Variables|Default|SetIs%20Carrier%20Active active))
  (if (not _output_get)
    (CallFunction|ResetSpores)))

(fn GetSporeData
  (params (carried%20spore :type Name))
  (if (Utilities|Array|ContainsItem (Variables|Default|GetCarried%20Spores) carried%20spore)
    (bind _returnvalue (Utilities|GetDataTableRow "/Game/Patchwork/Data/Datatables/DT_SporeEffects.DT_SporeEffects" carried%20spore)
      (:then
        (return true _returnvalue))
      (:RowNotFound
        _)))
  (return false ""))

(fn HasAnySpores
  (return (> (Utilities|Array|Length (Variables|Default|GetCarried%20Spores)) 0)))

(fn AddSporeType
  (params (Spore :type Name) (Instigator :type Actor%20Object%20Reference))
  (if (and (!= Spore "") (not (Utilities|Array|ContainsItem (Variables|Default|GetCarried%20Spores) Spore)))
    (Utilities|Array|AddUnique (Variables|Default|GetCarried%20Spores) Spore)
    (Default|CallOnSporeGained Spore 0 Instigator)
    (return)))

(fn HasSpore
  (params (SporeType :type Name))
  (return (Utilities|Array|ContainsItem (Variables|Default|GetCarried%20Spores) SporeType)))