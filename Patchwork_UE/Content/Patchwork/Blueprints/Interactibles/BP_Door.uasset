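; BP_Door is an interactable door that opens once, optionally from one side only, and keeps that state across loads.
; A flattened dot product against the door's right vector checks the player's side, showing a message when blocked.
; Opening invokes the DoorID world event and slerps the mesh toward EndRotation on a timeline.
; On load, the game mode's saved event state snaps the mesh open or closed.
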(event Custom|On%20Load
  (params (game%20data :type Game%20Data%20Object%20Reference))
  (bind _event_name (CallFunction|GetEventName))
  (bind _event_occured (Default|HasEventOccured game%20data _event_name))
  (CallFunction|LoadEvent _event_occured))

(event Custom|Open%20Door
  (if (not (Variables|Default|Getopened))
    (Variables|Default|Setopened true)
    (Default|InvokeWorldEvent (Variables|Default|GetAs%20GM%20Base%20Game%20Mode) (Variables|Default|GetDoor%20ID))
    (bind _rotation (Timeline|Animate%20Door Play)
      (:Update
        (Transformation|SetRelativeRotation (Variables|Default|Getdoor%20mesh) (Class|KismetMathLibrary|QuatRotator (Class|KismetMathLibrary|QuatSlerp (Math|Conversions|ToQuaternion(Rotator) (Variables|/Script/Engine.SceneComponent|GetRelativeRotation (Variables|Default|GetScene))) (Math|Conversions|ToQuaternion(Rotator) (Variables|/Script/Engine.SceneComponent|GetRelativeRotation (Variables|Default|Getend%20rotation))) _rotation)) false false)))))

(event EventBeginPlay
  (|CallParentFunction)
  (bind _asgm_base_game_mode (Utilities|Casting|CastToGM_BaseGameMode (Game|GetGameMode)))
  (Variables|Default|SetAs%20GM%20Base%20Game%20Mode _asgm_base_game_mode)
  (EventDispatchers|BindEventtoOnLoadOccured _asgm_base_game_mode (delegate Custom|On%20Load)))

(event Collision|EventActorBeginOverlap
  (params (OtherActor :type Actor%20Object%20Reference))
  (|CallParentFunction OtherActor) ; This node is disabled and will not be called.\nDrag off pins to build functionality.
)

(event EventTick
  (params (DeltaSeconds :type Float%20%28single-precision%29))
  (|CallParentFunction DeltaSeconds) ; This node is disabled and will not be called.\nDrag off pins to build functionality.
)

(event EventOnInteract
  (if (not (Variables|Default|Getopened))
    (if (Variables|Default|Getone%20sided)
      (if (> (Math|Vector|DotProduct (Math|Vector|Normalize (- (* (Transformation|GetActorLocation (Game|Player|GetPlayerPawn 0)) "1.000000,1.000000,0.000000") (* (Transformation|GetActorLocation) "1.000000,1.000000,0.000000"))) (Transformation|GetActorRightVector)) 0.0)
        (Variables|Default|Setopened true :!label _label)
        (Default|InvokeWorldEvent (Variables|Default|GetAs%20GM%20Base%20Game%20Mode) (Variables|Default|GetDoor%20ID))
        (bind _rotation (Timeline|Animate%20Door Play)
          (:Update
            (Transformation|SetRelativeRotation (Variables|Default|Getdoor%20mesh) (Class|KismetMathLibrary|QuatRotator (Class|KismetMathLibrary|QuatSlerp (Math|Conversions|ToQuaternion(Rotator) (Variables|/Script/Engine.SceneComponent|GetRelativeRotation (Variables|Default|GetScene))) (Math|Conversions|ToQuaternion(Rotator) (Variables|/Script/Engine.SceneComponent|GetRelativeRotation (Variables|Default|Getend%20rotation))) _rotation)) false false)))
        (else
          (bind _asgm_base_game_mode (Utilities|Casting|CastToGM_BaseGameMode (Game|GetGameMode)))
          (Default|DisplayMessage _asgm_base_game_mode "Door doesn't open from this side")))
      (else
        (goto _label)))))

(event EventLoadEvent
  (params (occured :type Boolean))
  (Variables|Default|Setopened occured)
  (Transformation|SetRelativeRotation (Variables|Default|Getdoor%20mesh) (Math|Rotator|SelectRotator (Variables|/Script/Engine.SceneComponent|GetRelativeRotation (Variables|Default|Getend%20rotation)) (Variables|/Script/Engine.SceneComponent|GetRelativeRotation (Variables|Default|GetScene)) occured) false false))

(fn ConstructionScript
  (|CallParentFunction)
  (if (not (Guid|IsValidGuid (Variables|Default|Getid)))
    (Variables|Default|Setid (Guid|NewGuid))))

(fn GetActionVerb
  (return "Open"))

(fn GetEventName
  (return (Variables|Default|GetDoor%20ID)))