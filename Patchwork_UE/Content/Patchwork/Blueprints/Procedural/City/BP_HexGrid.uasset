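; BP_HexGrid is a procedural city hex grid Blueprint that extends a parent class with a PCG bounding box.
; Its construction script runs the parent's, then derives Extents from triple the box's horizontal extent and a fixed height.
; It overrides GetBoundsVerticalHeight to return a constant without calling the parent.
; The event graph holds only disabled default events, so the Blueprint adds no runtime event logic.
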(event EventBeginPlay
  (|CallParentFunction) ; This node is disabled and will not be called.\nDrag off pins to build functionality.
)

(event Collision|EventActorBeginOverlap
  (params (OtherActor :type Actor%20Object%20Reference))
  (|CallParentFunction OtherActor) ; This node is disabled and will not be called.\nDrag off pins to build functionality.
)

(event EventTick
  (params (DeltaSeconds :type Float%20%28single-precision%29))
  (|CallParentFunction DeltaSeconds) ; This node is disabled and will not be called.\nDrag off pins to build functionality.
)

(fn ConstructionScript
  (bind _pcgboundingbox (Variables|Default|GetPCGBoundingBox))
  (bind _boxextent (Variables|/Script/Engine.BoxComponent|GetBoxExtent _pcgboundingbox))
  (bind _returnvalue (* _boxextent 3.0))
  (bind (_x _y) (Math|Vector|BreakVector _returnvalue))
  (|CallParentFunction)
  (Variables|Default|SetExtents (Math|Vector|MakeVector _x _y 1e+02)))

(fn GetBoundsVerticalHeight
  (return 2e+03))