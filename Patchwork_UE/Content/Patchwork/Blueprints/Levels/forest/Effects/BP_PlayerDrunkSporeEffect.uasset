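; Actor component that shows drunk spore toxicity on its owner through bubbles and, for players, camera shake.
; BeginPlay adds a Niagara bubble system with zero spawn rate, plus a camera shake source if the owner is the player.
; Toxicity changes set the bubble spawn rate directly.
; Tick restarts the shake on a countdown while toxicity is positive, scaling it by current toxicity and a multiplier.
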(event EventBeginPlay
  (|CallParentFunction)
  (Utilities|FlowControl|Sequence
    (:then_0
      ;[1 1 1] Drunk Bubbles
      (bind _returnvalue (Game|AddComponentbyClass (Components|GetOwner) "/Script/Niagara.NiagaraComponent" false (Math|Transform|MakeTransform "0, 0, 0")))
      (bind _output_get (Variables|Default|Setbubble%20effect _returnvalue))
      (Class|NiagaraComponent|SetAsset _output_get "/Game/Patchwork/Effects/NS_Bubbles.NS_Bubbles" true)
      (Effects|Components|ParticleSystem|SetFloatParameter _output_get (Variables|Default|GetSpawn%20Rate%20Parameter%20Name) 0.0))
    (:then_1
      ;[0.1667 0.1667 0.1667] Add Camera Shake to player
      (if (Variables|Default|GetIs%20Player)
        (bind _returnvalue_2 (Game|AddComponentbyClass (Components|GetOwner) "/Script/Engine.CameraShakeSourceComponent" false (Math|Transform|MakeTransform "0, 0, 0")))
        (bind _output_get_2 (Variables|Default|Setcamera%20shake _returnvalue_2))
        (Variables|/Script/Engine.CameraShakeSourceComponent|SetCameraShake _output_get_2 "/Game/Patchwork/Blueprints/Levels/forest/BP_DrunkCameraShake.BP_DrunkCameraShake_C")
        (CameraShakes|StartCameraShake (Variables|Default|Getcamera%20shake) "/Game/Patchwork/Blueprints/Levels/forest/BP_DrunkCameraShake.BP_DrunkCameraShake_C" 1.0 "CameraLocal" "0, 0, 0")))))

(event EventTick
  (params (DeltaSeconds :type Float%20%28single-precision%29))
  (|CallParentFunction DeltaSeconds)
  (if (Variables|Default|GetIs%20Player)
    (Utilities|IsValid (Variables|Default|Getcamera%20shake)
      (:Is%20Valid
        (if (> (Variables|Default|GetCurrent%20Toxicity) 0.0)
          (Variables|Default|Settime%20until%20next%20shake (- (Variables|Default|Gettime%20until%20next%20shake) DeltaSeconds))
          (if (<= (- (Variables|Default|Gettime%20until%20next%20shake) DeltaSeconds) 0.0)
            (Variables|Default|Settime%20until%20next%20shake (Variables|Default|Gettime%20between%20shakes))
            (CameraShakes|StartCameraShake (Variables|Default|Getcamera%20shake) "/Game/Patchwork/Blueprints/Levels/forest/BP_DrunkCameraShake.BP_DrunkCameraShake_C" (* (Variables|Default|GetCurrent%20Toxicity) (Variables|Default|Getshake%20multiplier)) "CameraLocal" "0, 0, 0")))))))

(fn OnToxicityChanged
  (params (new%20toxicity :type Float%20%28double-precision%29))
  (LocalVariables|Settoxicity new%20toxicity)
  (|CallParentFunction new%20toxicity)
  (Effects|Components|ParticleSystem|SetFloatParameter (Variables|Default|Getbubble%20effect) (Variables|Default|GetSpawn%20Rate%20Parameter%20Name) (LocalVariables|Gettoxicity)))