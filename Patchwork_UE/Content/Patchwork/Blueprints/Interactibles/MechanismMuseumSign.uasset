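; MechanismMuseumSign is an editor-configured sign Blueprint that labels a target object and its activation type, apparently for a showcase of mechanisms.
; The construction script shows the InfoTarget's class name, minus its last two characters (likely the "_C" suffix), and hides that label when no valid target exists.
; A second text render shows binary or analog activation from the Continuous flag.
; It has no active runtime logic.
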(event EventBeginPlay
  (|CallParentFunction) ; This node is disabled and will not be called.\nDrag off pins to build functionality.
)

(event Collision|EventActorBeginOverlap
  (params (OtherActor :type Actor%20Object%20Reference))
  (|CallParentFunction OtherActor) ; This node is disabled and will not be called.\nDrag off pins to build functionality.
)

(event EventTick
  (params (DeltaSeconds :type Float%20%28single-precision%29))
  (|CallParentFunction DeltaSeconds) ; This node is disabled and will not be called.\nDrag off pins to build functionality.
)

(fn ConstructionScript
  (bind _label_textrender1 (Variables|Default|GetLabel_TextRender1))
  (|CallParentFunction)
  (Utilities|FlowControl|Sequence
    (:then_0
      (bind _infotarget (Variables|Default|GetInfoTarget)
        (:then
          (Rendering|Components|TextRender|SetText _label_textrender1 (Utilities|Text|ToText(String) (Utilities|String|GetSubstring (Utilities|GetClassDisplayName (Utilities|GetClass _infotarget)) 0 (- (Utilities|String|Len (Utilities|GetClassDisplayName (Utilities|GetClass _infotarget))) 2))))
          (Rendering|SetVisibility _label_textrender1 true false))
        (:else
          (Rendering|SetVisibility _label_textrender1 false false))))
    (:then_1
      (Rendering|Components|TextRender|SetText (Variables|Default|GetMode_TextRender1) (Utilities|Text|FormatText "ActivationType: {0}" (Utilities|String|SelectText "Binary (on/off)" "Analog (continous)" (not (Variables|Default|GetContinuous))))))))