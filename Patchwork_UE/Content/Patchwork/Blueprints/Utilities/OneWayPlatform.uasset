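; One-way platform scene component that makes its child meshes solid only while the player is above it.
; On BeginPlay it caches child static meshes and Niagara systems.
; Each Tick it tests the player's lowered left-foot bone in local space, toggling mesh collision by the Z sign and passing a "colliding" bool to Niagara.
; An optional required tag, on the owner or each mesh, gates solidity and is reapplied by OnTagsChanged.
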(event EventBeginPlay
  (Utilities|FlowControl|Sequence
    (:then_0
      (CallFunction|Setup))
    (:then_1
      (Utilities|UpdateCollisions))))

(event EventTick
  (params (DeltaSeconds :type Float%20%28single-precision%29))
  (CallFunction|UpdateCollisions))

(fn OnTagsChanged
  (if (Variables|Default|GetRequireTag)
    (if (Variables|Default|Getwas%20colliding)
      (Utilities|SetCollisionsAll true)
      (else
        (Utilities|SetCollisionsAll false)))))

(fn Setup
  (for _array_element (Components|GetChildrenComponents true)
    (bind _asstatic_mesh_component (Utilities|Casting|CastToStaticMeshComponent _array_element)
      (:then
        (Utilities|Array|Add (Variables|Meshes|Getmeshes) _asstatic_mesh_component))
      (:CastFailed
        (bind _asniagara_particle_system_component (Utilities|Casting|CastToNiagaraComponent _array_element))
        (Utilities|Array|Add (Variables|Default|Getsystems) _asniagara_particle_system_component)))))

(fn UpdateCollisions
  (bind _output_get (Variables|Default|Setwas%20colliding (> (.Z (Math|Vector|BreakVector (Math|Transform|InverseTransformLocation (Transformation|GetWorldTransform) (+ (.Location (Math|Transform|BreakTransform (Transformation|GetBoneTransform (Variables|/Script/Engine.Character|GetMesh (CallFunction|GetBasePlayerPawn)) "foot_l" "RTS_World"))) "0.000000,0.000000,-20.000000")))) 0.0)))
  (if _output_get
    (Utilities|SetCollisionsAll true)
    (else
      (Utilities|SetCollisionsAll false))))

(fn SetCollisionsAll
  (params (InputPin :type Boolean))
  (LocalVariables|SetcheckTag (Variables|Default|GetRequireTag))
  (Utilities|FlowControl|Sequence
    (:then_0
      ;[0.6233 0.6233 0.6233 0.5] If owner has tag, don't check components
      (if (LocalVariables|GetcheckTag)
        (if (Actor|ActorHasTag (Components|GetOwner) (Variables|Default|GetRequiredTag))
          (LocalVariables|SetcheckTag false))))
    (:then_1
      (for _array_element (Variables|Meshes|Getmeshes)
        (Utilities|IsValid _array_element
          (:Is%20Valid
            (if (and (LocalVariables|GetcheckTag) InputPin)
              (if (Components|ComponentHasTag _array_element (Variables|Default|GetRequiredTag))
                (Utilities|SetCollisions _array_element InputPin :!label _label
                  (:Completed
                    (for _array_element_2 (Variables|Default|Getsystems)
                      (Utilities|UpdateSystemColliding _array_element_2 InputPin))))
                (else
                  (Utilities|SetCollisions _array_element false
                    (:Completed
                      (for _array_element_3 (Variables|Default|Getsystems)
                        (Utilities|UpdateSystemColliding _array_element_3 false))))))
              (else
                (goto _label)))))))))