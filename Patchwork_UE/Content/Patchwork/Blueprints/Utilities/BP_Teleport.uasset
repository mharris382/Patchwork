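; BP_Teleport is a teleporter that sends the player pawn to the TeleportArrive component of its TargetLocation.
; Player pawn overlap, or the TeleportPlayer event with any passed actor, calls TryTeleportActor, and failures print a message.
; A successful teleport zeroes actor rotation and sets player 0's control rotation to the arrival component's.
; An invalid TargetLocation only logs during the overlap check and does not block the teleport attempt.
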(event Custom|Event%20TeleportPlayer
  (params (Actor :type Actor%20Object%20Reference))
  (Utilities|TryTeleportActor Actor
    (:False
      (Development|PrintText "Teleportation Player failed" true true "(R=1.000000,G=0.000000,B=0.014042,A=1.000000)"))))

(event EventBeginPlay)

(event Collision|EventActorBeginOverlap
  (params (OtherActor :type Actor%20Object%20Reference))
  (bind _isplayer (CallFunction|IsPlayerPawn OtherActor))
  (if _isplayer
    (Utilities|TryTeleportActor OtherActor
      (:False
        (Development|PrintText "Teleportation failed" true true "(R=1.000000,G=0.000000,B=0.014042,A=1.000000)")))))

(fn ConstructionScript)

(fn IsPlayerPawn
  (params (Actor :type Object%20Object%20Reference))
  (bind _returnvalue (Game|Player|GetPlayerPawn 0))
  (bind _returnvalue_2 (== Actor _returnvalue))
  (Utilities|IsValid (Variables|Default|GetTargetLocation)
    (:Is%20Valid
      (return _returnvalue_2))
    (:Is%20Not%20Valid
      (Development|PrintString "Invalid location")
      (return _returnvalue_2))))