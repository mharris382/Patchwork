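; Trigger area that starts dialogue when the player overlaps it, optionally only while its Speaker NPC is following.
; It invokes an optional world event, can teleport the Speaker behind the camera's facing, then interacts with the Speaker or starts its assigned datatable dialogue through the game mode.
; One-shot triggers report that event ID and restore their fired state on load.
; Look-at location requests are forwarded to the Speaker.
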(event EventBeginPlay
  (bind _asgm_base_game_mode (Utilities|Casting|CastToGM_BaseGameMode (Game|GetGameMode)))
  (Variables|Default|SetGM%20Base%20Game%20Mode _asgm_base_game_mode))

(event Collision|EventActorBeginOverlap
  (params (OtherActor :type Actor%20Object%20Reference))
  (bind _event_id (Variables|Default|Getevent%20ID))
  (bind _speaker (Variables|Default|GetSpeaker))
  (if (and (== OtherActor (Game|Player|GetPlayerPawn 0)) (not (Variables|Default|GetHas%20Dialogue%20Happened)))
    (if (or (not (Variables|Default|GetOnly%20Trigger%20If%20NPC%20is%20following)) (and (Utilities|IsValid _speaker) (Variables|/Game/Patchwork/Blueprints/Character/BP_DialogueNPC.BP_DialogueNPC_C|GetFollowing%20Player _speaker)))
      (Utilities|FlowControl|Sequence
        (:then_0
          (if (!= _event_id "None")
            (Default|InvokeWorldEvent (Variables|Default|GetGM%20Base%20Game%20Mode) _event_id))
          (CallFunction|TriggerDialogue))
        (:then_1
          (if (Variables|Default|GetOnly%20Trigger%20Once)
            (Variables|Default|SetHas%20Dialogue%20Happened true)))))))

(event EventTick
  (params (DeltaSeconds :type Float%20%28single-precision%29)))

(event EventWorldEventOccuredfromLoad
  (params (event%20name :type Name :default "None") (has%20occured :type Boolean))
  (if (Variables|Default|GetOnly%20Trigger%20Once)
    (Variables|Default|SetHas%20Dialogue%20Happened has%20occured)))

(fn ConstructionScript
  (Variables|/Game/Defender/Blueprints/Components/DialogueComp.DialogueComp_C|SetDialogueDT (Variables|Default|GetDialogueComp) (Variables|Default|GetDialogue%20Datatable)))

(fn TriggerDialogue
  (bind _returnvalue (Game|Player|GetPlayerPawn 0))
  (bind (_aspaperperson _bsuccess) (Utilities|Casting|CastTopaperperson _returnvalue))
  (bind _camera (Variables|/Game/Patchwork/Blueprints/Pawns/BP_BaseCharacter.BP_BaseCharacter_C|GetCamera _aspaperperson))
  (bind _returnvalue_2 (Math|Vector|GetForwardVector _camera))
  (Utilities|IsValid (Variables|Default|GetDialogue%20Datatable)
    (:Is%20Valid
      (Utilities|FlowControl|Sequence
        (:then_0
          (if (and (Variables|Default|GetTeleport%20NPC%20behind%20player) _bsuccess)
            (Transformation|SetActorLocation (Variables|Default|GetSpeaker) (+ (* (Math|Vector|Normalize (Math|Vector|MakeVector (.x _returnvalue_2) (.y _returnvalue_2) 0.0)) (* (Variables|Default|Getdistance%20from%20player) -1.0)) (Transformation|GetActorLocation _returnvalue)) false false)))
        (:then_1
          (if (Variables|Default|GetUse%20Speaker%20Dialogue%20Component)
            (Default|Interaction (Variables|Default|GetSpeaker) (Game|Player|GetPlayerPawn 0))
            (else
              (Default|StartSpecificDialogue (Variables|Default|GetGM%20Base%20Game%20Mode) (Variables|Default|GetDialogue%20Datatable) self))))))
    (:Is%20Not%20Valid
      (Development|PrintText (Utilities|Text|FormatText "Dialogue Trigger {0} has no dialogue datatable assigned" (Utilities|GetDisplayName self))))))

(fn GetFPLookatLocationWS
  (bind _look_at_location (Default|GetFPLookatLocationWS (Variables|Default|GetSpeaker)))
  (return _look_at_location))

(fn GetReleventWorldEvents
  (bind _event_id (Variables|Default|Getevent%20ID))
  (return (select (or (== _event_id "None") (not (Variables|Default|GetOnly%20Trigger%20Once))) (Utilities|Array|MakeArray) (Utilities|Array|MakeArray _event_id))))