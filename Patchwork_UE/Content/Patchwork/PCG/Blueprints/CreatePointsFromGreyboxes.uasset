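; Custom PCG Blueprint element that turns tagged greybox static mesh actors into PCG points, one per actor by transform and local mesh bounds.
; Execute gathers the actors into Targets and builds points, or repeats a single point when not in FromPointArray mode; position-based creation is disconnected.
; IterationLoopBody then writes Index, MaxIndex and mesh path attributes and reapplies each actor's transform and bounds.
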(fn ExecutewithContext
  (params (InContext :type PCG%20Context%20Structure%20%28by%20ref%29) (Input :type PCG%20Data%20Collection%20Structure%20%28by%20ref%29))
  (bind _returnvalue (PCG|Temporary|GetActorData InContext))
  (bind _aspcgspatial_data (Utilities|Casting|CastToPCGSpatialData _returnvalue))
  (Variables|Default|SetAs%20BP%20PCG%20Greybox%20To%20Asset 0)
  (LocalVariables|SetTargetActor (Variables|/Script/PCG.PCGSpatialData|GetTargetActor _aspcgspatial_data))
  (Utilities|Array|Clear (Variables|Default|GetTargets))
  (Utilities|Array|Clear (Variables|Default|GetPointsToCreate))
  (bind _outactors (Actor|GetAllActorswithTag (Variables|Default|GetTargetTag)))
  (for _array_element _outactors
    (bind _asstatic_mesh_actor (Utilities|Casting|CastToStaticMeshActor _array_element))
    (Utilities|Array|Add (Variables|Default|GetTargets) _asstatic_mesh_actor)
    (Utilities|Array|Add (Variables|Default|GetPointsToCreate) (Utilities|Struct|MakePCGPoint (Transformation|GetActorTransform _asstatic_mesh_actor) 1.0 (.Min (Components|StaticMesh|GetLocalBounds (Variables|/Script/Engine.StaticMeshActor|GetStaticMeshComponent _asstatic_mesh_actor))) (.Max (Components|StaticMesh|GetLocalBounds (Variables|/Script/Engine.StaticMeshActor|GetStaticMeshComponent _asstatic_mesh_actor))) "(X=1.000000,Y=1.000000,Z=1.000000,W=1.000000)" 0.5 0)))
  (if (Utilities|Enum|Equal(Enum) (Variables|Default|GetPointCreationMethod) "NewEnumerator0")
    (LocalVariables|SetPoints%20to%20Loop%20On (Variables|Default|GetPointsToCreate))
    (else
      (Utilities|Array|Clear (LocalVariables|GetPoints%20to%20Loop%20On))
      (for _index (range 0 (- (Variables|Default|GetCount) 1))
        (Utilities|Array|Add (LocalVariables|GetPoints%20to%20Loop%20On) (Variables|Default|GetSinglePoint)))))
  (bind _returnvalue_2 (Game|ConstructObjectfromClass "/Script/PCG.PCGPointData"))
  (bind _output_get (Variables|Default|SetPtData _returnvalue_2))
  (SpatialData|InitializefromData _output_get _aspcgspatial_data 0 true true)
  (bind _returnvalue_3 (Metadata|MutableMetadata (Variables|Default|GetPtData)))
  (PCG|Metadata|CreateFloatAttribute _returnvalue_3 "Index" 0.0 false true)
  (PCG|Metadata|CreateFloatAttribute _returnvalue_3 "MaxIndex" 0.0 false true)
  (SpatialData|SetPoints (Variables|Default|GetPtData) (LocalVariables|GetPoints%20to%20Loop%20On))
  (Variables|Default|SetPtCount (Utilities|Array|Length (LocalVariables|GetPoints%20to%20Loop%20On)))
  (bind _outdata (PCG|FlowControl|IterationLoop InContext (Class|KismetMathLibrary|ToInt64(Integer) (Utilities|Array|Length (LocalVariables|GetPoints%20to%20Loop%20On))) 0 0 (Variables|Default|GetPtData)))
  (return (Utilities|Struct|MakePCGDataCollection (Utilities|Array|MakeArray (Utilities|Struct|MakePCGTaggedData _outdata 0 "None")))))

(fn IterationLoopBody
  (params (InContext :type PCG%20Context%20Structure%20%28by%20ref%29) (Iteration :type Integer64) (InA :type PCG%20Spatial%20Data%20Object%20Reference) (InB :type PCG%20Spatial%20Data%20Object%20Reference) (OutMetadata :type PCG%20Metadata%20Object%20Reference))
  (LocalVariables|Setcontext InContext)
  (LocalVariables|Setindex Iteration)
  (LocalVariables|SetoutMeta OutMetadata)
  (LocalVariables|SetmaxIndex (Class|KismetMathLibrary|ToInt64(Integer) (Variables|Default|GetPtCount)))
  (LocalVariables|SetinPoint (SpatialData|GetPoint (Variables|Default|GetPtData) (Math|Conversions|ToInteger(Byte) (LocalVariables|Getindex))))
  (bind _returnvalue (PCG|Temporary|GetActorData (LocalVariables|Getcontext)))
  (bind _aspcgspatial_data (Utilities|Casting|CastToPCGSpatialData _returnvalue))
  (LocalVariables|SetinLoopInContextSpatialData _aspcgspatial_data)
  (LocalVariables|SettargetMesh (Utilities|Array|Get(acopy) (Variables|Default|GetTargets) (Math|Conversions|ToInteger(Byte) (LocalVariables|Getindex))))
  (PCG|Metadata|SetFloatAttribute (LocalVariables|GetinPoint) (LocalVariables|GetoutMeta) "Index" (Math|Conversions|ToFloat(Integer) (Math|Conversions|ToInteger(Byte) (LocalVariables|Getindex))))
  (PCG|Metadata|SetFloatAttribute (LocalVariables|GetinPoint) (LocalVariables|GetoutMeta) "MaxIndex" (Math|Conversions|ToFloat(Integer) (LocalVariables|GetmaxIndex)))
  (Class|PCGMetadataAccessorHelpers|SetSoftObjectPathAttribute (LocalVariables|GetinPoint) (LocalVariables|GetoutMeta) "Mesh" (Utilities|GetSoftObjectPath (Variables|/Script/Engine.StaticMeshComponent|GetStaticMesh (Variables|/Script/Engine.StaticMeshActor|GetStaticMeshComponent (LocalVariables|GettargetMesh)))))
  (bind _structout (Utilities|Struct|SetmembersinPCGPoint (LocalVariables|GetinPoint) (Transformation|GetActorTransform (LocalVariables|GettargetMesh)) 1.0 (.Min (Components|StaticMesh|GetLocalBounds (Variables|/Script/Engine.StaticMeshActor|GetStaticMeshComponent (LocalVariables|GettargetMesh)))) (.Max (Components|StaticMesh|GetLocalBounds (Variables|/Script/Engine.StaticMeshActor|GetStaticMeshComponent (LocalVariables|GettargetMesh))))))
  (return _structout true))