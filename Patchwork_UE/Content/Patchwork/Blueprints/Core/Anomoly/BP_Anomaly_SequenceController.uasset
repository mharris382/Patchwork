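; BP_Anomaly_SequenceController is a controller for an anomaly's Level Sequence, exposing a PauseSequence function that pauses the player of a referenced LevelSequenceActor.
; BeginPlay checks that actor, logging an error if it is invalid and otherwise setting its SequencePlayer variable to None.
; PauseSequence reads the player directly from the actor without a validity check.
; The LevelSequenceGraph and remaining event logic are unused stubs.
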(event EventBeginPlay
  (if (Utilities|IsValid (Variables|Default|GetLevel%20Sequence%20Actor))
    (Variables|Default|SetSequence%20Player 0)
    (else
      (Class|VisualLoggerKismetLibrary|LogText 0 "ERROR: Anomaly Sequence Actor is not valid" "VisLogBP"))))

(event Collision|EventActorBeginOverlap
  (params (OtherActor :type Actor%20Object%20Reference)))

(event EventTick
  (params (DeltaSeconds :type Float%20%28single-precision%29)))

(fn ConstructionScript)

(fn PauseSequence
  (Sequencer|Player|Pause (Variables|/Script/LevelSequence.LevelSequenceActor|GetSequencePlayer (Variables|Default|GetLevel%20Sequence%20Actor))))