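; BP_Lever is an interactable lever that cycles its handle through a list of preset rotations each time it is used.
; Interaction advances a wrapping index, then a timeline slerps the handle between the two rotations via quaternions, ignoring input until the move finishes.
; On completion it fires a position-changed call with the new index.
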(event Custom|Move%20Next%20Position
  (if (not (Variables|Default|Getis%20transitioning))
    ;[1 1 1] cache start and end position and update index
    (Variables|Default|Setstart%20pos (Utilities|Array|Get(acopy) (Variables|Default|Getpositions) (Variables|Default|Getcurrent%20position)))
    (Variables|Default|Setcurrent%20position (CallFunction|NextPosition))
    (Variables|Default|Setend%20pos (Utilities|Array|Get(acopy) (Variables|Default|Getpositions) (Variables|Default|Getcurrent%20position)))
    (if (Utilities|Operators|EqualEqual (Variables|Default|Getstart%20pos) (Variables|Default|Getend%20pos) 0.1)
      (Development|PrintString "start and end positions are the same"))
    (Variables|Default|Setis%20transitioning true)
    (bind _pos (Timeline|Move%20Position PlayFromStart)
      (:Update
        (Transformation|SetRelativeRotation (Variables|Default|Gethandle) (Class|KismetMathLibrary|QuatRotator (Class|KismetMathLibrary|QuatSlerp (Math|Conversions|ToQuaternion(Rotator) (Variables|Default|Getstart%20pos)) (Math|Conversions|ToQuaternion(Rotator) (Variables|Default|Getend%20pos)) _pos)) false false))
      (:Finished
        (Variables|Default|Setis%20transitioning false)
        (Default|CallOnPositionChanged (Variables|Default|Getcurrent%20position))))))

(event Collision|EventActorBeginOverlap
  (params (OtherActor :type Actor%20Object%20Reference))
  (|CallParentFunction OtherActor) ; This node is disabled and will not be called.\nDrag off pins to build functionality.
)

(event EventTick
  (params (DeltaSeconds :type Float%20%28single-precision%29))
  (|CallParentFunction DeltaSeconds) ; This node is disabled and will not be called.\nDrag off pins to build functionality.
)

(event EventInteractionPressed
  (params (Interactor :type Actor%20Object%20Reference))
  (CallFunction|MoveNextPosition))

(event EventInteractionReleased
  (params (Interactor :type Actor%20Object%20Reference)))

(event EventBeginPlay)

(event EventOnInteract
  (CallFunction|MoveNextPosition))

(fn ConstructionScript)

(fn NextPosition
  (return (Math|Integer|%(Integer) (+ (Variables|Default|Getcurrent%20position) 1) (Utilities|Array|Length (Variables|Default|Getpositions)))))