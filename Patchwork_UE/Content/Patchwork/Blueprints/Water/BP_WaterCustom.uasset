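; BP_WaterCustom is a water actor that lets the player walk on water while the "WaterWalker" spore effect is active.
; On BeginPlay it binds to the game mode's player spore effect change event.
; Enabling the effect switches WaterSurface to a water-walking collision profile and disabling restores the standard one.
; Two paired DoOnce nodes re-arm each other so each switch runs once per change, with a leftover debug print on enable.
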(event Custom|CustomEvent
  (params (SporeEffectName :type Name) (Toxicity :type Float%20%28double-precision%29) (Enabled :type Boolean))
  (if (== SporeEffectName "WaterWalker")
    (if Enabled
      (Utilities|FlowControl|DoOnce false :!label _label
        (:Completed
          (Utilities|FlowControl|Sequence
            (:then_0
              (Collision|SetCollisionProfileName (Variables|Default|GetWaterSurface) "WaterBodyCollision_WaterWalking" true :!class /Script/Engine.PrimitiveComponent)
              (Development|PrintString "Rancid Anus"))
            (:then_1
              (goto _label_2 Reset)))))
      (else
        (Utilities|FlowControl|DoOnce true :!label _label_2
          (:Completed
            (Utilities|FlowControl|Sequence
              (:then_0
                (Collision|SetCollisionProfileName (Variables|Default|GetWaterSurface) "WaterBodyCollision" true :!class /Script/Engine.PrimitiveComponent))
              (:then_1
                (goto _label Reset)))))))))

(event EventBeginPlay
  (EventDispatchers|BindEventtoOnPlayerSporeEffectChanged (CallFunction|GetBaseGameMode) (delegate Custom|CustomEvent)))

(event Collision|EventActorBeginOverlap
  (params (OtherActor :type Actor%20Object%20Reference)))

(event EventTick
  (params (DeltaSeconds :type Float%20%28single-precision%29)))

(fn ConstructionScript)