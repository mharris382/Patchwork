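; BP_NY_Simple_Building is a procedural building actor that currently generates only a ring of horizontal plane tiles at the building's top height.
; The construction script derives a corner from Width, Depth and Height on a 200-unit grid centered on the actor.
; Two loops step along the X and Y edges, mirroring that corner to add opposite rows of static mesh components using PlaneMaterial.
; It builds no walls or interior fill, and some corner tiles overlap.
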(event EventBeginPlay)

(event Collision|EventActorBeginOverlap
  (params (OtherActor :type Actor%20Object%20Reference)))

(event EventTick
  (params (DeltaSeconds :type Float%20%28single-precision%29)))

(fn ConstructionScript
  (bind _returnvalue (Math|Vector|MakeVector 2.0 2.0 1.0))
  (bind _returnvalue_2 (Math|Vector|MakeVector 2e+02 2e+02 2e+02))
  (bind _width (Variables|Default|GetWidth))
  (bind _height (Variables|Default|GetHeight))
  (bind _depth (Variables|Default|GetDepth))
  (bind _returnvalue_3 (Math|Conversions|ToFloat(Integer) _width))
  (bind _returnvalue_4 (Math|Conversions|ToFloat(Integer) _height))
  (bind _returnvalue_5 (Math|Conversions|ToFloat(Integer) _depth))
  (bind _returnvalue_6 (Math|Vector|MakeVector _returnvalue_3 _returnvalue_5 _returnvalue_4))
  (bind _returnvalue_7 (* _returnvalue_6 _returnvalue_2))
  (bind _returnvalue_8 (/ _returnvalue_7 _returnvalue))
  (bind _returnvalue_9 (- _returnvalue_8 "100.000000,100.000000,0.000000"))
  (bind _returnvalue_10 (AddComponent|AddStaticMeshComponent false (Math|Transform|MakeTransform _returnvalue_9 "0, 0, 0" "2.000000,2.000000,2.000000")))
  (Components|StaticMesh|SetStaticMesh _returnvalue_10 "/Engine/BasicShapes/Plane.Plane")
  (Rendering|Material|SetMaterial _returnvalue_10 0 (Variables|Default|Getplane%20material))
  (for _index (range 0 (- (Variables|Default|GetWidth) 1))
    (bind _returnvalue_11 (AddComponent|AddStaticMeshComponent false (Math|Transform|MakeTransform (- _returnvalue_9 (* (Math|Vector|MakeVector 2e+02 0.0 0.0) _index)) "0, 0, 0" "2.000000,2.000000,2.000000")))
    (Components|StaticMesh|SetStaticMesh _returnvalue_11 "/Engine/BasicShapes/Plane.Plane")
    (Rendering|Material|SetMaterial _returnvalue_11 0 (Variables|Default|Getplane%20material))
    (bind _returnvalue_12 (AddComponent|AddStaticMeshComponent false (Math|Transform|MakeTransform (- (* _returnvalue_9 "1.000000,-1.000000,1.000000") (* (Math|Vector|MakeVector 2e+02 0.0 0.0) _index)) "0, 0, 0" "2.000000,2.000000,2.000000")))
    (Components|StaticMesh|SetStaticMesh _returnvalue_12 "/Engine/BasicShapes/Plane.Plane")
    (Rendering|Material|SetMaterial _returnvalue_12 0 (Variables|Default|Getplane%20material)))
  (for _index_2 (range 1 (- (Variables|Default|GetDepth) 1))
    (bind _returnvalue_13 (AddComponent|AddStaticMeshComponent false (Math|Transform|MakeTransform (- _returnvalue_9 (* (Math|Vector|MakeVector 0.0 2e+02 0.0) _index_2)) "0, 0, 0" "2.000000,2.000000,2.000000")))
    (Components|StaticMesh|SetStaticMesh _returnvalue_13 "/Engine/BasicShapes/Plane.Plane")
    (Rendering|Material|SetMaterial _returnvalue_13 0 (Variables|Default|Getplane%20material))
    (bind _returnvalue_14 (AddComponent|AddStaticMeshComponent false (Math|Transform|MakeTransform (- (* _returnvalue_9 "-1.000000,1.000000,1.000000") (* (Math|Vector|MakeVector 0.0 2e+02 0.0) _index_2)) "0, 0, 0" "2.000000,2.000000,2.000000")))
    (Components|StaticMesh|SetStaticMesh _returnvalue_14 "/Engine/BasicShapes/Plane.Plane")
    (Rendering|Material|SetMaterial _returnvalue_14 0 (Variables|Default|Getplane%20material))))