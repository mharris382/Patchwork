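; Editor utility actor, apparently for testing jump and fall trajectories of the player from its placed transform.
; The construction script clears its spline and runs a collision-traced projectile prediction with the player's capsule radius.
; Launch velocity follows the actor's orientation, with toggles for sprint speed and bounce-mushroom lift.
; It looks unfinished: the predicted path is unused, DrawPath has an empty loop, and several node chains are disconnected.
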(event EventBeginPlay)

(event Collision|EventActorBeginOverlap
  (params (OtherActor :type Actor%20Object%20Reference)))

(event EventTick
  (params (DeltaSeconds :type Float%20%28single-precision%29)))

(fn ConstructionScript
  (bind _returnvalue (Transformation|GetActorTransform))
  (Utilities|FlowControl|Sequence
    (:then_0
      (Spline|ClearSplinePoints (Variables|Default|GetSpline) true)
      (bind _predictresult (Class|GameplayStatics|BlueprintPredictProjectilePathAdvanced (Utilities|Struct|MakePredictProjectilePathParams (+ (.Location (Math|Transform|BreakTransform _returnvalue)) (Math|Vector|MakeVector 0.0 0.0 (+ (Variables|Default|Getplayer%20capsule%20radius) 1.0))) (Math|Transform|TransformDirection _returnvalue (Math|Vector|MakeVector (Math|Float|SelectFloat (.Sprinting%20Move%20Speed (Utilities|GetClassDefaults (Variables|Default|Getclass))) (Variables|Default|Getinitial%20move%20speed) (Variables|Default|Getuse%20player%20max%20speed)) 0.0 (Math|Float|SelectFloat 1e+03 (Variables|Default|Getjump%20z%20velocity) (Variables|Default|Getuse%20bounce%20mushroom)))) true (Variables|Default|Getplayer%20capsule%20radius) (Variables|Default|Gettest%20time%20limit) true "ECC_WorldStatic" "ObjectTypeQuery1" 0 (Variables|Default|Gettime%20increment)))))))

(fn DrawPath
  (params (path :type Array%20of%20Predict%20Projectile%20Path%20Point%20Data%20Structures))
  (for _array_element path
    _))