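; Utility actor that fades the screen out and in by animating a post-process blend weight, with an editor preview.
; FadeOut plays the Fade timeline forward and FadeIn reverses it, firing start and completion dispatchers.
; FadeInOut stores a delay and sets FullLoop, though the delayed fade-in sits on the branch where FullLoop is false.
; The timer-driven animation path and player-control hooks are unfinished stubs.
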(event Custom|Fade%20Out
  (Variables|Default|Setfade%20state "NewEnumerator0")
  (Default|CallOnFadeOutStarted)
  (bind _fade (Timeline|Fade PlayFromStart)
    (:Update
      (Variables|/Script/Engine.PostProcessComponent|SetBlendWeight (Variables|Default|GetPostProcess) _fade))
    (:Finished
      ;[0.6233 0.6233 0.6233 0.5] If full cycle then do fade in next
      (if (Variables|Default|Getfull%20loop)
        ;[0.6233 0.6233 0.6233 0.5] Call Events
        (Utilities|FlowControl|Sequence
          (:then_0
            (if (Utilities|Enum|Equal(Enum) (Variables|Default|Getfade%20state) "NewEnumerator0")
              (Default|CallOnFadeOutCompleted)
              (else
                (Default|CallOnFadeinCompleted))))
          (:then_1
            (Variables|Default|Setfade%20state "NewEnumerator2")))
        (else
          (switch Utilities|FlowControl|Switch|SwitchonEFadeState (Variables|Default|Getfade%20state)
            (:NewEnumerator0
              (Default|CallOnFadeOutCompleted)
              (Utilities|FlowControl|Delay (Variables|Default|GetWait%20Time))
              (CallFunction|Fadein))
            (:NewEnumerator1
              (Default|CallOnFadeinCompleted)
              (Variables|Default|Setfade%20state "NewEnumerator2"))))))))

(event Custom|Fade%20In
  (Variables|Default|Setfade%20state "NewEnumerator1")
  (bind _fade (Timeline|Fade ReverseFromEnd)
    (:Update
      (Variables|/Script/Engine.PostProcessComponent|SetBlendWeight (Variables|Default|GetPostProcess) _fade))
    (:Finished
      ;[0.6233 0.6233 0.6233 0.5] If full cycle then do fade in next
      (if (Variables|Default|Getfull%20loop)
        ;[0.6233 0.6233 0.6233 0.5] Call Events
        (Utilities|FlowControl|Sequence
          (:then_0
            (if (Utilities|Enum|Equal(Enum) (Variables|Default|Getfade%20state) "NewEnumerator0")
              (Default|CallOnFadeOutCompleted)
              (else
                (Default|CallOnFadeinCompleted))))
          (:then_1
            (Variables|Default|Setfade%20state "NewEnumerator2")))
        (else
          (switch Utilities|FlowControl|Switch|SwitchonEFadeState (Variables|Default|Getfade%20state)
            (:NewEnumerator0
              (Default|CallOnFadeOutCompleted)
              (Utilities|FlowControl|Delay (Variables|Default|GetWait%20Time))
              (CallFunction|Fadein))
            (:NewEnumerator1
              (Default|CallOnFadeinCompleted)
              (Variables|Default|Setfade%20state "NewEnumerator2"))))))))

(event Custom|Fade%20In%20Out
  (params (delay :type Float%20%28double-precision%29))
  (Variables|Default|SetWait%20Time delay)
  (Variables|Default|Setfull%20loop true)
  (CallFunction|FadeOut))

(event Custom|do%20fade%20out
  (bind _output_get (Variables|Default|Sett (+ (Variables|Default|Gett) (/ (Variables|Default|Getanim%20update%20interval) (Variables|Default|Getanim%20duration)))))
  (CallFunction|UpdateFade _output_get)
  (if true
    _))

(event Custom|Do%20Animation
  (params (time :type Float%20%28double-precision%29) (start :type Float%20%28double-precision%29) (end :type Float%20%28double-precision%29))
  (if (> time 0.0)
    (Variables|Default|SetStart start)
    (Variables|Default|SetEnd end)
    (Variables|Default|Setplaying true)
    (bind _returnvalue (Utilities|Time|SetTimerbyEvent (delegate Custom|do%20fade%20out) (Variables|Default|Getanim%20update%20interval) true))
    (Variables|Default|Setfade%20timer _returnvalue)))

(event Custom|disable%20player%20control)

(event Custom|enable%20player%20control)

(event EventBeginPlay
  (Variables|/Script/Engine.PostProcessComponent|SetBlendWeight (Variables|Default|GetPostProcess) 0.0))

(event Collision|EventActorBeginOverlap
  (params (OtherActor :type Actor%20Object%20Reference)))

(event EventTick
  (params (DeltaSeconds :type Float%20%28single-precision%29)))

(fn ConstructionScript
  (if (Variables|Default|Getpreview)
    (Variables|/Script/Engine.PostProcessComponent|SetBlendWeight (Variables|Default|GetPostProcess) (Variables|Default|Getpreview%20weight))))

(fn UpdateFade
  (params (t :type Float%20%28double-precision%29)))