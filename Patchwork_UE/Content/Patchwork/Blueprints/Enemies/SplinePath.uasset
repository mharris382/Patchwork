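; Spline path actor that gives enemy pawns a route of waypoints.
; It keeps a list of assigned agents, notifying each pawn on assignment, and finds the spline point nearest a world position.
; All agents share the default spline, falling back to the built-in one.
; BeginPlay checks for a PCG graph, but its generated-path loop over spline components has an empty body.
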(event EventBeginPlay
  (Utilities|IsValid (Variables|/Script/PCG.PCGComponent|GetGraphInstance (Variables|Default|GetPCG_Main))
    (:Is%20Valid
      (if (Variables|Default|GetUseGeneratedPath)
        (for _array_element (Actor|GetComponentsByClass "/Script/Engine.SplineComponent")
          _)))
    (:Is%20Not%20Valid
      (Variables|Default|SetDefaultPathSpline (Variables|Default|GetSpline)))))

(event Collision|EventActorBeginOverlap
  (params (OtherActor :type Actor%20Object%20Reference)))

(event EventTick
  (params (DeltaSeconds :type Float%20%28single-precision%29)))

(fn ConstructionScript)

(fn SetAssignedAgent
  (params (Pawn :type Pawn%20Object%20Reference))
  (Utilities|IsValid Pawn
    (:Is%20Valid
      (Utilities|Array|Add (Variables|Default|GetAssignedAgents) Pawn)
      (Class|BPIAgent|SetPath(Message) Pawn self))))

(fn UnassignAgent
  (params (Agent :type Pawn%20Object%20Reference))
  (Utilities|Array|RemoveItem (Variables|Default|GetAssignedAgents) Agent))

(fn CanAgentbeAssigned
  (params (Agent :type Pawn%20Object%20Reference))
  (Utilities|IsValid Agent
    (:Is%20Valid
      (return true))
    (:Is%20Not%20Valid
      (return false))))

(fn GetNearestWaypoint
  (params (Position :type Vector) (Agent :type Pawn%20Object%20Reference))
  (bind _spline (CallFunction|GetAgentPath Agent))
  (LocalVariables|SetsmallestDis 1e+11)
  (for _index (range 0 (- (Spline|GetNumberOfSplinePoints _spline) 1))
    (if (< (Class|KismetMathLibrary|VectorDistanceSquared (Spline|GetLocationatSplinePoint _spline _index "World") Position) (LocalVariables|GetsmallestDis))
      (LocalVariables|SetBestIndex _index)
      (LocalVariables|SetsmallestDis (Class|KismetMathLibrary|VectorDistanceSquared (Spline|GetLocationatSplinePoint _spline _index "World") Position))))
  (return (LocalVariables|GetBestIndex)))

(fn GetAgentPath
  (params (Pawn :type Pawn%20Object%20Reference))
  (bind _defaultpathspline (Variables|Default|GetDefaultPathSpline)
    (:then
      (return _defaultpathspline))
    (:else
      (return (Variables|Default|GetSpline)))))