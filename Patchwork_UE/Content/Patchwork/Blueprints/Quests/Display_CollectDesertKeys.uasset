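; Quest step display for collecting artifacts (desert keys) in the Walled Ruins, supplying progress text out of three.
; CountKeys loops over KeyEventNames and asks the GameMode whether each world event has occurred, tallying those that have.
; GetStepInfo formats that tally into a rich-text step description, so progress derives from world events with no counter stored here.
; The event graph holds only disabled default stubs.
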(event EventBeginPlay
  (|CallParentFunction) ; This node is disabled and will not be called.\nDrag off pins to build functionality.
)

(event Collision|EventActorBeginOverlap
  (params (OtherActor :type Actor%20Object%20Reference)))

(event EventTick
  (params (DeltaSeconds :type Float%20%28single-precision%29)))

(fn ConstructionScript
  (|CallParentFunction))

(fn GetStepInfo
  (bind _keys_collected (CallFunction|CountKeys))
  (return (Utilities|Text|FormatText "Collect Artifacts in Walled Ruins <b>({0}/3)</>" _keys_collected)))

(fn CountKeys
  (LocalVariables|Setcnt 0)
  (for _array_element (Variables|Default|GetKey%20Event%20Names)
    (bind _event_occured (Default|HasWorldEventOccured (Variables|Default|GetGame%20Mode) _array_element))
    (if _event_occured
      (LocalVariables|Setcnt (+ (LocalVariables|Getcnt) 1))))
  (return (LocalVariables|Getcnt)))