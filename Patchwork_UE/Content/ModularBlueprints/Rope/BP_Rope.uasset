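; BP_Rope is a rope actor that can reference an actor for each of its ends, AttachToStart and AttachToEnd.
; The construction script moves each valid referenced actor to the Start or End component's location.
; AttachActorOnConstraint only sorts parent, child and bone variables, never applying them to the constraint.
; Runtime events are empty, and the nodes for spawning physics constraints and attaching components are disconnected.
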(event EventBeginPlay)

(event Collision|EventActorBeginOverlap
  (params (OtherActor :type Actor%20Object%20Reference)))

(event EventTick
  (params (DeltaSeconds :type Float%20%28single-precision%29)))

(fn ConstructionScript
  (bind _attach_to_start (Variables|Default|GetAttach%20to%20Start))
  (bind _attach_to_end (Variables|Default|GetAttach%20to%20End))
  (Utilities|FlowControl|Sequence
    (:then_0
      (Utilities|IsValid _attach_to_start
        (:Is%20Valid
          (Transformation|SetActorLocation _attach_to_start (Transformation|GetWorldLocation (Variables|Default|GetStart)) false false))))
    (:then_1
      (Utilities|IsValid _attach_to_end
        (:Is%20Valid
          (Transformation|SetActorLocation _attach_to_end (Transformation|GetWorldLocation (Variables|Default|GetEnd)) false false))))))

(fn AttachActoronConstraint
  (params (actor :type Actor%20Object%20Reference) (actor%20is%20child :type Boolean) (attach%20bone :type Name) (constraint%20actor :type Physics%20Constraint%20Actor%20Object%20Reference))
  (LocalVariables|Setconstraint constraint%20actor)
  (LocalVariables|Setrope%20bone%20name attach%20bone)
  (Utilities|FlowControl|Sequence
    (:then_0
      (if actor%20is%20child
        (LocalVariables|Setchild%20actor actor)
        (LocalVariables|Setparent%20actor self)
        (LocalVariables|Setparent%20bone (LocalVariables|Getrope%20bone%20name))
        (else
          (LocalVariables|Setchild%20actor self)
          (LocalVariables|Setparent%20actor actor)
          (LocalVariables|Setchild%20bone (LocalVariables|Getrope%20bone%20name)))))))