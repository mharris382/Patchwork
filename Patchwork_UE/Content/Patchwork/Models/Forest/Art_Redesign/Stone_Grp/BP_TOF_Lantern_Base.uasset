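; BP_TOF_Lantern_Base is a lantern Blueprint, apparently a base for forest stone props, pairing a point light with a Niagara fire effect.
; The construction script applies exposed settings to the light's attenuation radius and indirect lighting intensity, then passes color and size to the fire effect.
; It overrides the parent's GetLight to return its point light, and its event graph has no active logic.
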(event EventBeginPlay)

(event Collision|EventActorBeginOverlap
  (params (OtherActor :type Actor%20Object%20Reference)))

(event EventTick
  (params (DeltaSeconds :type Float%20%28single-precision%29)))

(fn ConstructionScript
  (bind _pointlight (Variables|Default|GetPointLight))
  (bind _ns_firespeedrun (Variables|Default|GetNS_FireSpeedrun))
  (|CallParentFunction)
  (Utilities|FlowControl|Sequence
    (:then_0
      (Rendering|Lighting|SetAttenuationRadius _pointlight (Variables|Default|GetAttentionRadius))
      (Class|LightComponent|SetIndirectLightingIntensity _pointlight (Variables|Default|GetIndirect%20Lighting%20Intensity)))
    (:then_1
      (Niagara|SetNiagaraVariable(LinearColor) _ns_firespeedrun "Color" (Variables|Default|GetLight%20Color))
      (Niagara|SetNiagaraVariable(Float) _ns_firespeedrun "Size" (Variables|Default|GetFireSize)))))

(fn GetLight
  (|CallParentFunction)
  (return (Variables|Default|GetPointLight)))