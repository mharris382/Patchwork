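; Component that holds an actor's gameplay state as a gameplay tag container, including spore effect tags.
; Add and remove functions edit the container and broadcast OnGameplayStateChanged so listeners can react.
; Adding rejects exact duplicates of SporeEffects.EffectType tags with a red debug message; other tags skip that check.
; Getters expose the component and its tags, and PrintTags outputs the owner's current state for debugging.
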(event EventBeginPlay)

(event EventTick
  (params (DeltaSeconds :type Float%20%28single-precision%29)))

(fn RemoveGameplayTag
  (params (Tag :type Gameplay%20Tag%20Structure))
  (bind _returnvalue (GameplayTags|RemoveGameplayTag (Variables|Default|GetGameplayState) Tag :!class /Script/GameplayTags.BlueprintGameplayTagLibrary))
  (if _returnvalue
    (Default|CallOnGameplayStateChanged (Variables|Default|GetGameplayState))))

(fn AddGameplayTag
  (params (Tag :type Gameplay%20Tag%20Structure))
  (if (GameplayTags|MatchesTag Tag "(TagName=\"SporeEffects.EffectType\")")
    (if (GameplayTags|HasTag (Variables|Default|GetGameplayState) Tag true)
      (Development|PrintText (Utilities|Text|FormatText "tried to add the same spore effect {0}  more than once.  BAD COMPUTER!" (GameplayTags|GetTagName Tag)) true true "(R=1.000000,G=0.000000,B=0.000000,A=1.000000)")
      (else
        (GameplayTags|AddGameplayTag (Variables|Default|GetGameplayState) Tag :!class /Script/GameplayTags.BlueprintGameplayTagLibrary :!label _label)
        (Default|CallOnGameplayStateChanged (Variables|Default|GetGameplayState) (Components|GetOwner))))
    (else
      (goto _label))))

(fn PrintTags
  (params (bPrintToScreen :type Boolean) (bPrintToLog :type Boolean) (TextColor :type Linear%20Color%20Structure :default "(R=0.000000,G=1.000000,B=0.323809,A=1.000000)") (Duration :type Float%20%28single-precision%29))
  (Utilities|FlowControl|Sequence
    (:then_0
      (LocalVariables|Setstring (Utilities|String|Append "Actor State for " (Utilities|GetDisplayName (Components|GetOwner)) "= ")))
    (:then_1
      (for _array_element (GameplayTags|BreakGameplayTagContainer (Variables|Default|GetGameplayState))
        (LocalVariables|Setstring (Utilities|String|Append (LocalVariables|Getstring) (Utilities|String|ToString(Name) (GameplayTags|GetTagName _array_element)) ",  ")))
      (Development|PrintString (LocalVariables|Getstring) bPrintToScreen bPrintToLog TextColor Duration))))

(fn GetGameplayStateComponent
  (return self))

(fn GetGameplayStateTags
  (return (Variables|Default|GetGameplayState)))