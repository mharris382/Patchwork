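; Dreamwalker decal spawner that, as written, only locates tagged components on its owner and does not yet spawn a decal.
; On BeginPlay, SetupDecal searches the owner for static mesh and Niagara components carrying TargetTag.
; When both exist, it caches the first of each as Sm and Vfx, then runs an empty sequence.
; The cached references drive nothing further, and Tick is disabled.
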(event Custom|SetupDecal
  (bind _returnvalue (Components|GetOwner))
  (bind _targettag (Variables|Default|GetTargetTag))
  (bind _targettag_2 (Variables|Default|GetTargetTag))
  (bind _returnvalue_2 (Actor|GetComponentsbyTag _returnvalue "/Script/Niagara.NiagaraComponent" _targettag))
  (bind _returnvalue_3 (Actor|GetComponentsbyTag _returnvalue "/Script/Engine.StaticMeshComponent" _targettag_2))
  (if (and (> (Utilities|Array|Length _returnvalue_3) 0) (> (Utilities|Array|Length _returnvalue_2) 0))
    (Variables|Default|Setsm (Utilities|Array|Get(acopy) _returnvalue_3))
    (Variables|Default|Setvfx (Utilities|Array|Get(acopy) _returnvalue_2))
    (Utilities|FlowControl|Sequence)))

(event EventBeginPlay
  (CallFunction|SetupDecal))

(event EventTick
  (params (DeltaSeconds :type Float%20%28single-precision%29)))