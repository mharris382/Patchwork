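; BP_ChangeMusic is an overlap-driven actor that switches the music track as the player pawn enters it.
; On begin overlap it passes MusicTrack to the level's BP_DynamicAudioController, and on end overlap it passes ExitMusicTrack if SetMusicOnExit is enabled.
; A helper with Is Valid outputs finds and caches that controller, starting at BeginPlay, and prints a warning when none exists in the level.
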(event EventBeginPlay
  (Utilities|GetDynamicAudio))

(event Collision|EventActorBeginOverlap
  (params (OtherActor :type Actor%20Object%20Reference))
  (if (== OtherActor (Game|Player|GetPlayerPawn 0))
    (bind _dynamic_audio (Utilities|GetDynamicAudio)
      (:Is%20Valid
        (Default|ChangeMusicTrack _dynamic_audio (Variables|Default|GetMusic%20Track))))))

(event Collision|EventActorEndOverlap
  (params (OtherActor :type Actor%20Object%20Reference))
  (if (and (Variables|Default|Getset%20music%20on%20exit) (== OtherActor (Game|Player|GetPlayerPawn 0)))
    (bind _dynamic_audio (Utilities|GetDynamicAudio)
      (:Is%20Valid
        (Default|ChangeMusicTrack _dynamic_audio (Variables|Default|GetExit%20Music%20Track))))))

(fn ConstructionScript)