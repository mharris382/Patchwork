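; Hanging mushroom actor for the procedural Inverted Forest, which overrides its parent's bounds query to fit the space above it.
; GetBoundsMinMax traces straight up on the Visibility channel and stretches the box height slightly past the hit, dividing by the actor's Z scale to compensate for scaling.
; Without a hit it returns a fixed default box; the event graph holds no active logic.
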(event EventBeginPlay
  (|CallParentFunction) ; This node is disabled and will not be called.\nDrag off pins to build functionality.
)

(event Collision|EventActorBeginOverlap
  (params (OtherActor :type Actor%20Object%20Reference))
  (|CallParentFunction OtherActor) ; This node is disabled and will not be called.\nDrag off pins to build functionality.
)

(event EventTick
  (params (DeltaSeconds :type Float%20%28single-precision%29))
  (|CallParentFunction DeltaSeconds) ; This node is disabled and will not be called.\nDrag off pins to build functionality.
)

(fn ConstructionScript
  (|CallParentFunction))

(fn GetBoundsMinMax
  (bind _returnvalue (Transformation|GetActorLocation))
  (|CallParentFunction)
  (bind (_outhit _returnvalue_2) (Collision|LineTraceByChannel _returnvalue (+ _returnvalue (* (Math|Vector|VectorUp) 5e+05)) "TraceTypeQuery1" false 0 "None"))
  (bind _output_get (Variables|PCGINTERNAL|SetValid _returnvalue_2))
  (if _output_get
    (bind _output_get_2 (Variables|PCGINTERNAL|SetImpactDistance (.Distance (Collision|BreakHitResult _outhit))))
    (return "-100.000000,-100.000000,0.000000" (Math|Vector|MakeVector 1e+02 1e+02 (/ (+ _output_get_2 1e+02) (.z (Transformation|GetActorScale3D)))))
    (else
      (return "-100.000000,-100.000000,0.000000" "100.000000,100.000000,1000.000000"))))