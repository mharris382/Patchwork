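; Fog controller actor that moves a referenced Fog actor vertically according to the player pawn's height.
; Each tick, while enabled, the pawn's Z is normalized between min and max heights, shaped by a curve, and lerped between the offset bounds.
; The construction script takes the bounds from position properties and previews the fog at a simulated height.
; Up/down speed smoothing exists but is unconnected, so the fog snaps directly.
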(event EventBeginPlay
  (bind _returnvalue (Game|Player|GetPlayerPawn 0))
  (Actor|Tick|SetActorTickEnabled (Variables|Default|Getenabled))
  (Utilities|FlowControl|Delay 0.1)
  (Utilities|IsValid _returnvalue
    (:Is%20Valid
      (Variables|Default|Setcurrent (.z (Transformation|GetActorLocation _returnvalue))))))

(event Collision|EventActorBeginOverlap
  (params (OtherActor :type Actor%20Object%20Reference)))

(event EventTick
  (params (DeltaSeconds :type Float%20%28single-precision%29))
  (bind _returnvalue (Game|Player|GetPlayerPawn 0))
  (if (Variables|Default|Getenabled)
    (Utilities|IsValid _returnvalue
      (:Is%20Valid
        (CallFunction|UpdateFogfromZ DeltaSeconds (.z (Transformation|GetActorLocation _returnvalue)) false)))))

(fn ConstructionScript
  (if (Variables|Default|Getenabled)
    (Variables|Default|SetMin%20Height (.z (Variables|Default|Getmin%20position)))
    (Variables|Default|SetMax%20Height (.z (Variables|Default|Getmax%20position)))
    (CallFunction|UpdateFogfromZ 0.0 (.Z (Math|Vector|BreakVector (Variables|Default|Getsimulated%20height))) false)))

(fn GetFogHeightfromPosition
  (params (height :type Float%20%28double-precision%29))
  (bind _max_height (Variables|Default|GetMax%20Height))
  (bind _min_height (Variables|Default|GetMin%20Height))
  (return (Math|Float|Lerp (+ (Variables|Default|GetMax%20Height%20Offset) _max_height) (+ _min_height (Variables|Default|GetMin%20Height%20Offset)) (Math|Curves|GetFloatValue (Variables|Default|GetHeight%20Curve) (Math|Float|MapRangeClamped height _max_height _min_height 0.0 1.0)))))

(fn UpdateFogHeight
  (params (Value :type Float%20%28double-precision%29))
  (bind _fog (Variables|Default|GetFog)
    (:then
      (Transformation|SetActorLocation _fog (Math|Vector|MakeVector (.X (Math|Vector|BreakVector (Transformation|GetActorLocation _fog))) (.Y (Math|Vector|BreakVector (Transformation|GetActorLocation _fog))) (CallFunction|GetFogHeightfromPosition (Math|Float|MapRangeClamped Value 0.0 1.0 (Variables|Default|GetMin%20Height) (Variables|Default|GetMax%20Height)))) false false))
    (:else)))

(fn UpdateFogfromZ
  (params (dt :type Float%20%28double-precision%29) (height :type Float%20%28double-precision%29) (is%20editor :type Boolean))
  (bind _fog (Variables|Default|GetFog)
    (:then
      (Transformation|SetActorLocation _fog (Math|Vector|MakeVector (.X (Math|Vector|BreakVector (Transformation|GetActorLocation _fog))) (.Y (Math|Vector|BreakVector (Transformation|GetActorLocation _fog))) (CallFunction|GetFogHeightfromPosition height)) false false))
    (:else)))