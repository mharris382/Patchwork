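; BP_Cliffs_2 is a cliff actor Blueprint in the PCG Cliffs set that computes the bounds of a scaled cliff assembly.
; Its construction script sets bounds padding from assembly extents times cliff scale before running the parent script, then derives generation min and max bounds from extents, pivot offset and scale.
; It overrides the vertical bounds height getter to return its Height variable, and its event graph has no active logic.
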(event EventBeginPlay
  (|CallParentFunction) ; This node is disabled and will not be called.\nDrag off pins to build functionality.
)

(event Collision|EventActorBeginOverlap
  (params (OtherActor :type Actor%20Object%20Reference))
  (|CallParentFunction OtherActor) ; This node is disabled and will not be called.\nDrag off pins to build functionality.
)

(event EventTick
  (params (DeltaSeconds :type Float%20%28single-precision%29))
  (|CallParentFunction DeltaSeconds) ; This node is disabled and will not be called.\nDrag off pins to build functionality.
)

(fn ConstructionScript
  (bind _cliffassemblyextents (Variables|01-Cliffs|Size|GetCliffAssemblyExtents))
  (bind _cliffscale (Variables|01-Cliffs|Size|GetCliffScale))
  (bind _cliffpivotoffset (Variables|01-Cliffs|Size|GetCliffPivotOffset))
  (bind (_min _max) (CallFunction|GetAssemblyBoundsMinMax _cliffassemblyextents _cliffpivotoffset _cliffscale))
  (Variables|Default|SetBoundsPadding (* (Variables|01-Cliffs|Size|GetCliffAssemblyExtents) (Variables|01-Cliffs|Size|GetCliffScale)))
  (|CallParentFunction)
  (Utilities|FlowControl|Sequence
    (:then_0
      ;[0.6233 0.6233 0.6233 0.5] Bounds
      (Variables|PCGINTERNAL|SetGEN_BoundsMin _min)
      (Variables|PCGINTERNAL|SetGEN_BoundsMax _max))))

(fn GetBoundsVerticalHeight
  (return (Variables|01-Cliffs|GetHeight)))