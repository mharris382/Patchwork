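; BP_InvisibleWalls is an environment actor whose child components act as invisible walls, visible in the editor when ShowWallsInEditor is set.
; The construction script applies that editor visibility to the InvisibleWalls root and its children.
; BeginPlay hides them and sets the default collision type on each direct child primitive component.
; SetInvisibleWallCollisions can switch that collision type for all direct child walls.
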(event EventBeginPlay
  (Utilities|SetWallVisibility false)
  (CallFunction|SetInvisibleWallCollisions (Variables|Default|GetDefault%20Invisible%20wall%20collsion)))

(event Collision|EventActorBeginOverlap
  (params (OtherActor :type Actor%20Object%20Reference)))

(event EventTick
  (params (DeltaSeconds :type Float%20%28single-precision%29)))

(fn ConstructionScript
  (Utilities|SetWallVisibility (Variables|Default|GetShow%20walls%20in%20editor)))

(fn SetInvisibleWallCollisions
  (params (NewType :type ECollisionEnabled%20Enum :default "NoCollision"))
  (for _array_element (Components|GetChildrenComponents (Variables|Default|GetInvisible%20Walls) false)
    (bind _asprimitive_component (Utilities|Casting|CastToPrimitiveComponent _array_element))
    (Collision|SetCollisionEnabled _asprimitive_component NewType)))