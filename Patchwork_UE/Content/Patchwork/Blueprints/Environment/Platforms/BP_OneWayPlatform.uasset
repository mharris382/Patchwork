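; One-way platform actor whose Blueprint graphs only fit Niagara effects to the platform meshes, with no gameplay logic.
; The construction script scans all descendants of the OneWayPlatform component for Niagara components attached to static meshes.
; Each effect gets its "Box Size" parameter set to half the parent mesh's local bounds size.
; Its relative scale is reset to one.
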(event EventBeginPlay)

(event Collision|EventActorBeginOverlap
  (params (OtherActor :type Actor%20Object%20Reference)))

(event EventTick
  (params (DeltaSeconds :type Float%20%28single-precision%29)))

(fn ConstructionScript
  (for _array_element (Components|GetChildrenComponents (Variables|Default|GetOneWayPlatform) true)
    (bind _asniagara_particle_system_component (Utilities|Casting|CastToNiagaraComponent _array_element))
    (bind _asstatic_mesh_component (Utilities|Casting|CastToStaticMeshComponent (Transformation|GetAttachParent _asniagara_particle_system_component)))
    (Effects|Components|ParticleSystem|SetVectorParameter _asniagara_particle_system_component "Box Size" (/ (- (.Max (Components|StaticMesh|GetLocalBounds _asstatic_mesh_component)) (.Min (Components|StaticMesh|GetLocalBounds _asstatic_mesh_component))) 2.0))
    (Transformation|SetRelativeScale3D _asniagara_particle_system_component "1.000000,1.000000,1.000000")))