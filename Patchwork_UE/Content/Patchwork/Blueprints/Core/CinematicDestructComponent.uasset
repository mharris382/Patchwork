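; Actor component that triggers a cinematic destruction effect using a pre-placed Geometry Collection actor.
; On BeginPlay it caches that actor's Geometry Collection component, then deactivates and hides it.
; CineDestruct moves the collection actor to the target actor's location and rotation, then activates and reveals the component.
; A spawn-class check leads to no logic, and the UsePooled variable is unused.
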(event Custom|CineDestruct
  (bind _target_geometry_collection_component (Variables|Default|GetTarget%20Geometry%20Collection%20Component))
  (bind _targetactor (Variables|Default|GetTargetActor))
  (Utilities|FlowControl|Sequence
    (:then_0
      (bind _geometrycollectionactor (Variables|Default|GetGeometryCollectionActor)
        (:then
          (Transformation|SetActorLocationAndRotation _geometrycollectionactor (Transformation|GetActorLocation _targetactor) (Transformation|GetActorRotation _targetactor))
          (Components|Activation|SetActive _target_geometry_collection_component true true)
          (Rendering|SetVisibility _target_geometry_collection_component true true))
        (:else)))
    (:then_2
      (if (Utilities|IsValidClass (Variables|Default|GetSpawnActor))
        _))))

(event EventBeginPlay
  (bind _geometrycollectionactor (Variables|Default|GetGeometryCollectionActor))
  (bind _geometrycollectioncomponent (Variables|/Script/GeometryCollectionEngine.GeometryCollectionActor|GetGeometryCollectionComponent _geometrycollectionactor))
  (Utilities|IsValid _geometrycollectionactor
    (:Is%20Valid
      (Utilities|IsValid _geometrycollectioncomponent
        (:Is%20Valid
          (Variables|Default|SetTarget%20Geometry%20Collection%20Component _geometrycollectioncomponent)
          (Components|Activation|SetActive (Variables|Default|GetTarget%20Geometry%20Collection%20Component) false true)
          (Rendering|SetVisibility (Variables|Default|GetTarget%20Geometry%20Collection%20Component) false false))))))

(event EventTick
  (params (DeltaSeconds :type Float%20%28single-precision%29)))