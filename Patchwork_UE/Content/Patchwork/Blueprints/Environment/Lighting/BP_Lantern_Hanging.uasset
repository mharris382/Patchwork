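; BP_Lantern_Hanging is a hanging lantern environment prop built from a stable mesh, a lantern and a physics constraint.
; The construction script sets the constraint's linear Z motion to Limited, sized to the world distance between StableMesh and Lantern, so the hang length follows their placement.
; The event graph holds only disabled default events, so the Blueprint adds no runtime logic.
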(event EventBeginPlay
  (|CallParentFunction) ; This node is disabled and will not be called.\nDrag off pins to build functionality.
)

(event Collision|EventActorBeginOverlap
  (params (OtherActor :type Actor%20Object%20Reference))
  (|CallParentFunction OtherActor) ; This node is disabled and will not be called.\nDrag off pins to build functionality.
)

(event EventTick
  (params (DeltaSeconds :type Float%20%28single-precision%29))
  (|CallParentFunction DeltaSeconds) ; This node is disabled and will not be called.\nDrag off pins to build functionality.
)

(fn ConstructionScript
  (|CallParentFunction)
  (Class|PhysicsConstraintComponent|SetLinearZLimit (Variables|Default|GetPhysicsConstraint) "LCM_Limited" (Math|Vector|Distance(Vector) (Transformation|GetWorldLocation (Variables|Default|Getstable%20mesh)) (Transformation|GetWorldLocation (Variables|Default|Getlantern)))))