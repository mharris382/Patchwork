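; Scene component that kills the player when fully submerged in its owning actor's volume, such as water.
; The owner's overlap events toggle an "InWater" tag on the player pawn and start or stop a looping timer, used instead of Tick.
; The timer compares the component's world Z with the top of the player's capsule, using a cached half height, and calls the game mode's FadeAndKill once the component is higher.
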(event Custom|OnOverlapBegin
  (params (OverlappedActor :type Actor%20Object%20Reference) (OtherActor :type Actor%20Object%20Reference))
  (bind _returnvalue (Game|Player|GetPlayerPawn 0))
  (if (== OtherActor _returnvalue)
    (Utilities|Array|AddUnique (Variables|/Script/Engine.Actor|GetTags _returnvalue) "InWater")
    (Utilities|Time|ClearandInvalidateTimerbyHandle (Variables|Default|GetTimerHandle))
    (bind _returnvalue_2 (Utilities|Time|SetTimerbyEvent (delegate Custom|TrackPlayerUnderwater) 0.1 true true))
    (Variables|Default|SetTimerHandle _returnvalue_2)))

(event Custom|TrackPlayerUnderwater
  (if (> (.Z (Math|Vector|BreakVector (Transformation|GetWorldLocation))) (+ (.Z (Math|Vector|BreakVector (Transformation|GetActorLocation (Game|Player|GetPlayerPawn 0)))) (Variables|Default|GetHalf%20Height)))
    (Default|FadeandKill (CallFunction|GetBaseGameMode))
    (CallFunction|StopTracking)))

(event Custom|CustomEvent
  (params (OverlappedActor :type Actor%20Object%20Reference) (OtherActor :type Actor%20Object%20Reference))
  (if (== OtherActor (Game|Player|GetPlayerPawn 0))
    (CallFunction|StopTracking)
    (Utilities|Array|RemoveItem (Variables|/Script/Engine.Actor|GetTags (Game|Player|GetPlayerPawn 0)) "InWater")))

(event Custom|StopTracking
  (Utilities|Time|ClearandInvalidateTimerbyHandle (Variables|Default|GetTimerHandle)))

(event EventBeginPlay
  (bind _returnvalue (Components|GetOwner))
  (Collision|BindEventtoOnActorBeginOverlap _returnvalue (delegate Custom|OnOverlapBegin))
  (Collision|BindEventtoOnActorEndOverlap _returnvalue (delegate Custom|CustomEvent))
  (bind _ascharacter (Utilities|Casting|CastToCharacter (Game|Player|GetPlayerPawn 0)))
  (bind _halfheight (Class|BPIPlayerPawn|GetPlayerHalfHeight(Message) _ascharacter))
  (Variables|Default|SetHalf%20Height _halfheight))

(event EventTick
  (params (DeltaSeconds :type Float%20%28single-precision%29)))