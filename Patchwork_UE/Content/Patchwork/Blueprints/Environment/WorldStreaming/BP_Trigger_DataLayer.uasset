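; Trigger actor that switches World Partition data layer runtime states when the player pawn overlaps it.
; On overlap it gets the Data Layer Manager and passes three layer arrays, Unloaded, Loaded and Activated, to a shared helper in that order.
; The helper sets each valid layer asset to the target state, with the Unloaded pass relying on the default state value.
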(event EventBeginPlay)

(event Collision|EventActorBeginOverlap
  (params (OtherActor :type Actor%20Object%20Reference))
  (if (== OtherActor (Game|Player|GetPlayerPawn 0))
    (bind _returnvalue (WorldPartition|GetDataLayerManager))
    (Utilities|IsValid _returnvalue
      (:Is%20Valid
        (CallFunction|SetDataLayerStates _returnvalue (Variables|Default|GetUnloaded) "Unloaded" false)
        (CallFunction|SetDataLayerStates _returnvalue (Variables|Default|GetLoaded) "Loaded" false)
        (CallFunction|SetDataLayerStates _returnvalue (Variables|Default|GetActivated) "Activated" false)))))

(event EventTick
  (params (DeltaSeconds :type Float%20%28single-precision%29)))

(fn ConstructionScript)

(fn SetDataLayerStates
  (params (DL%20manager :type Data%20Layer%20Manager%20Object%20Reference) (Layers :type Array%20of%20Data%20Layer%20Asset%20Object%20References) (Target%20State :type EDataLayerRuntimeState%20Enum :default "Unloaded") (bInIsRecursive :type Boolean))
  (LocalVariables|Setstate Target%20State)
  (for _array_element Layers
    (Utilities|IsValid _array_element
      (:Is%20Valid
        (DataLayers|SetDataLayerRuntimeState DL%20manager _array_element (LocalVariables|Getstate) bInIsRecursive :!class /Script/Engine.DataLayerManager)))))