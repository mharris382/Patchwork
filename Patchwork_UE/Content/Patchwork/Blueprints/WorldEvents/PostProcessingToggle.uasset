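; World event Blueprint that switches between day and night post-processing by animating the blend weights of two post-process objects.
; BeginPlay starts with day at full weight and night at zero.
; SetSwitchValue stops one of two timelines and plays the other from the start, one for on and one for off.
; Each timeline drives both weights from its own curves, so interrupted blends restart rather than reverse.
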(event EventBeginPlay
  (Variables|/Script/Engine.PostProcessVolume|SetBlendWeight (Variables|Default|GetDay%20Post%20Process) 1.0)
  (Variables|/Script/Engine.PostProcessVolume|SetBlendWeight (Variables|Default|GetNight%20Post%20Process) 0.0))

(event EventSetSwitchValue
  (params (is%20On :type Boolean))
  (if is%20On
    (Utilities|FlowControl|Sequence
      (:then_0
        (bind (_direction _day_volume _night_volume) (Timeline|Timeline Stop)
          (:Update
            (Variables|/Script/Engine.PostProcessVolume|SetBlendWeight (Variables|Default|GetDay%20Post%20Process) _day_volume)
            (Variables|/Script/Engine.PostProcessVolume|SetBlendWeight (Variables|Default|GetNight%20Post%20Process) _night_volume))))
      (:then_1
        (bind (_direction_2 _night _day) (Timeline|Timeline_0 PlayFromStart)
          (:Update
            (Variables|/Script/Engine.PostProcessVolume|SetBlendWeight (Variables|Default|GetDay%20Post%20Process) _day)
            (Variables|/Script/Engine.PostProcessVolume|SetBlendWeight (Variables|Default|GetNight%20Post%20Process) _night)))))
    (else
      (Utilities|FlowControl|Sequence
        (:then_0
          (Timeline|Timeline_0 Stop))
        (:then_1
          (Timeline|Timeline PlayFromStart))))))

(fn ConstructionScript)