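; Mushroom ability that throws a projectile to place a bouncy mushroom, with throw strength charged by holding the Ability 1 input.
; Hold time, capped at a maximum, interpolates launch speed between min and max; release or cancel triggers the throw.
; One mushroom is pre-spawned far below the world and pooled: each throw destroys the previous projectile, despawns the mushroom and hands it to the new projectile.
; The projectile's spawn event updates the tracked mushroom.
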(event Custom|Throw%20Mushroom
  (bind _current_spawned_mushroom (Variables|Default|Getcurrent%20spawned%20mushroom))
  (bind _current_spawned_mushroom_2 (Variables|Default|Getcurrent%20spawned%20mushroom))
  (Utilities|FlowControl|Sequence
    (:then_0
      ;[1 1 1] Cleanup previous projectiles and mushrooms
      (Utilities|IsValid (Variables|Default|Getlast%20projectile)
        (:Is%20Valid
          (EventDispatchers|UnbindEventfromOnMushroomSpawned (Variables|Default|Getlast%20projectile) (delegate Custom|On%20Mushroom%20Spawned))
          (Actor|DestroyActor (Variables|Default|Getlast%20projectile))
          (Variables|Default|Setlast%20projectile 0))))
    (:then_1
      (Utilities|IsValid _current_spawned_mushroom
        (:Is%20Valid
          (Default|Despawn _current_spawned_mushroom))))
    (:then_2
      ;[1 1 1] Throw new projectile
      (bind _returnvalue (Game|SpawnActorfromClass "/Game/Patchwork/Blueprints/Pawns/Abilities/BP_Mushroom_Projectile.BP_Mushroom_Projectile_C" (Transformation|GetWorldTransform) "Undefined" "MultiplyWithRoot" 0 0))
      (bind _output_get (Variables|Default|Setlast%20projectile _returnvalue))
      (Utilities|FlowControl|Sequence
        (:then_0
          (Utilities|IsValid _current_spawned_mushroom_2
            (:Is%20Valid
              (Default|AssignPooledBouncer _output_get _current_spawned_mushroom_2))))
        (:then_1
          (EventDispatchers|BindEventtoOnMushroomSpawned _output_get (delegate Custom|On%20Mushroom%20Spawned))
          (Variables|/Script/Engine.ProjectileMovementComponent|SetInitialSpeed (Variables|/Game/Patchwork/Blueprints/Pawns/Abilities/BP_Mushroom_Projectile.BP_Mushroom_Projectile_C|GetProjectileMovement _output_get) (CallFunction|GetThrowVelocity)))))))

(event Custom|On%20Mushroom%20Spawned
  (params (mushroom :type BP%20Bouncy%20Mushroom%20Object%20Reference))
  ;[1 1 1] Throw new projectile
  (Variables|Default|Setcurrent%20spawned%20mushroom mushroom))

(event Input|EnhancedActionEvents|EnhancedInputActionIA_Ability_1
  (params (ActionValue :type Boolean) (ElapsedSeconds :type Float%20%28double-precision%29) (TriggeredSeconds :type Float%20%28double-precision%29) (InputAction :type Input%20Action%20Object%20Reference :default "/Game/Patchwork/Data/Input/IA_Ability_1.IA_Ability_1"))
  (:Started
    (Variables|Default|Sethold%20time 0.0)
    (Variables|Default|Setis%20holding true)
    (Default|CallOnAbilityStarted))
  (:Ongoing
    (Variables|Default|Sethold%20time (Math|Float|Min(Float) ElapsedSeconds (Variables|Default|Getmax%20hold%20time))))
  (:Canceled
    (Variables|Default|Setis%20holding false :!label _label)
    (Default|CallOnAbilityCompleted)
    (CallFunction|ThrowMushroom))
  (:Completed
    (goto _label)))

(event EventBeginPlay
  (bind _returnvalue (Game|SpawnActorfromClass "/Game/Patchwork/Blueprints/Pawns/Abilities/BP_Bouncy_Mushroom.BP_Bouncy_Mushroom_C" (Math|Transform|MakeTransform "0.000000,0.000000,-10000000.000000") "Undefined" "MultiplyWithRoot" 0 0))
  (Variables|Default|Setcurrent%20spawned%20mushroom _returnvalue))

(event EventTick
  (params (DeltaSeconds :type Float%20%28single-precision%29)))

(fn GetThrowPowerPercent
  (return (/ (Variables|Default|Gethold%20time) (Variables|Default|Getmax%20hold%20time))))

(fn GetThrowVelocity
  (return (Math|Float|Lerp (Variables|Default|Getmin%20throw%20velocity) (Variables|Default|Getmax%20throw%20velocity) (CallFunction|GetThrowPowerPercent))))