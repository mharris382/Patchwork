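; BP_PCG_CurvedPillar is an actor, by name a PCG curved pillar, whose construction script fits a Cube component to the pillar's height.
; CellSize times SizeZ gives the height, placing the cube at half height and scaling it by that height over 50, times BlockingCubeScale.
; X and Y are zeroed in both vectors, leaving SizeX and SizeY unused.
; The event graph has no active logic.
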(event EventBeginPlay)

(event Collision|EventActorBeginOverlap
  (params (OtherActor :type Actor%20Object%20Reference)))

(event EventTick
  (params (DeltaSeconds :type Float%20%28single-precision%29)))

(fn ConstructionScript
  (bind _cell_size (Variables|Default|GetCell%20Size))
  (bind _size_z (Variables|Default|GetSize%20Z))
  (bind _returnvalue (Math|Conversions|ToFloat(Integer) _size_z))
  (bind _returnvalue_2 (Math|Vector|MakeVector 0.0 0.0 _returnvalue))
  (bind _returnvalue_3 (* _cell_size _returnvalue_2))
  (Transformation|SetRelativeLocation (Variables|Default|GetCube) (/ _returnvalue_3 (Math|Vector|MakeVector 2.0 2.0 2.0)) false false)
  (Transformation|SetRelativeScale3D (Variables|Default|GetCube) (* (/ _returnvalue_3 (Math|Vector|MakeVector 5e+01 5e+01 5e+01)) (Variables|Default|GetBlocking%20Cube%20Scale%20))))