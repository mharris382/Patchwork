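; Trigger actor that fires Chaos field forces once, presumably to break geometry collections, when the player pawn overlaps it.
; PlayForces activates each valid Forces actor's field system and calls its CETrigger; SpawnForcesOnSimulate also fires it shortly after BeginPlay.
; The construction script sizes the Box from BoxSize.
; Logic for spawning forces at SpawnPoints and auto-finding geometry collections is present but disconnected.
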(event Custom|PlayForces
  (Utilities|FlowControl|DoOnce false
    (:Completed
      (for _array_element (Variables|Default|GetForces)
        (Utilities|IsValid _array_element
          (:Is%20Valid
            (Components|Activation|Activate (Variables|/Script/FieldSystemEngine.FieldSystemActor|GetFieldSystemComponent _array_element) false)
            (Default|CETrigger _array_element)))))))

(event EventBeginPlay
  (if (Variables|Default|GetSpawnForcesOnSimulate)
    (Utilities|FlowControl|Delay 2.0)
    (CallFunction|PlayForces)))

(event Collision|EventActorBeginOverlap
  (params (OtherActor :type Actor%20Object%20Reference))
  (if (== OtherActor (Game|Player|GetPlayerPawn 0))
    (CallFunction|PlayForces)))

(event EventTick
  (params (DeltaSeconds :type Float%20%28single-precision%29)))

(fn ConstructionScript
  (Utilities|FlowControl|Sequence
    (:then_2
      (Components|Box|SetBoxExtent (Variables|Default|GetBox) (/ (Variables|Default|GetBoxSize) 2.0) true))))