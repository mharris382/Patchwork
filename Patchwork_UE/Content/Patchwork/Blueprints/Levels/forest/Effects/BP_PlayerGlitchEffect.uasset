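; Toxicity-driven effect that makes its owner glitch-teleport at random intervals while toxicity is above a threshold.
; For players, the timer starts the glitch post-process, whose OnGlitch event performs the teleport; other owners teleport immediately.
; An overlapping BP_GlitchPortal supplies the destination; otherwise the owner makes a swept random horizontal jump with distance scaled by toxicity.
; Each glitch re-rolls the next delay from a random stream.
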(event Custom|Trigger%20Glitch
  (bind _returnvalue (Components|GetOwner))
  (bind _overlappingactors (Collision|GetOverlappingActors _returnvalue "/Game/Patchwork/Blueprints/Levels/forest/BP_GlitchPortal.BP_GlitchPortal_C" :!class /Script/Engine.Actor))
  (if (> (Utilities|Array|Length _overlappingactors) 0)
    (bind _asbp_glitch_portal (Utilities|Casting|CastToBP_GlitchPortal (Utilities|Array|Get(acopy) _overlappingactors))
      (:then
        (bind _location (Default|GetGlitchLocation _asbp_glitch_portal))
        (Transformation|SetActorLocationAndRotation (Components|GetOwner) (.location _location) (.rotation _location) false true))
      (:CastFailed
        (CallFunction|TriggerRandomGlitchonTerrain :!label _label)))
    (else
      (goto _label)))
  (Variables|Default|SetTime%20Until%20Next%20Glitch (Math|Random|RandomFloatinRangefromStream (Variables|Default|GetRandom%20Stream) (Variables|Default|GetMin%20Time%20Between%20Glitches) (Variables|Default|GetMax%20Time%20Between%20Glitches)))
  (Variables|Default|Setglitching false))

(event EventBeginPlay
  (|CallParentFunction)
  (bind _asbp_glitch_post_processing (Utilities|Casting|CastToBP_GlitchPostProcessing (Variables|Default|GetSpore%20Post%20Processing)))
  (EventDispatchers|BindEventtoOnGlitch _asbp_glitch_post_processing (delegate Custom|Trigger%20Glitch)))

(event EventTick
  (params (DeltaSeconds :type Float%20%28single-precision%29))
  (bind _returnvalue (Components|GetOwner))
  (bind _overlappingactors (Collision|GetOverlappingActors _returnvalue "/Game/Patchwork/Blueprints/Levels/forest/BP_GlitchPortal.BP_GlitchPortal_C" :!class /Script/Engine.Actor))
  (|CallParentFunction DeltaSeconds)
  (if (and (CallFunction|AbletoGlitch) (not (Variables|Default|Getglitching)))
    (bind _output_get (Variables|Default|SetTime%20Until%20Next%20Glitch (- (Variables|Default|GetTime%20Until%20Next%20Glitch) DeltaSeconds)))
    (if (<= _output_get 0.0)
      (Variables|Default|Setglitching true)
      (if (Variables|Default|GetIs%20Player)
        (bind _asbp_glitch_post_processing (Utilities|Casting|CastToBP_GlitchPostProcessing (Variables|Default|GetSpore%20Post%20Processing)))
        (Default|TriggerGlitchEffect _asbp_glitch_post_processing)
        (else
          (if (> (Utilities|Array|Length _overlappingactors) 0)
            (bind _asbp_glitch_portal (Utilities|Casting|CastToBP_GlitchPortal (Utilities|Array|Get(acopy) _overlappingactors))
              (:then
                (bind _location (Default|GetGlitchLocation _asbp_glitch_portal))
                (Transformation|SetActorLocationAndRotation (Components|GetOwner) (.location _location) (.rotation _location) false true))
              (:CastFailed
                (CallFunction|TriggerRandomGlitchonTerrain :!label _label)))
            (else
              (goto _label)))
          (Variables|Default|SetTime%20Until%20Next%20Glitch (Math|Random|RandomFloatinRangefromStream (Variables|Default|GetRandom%20Stream) (Variables|Default|GetMin%20Time%20Between%20Glitches) (Variables|Default|GetMax%20Time%20Between%20Glitches)))
          (Variables|Default|Setglitching false))))))

(fn OnToxicityChanged
  (params (new%20toxicity :type Float%20%28double-precision%29))
  (|CallParentFunction new%20toxicity))

(fn TriggerRandomGlitchonTerrain
  (bind _returnvalue (Components|GetOwner))
  (Transformation|SetActorLocationAndRotation _returnvalue (+ (Transformation|GetActorLocation _returnvalue) (* (Math|Vector|Normalize (* (Math|Random|RandomUnitVector) "1.000000,1.000000,0.000000")) (* (Variables|Default|GetCurrent%20Toxicity) (Variables|Default|GetMax%20Glitch%20Distance)))) (Transformation|GetActorRotation _returnvalue) true))

(fn AbletoGlitch
  (return (> (Variables|Default|GetCurrent%20Toxicity) 0.2)))