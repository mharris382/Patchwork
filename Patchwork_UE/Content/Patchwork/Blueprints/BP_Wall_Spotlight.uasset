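; BP_Wall_Spotlight is a configurable spotlight actor, named as a wall fixture.
; Its construction script pushes the intensity, color, attenuation radius and inner and outer cone angle variables onto the SpotLight component, so changes apply at construction.
; The event graph holds only disabled placeholder events, so it adds no runtime logic.
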(event EventBeginPlay)

(event Collision|EventActorBeginOverlap
  (params (OtherActor :type Actor%20Object%20Reference)))

(event EventTick
  (params (DeltaSeconds :type Float%20%28single-precision%29)))

(fn ConstructionScript
  (bind _spotlight (Variables|Default|GetSpotLight))
  (Rendering|Components|Light|SetIntensity _spotlight (Variables|Light|GetIntensity))
  (Rendering|Components|Light|SetLightColor _spotlight (Variables|Light|GetLight%20Color) true)
  (Rendering|Lighting|SetAttenuationRadius _spotlight (Variables|Light|GetAttenuation%20Radius))
  (Rendering|Lighting|SetInnerConeAngle _spotlight (Variables|Light|GetInner%20Angle))
  (Rendering|Lighting|SetOuterConeAngle _spotlight (Variables|Light|GetOuter%20Angle)))