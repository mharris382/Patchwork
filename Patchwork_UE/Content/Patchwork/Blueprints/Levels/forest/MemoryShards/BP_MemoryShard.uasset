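; BP_MemoryShard is a collectible Dreamer memory fragment, apparently placed in the forest level, that spins continuously until picked up.
; It extends a parent collectible, exposing its ShardId as the collectable ID and hiding the shard mesh when marked collected.
; On collection it fires OnShardCollected, saves the game through PatchworkGameInstance and shows a found message via the game mode.
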(event EventBeginPlay
  (|CallParentFunction)
  (bind _aspatchwork_game_instance (Utilities|Casting|CastToPatchworkGameInstance (Game|GetGameInstance)))
  (Variables|Default|SetAs%20Patchwork%20Game%20Instance _aspatchwork_game_instance))

(event Collision|EventActorBeginOverlap
  (params (OtherActor :type Actor%20Object%20Reference))
  (|CallParentFunction OtherActor))

(event EventTick
  (params (DeltaSeconds :type Float%20%28single-precision%29))
  (Transformation|AddRelativeRotation (Variables|Default|Getmemory_shard) (Math|Rotator|MakeRotator 0.0 0.0 (* DeltaSeconds (Variables|Default|GetRotation%20Rate))) false false))

(event EventCollect
  (|CallParentFunction)
  (Default|CallOnShardCollected)
  (Default|SaveGame (Variables|Default|GetAs%20Patchwork%20Game%20Instance) true)
  (Default|DisplayMessage (Variables|Default|GetGame%20Mode) "Found Dreamer Memory Fragment"))

(fn ConstructionScript)

(fn SetCollected
  (params (collected :type Boolean))
  (|CallParentFunction collected)
  (Rendering|SetVisibility (Variables|Default|Getmemory_shard) (not collected) false))

(fn GetCollectableID
  (return (Variables|Default|GetShardId)))