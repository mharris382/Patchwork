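; BP_Collectable is a pickup that the player collects by overlapping it, with its collected state persisted as a world event keyed by a collectable ID.
; On BeginPlay and game mode load events, it reads that state from game data and toggles the sphere's collision.
; Collecting invokes the event and plays optional sound and VFX.
; GetCollectableID returns "None" here, which disables persistence and logs a warning at BeginPlay.
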(event Custom|On%20Loaded
  (params (game%20data :type Game%20Data%20Object%20Reference))
  (bind _event_occured (Default|HasEventOccured game%20data (CallFunction|GetCollectableID)))
  (bind _output_get (Variables|Default|Setcollected _event_occured))
  (CallFunction|SetCollected _output_get))

(event Custom|Collect
  (bind _collect_sfx (Variables|Default|GetCollect%20SFX))
  (bind _collect_vfx (Variables|Default|GetCollect%20VFX))
  (Utilities|IsValid (Variables|Default|GetGame%20Mode)
    (:Is%20Valid
      (bind _asgm_base_game_mode (Utilities|Casting|CastToGM_BaseGameMode (Game|GetGameMode)))
      (Variables|Default|SetGame%20Mode _asgm_base_game_mode)
      (Default|InvokeWorldEvent (Variables|Default|GetGame%20Mode) (CallFunction|GetCollectableID))
      (CallFunction|SetCollected true)
      (Utilities|FlowControl|Sequence
        (:then_0
          ;[1 1 1] Play SFX
          (Utilities|IsValid _collect_sfx
            (:Is%20Valid
              (Audio|PlaySoundatLocation _collect_sfx (Transformation|GetActorLocation) "0, 0, 0" 1.0 1.0 0.0 0 0 0 0))))
        (:then_1
          ;[1 1 1] Play VFX
          (Utilities|IsValid _collect_vfx
            (:Is%20Valid
              (Niagara|SpawnSystematLocation _collect_vfx (Transformation|GetActorLocation) (Transformation|GetActorRotation (Game|Player|GetPlayerPawn 0))))))))))

(event EventBeginPlay
  (bind _aspatchwork_game_instance (Utilities|Casting|CastToPatchworkGameInstance (Game|GetGameInstance)))
  (Variables|Default|SetPatchwork%20Game%20Instance _aspatchwork_game_instance)
  (bind _asgm_base_game_mode (Utilities|Casting|CastToGM_BaseGameMode (Game|GetGameMode)))
  (bind _output_get (Variables|Default|SetGame%20Mode _asgm_base_game_mode))
  (if (not (== (CallFunction|GetCollectableID) ""))
    (EventDispatchers|BindEventtoOnLoadOccured _output_get (delegate Custom|On%20Loaded))
    (bind _event_occured (Default|HasEventOccured (Variables|/Game/Patchwork/Blueprints/PatchworkGameInstance.PatchworkGameInstance_C|GetCurrentGameData (Variables|Default|GetPatchwork%20Game%20Instance)) (CallFunction|GetCollectableID)))
    (bind _output_get_2 (Variables|Default|Setcollected _event_occured))
    (CallFunction|SetCollected _output_get_2)
    (else
      (Development|PrintString "Collectable Has No ID"))))

(event Collision|EventActorBeginOverlap
  (params (OtherActor :type Actor%20Object%20Reference))
  (if (and (== OtherActor (Game|Player|GetPlayerPawn 0)) (not (Variables|Default|Getcollected)))
    (Variables|Default|Setcollected true)
    (CallFunction|Collect)))

(fn ConstructionScript)

(fn GetCollectableID
  (return "None"))

(fn SetCollected
  (params (collected :type Boolean))
  (if collected
    (Collision|SetCollisionProfileName (Variables|Default|GetSphere) "NoCollision" true :!class /Script/Engine.PrimitiveComponent)
    (else
      (Collision|SetCollisionProfileName (Variables|Default|GetSphere) "OverlapAllDynamic" true :!class /Script/Engine.PrimitiveComponent))))