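; Japanese lantern lighting prop that sets its glow material during construction.
; The construction script either gets a material for its light color from the scene's MaterialInstanceManager or uses an assigned glow material, printing a warning if the manager is missing.
; It applies the result to slot 0 of static mesh components tagged "Emissive".
; GetLight overrides the parent to expose the lantern's point light, and the event graph has no active logic.
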(event EventBeginPlay
  (|CallParentFunction) ; This node is disabled and will not be called.\nDrag off pins to build functionality.
)

(event Collision|EventActorBeginOverlap
  (params (OtherActor :type Actor%20Object%20Reference))
  (|CallParentFunction OtherActor) ; This node is disabled and will not be called.\nDrag off pins to build functionality.
)

(event EventTick
  (params (DeltaSeconds :type Float%20%28single-precision%29))
  (|CallParentFunction DeltaSeconds) ; This node is disabled and will not be called.\nDrag off pins to build functionality.
)

(fn ConstructionScript
  (|CallParentFunction)
  ;[0.6233 0.6233 0.6233 0.5] Auto setup glow based on material color
  (if (or (Variables|Light|GetUseManagedMaterial) (Utilities|IsValid (Variables|Light|GetGlowMaterial)))
    (Utilities|FlowControl|Sequence
      (:then_0
        (if (Variables|Light|GetUseManagedMaterial)
          (bind _returnvalue (Actor|GetActorOfClass "/Game/Patchwork/Blueprints/Utilities/MaterialInstanceManager.MaterialInstanceManager_C"))
          (Utilities|IsValid _returnvalue
            (:Is%20Valid
              (bind _material (Default|GetMaterialInstanceforColor _returnvalue (Variables|Default|GetLight%20Color)))
              (LocalVariables|SetGlowMat _material))
            (:Is%20Not%20Valid
              (Development|PrintText "No MaterialInstanceManager in scene" true true "(R=1.000000,G=0.000000,B=0.020756,A=1.000000)")))
          (else
            (LocalVariables|SetGlowMat (Variables|Light|GetGlowMaterial)))))
      (:then_1
        (for _array_element (CallFunction|GetEmissiveParts)
          (Rendering|Material|SetMaterial _array_element 0 (LocalVariables|GetGlowMat)))))))

(fn GetLight
  (|CallParentFunction)
  (return (Variables|Default|GetPointLight_0)))

(fn GetEmissiveParts
  (return (Actor|GetComponentsbyTag "/Script/Engine.StaticMeshComponent" "Emissive")))