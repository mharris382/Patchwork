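; Lever Blueprint that moves a target actor between an On and an Off transform when its switch is toggled.
; SetSwitch sets a direction, and a looping timer steps a clamped alpha over Duration, lerping the transform until it hits either end.
; In relative mode, BeginPlay attaches a parentless target to a spawned actor so its initial transform becomes the reference.
; The construction script can preview the blend in the editor.
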(event Custom|update%20timer
  (bind _output_get (Variables|Default|Sett (Math|Float|Clamp(Float) (+ (Variables|Default|Gett) (* (/ (Utilities|Time|GetWorldDeltaSeconds) (Variables|Default|Getduration)) (Variables|Default|Getdirection))))))
  (bind _finished (CallFunction|UpdateTransform (Variables|Default|GetTarget) _output_get))
  (if _finished
    (Utilities|StopandClearTimer)))

(event Custom|Turn%20On
  (Variables|Default|Setdirection 1.0)
  (CallFunction|DoTransformation))

(event Custom|Turn%20Off
  (Variables|Default|Setdirection -1.0)
  (CallFunction|DoTransformation))

(event Custom|Do%20Transformation
  (Utilities|StopandClearTimer)
  (Utilities|IsValid (Variables|Default|GetTarget)
    (:Is%20Valid
      (bind _returnvalue (Utilities|Time|SetTimerbyEvent (delegate Custom|update%20timer) 0.01 true true))
      (Variables|Default|Settimer%20handle _returnvalue))
    (:Is%20Not%20Valid
      (Development|PrintString "Lever Has No Timer"))))

(event EventBeginPlay
  (bind _target (Variables|Default|GetTarget))
  (|CallParentFunction)
  (Utilities|FlowControl|Sequence
    (:then_0
      ;[0.6233 0.6233 0.6233 0.5] iuf using relative transform and has nio parent use the object's initial transform as the parent
      (if (Variables|Default|GetSet%20Relative%20Transform)
        (Utilities|IsValid _target
          (:Is%20Valid
            (if (not (Utilities|IsValid (Actor|GetParentActor _target)))
              (bind _returnvalue (Game|SpawnActorfromClass "/Script/Engine.Actor" (Transformation|GetActorTransform _target) "Undefined" "MultiplyWithRoot" 0 0))
              (Transformation|AttachActorToActor _target _returnvalue "None" "KeepRelative" "KeepRelative" "KeepRelative" true))))))))

(event Collision|EventActorBeginOverlap
  (params (OtherActor :type Actor%20Object%20Reference))
  (|CallParentFunction OtherActor) ; This node is disabled and will not be called.\nDrag off pins to build functionality.
)

(event EventTick
  (params (DeltaSeconds :type Float%20%28single-precision%29))
  (|CallParentFunction DeltaSeconds) ; This node is disabled and will not be called.\nDrag off pins to build functionality.
)

(fn ConstructionScript
  (bind _target (Variables|Default|GetTarget))
  (|CallParentFunction)
  (if (Variables|Default|GetPreview)
    (Utilities|IsValid _target
      (:Is%20Valid
        (CallFunction|UpdateTransform _target (Variables|Default|GetPreview%20Value))))))

(fn SetSwitch
  (params (is%20on :type Boolean))
  (|CallParentFunction is%20on)
  (if is%20on
    (CallFunction|Turnon)
    (else
      (CallFunction|TurnOff))))

(fn UpdateTransform
  (params (target :type Actor%20Object%20Reference) (t :type Float%20%28double-precision%29))
  (bind _on_transform (Variables|Default|GetOn%20Transform))
  (bind _rotation_interp_mode (Variables|Default|GetRotation%20Interp%20Mode))
  (bind _off_transform (Variables|Default|GetOff%20Transform))
  (bind _returnvalue (Math|Transform|Lerp(Transform) _on_transform _off_transform t _rotation_interp_mode))
  (Utilities|FlowControl|Sequence
    (:then_0
      (if (Variables|Default|GetSet%20Relative%20Transform)
        (Transformation|SetActorRelativeTransform target _returnvalue false false)
        (else
          (Transformation|SetActorTransform target _returnvalue))))
    (:then_1
      (return (or (>= t 1.0) (<= t 0.0))))))