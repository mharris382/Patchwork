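; Trigger actor that switches the level's ambient audio track when the player enters or leaves it.
; On BeginPlay it finds and caches the level's BP_DynamicAudioController, printing a warning if none exists.
; Player pawn overlap calls ChangeAmbTrack with AmbTrack, and ending the overlap sends ExitAmbTrack only when SetAmbnOnExit is enabled.
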(event EventBeginPlay
  (bind _returnvalue (Actor|GetActorOfClass "/Game/Patchwork/Blueprints/Audio/BP_DynamicAudioController.BP_DynamicAudioController_C"))
  (Utilities|IsValid _returnvalue
    (:Is%20Valid
      (Variables|Default|Setdynamic%20audio _returnvalue))
    (:Is%20Not%20Valid
      (Development|PrintString "Missing Dynamic Audio Controller in Level" true true "(R=1.000000,G=0.000000,B=0.146898,A=1.000000)"))))

(event Collision|EventActorBeginOverlap
  (params (OtherActor :type Actor%20Object%20Reference))
  (bind _dynamic_audio (Variables|Default|Getdynamic%20audio))
  (if (== OtherActor (Game|Player|GetPlayerPawn 0))
    (Utilities|IsValid _dynamic_audio
      (:Is%20Valid
        (Default|ChangeAmbTrack _dynamic_audio (Variables|Default|GetAmb%20Track))))))

(event Collision|EventActorEndOverlap
  (params (OtherActor :type Actor%20Object%20Reference))
  (bind _dynamic_audio (Variables|Default|Getdynamic%20audio))
  (if (and (Variables|Default|Getset%20ambn%20on%20exit) (== OtherActor (Game|Player|GetPlayerPawn 0)))
    (Utilities|IsValid _dynamic_audio
      (:Is%20Valid
        (Default|ChangeAmbTrack _dynamic_audio (Variables|Default|GetExit%20Amb%20Track))))))

(fn ConstructionScript)