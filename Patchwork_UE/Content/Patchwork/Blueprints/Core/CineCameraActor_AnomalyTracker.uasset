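; A cine camera actor that rides at the player pawn's camera position while always aiming at the anomaly's first-person look-at point.
; On BeginPlay it starts a fast looping timer, then polls until the pawn exists and caches its CameraComponent as HeadCam.
; Each timer update finds BP_Anomoly and moves and rotates the actor using a look-at rotation.
; SetCineCamActive and SetCineCamInactive start and clear that timer, which replaces Tick.
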(event Custom|SetCineCamActive
  (bind _returnvalue (Utilities|Time|SetTimerbyEvent (delegate Custom|UpdateCam) 0.01 true true))
  (Variables|Default|Setupdate%20timer _returnvalue))

(event Custom|SetCineCamInactive
  (Utilities|FlowControl|Sequence
    (:then_0
      (Utilities|Time|ClearandInvalidateTimerbyHandle (Variables|Default|Getupdate%20timer)))))

(event Custom|UpdateCam
  (bind _headcam (Variables|Default|GetHeadCam)
    (:then
      (bind _returnvalue (Actor|GetActorOfClass "/Game/Patchwork/Blueprints/Core/Anomoly/BP_Anomoly.BP_Anomoly_C"))
      (bind _look_at_location (Default|GetFPLookatLocationWS _returnvalue))
      (Transformation|SetActorLocationAndRotation self (Transformation|GetWorldLocation _headcam) (Math|Rotator|FindLookatRotation (Transformation|GetWorldLocation _headcam) _look_at_location)))
    (:else)))

(event EventBeginPlay
  (bind _returnvalue (Game|Player|GetPlayerPawn 0))
  (CallFunction|SetCineCamActive)
  (while (not (Utilities|IsValid _returnvalue)) :!label _label
    (Utilities|FlowControl|Delay 0.2)
    (Development|PrintString "Cam Waiting")
    (goto _label))
  (Variables|Default|SetHeadCam (Actor|GetComponentbyClass _returnvalue "/Script/Engine.CameraComponent")))

(event Collision|EventActorBeginOverlap
  (params (OtherActor :type Actor%20Object%20Reference)))

(event EventTick
  (params (DeltaSeconds :type Float%20%28single-precision%29)))

(fn ConstructionScript)