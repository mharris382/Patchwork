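; SporeEffectListener watches for spore effect components on the player pawn and announces each one as it is found.
; A fast looping timer checks every data table row not yet cached and stops once the cache count matches the row count.
; TryGetEffect returns a valid cached component or looks up the row's class on player 0's pawn, then caches it and calls OnSporeEffectAdded.
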(event Custom|check%20for%20effects
  (bind _outrownames (DataTable|GetDataTableRowNames (Variables|Default|Getdatatable)))
  (if (== (Utilities|Array|Length _outrownames) (Utilities|Map|Length (Variables|Default|Geteffect%20cache)))
    (Utilities|Time|ClearandInvalidateTimerbyHandle (Variables|Default|Getwait%20for%20effects))
    (else
      (for _array_element _outrownames
        (Utilities|FindEffectinMap _array_element
          (:not%20found
            (CallFunction|TryGetEffect _array_element)))))))

(event EventBeginPlay
  (bind _returnvalue (Utilities|Time|SetTimerbyEvent (delegate Custom|check%20for%20effects) 0.1 true))
  (Variables|Default|Setwait%20for%20effects _returnvalue))

(fn ConstructionScript)

(fn GetRow
  (params (effect%20name :type Name))
  (bind _returnvalue (Utilities|GetDataTableRow (Variables|Default|Getdatatable) effect%20name)
    (:then
      (return true _returnvalue))
    (:RowNotFound
      (return false ""))))

(fn TryGetEffect
  (params (row%20name :type Name))
  (bind _value (Utilities|FindEffectinMap row%20name)
    (:then
      (return true _value))
    (:not%20found
      (bind (_found _out_row) (CallFunction|GetRow row%20name))
      (if _found
        (Utilities|IsValid (Actor|GetComponentbyClass (Game|Player|GetPlayerPawn 0) (.PlayerEffectClass (Utilities|Struct|BreakS_SporeEffectData _out_row)))
          (:Is%20Valid
            (Utilities|Map|Add (Variables|Default|Geteffect%20cache) row%20name (Actor|GetComponentbyClass (Game|Player|GetPlayerPawn 0) (.PlayerEffectClass (Utilities|Struct|BreakS_SporeEffectData _out_row))))
            (Default|CallOnSporeEffectAdded row%20name (Actor|GetComponentbyClass (Game|Player|GetPlayerPawn 0) (.PlayerEffectClass (Utilities|Struct|BreakS_SporeEffectData _out_row))))
            (return true (Actor|GetComponentbyClass (Game|Player|GetPlayerPawn 0) (.PlayerEffectClass (Utilities|Struct|BreakS_SporeEffectData _out_row)))))
          (:Is%20Not%20Valid
            (return false 0)))
        (else
          (return false 0))))))