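; Spore effect for the forest level that cancels its owner's long fall while toxicity is present.
; On BeginPlay it finds the owner's FallHeight component, printing an error if it is missing.
; Each tick, while toxicity is above a near-zero value and the character has fallen past a threshold distance, it calls CancelLongFall on that component.
; The toxicity change handler only forwards to the parent.
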(event EventBeginPlay
  (|CallParentFunction)
  (bind _output_get (Variables|Refernces|SetFallHeight (Actor|GetComponentbyClass (Components|GetOwner) "/Game/Patchwork/Blueprints/Core/Pawns/Components/FallHeight.FallHeight_C")))
  (Utilities|IsValid _output_get
    (:Is%20Not%20Valid
      ;[0.6233 0.6233 0.6233 0.5] Error Logging
      (Development|PrintString (Utilities|String|Append (Utilities|GetDisplayName (Components|GetOwner)) " does not have long fall componet")))))

(event EventTick
  (params (DeltaSeconds :type Float%20%28single-precision%29))
  (bind _fallheight (Variables|Refernces|GetFallHeight))
  (|CallParentFunction DeltaSeconds)
  (if (> (Variables|Default|GetCurrent%20Toxicity) 0.01)
    (if (and (Default|IsCharacterFalling _fallheight) (> (Default|GetCurrentFallDistance _fallheight) (Variables|Default|GetFall%20Height%20Threshold)))
      (Default|CancelLongFall (Variables|Refernces|GetFallHeight)))))

(fn OnToxicityChanged
  (params (new%20toxicity :type Float%20%28double-precision%29))
  (|CallParentFunction new%20toxicity))