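; BP_SpinningHallway is a hallway actor that rotates continuously around its root, with optional top, back, front and bottom sides.
; Tick adds a local rotation to DefaultSceneRoot from SpinDirection and SpinRate, scaled by delta time.
; The Construction Script checks each side's Has flag and calls DeleteWalls for disabled ones.
; DeleteWalls uses GetWalls to gather a parent component's direct static mesh children, then destroys them.
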(event EventBeginPlay)

(event Collision|EventActorBeginOverlap
  (params (OtherActor :type Actor%20Object%20Reference)))

(event EventTick
  (params (DeltaSeconds :type Float%20%28single-precision%29))
  (Transformation|AddLocalRotation (Variables|Default|GetDefaultSceneRoot) (* (Variables|Default|GetSpin%20Direction) (* DeltaSeconds (Variables|Default|GetSpin%20Rate))) false false))

(fn ConstructionScript
  (Utilities|FlowControl|Sequence
    (:then_0
      (if (not (Variables|Default|GetHas%20Top))
        (CallFunction|DeleteWalls)))
    (:then_1
      (if (not (Variables|Default|GetHas%20Back))
        (CallFunction|DeleteWalls)))
    (:then_2
      (if (not (Variables|Default|GetHas%20Front))
        (CallFunction|DeleteWalls)))
    (:then_3
      (if (not (Variables|Default|GetHas%20Bottom))
        (CallFunction|DeleteWalls)))))

(fn GetWalls
  (params (parent :type Scene%20Component%20Object%20Reference))
  (LocalVariables|Setwalls (Utilities|Array|MakeArray 0))
  (for _array_element (Components|GetChildrenComponents parent false)
    (bind _asstatic_mesh_component (Utilities|Casting|CastToStaticMeshComponent _array_element))
    (Utilities|Array|Add (LocalVariables|Getwalls) _asstatic_mesh_component))
  (return (LocalVariables|Getwalls)))

(fn DeleteWalls
  (params (parent :type Scene%20Component%20Object%20Reference))
  (bind _back_walls (CallFunction|GetWalls parent))
  (for _array_element _back_walls
    (Utilities|IsValid _array_element
      (:Is%20Valid
        (Components|DestroyComponent _array_element)))))