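; Storm manager actor for the paper desert level that ramps up a storm's intensity and wind.
; StartStorm plays the StormBuildup timeline from the start, writing its Intensity and Wind tracks into scalar parameters of a material parameter collection on each update.
; A StartStormImmediately flag triggers the buildup on BeginPlay; otherwise the StartStorm event must be called.
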(event Custom|Start%20Storm
  (bind (_direction _intensity _wind) (Timeline|Storm%20Buildup PlayFromStart)
    (:Update
      (Rendering|Material|SetScalarParameterValue (Variables|Default|Getparam%20collection) (Variables|Default|Getintensity%20name) _intensity :!class /Script/Engine.KismetMaterialLibrary)
      (Rendering|Material|SetScalarParameterValue (Variables|Default|Getparam%20collection) (Variables|Default|Getwind%20strength%20name) _wind :!class /Script/Engine.KismetMaterialLibrary))))

(event EventBeginPlay
  (if (Variables|Default|GetStart%20Storm%20Immediately)
    (CallFunction|StartStorm)))

(event Collision|EventActorBeginOverlap
  (params (OtherActor :type Actor%20Object%20Reference)))

(event EventTick
  (params (DeltaSeconds :type Float%20%28single-precision%29)))

(fn ConstructionScript)