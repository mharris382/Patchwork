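; Data layer manager that sets World Streaming data layer runtime states from BP_DLStateVolume overlaps.
; Updates follow a delayed BeginPlay and trigger events, testing overlaps against the player pawn, or against the streaming target during teleports.
; Volume states merge by priority into ModifiedState, and a defaults pass writes to CurrentState.
; ApplyWorldState then replaces CurrentState with ModifiedState and pushes it to the DataLayerManager; an override event applies explicit states directly.
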(event Custom|DLTransition%20Start%20Trigger
  (if (not (Utilities|IsPlayerTeleporting))
    (CallFunction|UpdateWorldState)))

(event Custom|Event_OverrideWorldState
  (params (Activated :type Array%20of%20Data%20Layer%20Asset%20Object%20References) (Loaded :type Array%20of%20Data%20Layer%20Asset%20Object%20References) (Unloaded :type Array%20of%20Data%20Layer%20Asset%20Object%20References))
  (CallFunction|OverrideWorldState Activated Loaded Unloaded))

(event Custom|DLStream%20Triggered
  (params (Streaming%20Target :type BP%20Streaming%20Target%20Object%20Reference))
  (if (Utilities|IsPlayerTeleporting)
    (CallFunction|UpdatefromStreamingTarget Streaming%20Target)))

(event Custom|DLStateVolume%20Triggered
  (if (not (Utilities|IsPlayerTeleporting))
    (CallFunction|UpdateWorldState)))

(event EventBeginPlay
  (Utilities|FlowControl|Delay 7.0)
  (CallFunction|UpdateWorldState)
  (Development|PrintString "Update called from manager"))

(fn ConstructionScript)

(fn OverrideDefault
  (params (Override%20States :type Map%20of%20Data%20Layer%20Asset%20Object%20References%20to%20Bytes))
  (Development|PrintText (Utilities|Text|ToText(Integer) (Utilities|Map|Length Override%20States))))

(fn UpdateWorldState
  (Utilities|FlowControl|Sequence
    (:then_0
      (Utilities|Map|Clear (Variables|Default|GetmodifiedState)) ; not necessary but included for verbosity
      ;[0.6233 0.6233 0.6233 0.5] First Resolve as much of World State from Volumes as we can
      (bind _output_get (LocalVariables|SetoverlappingVolumes (Collision|GetOverlappingActors (Game|Player|GetPlayerPawn 0) "/Game/Patchwork/Blueprints/Environment/WorldStreaming/BP_DLStateVolume.BP_DLStateVolume_C" :!class /Script/Engine.Actor)))
      (switch int (Utilities|Array|Length _output_get)
        (:Default
          (for _array_element (LocalVariables|GetoverlappingVolumes)
            (bind _priority (Default|GetPriority _array_element))
            (CallFunction|ResolveVolume _array_element true _priority)))
        (:0
          (Development|PrintText "No overlapping volumes")
          (return))
        (:1
          (CallFunction|ResolveVolume (Utilities|Array|Get(acopy) (LocalVariables|GetoverlappingVolumes)) false 1))))
    (:then_1
      ;[0.6233 0.6233 0.6233 0.5] Resolve any unspecified DL states using defaults
      (CallFunction|ResolveDefaultWorldStates)
      ;[0.6233 0.6233 0.6233 0.5] Apply world state
      (CallFunction|ApplyWorldState))))

(fn ApplyWorldState
  (bind _modifiedstate (Variables|Default|GetmodifiedState))
  (Utilities|FlowControl|Sequence
    (:then_0
      ;[0.6233 0.6233 0.6233 0.5] Set current state to modified, then clear modifiedState
      (Variables|Default|SetcurrentState _modifiedstate)
      (Utilities|Map|Clear _modifiedstate))
    (:then_1
      ;[0.6233 0.6233 0.6233 0.5] Apply all data layer states from currentState
      (bind _returnvalue (WorldPartition|GetDataLayerManager))
      (bind _keys (Utilities|Map|Keys (Variables|Default|GetcurrentState)))
      (for _array_element _keys
        (DataLayers|SetDataLayerRuntimeState _returnvalue _array_element (.state (.Value (Utilities|Map|Find (Variables|Default|GetcurrentState) _array_element))) false :!class /Script/Engine.DataLayerManager)))))

(fn ResolveDefaultWorldStates
  (bind _keys (Utilities|Map|Keys (Variables|Default|GetcurrentState)))
  (for _array_element _keys
    (LocalVariables|Setcurr%20data%20layer _array_element)
    (if (.ReturnValue (Utilities|Map|Find (Variables|Default|GetmodifiedState) _array_element))
      (Utilities|Map|Add (Variables|Default|GetcurrentState) (LocalVariables|Getcurr%20data%20layer) (.Value (Utilities|Map|Find (Variables|Default|GetmodifiedState) _array_element)))
      (elif (.ReturnValue (Utilities|Map|Find (Variables|Default|GetDefaultStates) (LocalVariables|Getcurr%20data%20layer)))
        (Utilities|Map|Add (Variables|Default|GetcurrentState) (LocalVariables|Getcurr%20data%20layer) (Utilities|Struct|MakeS_DLStateInfo (.state (.Value (Utilities|Map|Find (Variables|Default|GetDefaultStates) (LocalVariables|Getcurr%20data%20layer)))) 0))
        (else
          (Development|PrintString "data layer[Name] not in default" true true "(R=1.000000,G=0.049562,B=0.000000,A=1.000000)"))))))

(fn ResolveVolume
  (params (InVolume :type BP%20DL%20Volume%20Base%20Object%20Reference) (CheckPriority :type Boolean) (Priority :type Integer))
  (bind (_activated _loaded _unloaded) (Default|GetStates InVolume))
  (CallFunction|SetModifiedState _activated _loaded _unloaded CheckPriority Priority)
  (return))

(fn OverrideWorldState
  (params (Activated :type Array%20of%20Data%20Layer%20Asset%20Object%20References) (Loaded :type Array%20of%20Data%20Layer%20Asset%20Object%20References) (Unloaded :type Array%20of%20Data%20Layer%20Asset%20Object%20References))
  (CallFunction|SetModifiedState Activated Loaded Unloaded false)
  (CallFunction|ApplyWorldState))

(fn SetModifiedState
  (params (Activated :type Array%20of%20Data%20Layer%20Asset%20Object%20References) (Loaded :type Array%20of%20Data%20Layer%20Asset%20Object%20References) (Unloaded :type Array%20of%20Data%20Layer%20Asset%20Object%20References) (CheckPriority :type Boolean) (InPriority :type Integer))
  (Utilities|FlowControl|Sequence
    (:then_0
      (for _array_element Activated
        (Utilities|TryAddValue CheckPriority _array_element InPriority "Activated")))
    (:then_1
      (for _array_element_2 Loaded
        (Utilities|TryAddValue CheckPriority _array_element_2 InPriority "Loaded")))
    (:then_2
      (for _array_element_3 Unloaded
        (Utilities|TryAddValue CheckPriority _array_element_3 InPriority "Unloaded")))
    (:then_3
      (return))))

(fn UpdatefromStreamingTarget
  (params (Streaming%20Target :type BP%20Streaming%20Target%20Object%20Reference))
  (Utilities|FlowControl|Sequence
    (:then_0
      (Utilities|Map|Clear (Variables|Default|GetmodifiedState))
      (bind _output_get (LocalVariables|SetOverlapping%20Volumes (Collision|GetOverlappingActors Streaming%20Target "/Game/Patchwork/Blueprints/Environment/WorldStreaming/BP_DLStateVolume.BP_DLStateVolume_C" :!class /Script/Engine.Actor)))
      (switch int (Utilities|Array|Length _output_get)
        (:Default
          (for _array_element (LocalVariables|GetOverlapping%20Volumes)
            (bind _priority (Default|GetPriority _array_element))
            (CallFunction|ResolveVolume _array_element true _priority)))
        (:0
          (Development|PrintText "No overlapping volumes")
          (return))
        (:1
          (CallFunction|ResolveVolume (Utilities|Array|Get(acopy) (LocalVariables|GetOverlapping%20Volumes)) false 1))))
    (:then_1
      ;[0.6233 0.6233 0.6233 0.5] Resolve any unspecified DL states using defaults
      (CallFunction|ResolveDefaultWorldStates)
      ;[0.6233 0.6233 0.6233 0.5] Apply world state
      (CallFunction|ApplyWorldState))))