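; Interactable climbable ladder that builds itself from a configurable count of stacked mesh segments, fitting its box and top markers to the height.
; BeginPlay caches a backward climb offset and traces between climb points to find the bottom.
; Interacting hands the ladder to the player, changes movement mode and snaps them to the height-matched point on the climb line.
; Interaction is blocked during certain player movement modes, otherwise deferring to the parent check.
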(event EventBeginPlay
  (bind _climb_bottom_point (Variables|Default|Getclimb%20bottom%20point))
  (bind _returnvalue (Transformation|GetWorldLocation _climb_bottom_point))
  (bind _aspaperperson (Utilities|Casting|CastTopaperperson (Game|Player|GetPlayerPawn 0)))
  (Variables|Default|Setplayer%20character _aspaperperson)
  (Utilities|FlowControl|Sequence
    (:then_0
      (Variables|Default|Setclimb%20offset (* (* (Transformation|GetActorForwardVector) -1.0) (Variables|Default|Getclimb%20offset%20distance))))
    (:then_1
      (bind (_outhit _returnvalue_2) (Collision|LineTraceForObjects (Transformation|GetWorldLocation (Variables|Default|Getclimb%20top%20point)) _returnvalue (Utilities|Array|MakeArray "ObjectTypeQuery1") false 0 "None"))
      (if _returnvalue_2
        (Variables|Default|SetClimb%20bottom (.Location (Collision|BreakHitResult _outhit)))
        (else
          (Variables|Default|SetClimb%20bottom _returnvalue))))))

(event Collision|EventActorBeginOverlap
  (params (OtherActor :type Actor%20Object%20Reference)))

(event EventOnInteract
  (bind _player_character (Variables|Default|Getplayer%20character))
  (Variables|/Game/Patchwork/Blueprints/Core/Pawns/paperperson.paperperson_C|SetLadder _player_character self)
  (Default|ChangeMovementMode _player_character "NewEnumerator1")
  (bind _location (CallFunction|GetNearestClimbPoint _player_character))
  (Transformation|SetActorLocation _player_character _location false false))

(fn ConstructionScript
  (bind _returnvalue (Math|Vector|VectorUp))
  (bind _exit_position (Variables|Default|Getexit%20position))
  (bind _ladder_segment_mesh (Variables|Default|GetLadder%20Segment%20Mesh))
  (bind _offset (Variables|Default|GetOffset))
  (bind _segment_count (Variables|Default|GetSegment%20Count))
  (bind _box (Variables|Default|GetBox))
  (bind _returnvalue_2 (Transformation|GetWorldLocation _exit_position))
  (bind _returnvalue_3 (* _returnvalue _offset))
  (bind _returnvalue_4 (* _returnvalue_3 _segment_count))
  (bind _returnvalue_5 (/ _returnvalue_4 2.0))
  (Utilities|FlowControl|Sequence
    (:then_0
      (for _index (range 0 (- (Variables|Default|GetSegment%20Count) 1))
        (bind _returnvalue_6 (AddComponent|AddStaticMeshComponent false (Math|Transform|MakeTransform (* _index _returnvalue_3) "0, 0, 0" (Variables|Default|GetScale))))
        (Utilities|IsValid _ladder_segment_mesh
          (:Is%20Valid
            (Components|StaticMesh|SetStaticMesh _returnvalue_6 _ladder_segment_mesh))
          (:Is%20Not%20Valid
            (Development|PrintText (Utilities|Text|FormatText "missing ladder segment mesh on ladder ({0})" (Utilities|GetDisplayName self)))))))
    (:then_1
      (Transformation|SetRelativeLocation (Variables|Default|GetLadder_Top) _returnvalue_4 false false)
      (Transformation|SetRelativeLocation _box _returnvalue_5 false false)
      (Components|Box|SetBoxExtent _box (+ _returnvalue_5 (Math|Vector|MakeVector 3e+01 1e+01 (Variables|Default|GetExtra%20Z%20Extents))) true)
      (Transformation|SetRelativeLocation (Variables|Default|GetGet%20On%20From%20top) (+ _returnvalue_4 (Math|Vector|MakeVector 0.0 0.0 (Variables|Default|GetGet%20On%20From%20Top%20Offset))) false false))
    (:then_2
      (bind (_outhit _returnvalue_7) (Collision|LineTraceForObjects _returnvalue_2 (- _returnvalue_2 "0.000000,0.000000,100.000000") (Utilities|Array|MakeArray "ObjectTypeQuery1") false 0 "ForOneFrame"))
      (if _returnvalue_7
        _))))

(fn GetClimbTop
  (return (+ (Transformation|GetWorldLocation (Variables|Default|Getclimb%20top%20point)) (* (CallFunction|GetClimbUpVector) 1e+02) (Variables|Default|Getclimb%20offset))))

(fn GetClimbUpVector
  (return (Math|Vector|Normalize (- (Transformation|GetWorldLocation (Variables|Default|GetLadder_Top)) (Transformation|GetWorldLocation (Variables|Default|GetLadder_Bottom))))))

(fn GetNearestClimbPoint
  (params (actor :type Actor%20Object%20Reference))
  (bind _returnvalue (Transformation|GetActorLocation actor))
  (bind _ws_position (CallFunction|GetClimbTop))
  (bind _climb_bottom (Variables|Default|GetClimb%20bottom))
  (if (> (.z _returnvalue) (.z _ws_position))
    (return (CallFunction|GetClimbTop))
    (elif (< (.z _returnvalue) (.z _climb_bottom))
      (return (Variables|Default|GetClimb%20bottom))
      (else
        (return (Math|Vector|Lerp(Vector) (Variables|Default|GetClimb%20bottom) (CallFunction|GetClimbTop) (Math|Float|MapRangeClamped (.z _returnvalue) (.z _climb_bottom) (.z _ws_position) 0.0 1.0)))))))

(fn GetActionVerb
  (return "Climb"))

(fn IsInteractionAvailable
  (bind _aspaperperson_ledge_grab (Utilities|Casting|CastTopaperperson_ledge_grab (Game|Player|GetPlayerPawn 0))
    (:then
      (if (Math|Boolean|ORBoolean (Utilities|Enum|Equal(Enum) (Variables|/Game/Patchwork/Blueprints/Core/Pawns/paperperson.paperperson_C|GetMovement%20Mode _aspaperperson_ledge_grab) "NewEnumerator1") (Utilities|Enum|Equal(Enum) (Variables|/Game/Patchwork/Blueprints/Core/Pawns/paperperson.paperperson_C|GetMovement%20Mode _aspaperperson_ledge_grab) "NewEnumerator3") (Utilities|Enum|Equal(Enum) (Variables|/Game/Patchwork/Blueprints/Core/Pawns/paperperson.paperperson_C|GetMovement%20Mode _aspaperperson_ledge_grab) "NewEnumerator5"))
        (return false)
        (else
          _)))
    (:CastFailed
      _))
  (return (|CallParentFunction)))