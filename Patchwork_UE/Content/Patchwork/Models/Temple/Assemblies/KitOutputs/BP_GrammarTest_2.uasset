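; BP_GrammarTest_2 is a test Blueprint among the temple kit-output assemblies, mainly overriding the bounds queries of its parent class.
; GetBoundsMinMax expands the parent's bounds in X and Y by half of OffsetDistance on each side, leaving Z untouched.
; GetBoundsVerticalHeight returns the Height variable in place of the parent's result.
; The construction script only calls the parent, and the event graph holds only disabled default events.
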(event EventBeginPlay
  (|CallParentFunction) ; This node is disabled and will not be called.\nDrag off pins to build functionality.
)

(event Collision|EventActorBeginOverlap
  (params (OtherActor :type Actor%20Object%20Reference))
  (|CallParentFunction OtherActor) ; This node is disabled and will not be called.\nDrag off pins to build functionality.
)

(event EventTick
  (params (DeltaSeconds :type Float%20%28single-precision%29))
  (|CallParentFunction DeltaSeconds) ; This node is disabled and will not be called.\nDrag off pins to build functionality.
)

(fn ConstructionScript
  (|CallParentFunction))

(fn GetBoundsMinMax
  (bind _offsetdistance (Variables|Default|GetOffsetDistance))
  (bind _returnvalue (/ _offsetdistance 2.0))
  (bind (_min _max) (|CallParentFunction))
  (return (- _min (Math|Vector|MakeVector _returnvalue _returnvalue 0.0)) (+ _max (Math|Vector|MakeVector _returnvalue _returnvalue 0.0))))

(fn GetBoundsVerticalHeight
  (return (Variables|Default|GetHeight)))