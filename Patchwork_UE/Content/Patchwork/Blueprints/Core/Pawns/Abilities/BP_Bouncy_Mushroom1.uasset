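; Bouncy mushroom that launches characters with sound, scales in and out on spawn and despawn, and is destroyed on player death.
; Extends parent bounce force, rescaling it for some launch angles when horizontal velocity opposes the bounce.
; Spore carrier events attach or remove data-table-driven spore actors, with a dissipate effect on loss.
; Darkness brightens its lights via a reversible timeline; camera quick-turn logic exists but its check is unwired.
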(event Custom|Despawn
  ;[0.6233 0.6233 0.6233 0.5] Despawn
  (Default|ResetSpores (Variables|Default|GetBP_SporeCarrierController))
  (Variables|Default|Setis%20spawned false)
  (Utilities|FlowControl|DoOnce false
    (:Completed
      (bind _scale (Timeline|Despawn%20Timeline Play)
        (:Update
          (Transformation|SetActorScale3D (Math|Conversions|ToVector(Float) _scale)))))))

(event Custom|Respawn%20From
  (params (transform :type Transform))
  ;[0.6233 0.6233 0.6233 0.5] Spawning
  (Transformation|SetActorTransform transform)
  (Utilities|FlowControl|Sequence
    (:then_0
      (bind _scale (Timeline|Spawn%20Timeline PlayFromStart)
        (:Update
          (Transformation|SetRelativeScale3D (Variables|Default|GetMushroomPivot) (Math|Conversions|ToVector(Float) _scale)))))
    (:then_1
      (CallFunction|OnSpawned))
    (:then_2
      (Utilities|FlowControl|Delay 0.2)
      (Variables|Default|Setis%20spawned true))))

(event Custom|gained%20spore
  (params (type :type Name) (source :type BPI%20Spore%20Contagion%20Interface) (instigator :type Actor%20Object%20Reference))
  (Utilities|GetDataTableRow "/Game/Patchwork/Data/Datatables/DT_SporeEffects.DT_SporeEffects" type
    (:then
      (bind _returnvalue (Game|SpawnActorfromClass "/Game/Patchwork/Blueprints/Levels/forest/Spores/BP_Spore_Spawned.BP_Spore_Spawned_C" (Transformation|GetActorTransform) "Undefined" "MultiplyWithRoot" 0 0))
      (Utilities|Map|Add (Variables|Default|GetSpawned) type _returnvalue)
      (Transformation|AttachActorToActor _returnvalue self "None" "KeepWorld" "KeepWorld" "KeepWorld" true)
      (Default|ChangeSporeType _returnvalue (Utilities|Struct|MakeDataTableRowHandle "/Game/Patchwork/Data/Datatables/DT_SporeEffects.DT_SporeEffects" type)))))

(event Custom|lost%20spore
  (params (type :type Name))
  (bind _returnvalue (Transformation|GetActorTransform))
  (bind _spawned (Variables|Default|GetSpawned))
  (bind (_value _returnvalue_2) (Utilities|Map|Find _spawned type))
  (if _returnvalue_2
    (Actor|DestroyActor _value)
    (bind _returnvalue_3 (Niagara|SpawnSystematLocation "/Game/Patchwork/Effects/SporeEffects/NS_Spore_Dissapate.NS_Spore_Dissapate" (.location _returnvalue) (.rotation _returnvalue) (.scale _returnvalue) true true "AutoRelease"))
    (CallFunction|ApplySporeTypetoEffect type _returnvalue_3 1.0)))

(event Custom|On%20Spawned
  ;[0.6233 0.6233 0.6233 0.5] Despawn
  (Utilities|FlowControl|Sequence
    (:then_0
      (Utilities|FlowControl|DoOnce false) ; enters at Reset
    )
    (:then_1
      (bind _scale (Timeline|Despawn%20Timeline Stop)
        (:Update
          (Transformation|SetActorScale3D (Math|Conversions|ToVector(Float) _scale)))))))

(event Custom|CustomEvent
  ;[0.6233 0.6233 0.6233 0.5] Begin
  ;;[0.6233 0.6233 0.6233 0.5] Destroy on player long fall
  (Actor|DestroyActor))

(event Custom|go%20to%20rotation
  (if (not (Utilities|Enum|Equal(Enum) (Variables|/Game/Patchwork/Blueprints/Core/Pawns/paperperson.paperperson_C|GetMovement%20Mode (.AsPaperperson (Utilities|Casting|CastTopaperperson (CallFunction|GetBasePlayerPawn)))) "NewEnumerator0"))
    (CallFunction|StopQuickTurn)
    (Utilities|Time|ClearandInvalidateTimerbyHandle (Variables|Default|Getrotation))))

(event Custom|start%20quick%20turn
  (bind _returnvalue (Game|GetPlayerController 0))
  (bind _returnvalue_2 (Pawn|GetControlRotation _returnvalue :!class /Script/Engine.Controller))
  (Utilities|FlowControl|Sequence
    (:then_0
      (bind _t (Timeline|Quick%20Turn PlayFromStart)
        (:Update
          (Pawn|SetControlRotation _returnvalue (Math|Rotator|MakeRotator (.roll _returnvalue_2) (.pitch _returnvalue_2) (Math|Float|Lerp (Variables|Default|GetStart%20Yaw) (Variables|Default|Getdesired%20yaw) _t))))
        (:Finished
          (Utilities|ClearTimer))))
    (:then_1
      (Utilities|ClearTimer)
      (bind _returnvalue_3 (Utilities|Time|SetTimerbyEvent (delegate Custom|go%20to%20rotation) 0.1 true true))
      (Variables|Default|Setrotation _returnvalue_3))))

(event Custom|Stop%20quick%20turn
  (bind _returnvalue (Game|GetPlayerController 0))
  (bind _returnvalue_2 (Pawn|GetControlRotation _returnvalue :!class /Script/Engine.Controller))
  (Utilities|ClearTimer)
  (bind _t (Timeline|Quick%20Turn Stop)
    (:Update
      (Pawn|SetControlRotation _returnvalue (Math|Rotator|MakeRotator (.roll _returnvalue_2) (.pitch _returnvalue_2) (Math|Float|Lerp (Variables|Default|GetStart%20Yaw) (Variables|Default|Getdesired%20yaw) _t))))
    (:Finished
      (Utilities|ClearTimer))))

(event Custom|check%20for%20quick%20turn
  (bind _base_character (CallFunction|GetBasePlayerPawn))
  (bind _launch_direction (Variables|Default|GetLaunch%20Direction))
  (bind _returnvalue (Math|Vector|GetForwardVector _launch_direction))
  (bind _camera (Variables|/Game/Patchwork/Blueprints/Core/Pawns/BP_BaseCharacter.BP_BaseCharacter_C|GetCamera _base_character))
  (bind _returnvalue_2 (Math|Vector|GetForwardVector _camera))
  (bind _output_get (Variables|Default|Setlaunch%20forward%20direction _returnvalue))
  (if (not (> (Math|Float|Absolute(Float) (Math|Vector|DotProduct _output_get "0.000000,0.000000,1.000000")) 0.1)) ; check if pointing close to up
    (if (< (Math|Vector|DotProduct (Math|Vector|Normalize (* _returnvalue "1.000000,1.000000,0.000000")) (Math|Vector|Normalize (* _returnvalue_2 "1.000000,1.000000,0.000000"))) -0.2) ; looking opposite to bounce direction
      (Variables|Default|SetStart%20Yaw (.yaw (Math|Conversions|RotationFromXVector _returnvalue_2)))
      (Variables|Default|Setdesired%20yaw (.yaw (Math|Conversions|RotationFromXVector _returnvalue)))
      (CallFunction|StartQuickTurn)
      (CallFunction|StartQuickTurn))))

(event EventBeginPlay
  (bind _bp_sporecarriercontroller (Variables|Default|GetBP_SporeCarrierController))
  ;[0.6233 0.6233 0.6233 0.5] Begin
  (|CallParentFunction)
  (Utilities|FlowControl|Sequence
    (:then_0
      (EventDispatchers|BindEventtoOnSporeGained _bp_sporecarriercontroller (delegate Custom|gained%20spore))
      (EventDispatchers|BindEventtoOnSporeLost _bp_sporecarriercontroller (delegate Custom|lost%20spore)))
    (:then_1
      ;;[0.6233 0.6233 0.6233 0.5] Destroy on player long fall
      (EventDispatchers|BindEventtoOnPlayerDeathOccured (CallFunction|GetBaseGameMode) (delegate Custom|CustomEvent)))
    (:then_2
      ;[0.6233 0.6233 0.6233 0.5] Spawning
      (bind _scale (Timeline|Spawn%20Timeline PlayFromStart)
        (:Update
          (Transformation|SetRelativeScale3D (Variables|Default|GetMushroomPivot) (Math|Conversions|ToVector(Float) _scale)))))))

(event EventBounceCharacter
  (params (actor :type Actor%20Object%20Reference))
  (|CallParentFunction actor)
  (if (== actor (Game|Player|GetPlayerPawn 0))
    _))

(event EventSetInsideDarkness
  (params (is%20inside%20darkness :type Boolean))
  (bind _castlight (Variables|Default|GetCastLight))
  ;[0.07812 0.07812 0.07812 0.5 50] Darkness
  (Utilities|FlowControl|Sequence
    (:then_0
      (if is%20inside%20darkness
        (bind (_direction _intensity _distance) (Timeline|Lights PlayFromStart)
          (:Update
            (Utilities|FlowControl|Sequence
              (:then_0
                (Rendering|Components|Light|SetIntensity _castlight (Math|Float|MapRangeUnclamped _intensity 0.0 1.0 (Variables|Default|GetNormal%20Light%20Intensity) (Variables|Default|GetBright%20Light%20Intensity))))
              (:then_1
                (Rendering|Lighting|SetAttenuationRadius _castlight (Math|Float|MapRangeUnclamped _distance 0.0 1.0 (Variables|Default|GetNormal%20Light%20Radius) (Variables|Default|GetBright%20Light%20Radius)))))))
        (else
          (Timeline|Lights ReverseFromEnd))))
    (:then_1
      (Rendering|SetVisibility (Variables|Default|GetAreaAroundMushLight) is%20inside%20darkness false))))

(event EventBounce
  ;[0.6233 0.6233 0.6233 0.5 32] Bounce
  (Utilities|FlowControl|Sequence
    (:then_0
      (|CallParentFunction))
    (:then_1
      (Audio|PlaySoundatLocation "/Game/Patchwork/Audio/Abilities/BounceShroom/MS_BounceShroom_Jump_Container.MS_BounceShroom_Jump_Container" (Transformation|GetActorLocation) "0, 0, 0" 1.0 1.0 0.0 0 0 0 0))))

(fn ConstructionScript)

(fn GetBounceForce
  (params (direction :type Vector :default "0, 0, 0") (look%20direction :type Vector :default "0, 0, 0") (character%20velocity :type Vector :default "0, 0, 0") (is%20player :type Boolean))
  (bind _returnvalue (Math|Vector|DotProduct direction "0.000000,0.000000,1.000000"))
  (bind _amount (|CallParentFunction direction look%20direction character%20velocity is%20player))
  (bind _returnvalue_2 (Utilities|RemoveZ direction))
  (bind _returnvalue_3 (Utilities|RemoveZ character%20velocity))
  (bind _returnvalue_4 (Math|Vector|DotProduct _returnvalue_2 _returnvalue_3))
  (if (and (< (Math|Float|Absolute(Float) _returnvalue) 0.5) (> _returnvalue 0.0))
    (return _amount)
    (else
      (return (Math|Float|SelectFloat (* _amount (Math|Float|MapRangeClamped (Math|Float|Absolute(Float) _returnvalue_4) 0.0 1.0 1.0 (Variables|Forces|GetBounce%20Force%20Scale%20when%20changing%20direction))) _amount (< _returnvalue_4 0.0))))))