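; BP_FallBox is an overlap volume that teleports the player pawn back to a recovery point when it enters.
; If ReturnToLastGroundedLocation is enabled, it first tries the last ground location and rotation stored on BP_BaseCharacter.
; If that is disabled or unavailable, it falls back to the nearest teleport point supplied by GM_BaseGameMode, which it caches on BeginPlay.
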(event EventBeginPlay
  (bind _returnvalue (Actor|GetActorOfClass "/Script/Engine.PlayerStart"))
  (Variables|Default|Setplayer%20start _returnvalue)
  (bind _asgm_base_game_mode (Utilities|Casting|CastToGM_BaseGameMode (Game|GetGameMode)))
  (Variables|Default|SetGM%20Base%20Game%20Mode _asgm_base_game_mode))

(event Collision|EventActorBeginOverlap
  (params (OtherActor :type Actor%20Object%20Reference))
  (bind _returnvalue (Game|Player|GetPlayerPawn 0))
  (if (== OtherActor _returnvalue)
    (Utilities|TryReturntoLastGroundLocation
      (:failure
        (bind (_location _rotator) (Default|GetNearestTelepoint (Variables|Default|GetGM%20Base%20Game%20Mode)))
        (Transformation|SetActorLocationAndRotation _returnvalue _location _rotator false true)))))

(event EventTick
  (params (DeltaSeconds :type Float%20%28single-precision%29)))

(fn ConstructionScript)