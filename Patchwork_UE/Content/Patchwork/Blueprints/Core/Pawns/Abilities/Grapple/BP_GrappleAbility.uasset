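; Grapple ability component on the player pawn that fires a projectile and acts on what it hits.
; A valid hit moves an attach point to the impact and sets a state based on physics simulation.
; Kinematic hits zip the player with per-tick, normal-offset forces.
; Dynamic hits spawn an IronPuller, using a dummy target for actors lacking BPI_Pullable; long falls stay disabled during zips until landing, height limit or timeout.
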(event Custom|Fire%20Grapple%20Projectile
  (bind _returnvalue (Transformation|GetWorldTransform))
  ;[0.6233 0.6233 0.6233 0.5] Spawn Projecitle
  (Variables|Default|SetGrappleState "NewEnumerator1")
  (bind _returnvalue_2 (Game|SpawnActorfromClass (Getters|GetProjectileClass) (Math|Transform|MakeTransform (.location _returnvalue) (.rotation _returnvalue) "1.000000,1.000000,1.000000") "Undefined" "MultiplyWithRoot" (Components|GetOwner) (Variables|References|GetOwnerPawn)))
  (Variables|References|SetCurrentProjectile _returnvalue_2)
  (Utilities|FlowControl|Sequence
    (:then_0
      ;[0.6233 0.6233 0.6233 0.5] Init Grapple Settings
      (Variables|/Game/Patchwork/Blueprints/Core/Pawns/Abilities/Grapple/BP_Grapple_Projectile.BP_Grapple_Projectile_C|SetAllowedDistance (Variables|References|GetCurrentProjectile) (Getters|GetMaxGrappleDistance))
      (Grapple|UpdateGrappleVisualSettings) ; call in case we upgrade max distance
    )
    (:then_1
      ;[0.6233 0.6233 0.6233 0.5 25] Listen for Projectile Hit Events
      (Variables|Default|SetProjectileHitOccurred false)
      ;;[0.6233 0.6233 0.6233 0.5] Valid
      (EventDispatchers|BindEventtoOnGrappleHitValid (Variables|References|GetCurrentProjectile) (delegate Custom|Valid%20hit))
      ;;[0.6233 0.6233 0.6233 0.5] Invalid
      (EventDispatchers|BindEventtoOnGrappleHitInvalid (Variables|References|GetCurrentProjectile) (delegate Custom|Invalid%20Hit))
      (Game|BindEventtoOnDestroyed (Variables|References|GetCurrentProjectile) (delegate Custom|Projectile%20Destroyed)))))

(event Custom|Retract%20Grapple
  ;[0.6233 0.6233 0.6233 0.5] Retract Grapple (not sure if will be used)
  (if (Variables|Default|GetIsAttached)
    (CallFunction|PlayImpactatLocation "(TagName=\"Feedbacks.Abilities.Grapple.Detached\")" (Transformation|GetWorldLocation) self)))

(event Custom|Valid%20hit
  (params (Hit :type Hit%20Result%20Structure) (HitComponent :type Scene%20Component%20Object%20Reference) (SporeCarrier :type BP%20Spore%20Carrier%20Object%20Reference))
  ;[0.6233 0.6233 0.6233 0.5 25] Listen for Projectile Hit Events
  ;;[0.6233 0.6233 0.6233 0.5] Valid
  (Utilities|CheckProjectileHit
    (:then
      (Grapple|OnValidGrappleHit Hit HitComponent SporeCarrier))))

(event Custom|Invalid%20Hit
  (params (Hit :type Hit%20Result%20Structure))
  ;[0.6233 0.6233 0.6233 0.5 25] Listen for Projectile Hit Events
  ;;[0.6233 0.6233 0.6233 0.5] Invalid
  (Utilities|CheckProjectileHit
    (:then
      (CallFunction|GrappleProjectileFailed))))

(event Custom|Projectile%20Destroyed
  (params (DestroyedActor :type Actor%20Object%20Reference))
  ;[0.6233 0.6233 0.6233 0.5 25] Listen for Projectile Hit Events
  ;;[0.6233 0.6233 0.6233 0.5] Invalid
  (Utilities|CheckProjectileHit
    (:then
      (CallFunction|GrappleProjectileFailed))))

(event Custom|Grapple%20Projectile%20Failed
  ;[0.6233 0.6233 0.6233 0.5 25] Listen for Projectile Hit Events
  ;;[0.6233 0.6233 0.6233 0.5] Invalid
  ;;;[0.6233 0.6233 0.6233 0.5] Cleanup after invalid hit or projectile destroyed without hit
  (CallFunction|CompleteAbility false)
  (Utilities|PlayFXonSelf (Variables|Feedbacks|GetInvalidHitFX)
    (:then
      (Default|SetGrappleActive (Variables|References|GetGrapple) false))))

(event Input|EnhancedActionEvents|EnhancedInputActionIA_Ability_2
  (params (ActionValue :type Boolean) (ElapsedSeconds :type Float%20%28double-precision%29) (TriggeredSeconds :type Float%20%28double-precision%29) (InputAction :type Input%20Action%20Object%20Reference :default "/Game/Patchwork/Data/Input/IA_Ability_2.IA_Ability_2"))
  (:Started
    ;[0.6233 0.6233 0.6233 0.5] Ability Input Start
    (if (Utilities|Enum|Equal(Enum) (Variables|Default|GetGrappleState) "NewEnumerator0")
      (CallFunction|StartAbility)
      (else
        (switch Utilities|FlowControl|Switch|SwitchonEGrappleAbilityState (Variables|Default|GetGrappleState)
          (:NewEnumerator3
            _)
          (:NewEnumerator4
            _))
        (Default|Detach (Variables|References|GetGrapple) (Variables|Default|GetLastHit))
        (CallFunction|CompleteAbility true)
        (bind _currentprojectile (Variables|References|GetCurrentProjectile)
          (:then
            (Actor|DestroyActor _currentprojectile))
          (:else)))))
  (:Ongoing
    (Development|PrintString "Grapple Ongoing"))
  (:Canceled
    (Development|PrintString "Grapple Cancel"))
  (:Completed
    (Development|PrintString "Grapple Complete")))

(event Input|EnhancedActionEvents|EnhancedInputActionIA_Interact
  (params (ActionValue :type Boolean) (ElapsedSeconds :type Float%20%28double-precision%29) (TriggeredSeconds :type Float%20%28double-precision%29) (InputAction :type Input%20Action%20Object%20Reference :default "/Game/Patchwork/Data/Input/IA_Interact.IA_Interact"))
  ;[0.6233 0.6233 0.6233 0.5] Ability Input Start
  (if (not (Utilities|Enum|Equal(Enum) (Variables|Default|GetGrappleState) "NewEnumerator0"))
    (switch Utilities|FlowControl|Switch|SwitchonEGrappleAbilityState (Variables|Default|GetGrappleState)
      (:NewEnumerator3
        _)
      (:NewEnumerator4
        _))
    (Default|Detach (Variables|References|GetGrapple) (Variables|Default|GetLastHit))
    (CallFunction|CompleteAbility true)
    (bind _currentprojectile (Variables|References|GetCurrentProjectile)
      (:then
        (Actor|DestroyActor _currentprojectile))
      (:else))))

(event EventBeginPlay
  ;[0.6233 0.6233 0.6233 0.5 45] Begin
  (|CallParentFunction)
  (Utilities|FlowControl|Sequence
    (:then_0
      ;;[0.6233 0.6233 0.6233 0.5] Get Ref to Owner Pawn
      (bind _aspawn (Utilities|Casting|CastToPawn (Components|GetOwner)))
      (bind _output_get (Variables|References|SetOwnerPawn _aspawn))
      (Variables|Default|SetFallHeight (Actor|GetComponentbyClass _output_get "/Game/Patchwork/Blueprints/Core/Pawns/Components/FallHeight.FallHeight_C"))
      ;;[0.6233 0.6233 0.6233 0.5] Cache Sqr End Distance
      (Variables|AbilitySettings|SetGrappleEndDistanceSqr (Math|Float|Power (Variables|AbilitySettings|GetGrappleEndDistance) 2.0))
      (Variables|AbilitySettings|SetGrapplePullDistanceSqr (Math|Float|Power (Variables|AbilitySettings|GetGrapplePullDistance) 2.0)))
    (:then_1
      ;;[0.6233 0.6233 0.6233 0.5] Spawn Ability Actors
      (bind _attachpoint (Utilities|GetorSpawnAttachPoint))
      (bind _returnvalue (Game|SpawnActorfromClass "/Game/Patchwork/Blueprints/Core/Pawns/Abilities/Grapple/BP_Grapple.BP_Grapple_C" (Transformation|GetWorldTransform) "Undefined" "MultiplyWithRoot" 0 self (Variables|/Script/Engine.Actor|GetRootComponent _attachpoint) (Variables|References|GetOwnerPawn)))
      (bind _output_get_2 (Variables|References|SetGrapple _returnvalue))
      (Default|SetGrappleActive _output_get_2 false)
      (Variables|/Game/Patchwork/Blueprints/Core/Pawns/Abilities/Grapple/BP_Grapple.BP_Grapple_C|SetAttachPoint _output_get_2 (Variables|References|GetAttachPoint))
      (Grapple|UpdateGrappleVisualSettings)
      (Transformation|AttachComponentToComponent (Variables|References|GetGrapple) self "None" "KeepWorld" "KeepWorld" "KeepWorld" true))
    (:then_2
      (EventDispatchers|BindEventtoOnPlayerMushBounced (CallFunction|GetBaseGameMode) (EventDispatchers|CreateEvent :!event OnPlayerMushBounced)))))

(event EventTick
  (params (DeltaSeconds :type Float%20%28single-precision%29))
  (|CallParentFunction DeltaSeconds)
  (CallFunction|UpdateZipForces))

(event Custom|BeginZipToKinematic
  ;[0.6233 0.6233 0.6233 0.5 45] Start Zip
  (Variables|/Game/Patchwork/Blueprints/Core/Pawns/Components/FallHeight.FallHeight_C|Setallow%20long%20falls (Variables|Default|GetFallHeight) false)
  (Components|Tick|SetComponentTickEnabled true)
  (Class|BPIPlayerPawn|SetPlayerMoveState(Message) (Components|GetOwner) "NewEnumerator6")
  (Utilities|FlowControl|Sequence
    (:then_0
      (Utilities|Time|ClearandInvalidateTimerbyHandle (Variables|Default|Getwaithandle)))
    (:then_1
      ;[0.6233 0.6233 0.6233 0.5 45] End Zip
      (Utilities|FlowControl|DoOnce false) ; enters at Reset
    )))

(event Custom|EndZip
  ;[0.6233 0.6233 0.6233 0.5 45] End Zip
  (Components|Tick|SetComponentTickEnabled true)
  (bind _has_floor (Class|BPIPlayerPawn|GetPlayerFloor(Message) (Components|GetOwner)))
  (if _has_floor
    _
    (else
      (bind _returnvalue (Utilities|Time|SetTimerbyEvent (delegate Custom|WaitForFloor) 0.01 true true))
      (Variables|Default|Setwaithandle _returnvalue)
      (Utilities|FlowControl|Delay 1.0)
      (Utilities|FlowControl|DoOnce false
        (:Completed
          (Utilities|Time|ClearandInvalidateTimerbyHandle (Variables|Default|Getwaithandle))))))
  (Class|BPIPlayerPawn|SetPlayerMoveState(Message) (Components|GetOwner) "NewEnumerator0")
  (Variables|/Game/Patchwork/Blueprints/Core/Pawns/Components/FallHeight.FallHeight_C|Setallow%20long%20falls (Variables|Default|GetFallHeight) true))

(event Custom|update%20zip%20forces
  ;[0.6233 0.6233 0.6233 0.5 45] Update Zip
  (switch Utilities|FlowControl|Switch|SwitchonEGrappleAbilityState (Variables|Default|GetGrappleState)
    (:NewEnumerator3
      (if (Conditions|CheckGrappleDistance)
        (CallFunction|CompleteAbility true)
        (else
          (Physics|ApplyZipForcetoPlayer))))))

(event Custom|Begin%20Zip%20To%20Dynamic
  (IronPuller|SetupIronPullerforHit (Variables|Default|GetLastHit)))

(event Custom|WaitForFloor
  ;[0.6233 0.6233 0.6233 0.5 45] End Zip
  (bind _has_floor (Class|BPIPlayerPawn|GetPlayerFloor(Message) (Components|GetOwner)))
  (if (or _has_floor (> (- (.z (Transformation|GetActorLocation (Components|GetOwner))) (.z (Utilities|GetLastGrappleLocation))) (Variables|AbilitySettings|GetMaxFlingHeight)))
    (Utilities|FlowControl|DoOnce false
      (:Completed
        (Utilities|Time|ClearandInvalidateTimerbyHandle (Variables|Default|Getwaithandle))
        (Class|BPIPlayerPawn|SetPlayerMoveState(Message) (Components|GetOwner) "NewEnumerator0")
        (Variables|/Game/Patchwork/Blueprints/Core/Pawns/Components/FallHeight.FallHeight_C|Setallow%20long%20falls (Variables|Default|GetFallHeight) true)))))

(fn IsReady
  (switch Utilities|FlowControl|Switch|SwitchonEGrappleAbilityState (Variables|Default|GetGrappleState)
    (:NewEnumerator0
      (return (|CallParentFunction)))
    (:NewEnumerator1
      _)
    (:NewEnumerator2
      _)
    (:NewEnumerator3
      _)
    (:NewEnumerator4
      _))
  (return false))

(fn GetProjectileClass
  (return (Variables|Projectile|GetGrappleProjectileClass)))

(fn OnValidGrappleHit
  (params (Hit :type Hit%20Result%20Structure) (HitComponent :type Scene%20Component%20Object%20Reference) (SporeCarrier :type BP%20Spore%20Carrier%20Object%20Reference))
  (bind (_bblockinghit _binitialoverlap _time _distance _location _impactpoint _normal _impactnormal _physmat _hitactor _hitcomponent _hitbonename) (Collision|BreakHitResult Hit))
  (Utilities|FlowControl|Sequence
    (:then_0
      (Variables|Default|SetLastHit Hit))
    (:then_1
      ;[0.6233 0.6233 0.6233 0.5] Check if hit was skeletal mesh
      (bind _asskeletal_mesh_component (Utilities|Casting|CastToSkeletalMeshComponent HitComponent))
      (LocalVariables|Setskeletal%20mesh%20target _asskeletal_mesh_component))
    (:then_2
      ;[0.6233 0.6233 0.6233 0.5] Setup Attach Point
      (Utilities|GetorSpawnAttachPoint)
      (Transformation|SetActorLocation (Variables|References|GetAttachPoint) (.ImpactPoint (Collision|BreakHitResult Hit)) false false)
      (Transformation|AttachComponentToComponent (Variables|References|GetAttachPoint) _hitcomponent _hitbonename "KeepWorld" "KeepWorld" "KeepWorld" true))
    (:then_3
      ;[0.6233 0.6233 0.6233 0.5] Update Grapple State
      (bind _skeletal_mesh_target (LocalVariables|Getskeletal%20mesh%20target)
        (:then
          (if (Physics|IsSimulatingPhysics _skeletal_mesh_target (.BoneName (Collision|BreakHitResult Hit)))
            (CallFunction|SetGrappleState "NewEnumerator4")
            (else
              (CallFunction|SetGrappleState "NewEnumerator3"))))
        (:else
          (if (Physics|IsSimulatingPhysics HitComponent "None")
            (CallFunction|SetGrappleState "NewEnumerator4")
            (else
              (CallFunction|SetGrappleState "NewEnumerator3"))))))))

(fn CompleteAbility
  (params (Success :type Boolean))
  (|CallParentFunction Success)
  (Utilities|FlowControl|Sequence
    (:then_0
      (switch Utilities|FlowControl|Switch|SwitchonEGrappleAbilityState (Variables|Default|GetGrappleState)
        (:NewEnumerator3
          _)
        (:NewEnumerator4
          _))
      (CallFunction|EndZip))
    (:then_1
      (Variables|Default|SetGrappleState "NewEnumerator0")
      (Default|SetGrappleActive (Variables|References|GetGrapple) false))
    (:then_2
      (IronPuller|DestroyIronPuller))))

(fn GetMaxGrappleDistance
  (return (Variables|AbilitySettings|GetDefaultMaxGrappleDistance)))

(fn StartAbility
  (bind _grapple (Variables|References|GetGrapple))
  (bind (_started _start_vfx) (|CallParentFunction))
  (Utilities|FlowControl|Sequence
    (:then_0
      (if _started
        (CallFunction|FireGrappleProjectile)
        (Default|SetGrappleActive _grapple true)
        (Variables|/Game/Patchwork/Blueprints/Core/Pawns/Abilities/Grapple/BP_Grapple.BP_Grapple_C|SetProjectile _grapple (Variables|References|GetCurrentProjectile))))
    (:then_1
      (return _started _start_vfx))))

(fn SetGrappleState
  (params (GrappleState :type EGrappleAbilityState%20Enum :default "NewEnumerator0"))
  (bind _output_get (Variables|Default|SetGrappleState GrappleState))
  (switch Utilities|FlowControl|Switch|SwitchonEGrappleAbilityState _output_get
    (:NewEnumerator0
      (bind _movestate (Class|BPIPlayerPawn|GetPlayerMoveState(Message) (Components|GetOwner) :!label _label))
      (if (Utilities|Enum|Equal(Enum) _movestate "NewEnumerator6")
        (CallFunction|EndZip)))
    (:NewEnumerator1
      (goto _label))
    (:NewEnumerator2
      (goto _label))
    (:NewEnumerator3
      (CallFunction|BeginZiptoKinematic))
    (:NewEnumerator4
      (CallFunction|BeginZiptoDynamic))))

(fn UpdateGrappleVisualSettings
  (Variables|/Game/Patchwork/Blueprints/Core/Pawns/Abilities/Grapple/BP_Grapple.BP_Grapple_C|SetMaxDistance (Variables|References|GetGrapple) (Getters|GetMaxGrappleDistance)))

(fn ApplyZipForcetoPlayer
  (bind _returnvalue (Components|GetOwner))
  (bind _lasthit (Variables|Default|GetLastHit))
  (bind _zipforcerange (Variables|AbilitySettings|GetZipForceRange))
  (bind _normal (Collision|BreakHitResult _lasthit))
  (bind (_has_floor _floor_hit) (Class|BPIPlayerPawn|GetPlayerFloor(Message) _returnvalue))
  (if _has_floor
    (Class|BPIPlayerPawn|ApplyBounceForce(Message) _returnvalue (* (.Normal (Collision|BreakHitResult _floor_hit)) (Variables|AbilitySettings|GetZipGroundedBounceForce)) false true))
  (Utilities|FlowControl|Sequence
    (:then_0
      (if (Variables|AbilitySettings|GetUseConstantForce)
        (LocalVariables|SetZipForce (Variables|AbilitySettings|GetZipForceConstant))
        (else
          (LocalVariables|SetZipForce (Math|Float|MapRangeClamped (Math|Vector|Distance(Vector) (Transformation|GetActorLocation (Variables|References|GetAttachPoint)) (Transformation|GetWorldLocation)) (Variables|AbilitySettings|GetGrappleEndDistance) (Variables|AbilitySettings|GetDefaultMaxGrappleDistance) (.x _zipforcerange) (.y _zipforcerange))))))
    (:then_1
      ;[0.6233 0.6233 0.6233 0.5] Get Offset Amount
      (if (> (- 1.0 (Math|Float|Absolute(Float) (Math|Vector|DotProduct _normal "0.000000,0.000000,1.000000"))) 0.5)
        (LocalVariables|Setoffset (* (Variables|AbilitySettings|GetNormalOffsetAmountWall) _normal))
        (else
          (LocalVariables|Setoffset (* (Variables|AbilitySettings|GetNormalOffsetAmountFloor) _normal)))))
    (:then_2
      (Class|BPIPlayerPawn|AddForce(Message) (Components|GetOwner) (* (Math|Vector|Normalize (- (+ (Transformation|GetActorLocation (Variables|References|GetAttachPoint)) (LocalVariables|Getoffset)) (Transformation|GetWorldLocation))) (LocalVariables|GetZipForce))))))

(fn CheckGrappleDistance
  (return (<= (Class|KismetMathLibrary|VectorDistanceSquared (Transformation|GetActorLocation (Variables|References|GetAttachPoint)) (Transformation|GetWorldLocation)) (Variables|AbilitySettings|GetGrappleEndDistanceSqr))))

(fn OnPlayerMushBounced
  (params (Mushroom :type Actor%20Object%20Reference)))

(fn SetupIronPullerforHit
  (params (hit :type Hit%20Result%20Structure))
  (bind _returnvalue (Components|GetOwner))
  (bind _hitactor (Collision|BreakHitResult hit))
  (Utilities|FlowControl|Sequence
    (:then_0
      ;[0.6233 0.6233 0.6233 0.5] If no implementation is provided for BPI_Pullable use dummy puller
      (if (Utilities|DoesObjectImplementInterface _hitactor "/Game/Patchwork/Blueprints/Interfaces/BPI_Pullable.BPI_Pullable_C")
        (LocalVariables|SetTargetActor _hitactor)
        (else
          (bind _dummypuller (Utilities|GetorSpawnDummy hit))
          (LocalVariables|SetTargetActor _dummypuller))))
    (:then_1
      (IronPuller|DestroyIronPuller) ; destroy previous puller
    )
    (:then_2
      ;[0.6233 0.6233 0.6233 0.5] Spawn Puller
      (bind _returnvalue_2 (Game|AddComponentbyClass _returnvalue "/Game/Patchwork/Blueprints/Core/Pawns/Abilities/Grapple/IronPuller.IronPuller_C" true (Transformation|GetRelativeTransform) _returnvalue (LocalVariables|GetTargetActor) (Variables|/Script/Engine.Actor|GetRootComponent (Variables|References|GetAttachPoint)) self))
      (Variables|Default|SetCurrentIronPuller _returnvalue_2))))

(fn DestroyIronPuller
  (bind _currentironpuller (Variables|Default|GetCurrentIronPuller)
    (:then
      (Default|SetPullerActive _currentironpuller false)
      (Components|DestroyComponent _currentironpuller)
      (Development|PrintString "Destroyed Puller"))
    (:else)))

(fn CheckPullDistance
  (return (<= (Class|KismetMathLibrary|VectorDistanceSquared (Transformation|GetActorLocation (Variables|References|GetAttachPoint)) (Transformation|GetWorldLocation)) (Variables|AbilitySettings|GetGrapplePullDistanceSqr))))

(fn GetMass
  (return 0.0))