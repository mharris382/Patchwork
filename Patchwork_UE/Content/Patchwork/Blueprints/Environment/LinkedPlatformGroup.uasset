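; LinkedPlatformGroup is an environment actor that chains LinkedScalingPlatform actors into a sequence at construction time.
; It gathers targets by tag and from directly attached platforms, then links each to the next, closing the loop if Looped is set.
; Links carry the group's timing and behavior when ControlBehavior is on, and each linking platform receives the group's growth-based delay percentage.
; The start platform is set to auto-start and refreshes its designer arrows.
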(event EventBeginPlay)

(event Collision|EventActorBeginOverlap
  (params (OtherActor :type Actor%20Object%20Reference)))

(event EventTick
  (params (DeltaSeconds :type Float%20%28single-precision%29)))

(fn ConstructionScript
  (Utilities|FlowControl|Sequence
    (:then_0
      (if (not (== (Variables|Default|GetTarget%20Tag) "None"))
        (Utilities|Array|Clear (Variables|Default|GetTargets))
        (bind _outactors (Actor|GetAllActorsOfClasswithTag "/Game/Patchwork/Blueprints/Environment/LinkedScalingPlatform.LinkedScalingPlatform_C" (Variables|Default|GetTarget%20Tag)))
        (Variables|Default|Settargets _outactors)
        (Utilities|Array|Clear (LocalVariables|GetTmp))))
    (:then_1
      (Utilities|Array|Clear (LocalVariables|Gettmp))
      (for _array_element (Actor|GetAttachedActors true false)
        (bind _aslinked_scaling_platform (Utilities|Casting|CastToLinkedScalingPlatform _array_element))
        (Utilities|Array|Add (LocalVariables|GetTmp) _aslinked_scaling_platform))
      (for _array_element_2 (LocalVariables|GetTmp)
        (Utilities|Array|AddUnique (Variables|Default|GetTargets) _array_element_2)))
    (:then_2
      (CallFunction|UpdateFlow))))

(fn UpdateFlow
  (bind _returnvalue (Utilities|GetStartPlatform))
  (bind _targets (Variables|Default|Gettargets))
  (bind _behavior (Variables|Default|GetBehavior))
  (bind _targets_2 (Variables|Default|GetTargets))
  (bind _returnvalue_2 (Utilities|Array|Length _targets_2))
  (if (> _returnvalue_2 1)
    (for _index (range 0 _returnvalue_2)
      (LocalVariables|Setcurrent%20index _index)
      (LocalVariables|Setnext%20index (Math|Integer|%(Integer) (+ _index 1) _returnvalue_2))
      (if (< (LocalVariables|Getcurrent%20index) (LocalVariables|Getnext%20index))
        (Utilities|FlowControl|Sequence :!label _label
          (:then_0
            (if (and (Utilities|IsValid (Utilities|Array|Get(acopy) _targets (LocalVariables|Getcurrent%20index))) (Utilities|IsValid (Utilities|Array|Get(acopy) _targets (LocalVariables|Getnext%20index))))
              (Utilities|Array|SetArrayElem (Variables|/Game/Patchwork/Blueprints/Environment/LinkedScalingPlatform.LinkedScalingPlatform_C|Getlinked%20platforms (Utilities|Array|Get(acopy) _targets (LocalVariables|Getcurrent%20index))) 0 (select (Variables|Default|GetControl%20Behavior) (Utilities|Struct|MakeS_LinkedScalingPlatform (Utilities|Array|Get(acopy) _targets (LocalVariables|Getnext%20index)) (.delay _behavior) (.growthtime _behavior) (.waittime _behavior) (.shrinktime _behavior) (.behavior _behavior)) (Utilities|Struct|MakeS_LinkedScalingPlatform (Utilities|Array|Get(acopy) _targets (LocalVariables|Getnext%20index)) 0.0)) true)
              (if true
                (Variables|/Game/Patchwork/Blueprints/Environment/LinkedScalingPlatform.LinkedScalingPlatform_C|Setpercent%20of%20growth%20time%20to%20add%20to%20delay (Utilities|Array|Get(acopy) _targets (LocalVariables|Getcurrent%20index)) (.growthpercent _behavior))))))
        (elif (Variables|Default|GetLooped)
          (goto _label))))
    (Utilities|IsValid _returnvalue
      (:Is%20Valid
        (Variables|/Game/Patchwork/Blueprints/Environment/LinkedScalingPlatform.LinkedScalingPlatform_C|Setauto%20start _returnvalue true)
        (Default|UpdateDesignerArrowstoChildren _returnvalue (Utilities|Array|MakeArray))
        (return)))))