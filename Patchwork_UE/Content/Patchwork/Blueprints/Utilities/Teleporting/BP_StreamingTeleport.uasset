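; Trigger actor that teleports the player to a TeleportTarget once World Partition streaming there has finished.
; On overlap, a DoOnce flags the player as teleporting, freezes input, optionally fades the camera, enables the target's streaming source and updates BP_DataLayerManager.
; A looping timer polls for streaming completion, then moves the player and restores streaming, world state, camera, input and the trigger.
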(event Custom|CheckTeleportComplete
  ;[0.15 0.15 0.15 0.5] Do the teleport after streaming is complete
  (if (Class|WorldPartitionStreamingSourceComponent|IsStreamingCompleted (Variables|/Game/Patchwork/Blueprints/Utilities/Teleporting/BP_StreamingTarget.BP_StreamingTarget_C|GetWorldPartitionStreamingSource (Variables|Default|GetTeleport%20Target)))
    (Development|PrintString "Stream successful")
    (bind _successful (CallFunction|TryTeleportPlayer))
    (Development|PrintText (Utilities|Text|FormatText "Teleport successful: {0}" _successful) true true "(R=1.000000,G=0.397669,B=0.000000,A=1.000000)" 5.0)
    (Utilities|Time|ClearandInvalidateTimerbyHandle (Variables|Default|GetCheckStreamingTimer))
    (CallFunction|ResetTeleporter)))

(event Custom|DoTeleport
  (Utilities|FlowControl|Sequence
    (:then_0
      (CallFunction|FreezePlayer)
      (Utilities|FadetoColor))
    (:then_1
      (Default|SetStreamingSourceEnabled (Variables|Default|GetTeleport%20Target) true)
      (Default|UpdatefromStreamingTarget (Variables|Default|GetDataLayerManager) (Variables|Default|GetTeleport%20Target)))
    (:then_2
      (Utilities|CalcRayTracePoints 5e+02))
    (:then_3
      ;[0.15 0.15 0.15 0.5] Do the teleport after streaming is complete
      (Utilities|Time|ClearandInvalidateTimerbyHandle (Variables|Default|GetCheckStreamingTimer))
      (bind _returnvalue (Utilities|Time|SetTimerbyEvent (delegate Custom|CheckTeleportComplete) 0.1 true true 0.1))
      (Variables|Default|SetCheckStreamingTimer _returnvalue))))

(event Custom|ResetTeleporter
  ;[0.15 0.15 0.15 0.5] Returns all involved actors to their default state, and sets IsPlayerTeleporting to false
  (Default|SetStreamingSourceEnabled (Variables|Default|GetTeleport%20Target) false)
  (Default|UpdateWorldState (Variables|Default|GetDataLayerManager))
  (CallFunction|ResetTrigger)
  (Utilities|FadefromColor)
  (CallFunction|UnfreezePlayer)
  (Utilities|SetPlayerTeleporting false))

(event Custom|Reset%20Trigger
  ;[0.15 0.15 0.15 0.5] Try to start the teleport process when the player overlaps with the actor
  (Utilities|FlowControl|DoOnce false) ; enters at Reset
)

(event EventBeginPlay
  (bind _returnvalue (Actor|GetActorOfClass "/Game/Patchwork/Blueprints/Environment/WorldStreaming/BP_DataLayerManager.BP_DataLayerManager_C"))
  (Variables|Default|SetDataLayerManager _returnvalue))

(event Collision|EventActorBeginOverlap
  (params (OtherActor :type Actor%20Object%20Reference))
  ;[0.15 0.15 0.15 0.5] Try to start the teleport process when the player overlaps with the actor
  (if (== OtherActor (Game|GetPlayerCharacter 0))
    (Utilities|IsValid (Variables|Default|GetTeleport%20Target)
      (:Is%20Valid
        (Utilities|FlowControl|DoOnce false
          (:Completed
            (Utilities|SetPlayerTeleporting true)
            (CallFunction|DoTeleport))))
      (:Is%20Not%20Valid
        (Development|PrintText "ERROR: Invalid Streaming Target" true true "(R=1.000000,G=0.000000,B=0.015653,A=1.000000)" 6.0)))))

(fn ConstructionScript)

(fn TryTeleportPlayer
  (bind _teleport_target (Variables|Default|GetTeleport%20Target))
  (bind (_location _rotation) (Default|GetLocationandRotation _teleport_target))
  (bind _returnvalue (Transformation|SetActorLocationAndRotation (Game|GetPlayerCharacter 0) _location _rotation))
  (return _returnvalue))

(fn FreezePlayer
  (bind _returnvalue (Game|GetPlayerController 0))
  (Class|BPIPlayerPawn|SetPlayerVelocity(Message) (Game|Player|GetPlayerPawn 0) "0, 0, 0")
  (Input|SetIgnoreMoveInput _returnvalue true)
  (Input|SetIgnoreLookInput _returnvalue true))

(fn UnfreezePlayer
  (bind _returnvalue (Game|GetPlayerController 0))
  (Input|ResetIgnoreMoveInput _returnvalue)
  (Input|ResetIgnoreLookInput _returnvalue))