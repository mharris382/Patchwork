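; Level controller for the anomaly: links the BP_Anomoly actor to its BP_Fragment actors and runs its menu sequence.
; On BeginPlay it checks that the placed fragment count matches the anomaly's data table.
; After load completes it resets fragments and binds anomaly events, so first interaction spawns fragments and a loaded anomaly restores them.
; Opening the menu plays a reach montage with timeline-driven FOV zoom and post-process blend, animated out on close.
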(event Custom|Init%20Anomoly
  (bind _main_anomoly (Variables|Default|Getmain%20anomoly))
  (for _array_element (Variables|Default|Getfragments)
    (Default|SetasUnspawned _array_element))
  (EventDispatchers|BindEventtoOnFirstInteraction _main_anomoly (delegate Custom|Do%20First%20Interact))
  (EventDispatchers|BindEventtoOnAnomolyLoaded _main_anomoly (delegate Custom|On%20Anomoly%20Loaded))
  (EventDispatchers|BindEventtoOpenAnomolyMenu _main_anomoly (delegate Custom|open%20menu))
  (Variables|/Game/Patchwork/Blueprints/Anomoly/BP_Anomoly.BP_Anomoly_C|Setinteraction%20enabled _main_anomoly true)
  (Variables|/Script/Engine.PostProcessComponent|SetBlendWeight (Variables|Default|GetExit%20PostProcess) 0.0))

(event Custom|On%20Load%20Completed
  (CallFunction|InitAnomoly))

(event Custom|Do%20First%20Interact
  (for _array_element (Variables|Default|Getfragments)
    (Default|SpawnFragment _array_element)
    (CallFunction|OpenMenu)))

(event Custom|On%20Anomoly%20Loaded
  (for _array_element (Variables|Default|Getfragments)
    (Default|LoadasSpawned _array_element)))

(event Custom|open%20menu
  (Default|SetInteractEnabled (Variables|Default|Getmain%20anomoly) false)
  (bind _aspaperperson (Utilities|Casting|CastTopaperperson (Game|Player|GetPlayerPawn 0)))
  (Input|DisableInput _aspaperperson (Game|GetPlayerController 0))
  (Animation|Montage|PlayMontage (Variables|/Script/Engine.Character|GetMesh _aspaperperson) "/Game/Characters/Mannequins/Animations/Mixamo/AM_ReachingOut.AM_ReachingOut"
    (:then
      (bind _aspaperperson_2 (Utilities|Casting|CastTopaperperson (Game|Player|GetPlayerPawn 0)))
      (bind _output_get (Variables|Default|SetAs%20Paperperson _aspaperperson_2))
      (bind _output_get_2 (Variables|Default|Setstarting%20fov (Variables|/Script/Engine.CameraComponent|GetFieldOfView (Variables|/Game/Patchwork/Blueprints/Pawns/BP_BaseCharacter.BP_BaseCharacter_C|GetCamera _output_get))))
      (Variables|Default|Setending%20fov (/ _output_get_2 3.0))
      (Variables|/Game/Patchwork/Blueprints/Pawns/BP_BaseCharacter.BP_BaseCharacter_C|Setmanual%20field%20of%20view _output_get true)
      (bind (_direction _post_process_alpha _fov) (Timeline|Animate%20Enter PlayFromStart)
        (:Update
          (Variables|/Script/Engine.PostProcessComponent|SetBlendWeight (Variables|Default|GetExit%20PostProcess) _post_process_alpha)
          (Camera|SetFieldOfView (Variables|/Game/Patchwork/Blueprints/Pawns/BP_BaseCharacter.BP_BaseCharacter_C|GetCamera (Variables|Default|GetAs%20Paperperson)) (Math|Float|Lerp (Variables|/Game/Patchwork/Blueprints/SaveData/PlayerSettings.PlayerSettings_C|GetFOV (Variables|/Game/Patchwork/Blueprints/PatchworkGameInstance.PatchworkGameInstance_C|GetCurrentSettings (.AsPatchwork%20Game%20Instance (Utilities|Casting|CastToPatchworkGameInstance (Game|GetGameInstance))))) (Variables|Default|Getending%20fov) _fov)))))
    (:OnCompleted
      (Input|EnableInput (Game|Player|GetPlayerPawn 0) (Game|GetPlayerController 0))
      (Utilities|IsValid (Variables|Default|Getanomoly%20UI)
        (:Is%20Valid
          _)
        (:Is%20Not%20Valid
          (bind _returnvalue (UserInterface|CreateWidget "/Game/Patchwork/Blueprints/Anomoly/WB_AnomolyMenu.WB_AnomolyMenu_C" (Game|GetPlayerController 0) (Variables|/Game/Patchwork/Blueprints/Anomoly/BP_Anomoly.BP_Anomoly_C|GetAnomolyData (Variables|Default|Getmain%20anomoly))))
          (bind _output_get_3 (Variables|Default|Setanomoly%20UI _returnvalue))
          (EventDispatchers|BindEventtoBPonWidgetDeactivated _output_get_3 (delegate Custom|on%20ui%20closed))))
      (UserInterface|Viewport|AddtoViewport (Variables|Default|Getanomoly%20UI) 10)
      (Input|SetInputModeUIOnly (Game|GetPlayerController 0) (Variables|Default|Getanomoly%20UI) "DoNotLock" false)
      (Class|CommonActivatableWidget|ActivateWidget (Variables|Default|Getanomoly%20UI)))))

(event Custom|on%20ui%20closed
  (bind _returnvalue (Game|GetPlayerController 0))
  (bind _returnvalue_2 (Game|GetPlayerController 0))
  (Widget|RemovefromParent (Variables|Default|Getanomoly%20UI))
  (Utilities|IsValid _returnvalue_2
    (:Is%20Valid
      (Variables|/Script/Engine.PlayerController|SetbShowMouseCursor _returnvalue_2 false))
    (:Is%20Not%20Valid
      _))
  (Input|SetInputModeGameOnly _returnvalue false)
  (Input|EnableInput (Game|Player|GetPlayerPawn 0) _returnvalue)
  (bind (_direction _post_process_alpha _fov) (Timeline|Animate%20Exit PlayFromStart)
    (:Update
      (Variables|/Script/Engine.PostProcessComponent|SetBlendWeight (Variables|Default|GetExit%20PostProcess) _post_process_alpha)
      (Camera|SetFieldOfView (Variables|/Game/Patchwork/Blueprints/Pawns/BP_BaseCharacter.BP_BaseCharacter_C|GetCamera (Variables|Default|GetAs%20Paperperson)) (Math|Float|Lerp (Variables|/Game/Patchwork/Blueprints/SaveData/PlayerSettings.PlayerSettings_C|GetFOV (Variables|/Game/Patchwork/Blueprints/PatchworkGameInstance.PatchworkGameInstance_C|GetCurrentSettings (.AsPatchwork%20Game%20Instance (Utilities|Casting|CastToPatchworkGameInstance (Game|GetGameInstance))))) (Variables|Default|Getending%20fov) _fov)))
    (:Finished
      (Variables|/Game/Patchwork/Blueprints/Pawns/BP_BaseCharacter.BP_BaseCharacter_C|Setmanual%20field%20of%20view (Variables|Default|GetAs%20Paperperson) false)
      (Default|SetInteractEnabled (Variables|Default|Getmain%20anomoly) true))))

(event EventBeginPlay
  (Variables|/Script/Engine.PostProcessComponent|SetBlendWeight (Variables|Default|GetExit%20PostProcess) 0.0)
  (bind _returnvalue (Actor|GetActorOfClass "/Game/Patchwork/Blueprints/Anomoly/BP_Anomoly.BP_Anomoly_C"))
  (bind _output_get (Variables|Default|Setmain%20anomoly _returnvalue))
  (Utilities|IsValid _output_get
    (:Is%20Valid
      (if (and (Default|IsAnomolyValid _output_get) (Default|IsFragmentDatabaseValid _output_get))
        (bind _outrownames (DataTable|GetDataTableRowNames (.fragmentdatatable (Variables|/Game/Patchwork/Blueprints/Anomoly/BP_Anomoly.BP_Anomoly_C|GetAnomolyData (Variables|Default|Getmain%20anomoly)))))
        (bind _outactors (Actor|GetAllActorsOfClass "/Game/Patchwork/Blueprints/Anomoly/BP_Fragment.BP_Fragment_C"))
        (bind _output_get_2 (Variables|Default|Setfragments _outactors))
        (if (== (Utilities|Array|Length _output_get_2) (Utilities|Array|Length _outrownames))
          (Variables|Default|Setis%20valid true)
          (else
            (Variables|Default|Setis%20valid false)
            (Development|PrintText "Not all fragments found in level" true true "(R=1.000000,G=0.000000,B=0.022180,A=1.000000)")))
        (else
          (Development|PrintText "anomoly data is not valid" true true "(R=1.000000,G=0.000000,B=0.022180,A=1.000000)")
          (Variables|Default|Setis%20valid false))))
    (:Is%20Not%20Valid
      (Development|PrintText "no anomoly found in level" true true "(R=1.000000,G=0.753322,B=0.000000,A=1.000000)"))))

(fn ConstructionScript)