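; Spore toxicity effect for the forest level that gives the player a tripping screen distortion.
; It overrides the parent's toxicity-changed handler and, only when IsPlayer is set, writes toxicity scaled by MaxDistortion into a material parameter collection scalar.
; The visual itself comes from whichever materials read that parameter, and BeginPlay and Tick are unused.
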(event EventBeginPlay
  (|CallParentFunction) ; This node is disabled and will not be called.\nDrag off pins to build functionality.
)

(event EventTick
  (params (DeltaSeconds :type Float%20%28single-precision%29))
  (|CallParentFunction DeltaSeconds) ; This node is disabled and will not be called.\nDrag off pins to build functionality.
)

(fn OnToxicityChanged
  (params (new%20toxicity :type Float%20%28double-precision%29))
  (|CallParentFunction new%20toxicity)
  (if (Variables|Default|GetIs%20Player)
    (Rendering|Material|SetScalarParameterValue (Variables|Default|GetParameter%20Collection) (Variables|Default|GetDistortion%20Parameter%20Name) (* new%20toxicity (Variables|Default|GetMax%20Distortion)) :!class /Script/Engine.KismetMaterialLibrary)))