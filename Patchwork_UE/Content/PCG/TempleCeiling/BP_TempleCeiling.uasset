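; BP_TempleCeiling is a Blueprint for a temple ceiling in the PCG content, holding brick sizing for generation.
; Its construction script derives GEN brick extents from base extents and a scale multiplier, and a spacing offset from those extents and the overlap, before running the parent script.
; It overrides GetBoundsVerticalHeight to return the larger of the parent's value and its own Height.
; The event graph holds only disabled stubs.
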(event EventBeginPlay
  (|CallParentFunction) ; This node is disabled and will not be called.\nDrag off pins to build functionality.
)

(event Collision|EventActorBeginOverlap
  (params (OtherActor :type Actor%20Object%20Reference))
  (|CallParentFunction OtherActor) ; This node is disabled and will not be called.\nDrag off pins to build functionality.
)

(event EventTick
  (params (DeltaSeconds :type Float%20%28single-precision%29))
  (|CallParentFunction DeltaSeconds) ; This node is disabled and will not be called.\nDrag off pins to build functionality.
)

(fn ConstructionScript
  (Utilities|FlowControl|Sequence
    (:then_0
      (bind _output_get (Variables|PCGINTERNAL|SetGEN_BrickExtents (* (Variables|01-Temple|GetBrickExtents) (Variables|01-Temple|GetBrickScaleMultiplier))))
      (Variables|PCGINTERNAL|SetGEN_BrickSpacingOffset (* _output_get (Variables|01-Temple|GetBrickOverlap))))
    (:then_1
      (|CallParentFunction))))

(fn GetBoundsVerticalHeight
  (return (Math|Float|Max(Float) (|CallParentFunction) (Variables|01-Temple|GetHeight))))