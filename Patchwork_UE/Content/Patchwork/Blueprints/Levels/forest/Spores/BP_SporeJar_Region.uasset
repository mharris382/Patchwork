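; BP_SporeJar_Region is a timed spore region with a Niagara effect matching its spore type.
; The spore name selects a DT_SporeEffects row, applied to the Niagara system during construction and reassigned on BeginPlay with the spore tag before parent logic runs.
; BeginPlay passes Lifetime to Niagara and starts a timer that deactivates the region, then destroys the actor after a short delay.
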(event Custom|destroy
  (CallFunction|SetActive false)
  (Utilities|FlowControl|Delay 5.0)
  (Actor|DestroyActor))

(event EventBeginPlay
  (Variables|Default|SetSporeTypeTag (Variables|Default|GetSporeTag))
  (Variables|Default|SetEffect%20Type (Utilities|Struct|MakeDataTableRowHandle "/Game/Patchwork/Data/Datatables/DT_SporeEffects.DT_SporeEffects" (Variables|Default|GetSporeName)))
  (|CallParentFunction)
  (Niagara|SetNiagaraVariable(Float) (Variables|Default|GetNiagara) "Lifespan" (Variables|Default|GetLifetime))
  (Niagara|ResetSystem (Variables|Default|GetNiagara))
  (Utilities|Time|SetTimerbyEvent (delegate Custom|destroy) (Variables|Default|GetLifetime)))

(event Collision|EventActorBeginOverlap
  (params (OtherActor :type Actor%20Object%20Reference))
  (|CallParentFunction OtherActor) ; This node is disabled and will not be called.\nDrag off pins to build functionality.
)

(event EventTick
  (params (DeltaSeconds :type Float%20%28single-precision%29))
  (|CallParentFunction DeltaSeconds) ; This node is disabled and will not be called.\nDrag off pins to build functionality.
)

(fn ConstructionScript
  (bind _sporename (Variables|Default|GetSporeName))
  (|CallParentFunction)
  (if (!= _sporename "")
    (Variables|Default|SetEffect%20Type (Utilities|Struct|MakeDataTableRowHandle "/Game/Patchwork/Data/Datatables/DT_SporeEffects.DT_SporeEffects" _sporename))
    (CallFunction|ApplySporeEffecttoSystem (Variables|Default|GetNiagara))))