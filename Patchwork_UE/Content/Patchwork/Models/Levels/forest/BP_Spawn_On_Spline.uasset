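; Spline actor that lays a chosen static mesh along PipeSpline as a deforming pipe-like strip, built in the editor.
; The construction script destroys and clears its tracked spline meshes, then adds one spline mesh component per spline segment.
; Each takes position, tangent, scale and roll from the segment's two spline points, with scale multiplied by GlobalScaleMultiplier.
; The event graph has no runtime logic.
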(event EventBeginPlay)

(event Collision|EventActorBeginOverlap
  (params (OtherActor :type Actor%20Object%20Reference)))

(event EventTick
  (params (DeltaSeconds :type Float%20%28single-precision%29)))

(fn ConstructionScript
  (bind _pipe_spline (Variables|Default|GetPipe_Spline))
  (for _array_element (Variables|Default|GetSpline%20Meshes)
    (Components|DestroyComponent _array_element))
  (Utilities|Array|Clear (Variables|Default|GetSpline%20Meshes))
  (for _index (range 0 (- (Class|SplineComponent|GetNumberOfSplineSegments (Variables|Default|GetPipe_Spline)) 1))
    (bind _returnvalue (AddComponent|AddSplineMeshComponent false (Math|Transform|MakeTransform "0, 0, 0")))
    (Components|StaticMesh|SetStaticMesh _returnvalue (Variables|Default|GetMesh))
    (Utilities|Array|Add (Variables|Default|GetSpline%20Meshes) _returnvalue)
    (SplineMesh|SetStartPosition _returnvalue (.Position (Utilities|Struct|BreakSplinePoint (Spline|GetSplinePointAt _pipe_spline _index "Local"))) false)
    (SplineMesh|SetStartTangent _returnvalue (.LeaveTangent (Utilities|Struct|BreakSplinePoint (Spline|GetSplinePointAt _pipe_spline _index "Local"))) false :!class /Script/Engine.SplineMeshComponent)
    (SplineMesh|SetStartScale _returnvalue (* (Math|Vector2D|MakeVector2D (.y (.Scale (Utilities|Struct|BreakSplinePoint (Spline|GetSplinePointAt _pipe_spline _index "Local")))) (.z (.Scale (Utilities|Struct|BreakSplinePoint (Spline|GetSplinePointAt _pipe_spline _index "Local"))))) (Variables|Default|GetGlobal%20Scale%20Multiplier)) false :!class /Script/Engine.SplineMeshComponent)
    (SplineMesh|SetStartRollDegrees _returnvalue (.roll (.Rotation (Utilities|Struct|BreakSplinePoint (Spline|GetSplinePointAt _pipe_spline _index "Local")))) false)
    (SplineMesh|SetEndPosition _returnvalue (.Position (Utilities|Struct|BreakSplinePoint (Spline|GetSplinePointAt _pipe_spline (+ _index 1) "Local"))) false)
    (SplineMesh|SetEndTangent _returnvalue (.ArriveTangent (Utilities|Struct|BreakSplinePoint (Spline|GetSplinePointAt _pipe_spline (+ _index 1) "Local"))) false :!class /Script/Engine.SplineMeshComponent)
    (SplineMesh|SetEndScale _returnvalue (* (Math|Vector2D|MakeVector2D (.y (.Scale (Utilities|Struct|BreakSplinePoint (Spline|GetSplinePointAt _pipe_spline (+ _index 1) "Local")))) (.z (.Scale (Utilities|Struct|BreakSplinePoint (Spline|GetSplinePointAt _pipe_spline (+ _index 1) "Local"))))) (Variables|Default|GetGlobal%20Scale%20Multiplier)) false :!class /Script/Engine.SplineMeshComponent)
    (SplineMesh|SetEndRollDegrees _returnvalue (.roll (.Rotation (Utilities|Struct|BreakSplinePoint (Spline|GetSplinePointAt _pipe_spline (+ _index 1) "Local")))) true)))