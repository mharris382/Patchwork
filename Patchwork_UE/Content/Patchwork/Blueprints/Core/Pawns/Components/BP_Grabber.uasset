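; BP_Grabber is a scene component that picks up and releases physics objects through the owner's PhysicsHandle on IA_Interact, using a hit supplied by SetTrace.
; "Controlled Rotation" or "Controlled Position" tags on the actor or component select the grab mode, otherwise grabbing at the hit point.
; Tick makes held objects ignore the Pawn channel, restores blocking after release, and updates target rotation for rotation-controlled objects; it never sets target location.
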(event Custom|Reset%20CollisionResponse
  (Utilities|IsValid (Variables|Default|Getlast%20grabbed%20component)
    (:Is%20Valid
      (Collision|SetCollisionResponsetoChannel (Variables|Default|Getlast%20grabbed%20component) "ECC_Pawn" "ECR_Block"))))

(event Custom|Disable%20col%20Response
  (bind _last_grabbed_component (Variables|Default|Getlast%20grabbed%20component))
  (Utilities|IsValid _last_grabbed_component
    (:Is%20Valid
      (Collision|SetCollisionResponsetoChannel _last_grabbed_component "ECC_Pawn" "ECR_Ignore"))))

(event Input|EnhancedActionEvents|EnhancedInputActionIA_Interact
  (params (ActionValue :type Boolean) (ElapsedSeconds :type Float%20%28double-precision%29) (TriggeredSeconds :type Float%20%28double-precision%29) (InputAction :type Input%20Action%20Object%20Reference :default "/Game/Patchwork/Data/Input/IA_Interact.IA_Interact"))
  (bind _returnvalue (Transformation|GetWorldRotation))
  (bind _returnvalue_2 (Transformation|GetWorldLocation))
  (bind _hit (Variables|Default|Gethit))
  (Utilities|CarryingObject
    (:carrying
      (Physics|Components|PhysicsHandle|ReleaseComponent (Variables|Default|Gethandle)))
    (:not%20carrying
      (if (Variables|Default|Gethas%20hit)
        (Variables|Default|Sethit%20bonne (.hitbonename _hit))
        (Utilities|GetGrabMode (.hitcomponent _hit)
          (:control%20rotation
            (Transformation|SetWorldLocationAndRotation _returnvalue_2 _returnvalue false false)
            (Physics|Components|PhysicsHandle|GrabComponentatLocationwithRotation (Variables|Default|Gethandle) (.hitcomponent _hit) (.hitbonename _hit) _returnvalue_2 _returnvalue))
          (:control%20position
            (Transformation|SetWorldLocation _returnvalue_2 false false)
            (Class|PhysicsHandleComponent|GrabComponentatLocation (Variables|Default|Gethandle) (.hitcomponent _hit) (.hitbonename _hit) _returnvalue_2))
          (:default
            (Class|PhysicsHandleComponent|GrabComponentatLocation (Variables|Default|Gethandle) (.hitcomponent _hit) (.hitbonename _hit) (.location _hit))))))))

(event EventBeginPlay
  (Variables|Default|Sethandle (Actor|GetComponentbyClass (Components|GetOwner) "/Script/Engine.PhysicsHandleComponent")))

(event EventTick
  (params (DeltaSeconds :type Float%20%28single-precision%29))
  (bind _handle (Variables|Default|Gethandle))
  (bind _returnvalue (Class|PhysicsHandleComponent|GetGrabbedComponent _handle))
  (Utilities|IsValid _returnvalue
    (:Is%20Valid
      (Utilities|FlowControl|Sequence
        (:then_0
          (Utilities|IsValid (Variables|Default|Getlast%20grabbed%20component)
            (:Is%20Valid
              (if (not (== _returnvalue (Variables|Default|Getlast%20grabbed%20component)))
                _
                (else
                  (CallFunction|ResetCollisionResponse)))
              (Variables|Default|Setlast%20grabbed%20component _returnvalue)
              (CallFunction|DisableColResponse))
            (:Is%20Not%20Valid
              (Variables|Default|Setlast%20grabbed%20component _returnvalue)
              (CallFunction|DisableColResponse))))
        (:then_1
          (if (or (Actor|ActorHasTag (Components|GetOwner _returnvalue) "Controlled Rotation") (Components|ComponentHasTag _returnvalue "Controlled Rotation"))
            (Class|PhysicsHandleComponent|SetTargetRotation (Variables|Default|Gethandle) (Transformation|GetWorldRotation))))))
    (:Is%20Not%20Valid
      (Utilities|IsValid (Variables|Default|Getlast%20grabbed%20component)
        (:Is%20Valid
          (CallFunction|ResetCollisionResponse))))))

(fn SetTrace
  (params (has%20hit :type Boolean) (hit :type Hit%20Result%20Structure))
  (Variables|Default|Sethas%20hit has%20hit)
  (Variables|Default|Sethit hit))