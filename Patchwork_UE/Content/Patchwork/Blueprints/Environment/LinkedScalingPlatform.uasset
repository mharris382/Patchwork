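; A platform actor that scales between shrunken and grown sizes and triggers linked platforms in a chain, begun by instances set to auto-start.
; Each trigger resolves delay and timings against defaults, then passes per-link settings onward, offsetting delay by a share of growth time.
; Tick drives scale through optional per-axis vector curves, growing, then waiting and shrinking if the behavior calls for it.
; The construction script recursively draws color-coded arrows between links for designers.
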(event Custom|Next%20Growth
  (Variables|Default|Setcnt (+ (Variables|Default|Getcnt) 1))
  ;[0.6233 0.6233 0.6233 0.5] Assign Values for Next Scaling Action
  (switch int (Variables|Default|Getcnt)
    (:0
      (Variables|Default|Setis%20shrinking false)
      (Variables|Default|Settarget%20scale (Math|Vector|SelectVector (Variables|Behavior|GetGrow%20Scale) (Variables|Behavior|GetShrink%20Scale) (Variables|Default|Getis%20shrinking)) :!label _label)
      (Variables|Default|Setstart%20scale (Math|Vector|SelectVector (Variables|Behavior|GetGrow%20Scale) (Variables|Behavior|GetShrink%20Scale) (not (Variables|Default|Getis%20shrinking))))
      (Variables|Default|Settarget%20time (Math|Float|SelectFloat (Variables|Default|GetShrink%20Time) (Variables|Default|GetGrow%20Time) (Variables|Default|Getis%20shrinking)))
      (Variables|Default|Settarget%20curve (.AsCurve%20Float (Utilities|Casting|CastToCurveFloat (Utilities|SelectObject (Variables|Default|GetShrink%20Curve) (Variables|Default|GetGrow%20Curve) (Variables|Default|Getis%20shrinking)))))
      (Variables|Default|Settarget%20curve_0 (.AsCurve%20Vector (Utilities|Casting|CastToCurveVector (Utilities|SelectObject (Variables|Behavior|GetShrink%20Curve_0) (Variables|Behavior|GetGrow%20Curve_0) (Variables|Default|Getis%20shrinking)))))
      (Variables|Testing|Sett 0.0)
      (Variables|Default|Setis%20waiting false))
    (:1
      (Variables|Default|Setis%20waiting true)
      (switch Utilities|FlowControl|Switch|SwitchonEScalingPlatformMode (Variables|Default|GetBehavior)
        (:NewEnumerator0
          (Utilities|FlowControl|Delay (Variables|Default|GetWait%20Time))
          (Variables|Default|Setis%20shrinking true)
          (goto _label))))
    (:2
      (Variables|Default|Setis%20waiting true))))

(event Custom|Trigger%20Platform%20Behavior
  (params (behavior :type S%20Linked%20Scaling%20Platform%20Structure))
  (bind _behavior (CallFunction|GetBehavior behavior))
  (bind (_target _delay _growthtime _waittime _shrinktime _behavior_2) (Utilities|Struct|BreakS_LinkedScalingPlatform _behavior))
  ;[0.6233 0.6233 0.6233 0.5] Trigger Next Platform
  (Variables|Default|Setis%20waiting true)
  (Utilities|FlowControl|Delay _delay)
  (Variables|Default|SetBehavior _behavior_2)
  (Variables|Default|SetGrow%20Time _growthtime)
  (Variables|Default|SetWait%20Time _waittime)
  (Variables|Default|SetShrink%20Time _shrinktime)
  (Variables|Default|Setcnt -1)
  (CallFunction|ResetChainCount) ; only does anything if this is the autostart mushroom
  (CallFunction|NextGrowth)
  (for _array_element (Variables|Behavior|Getlinked%20platforms)
    (Utilities|IsValid (.Target (Utilities|Struct|BreakS_LinkedScalingPlatform _array_element))
      (:Is%20Valid
        (CallFunction|TriggerPlatformBehavior (.Target (Utilities|Struct|BreakS_LinkedScalingPlatform _array_element)) (Utilities|Struct|MakeS_LinkedScalingPlatform (.Target (Utilities|Struct|BreakS_LinkedScalingPlatform _array_element)) (+ (* (Variables|Default|GetGrow%20Time) (Variables|Behavior|Getpercent%20of%20growth%20time%20to%20add%20to%20delay)) (Utilities|SelectorDefault (.delay (Utilities|Struct|BreakS_LinkedScalingPlatform _array_element)) (.delay (Variables|LinkedScalingPlatform_C|Getdefault%20behavior (.Target (Utilities|Struct|BreakS_LinkedScalingPlatform _array_element)))))) (.growthtime (Utilities|Struct|BreakS_LinkedScalingPlatform _array_element)) (.waittime (Utilities|Struct|BreakS_LinkedScalingPlatform _array_element)) (.shrinktime (Utilities|Struct|BreakS_LinkedScalingPlatform _array_element)) (.behavior (Utilities|Struct|BreakS_LinkedScalingPlatform _array_element))))))))

(event EventBeginPlay
  (Variables|Default|Setis%20waiting true)
  (Transformation|SetRelativeScale3D (Variables|Default|GetScale%20Pivot) (Variables|Behavior|GetShrink%20Scale))
  (if (Variables|Behavior|Getauto%20start)
    (CallFunction|TriggerPlatformBehavior (Variables|Behavior|Getdefault%20behavior))))

(event Collision|EventActorBeginOverlap
  (params (OtherActor :type Actor%20Object%20Reference)))

(event EventTick
  (params (DeltaSeconds :type Float%20%28single-precision%29))
  ;[0.6233 0.6233 0.6233 0.5] Tick
  (if (not (Variables|Default|Getis%20waiting))
    (Utilities|FlowControl|Sequence
      (:then_0
        (Variables|Testing|Sett (Math|Float|Clamp(Float) (+ (/ DeltaSeconds (Variables|Default|Gettarget%20time)) (Variables|Testing|Gett))))
        (Transformation|SetRelativeScale3D (Variables|Default|GetScale%20Pivot) (CallFunction|EvaluateCurve (Variables|Testing|Gett) (Variables|Default|Gettarget%20curve_0) (Variables|Default|Gettarget%20scale) (Variables|Default|Getstart%20scale)))
        (if (>= (Variables|Testing|Gett) 1.0)
          (CallFunction|NextGrowth))))))

(fn ConstructionScript
  (bind _override_material (Variables|Visuals|GetOverride%20Material))
  (Utilities|FlowControl|Sequence
    (:then_0
      (Components|StaticMesh|SetStaticMesh (Variables|Default|GetStaticMesh1) (Variables|Visuals|GetMesh))
      (Variables|Default|Setis%20shrinking false)
      (Variables|Default|Setcnt (Math|Integer|SelectInt 0 1 (Variables|Default|Getis%20shrinking)))
      (CallFunction|UpdateScales (Math|Float|%(Float) (Variables|Testing|Gett) 1.0)))
    (:then_1
      (Utilities|IsValid _override_material
        (:Is%20Valid
          (Rendering|Material|SetMaterial (Variables|Default|GetStaticMesh1) 0 _override_material))))
    (:then_2
      (Utilities|FlowControl|Sequence
        (:then_0
          (CallFunction|UpdateDesignerArrows (Utilities|Array|MakeArray)))))))

(fn EvaluateCurve
  (params (InputPin :type Float%20%28double-precision%29) (InputPin2 :type Curve%20Vector%20Object%20Reference) (start :type Vector :default "50.000000,50.000000,50.000000") (end :type Vector :default "50.000000,50.000000,50.000000"))
  (bind (_x _y _z) (Math|Vector|BreakVector start))
  (bind (_x_2 _y_2 _z_2) (Math|Vector|BreakVector end))
  (bind _returnvalue (Math|Curves|GetVectorValue InputPin2 InputPin))
  (return (Math|Vector|SelectVector (Math|Vector|MakeVector (Math|Float|Lerp _x _x_2 (.x _returnvalue)) (Math|Float|Lerp _y _y_2 (.y _returnvalue)) (Math|Float|Lerp _z _z_2 (.z _returnvalue))) (Math|Vector|Lerp(Vector) start end InputPin) (Utilities|IsValid InputPin2))))

(fn GetBehavior
  (params (in%20behavior :type S%20Linked%20Scaling%20Platform%20Structure))
  (bind _default_behavior (Variables|Behavior|Getdefault%20behavior))
  (return (Utilities|Struct|MakeS_LinkedScalingPlatform self (Utilities|SelectorDefault (.delay in%20behavior) (.delay _default_behavior)) (Utilities|SelectorDefault (.growthtime in%20behavior) (.growthtime _default_behavior)) (Utilities|SelectorDefault (.waittime in%20behavior) (.waittime _default_behavior)) (Utilities|SelectorDefault (.shrinktime in%20behavior) (.shrinktime _default_behavior)) (.behavior in%20behavior))))

(fn UpdateDesignerArrows
  (params (visited :type Array%20of%20Linked%20Scaling%20Platform%20Object%20References))
  (bind _arrows (Variables|Default|GetArrows))
  (bind _arrows_2 (Variables|Default|GetArrows))
  (bind _returnvalue (Transformation|GetWorldLocation _arrows_2))
  (bind _output_get (LocalVariables|SetNewLocalVar visited))
  (if (not (Utilities|Array|ContainsItem _output_get self))
    (Utilities|Array|Add _output_get self))
  (Utilities|FlowControl|Sequence
    (:then_0
      (for _array_element (Components|GetChildrenComponents (Variables|Default|GetArrows) false)
        (Components|DestroyComponent _array_element)))
    (:then_1
      (for _array_element_2 (Variables|Behavior|Getlinked%20platforms)
        (Utilities|IsValid (.Target (Utilities|Struct|BreakS_LinkedScalingPlatform _array_element_2))
          (:Is%20Valid
            (LocalVariables|Setcurrent%20target (.Target (Utilities|Struct|BreakS_LinkedScalingPlatform _array_element_2)))
            (Utilities|FlowControl|Sequence
              (:then_0
                (bind _returnvalue_2 (AddComponent|AddArrowComponent self false (Transformation|GetRelativeTransform _arrows)))
                (LocalVariables|Setcurrent%20arrow _returnvalue_2)
                (Transformation|AttachComponentToComponent _returnvalue_2 _arrows "None" "KeepRelative" "KeepWorld" "KeepWorld" true)
                (Transformation|SetWorldRotation (LocalVariables|Getcurrent%20arrow) (Math|Rotator|FindLookatRotation _returnvalue (Transformation|GetWorldLocation (Variables|LinkedScalingPlatform_C|GetArrows (.Target (Utilities|Struct|BreakS_LinkedScalingPlatform _array_element_2))))) false false)
                (Variables|/Script/Engine.ArrowComponent|SetArrowLength (LocalVariables|Getcurrent%20arrow) (Math|Vector|Distance(Vector) (Transformation|GetWorldLocation (Variables|LinkedScalingPlatform_C|GetArrows (.Target (Utilities|Struct|BreakS_LinkedScalingPlatform _array_element_2)))) _returnvalue))
                (Transformation|SetWorldScale3D (Variables|Default|GetArrows) "1.000000,1.000000,1.000000")
                (Variables|/Script/Engine.ArrowComponent|SetArrowColor (LocalVariables|Getcurrent%20arrow) (select (Variables|Behavior|Getauto%20start) (Variables|designercolorcode|Getauto%20start%20color) (select (Variables|LinkedScalingPlatform_C|Getauto%20start (LocalVariables|Getcurrent%20target)) (Variables|designercolorcode|Getrestart%20color) (select (Utilities|Enum|Equal(Enum) (.behavior (Utilities|Struct|BreakS_LinkedScalingPlatform _array_element_2)) "NewEnumerator1") (Variables|designercolorcode|Getgrow%20only%20color) (select (Math|Boolean|ANDBoolean (<= (.delay (Utilities|Struct|BreakS_LinkedScalingPlatform _array_element_2)) 0.0) (<= (.growthtime (Utilities|Struct|BreakS_LinkedScalingPlatform _array_element_2)) 0.0) (<= (.waittime (Utilities|Struct|BreakS_LinkedScalingPlatform _array_element_2)) 0.0) (<= (.shrinktime (Utilities|Struct|BreakS_LinkedScalingPlatform _array_element_2)) 0.0)) (Variables|DesignerColorCode|Getdefault%20color) (Variables|DesignerColorCode|Getoveridden%20settings%20color))))))
                (if (Variables|LinkedScalingPlatform_C|Getauto%20start (LocalVariables|Getcurrent%20target))
                  (Transformation|AddLocalOffset (LocalVariables|Getcurrent%20arrow) "0.000000,0.000000,-100.000000" false false)))
              (:then_1
                (if (not (Utilities|Array|ContainsItem (LocalVariables|GetNewLocalVar) (.Target (Utilities|Struct|BreakS_LinkedScalingPlatform _array_element_2))))
                  (CallFunction|UpdateDesignerArrows (.Target (Utilities|Struct|BreakS_LinkedScalingPlatform _array_element_2)) (LocalVariables|GetNewLocalVar)))))))))))

(fn ResetChainCount
  (if (Variables|Behavior|Getauto%20start)
    (CallFunction|ResetChainCountRecursive (Utilities|Array|MakeArray))))

(fn ResetChainCountRecursive
  (params (visited :type Array%20of%20Linked%20Scaling%20Platform%20Object%20References))
  (bind _output_get (LocalVariables|SetNewLocalVar_0 visited))
  (Utilities|Array|AddUnique _output_get self)
  (Variables|Default|Setchain%20count 0)
  (for _array_element (Variables|Behavior|Getlinked%20platforms)
    (Utilities|IsValid (.Target (Utilities|Struct|BreakS_LinkedScalingPlatform _array_element))
      (:Is%20Valid
        (Variables|Default|Setchain%20count 0)
        (if (not (Utilities|Array|ContainsItem (LocalVariables|GetNewLocalVar_0) (.Target (Utilities|Struct|BreakS_LinkedScalingPlatform _array_element))))
          (CallFunction|ResetChainCountRecursive (.Target (Utilities|Struct|BreakS_LinkedScalingPlatform _array_element)) (LocalVariables|GetNewLocalVar_0)))))))

(fn UpdateScales
  (params (t :type Float%20%28double-precision%29))
  (if (Variables|Testing|GetIs%20Debugging)
    (Transformation|SetRelativeScale3D (Variables|Default|GetScale%20Pivot) (Math|Vector|SelectVector (CallFunction|EvaluateCurve t (Variables|Behavior|GetShrink%20Curve_0) (Variables|Behavior|GetGrow%20Scale) (Variables|Behavior|GetShrink%20Scale)) (CallFunction|EvaluateCurve t (Variables|Behavior|GetGrow%20Curve_0) (Variables|Behavior|GetShrink%20Scale) (Variables|Behavior|GetGrow%20Scale)) (Variables|Default|Getis%20shrinking)))
    (else
      (Transformation|SetRelativeScale3D (Variables|Default|GetScale%20Pivot) (Math|Vector|SelectVector (Variables|Behavior|GetShrink%20Scale) (Variables|Behavior|GetGrow%20Scale) (Variables|Default|Getis%20shrinking))))))