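; Player ability scene component that manages an ability's readiness, in-use state, optional cooldown and feedback effects.
; StartAbility and CompleteAbility toggle the in-use state and fire started and completed dispatchers.
; A successful completion timestamps the cooldown for readiness checks and starts a delay that triggers ready FX.
; Gameplay tags select the impact effects played at the component, though the cooldown's RemainingTime actually returns elapsed time.
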(event Custom|CustomEvent
  (params (Success :type Boolean))
  ;[0.6233 0.6233 0.6233 0.5] Start Cooldown Timer on Ability Complete
  (if Success
    (Variables|Cooldown|SetLastUseTimestamp (Utilities|Time|GetGameTimeinSeconds))
    (Utilities|FlowControl|Delay (Conditions|GetCooldownDuration))
    (CallFunction|CooldownCompleted)))

(event EventBeginPlay
  ;[0.6233 0.6233 0.6233 0.5] Start Cooldown Timer on Ability Complete
  (if (Variables|Cooldown|GetHasCooldown)
    (EventDispatchers|BindEventtoOnAbilityCompleted (delegate Custom|CustomEvent))))

(event EventTick
  (params (DeltaSeconds :type Float%20%28single-precision%29)))

(fn IsReady
  (if (not (Variables|Default|GetInUse))
    (if (Variables|Cooldown|GetHasCooldown)
      (return (not (.IsInCooldown (Conditions|CheckCooldown))))
      (else
        (return true)))))

(fn UseAbility
  (if (Conditions|IsReady)
    (return true)
    (else
      (return false))))

(fn CheckCooldown
  (bind _returnvalue (Utilities|Time|GetGameTimeinSeconds))
  (bind _lastusetimestamp (Variables|Cooldown|GetLastUseTimestamp))
  (bind _returnvalue_2 (- _returnvalue _lastusetimestamp))
  (if (Variables|Cooldown|GetHasCooldown)
    (return (> (Conditions|GetCooldownDuration) _returnvalue_2) _returnvalue_2)
    (else
      (return false 0.0))))

(fn GetCooldownDuration
  (return (Variables|Cooldown|GetDefaultCooldownDuration)))

(fn PlayAbilityStartFX
  (if (GameplayTags|IsGameplayTagValid (Variables|Feedbacks|GetAbilityStartedFXTag))
    (bind (_success _vfx) (CallFunction|PlayImpactatLocation (Variables|Feedbacks|GetAbilityStartedFXTag) (Transformation|GetWorldLocation) self))
    (if _success
      (return _success _vfx))
    (else
      (return false 0))))

(fn CompleteAbility
  (params (Success :type Boolean))
  (Variables|Default|SetInUse false)
  (Default|CallOnAbilityCompleted Success))

(fn StartAbility
  (if (Conditions|IsReady)
    (Variables|Default|SetInUse true)
    (Default|CallOnAbilityStarted)
    (bind _vfx (Utilities|PlayFXonSelf (Variables|Feedbacks|GetAbilityStartedFXTag))
      (:then
        (return true _vfx)))
    (else
      (Development|PrintText (Utilities|Text|FormatText "Grapple is in cooldown for {0} more seconds" (.RemainingTime (Conditions|CheckCooldown))))
      (return false 0))))

(fn CooldownCompleted
  (bind _abilityreadyfxtag (Variables|Feedbacks|GetAbilityReadyFXTag))
  (if (GameplayTags|IsGameplayTagValid _abilityreadyfxtag)
    (Utilities|PlayFXonSelf _abilityreadyfxtag)
    (else
      (Development|PrintString (Utilities|String|Append "No Valid Tag for player ability cooldown completed.  Ability Name = " (Utilities|GetClassDisplayName (Utilities|GetClass self)))))))