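; Base player character for Patchwork that manages a switchable first/third-person camera.
; Timelines blend the camera between views under perspective-mode locks, with a looping timer settling any leftover third-person offset.
; Tick records the last grounded transform, pins the first-person camera to its head target, and turns the view toward dialogue or anomaly targets through BPI_InteractLookAt.
; FOV follows game-instance settings, easing to a dialogue value in first person.
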(event Custom|Transition%20to%20TP
  (params (Restart :type Boolean))
  (bind _returnvalue (Pawn|GetController))
  (bind _returnvalue_2 (Pawn|GetControlRotation _returnvalue :!class /Script/Engine.Controller))
  (CallFunction|ClearTimers)
  (Transformation|AttachComponentToComponent (Variables|Default|GetCamera) (Variables|Collision|GetCapsuleComponent) "None" "KeepWorld" "KeepWorld" "KeepRelative" true)
  (Camera|OnTransitionStart true)
  (Variables|Default|SetCamera%20State "NewEnumerator3")
  (if Restart
    (bind (_direction _blend _pitch_curve) (Timeline|Transition%20to%20Third PlayFromStart)
      (:Update
        (Transformation|SetWorldTransform (Variables|Default|GetCamera) (Math|Transform|Lerp(Transform) (Transformation|GetWorldTransform (Variables|Default|GetFirstPerson)) (Transformation|GetWorldTransform (Variables|Default|GetThirdPerson)) _blend) false false)
        ;[1 1 1] SLerp Pitch Rotation
        (Pawn|SetControlRotation _returnvalue (Math|Rotator|MakeRotator (.roll _returnvalue_2) (.pitch (Class|KismetMathLibrary|QuatRotator (Class|KismetMathLibrary|QuatSlerp (Math|Conversions|ToQuaternion(Rotator) (Pawn|GetControlRotation (Pawn|GetController) :!class /Script/Engine.Controller)) (Math|Conversions|ToQuaternion(Rotator) (.Rotation (Math|Transform|BreakTransform (Transformation|GetRelativeTransform (Variables|Default|GetSpringArm))))) _pitch_curve))) (.yaw _returnvalue_2))))
      (:Finished
        (Variables|Default|SetCamera%20State "NewEnumerator1")
        (Transformation|AttachComponentToComponent (Variables|Default|GetCamera) (Variables|Default|GetThirdPerson) "None" "KeepWorld" "KeepWorld" "KeepWorld" true)
        (Camera|OnTransitionEnd true)
        (if (Utilities|Operators|NotEqual(!=) :A (Variables|/Script/Engine.SceneComponent|GetRelativeLocation (Variables|Default|GetCamera)) :ErrorTolerance 0.001)
          (bind _returnvalue_3 (Utilities|Time|SetTimerbyEvent (delegate Custom|move%20to%20zero) 0.001 true))
          (Variables|Default|Setmove%20to%20zero%20timer _returnvalue_3))))
    (else
      (Timeline|Transition%20to%20Third Play))))

(event Custom|Transition%20to%20FP
  (params (Restart :type Boolean))
  (CallFunction|ClearTimers)
  (Transformation|AttachComponentToComponent (Variables|Default|GetCamera) (Variables|Collision|GetCapsuleComponent) "None" "KeepWorld" "KeepWorld" "KeepRelative" true)
  (Camera|OnTransitionStart false)
  (Variables|Default|SetCamera%20State "NewEnumerator2")
  (if Restart
    (bind _camera_blend (Timeline|Transition%20to%20First PlayFromStart)
      (:Update
        ;[1 1 1] Blend Transforms
        (Transformation|SetWorldTransform (Variables|Default|GetCamera) (Math|Transform|Lerp(Transform) (Transformation|GetWorldTransform (Variables|Default|GetThirdPerson)) (Math|Transform|MakeTransform (Utilities|GetFPCameraTargetLocation) (Transformation|GetWorldRotation (Variables|Default|GetCamera))) _camera_blend) false false))
      (:Finished
        (Variables|Default|SetCamera%20State "NewEnumerator0")
        (Camera|OnTransitionEnd false)))
    (else
      (Timeline|Transition%20to%20First Play))))

(event Custom|move%20to%20zero
  (bind _camera (Variables|Default|GetCamera))
  (bind _relativelocation (Variables|/Script/Engine.SceneComponent|GetRelativeLocation _camera))
  (if (Utilities|Operators|NotEqual(!=) :A _relativelocation :ErrorTolerance 0.001)
    (Transformation|SetRelativeLocation _camera (Math|Vector|Lerp(Vector) _relativelocation "0, 0, 0" 0.001) false false)
    (else
      (CallFunction|ClearTimers))))

(event Custom|Set%20Perspective%20Mode
  (params (Mode :type EPerspectiveMode%20Enum :default "NewEnumerator0"))
  ;[0.2396 0.2396 0.2396 0] Change Perspective Mode
  (if (not (Variables|Default|GetinDialogue))
    (if (Utilities|Enum|NotEqual(Enum) Mode (Variables|Default|GetPerspective%20Mode))
      (bind _output_get (Variables|Default|SetPerspective%20Mode Mode))
      (switch Utilities|FlowControl|Switch|SwitchonEPerspectiveMode _output_get
        (:NewEnumerator0
          ;;[1 1 1] if locked to TP and in FP
          (if (or (Utilities|Enum|Equal(Enum) (Variables|Default|GetCamera%20State) "NewEnumerator0") (Utilities|Enum|Equal(Enum) (Variables|Default|GetCamera%20State) "NewEnumerator2"))
            (CallFunction|TransitiontoFP false)))
        (:NewEnumerator1
          ;;[1 1 1] if locked to FP and in TP
          (if (or (Utilities|Enum|Equal(Enum) (Variables|Default|GetCamera%20State) "NewEnumerator1") (Utilities|Enum|Equal(Enum) (Variables|Default|GetCamera%20State) "NewEnumerator3"))
            (CallFunction|TransitiontoTP false)))))))

(event Custom|OnCurrentSettingsChanged
  (params (CurrentSettings :type Player%20Settings%20Object%20Reference))
  (Camera|SetFieldOfView (Variables|Default|GetCamera) (Variables|/Game/Patchwork/Blueprints/SaveData/PlayerSettings.PlayerSettings_C|GetFOV CurrentSettings)))

(event Custom|Clear%20Timers
  (Utilities|Time|ClearandInvalidateTimerbyHandle (Variables|Default|Getmove%20to%20zero%20timer)))

(event Input|EnhancedActionEvents|EnhancedInputActionIA_Pause
  (params (ActionValue :type Boolean) (ElapsedSeconds :type Float%20%28double-precision%29) (TriggeredSeconds :type Float%20%28double-precision%29) (InputAction :type Input%20Action%20Object%20Reference :default "/Game/Patchwork/Data/Input/IA_Pause.IA_Pause")))

(event EventBeginPlay
  (bind _aspatchwork_game_instance (Utilities|Casting|CastToPatchworkGameInstance (Game|GetGameInstance)))
  (bind _output_get (Variables|Default|SetPatchwork%20Game%20Instance _aspatchwork_game_instance))
  (Camera|SetFieldOfView (Variables|Default|GetCamera) (Variables|/Game/Patchwork/Blueprints/SaveData/PlayerSettings.PlayerSettings_C|GetFOV (Variables|/Game/Patchwork/Blueprints/PatchworkGameInstance.PatchworkGameInstance_C|GetCurrentSettings _output_get)))
  (Variables|Default|Sethas%20last%20location false))

(event Collision|EventActorBeginOverlap
  (params (OtherActor :type Actor%20Object%20Reference)))

(event EventTick
  (params (DeltaSeconds :type Float%20%28single-precision%29))
  (bind _dialogue_target (Variables|Default|Getdialogue%20target))
  (bind _camera (Variables|Default|GetCamera))
  (bind _camera_2 (Variables|Default|GetCamera))
  (bind _patchwork_game_instance (Variables|Default|GetPatchwork%20Game%20Instance))
  (bind _currentsettings (Variables|/Game/Patchwork/Blueprints/PatchworkGameInstance.PatchworkGameInstance_C|GetCurrentSettings _patchwork_game_instance))
  (Utilities|FlowControl|Sequence
    (:then_1
      ;[1 1 1] Update Ground Location
      (bind _can_save (CallFunction|CanSavePlayerLocation))
      (if _can_save
        (Variables|Default|Sethas%20last%20location true)
        (Variables|Default|Setlast%20ground%20location (Transformation|GetActorLocation))
        (Variables|Default|Setlast%20ground%20rotation (Transformation|GetActorRotation))))
    (:then_2
      ;[0.6233 0.6233 0.6233 0.5] Camera Stuff
      (Utilities|FlowControl|Sequence
        (:then_0
          (if (Variables|Default|Getis%20Interacting%20With%20Anomaly)
            (bind _output_get (Utilities|GetAnomalyActor))
            (bind _asbpi_interact_look_at (Utilities|Casting|CastToBPI_InteractLookAt _output_get))
            (CallFunction|LookatTarget _asbpi_interact_look_at DeltaSeconds)
            (else
              ;;[0.6233 0.6233 0.6233 0.5] Update Camera Facing Direction while look target is set
              (if (Variables|Default|GetinDialogue)
                (Utilities|IsValid _dialogue_target
                  (:Is%20Valid
                    (bind _asbpi_interact_look_at_2 (Utilities|Casting|CastToBPI_InteractLookAt _dialogue_target))
                    (CallFunction|LookatTarget _asbpi_interact_look_at_2 DeltaSeconds)))))))
        (:then_1
          ;;[1 1 1] Update camera in dialogues
          (if (not (Variables|Default|Getmanual%20field%20of%20view))
            (if (Variables|Default|GetinDialogue)
              (if (Camera|IsCameraFP)
                (Camera|SetFieldOfView _camera (Math|Float|Lerp (Variables|/Script/Engine.CameraComponent|GetFieldOfView _camera) (Variables|Default|Getdialogue%20fov) (* DeltaSeconds (Variables|Default|Getdialogue%20fov%20rate)))))
              (else
                (Utilities|IsValid _currentsettings
                  (:Is%20Valid
                    (Camera|SetFieldOfView _camera_2 (Math|Float|Lerp (Variables|/Script/Engine.CameraComponent|GetFieldOfView _camera_2) (Variables|/Game/Patchwork/Blueprints/SaveData/PlayerSettings.PlayerSettings_C|GetFOV _currentsettings) (* DeltaSeconds (Variables|Default|Getdialogue%20fov%20rate)))))
                  (:Is%20Not%20Valid
                    (Development|PrintText "Settings Missing")))))))
        (:then_2
          ;;[0.6233 0.6233 0.6233 0.5] Update Camera FP Location
          (switch Utilities|FlowControl|Switch|SwitchonEPerspectiveState (Variables|Default|GetCamera%20State)
            (:NewEnumerator0
              (Transformation|SetWorldLocation (Variables|Default|GetCamera) (Utilities|GetFPCameraTargetLocation) false false))))))))

(fn ConstructionScript)

(fn IsCameraFP
  (return (or (Utilities|Enum|Equal(Enum) (Variables|Default|GetCamera%20State) "NewEnumerator0") (Utilities|Enum|Equal(Enum) (Variables|Default|GetCamera%20State) "NewEnumerator2"))))

(fn IsCameraTransitioning
  (return (or (Utilities|Enum|Equal(Enum) (Variables|Default|GetCamera%20State) "NewEnumerator3") (Utilities|Enum|Equal(Enum) (Variables|Default|GetCamera%20State) "NewEnumerator2"))))

(fn SwitchCameras
  (switch Utilities|FlowControl|Switch|SwitchonEPerspectiveMode (Variables|Default|GetPerspective%20Mode)
    (:NewEnumerator0
      (Development|PrintText "Cannot Change to First Person right now"))
    (:NewEnumerator1
      (Development|PrintText "Cannot Change to Third Person right now"))
    (:NewEnumerator2
      ;[1 1 1] Block changes while transitioning
      (if (or (not (Camera|IsCameraTransitioning)) (Variables|Default|GetAllow%20Interupt%20Transition))
        ;[1 1 1] Trigger Transition to other camera mode
        (if (Camera|IsCameraFP)
          (CallFunction|TransitiontoTP true)
          (else
            (CallFunction|TransitiontoFP true)))
        (return true)
        (else
          (return false)))))
  (return false))

(fn GetCurrentSettings
  (bind _aspatchwork_game_instance (Utilities|Casting|CastToPatchworkGameInstance (Game|GetGameInstance)))
  (return (Variables|/Game/Patchwork/Blueprints/PatchworkGameInstance.PatchworkGameInstance_C|GetCurrentSettings _aspatchwork_game_instance)))

(fn OnTransitionStart
  (params (is%20transition%20to%20TP :type Boolean)))

(fn OnTransitionEnd
  (params (is%20transition%20to%20TP :type Boolean)))

(fn CanSavePlayerLocation
  (return (not (AI|Components|NavMovement|IsFalling (Variables|Character|GetCharacterMovement)))))

(fn IsAutojumping
  (return (Actor|ActorHasTag "Autojump")))

(fn LookatTarget
  (params (self2 :type BPI%20Interact%20Look%20at%20Interface) (A :type Float%20%28double-precision%29))
  (bind _look_at_location (Default|GetFPLookatLocationWS self2))
  (Pawn|SetControlRotation (Game|GetPlayerController 0) (Math|Rotator|FindLookatRotation (Transformation|GetWorldLocation (Variables|Default|GetCamera)) _look_at_location)))