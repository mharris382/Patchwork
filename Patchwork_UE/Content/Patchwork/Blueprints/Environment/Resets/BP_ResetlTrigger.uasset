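; Reset trigger actor that respawns the player at their last ground location when the player pawn overlaps it.
; Actor overlap is filtered to player pawn 0 before calling the respawn function.
; The construction script snaps a PostProcess component onto the shape from GetComponentShape when that shape is valid.
; GetComponentShape returns no component here, so that attachment only runs if an override supplies one.
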(event OnComponentBeginOverlap(Plane)
  (params (OverlappedComponent :type Primitive%20Component%20Object%20Reference) (OtherActor :type Actor%20Object%20Reference) (OtherComp :type Primitive%20Component%20Object%20Reference) (OtherBodyIndex :type Integer) (bFromSweep :type Boolean) (SweepResult :type Hit%20Result%20Structure%20%28by%20ref%29)))

(event EventBeginPlay)

(event Collision|EventActorBeginOverlap
  (params (OtherActor :type Actor%20Object%20Reference))
  (if (== OtherActor (Game|Player|GetPlayerPawn 0))
    (CallFunction|RespawnPlayeratLastGroundLocation)))

(event EventTick
  (params (DeltaSeconds :type Float%20%28single-precision%29)))

(fn ConstructionScript
  (bind _shape (CallFunction|GetComponentShape))
  (Utilities|IsValid _shape
    (:Is%20Valid
      (Transformation|AttachComponentToComponent (Variables|Default|GetPostProcess) _shape "None" "SnapToTarget" "SnapToTarget" "SnapToTarget" true))))

(fn GetComponentShape
  (return 0))