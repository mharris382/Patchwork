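; BP_AntiSporeEffect is a spore effect component that counteracts the other spore effects on the same owner.
; Each tick it runs the parent update, then checks whether its own toxicity is above a threshold.
; While it is, it finds the owner's other BP_PlayerSporeEffectBase components and sets each one's instant toxicity change to minus half that component's current toxicity.
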(event EventBeginPlay
  (|CallParentFunction) ; This node is disabled and will not be called.\nDrag off pins to build functionality.
)

(event EventTick
  (params (DeltaSeconds :type Float%20%28single-precision%29))
  (|CallParentFunction DeltaSeconds)
  (if (> (Variables|Default|GetCurrent%20Toxicity) 0.56)
    (for _array_element (Actor|GetComponentsByClass (Components|GetOwner) "/Game/Patchwork/Blueprints/Levels/forest/BP_PlayerSporeEffectBase.BP_PlayerSporeEffectBase_C")
      (if (!= _array_element self)
        (Variables|/Game/Patchwork/Blueprints/Levels/forest/BP_SporeEffectBase.BP_SporeEffectBase_C|SetInstant%20Toxicity%20Change _array_element (* (/ (Variables|/Game/Patchwork/Blueprints/Levels/forest/BP_SporeEffectBase.BP_SporeEffectBase_C|GetCurrent%20Toxicity _array_element) 2.0) -1.0))))))