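; Spherical variant of a spore region in the forest levels, built on a parent spore region Blueprint.
; The construction script feeds Radius into both the Sphere collision component and the Niagara system's "Sphere Radius" variable, so collision and effect share one size.
; It then destroys the Box component and applies the spore effect to the Niagara system through the parent's implementation.
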(event EventBeginPlay
  (|CallParentFunction) ; This node is disabled and will not be called.\nDrag off pins to build functionality.
)

(event Collision|EventActorBeginOverlap
  (params (OtherActor :type Actor%20Object%20Reference))
  (|CallParentFunction OtherActor) ; This node is disabled and will not be called.\nDrag off pins to build functionality.
)

(event EventTick
  (params (DeltaSeconds :type Float%20%28single-precision%29))
  (|CallParentFunction DeltaSeconds) ; This node is disabled and will not be called.\nDrag off pins to build functionality.
)

(fn ConstructionScript
  (|CallParentFunction)
  (CallFunction|UpdateRadius (Variables|Default|GetRadius))
  (Components|DestroyComponent (Variables|Default|GetBox))
  (CallFunction|ApplySporeEffecttoSystem (Variables|Default|GetNiagara)))

(fn UpdateRadius
  (params (InputPin :type Float%20%28double-precision%29))
  (Niagara|SetNiagaraVariable(Float) (Variables|Default|GetNiagara) "Sphere Radius" InputPin)
  (Components|Sphere|SetSphereRadius (Variables|Default|GetSphere) InputPin true))

(fn ApplySporeEffecttoSystem
  (params (self2 :type FX%20System%20Component%20Object%20Reference))
  (|CallParentFunction self2))