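; BP_TrippingTestArea is a test area that fades in a tripping effect while the player pawn overlaps it.
; Entering plays the TrippingFade timeline and leaving reverses it.
; Each timeline update remaps TrippingAmount up to MaxTrippiness and writes it to a named scalar in a Material Parameter Collection, so any material reading that parameter follows the fade.
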(event EventBeginPlay)

(event Collision|EventActorBeginOverlap
  (params (OtherActor :type Actor%20Object%20Reference))
  (if (== OtherActor (Game|Player|GetPlayerPawn 0))
    (bind _tripping_amount (Timeline|Tripping%20Fade Play)
      (:Update
        (Rendering|Material|SetScalarParameterValue (Variables|Default|GetParameter%20Collection) (Variables|Default|GetTripping%20Intensity%20Name) (Math|Float|MapRangeClamped _tripping_amount 0.0 1.0 0.0 (Variables|Default|GetMax%20Trippiness)) :!class /Script/Engine.KismetMaterialLibrary)))))

(event EventTick
  (params (DeltaSeconds :type Float%20%28single-precision%29)))

(event Collision|EventActorEndOverlap
  (params (OtherActor :type Actor%20Object%20Reference))
  (if (== OtherActor (Game|Player|GetPlayerPawn 0))
    (bind _tripping_amount (Timeline|Tripping%20Fade Reverse)
      (:Update
        (Rendering|Material|SetScalarParameterValue (Variables|Default|GetParameter%20Collection) (Variables|Default|GetTripping%20Intensity%20Name) (Math|Float|MapRangeClamped _tripping_amount 0.0 1.0 0.0 (Variables|Default|GetMax%20Trippiness)) :!class /Script/Engine.KismetMaterialLibrary)))))

(fn ConstructionScript)