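; Interactable dialogue NPC with a Paper2D sprite that registers with GM_BaseGameMode and starts its DialogueComp conversation on interact.
; Tick yaws the sprite pivot toward the player based on a flag or distance check, and returns the NPC to its start if it falls out of the world.
; Named dialogue events run as functions via next-tick timers; a recorded event also triggers a world event and is saved with transform and dialogue progress, then replayed on load.
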(event Custom|Reset%20All%20Recorded%20Events)

(event EventBeginPlay
  (|CallParentFunction)
  (Variables|Default|SetStart%20Location (Transformation|GetActorLocation))
  (Development|PrintString (Utilities|GetDisplayName self))
  (bind _asgm_base_game_mode (Utilities|Casting|CastToGM_BaseGameMode (Game|GetGameMode))
    (:then
      (bind _output_get (Variables|Default|SetGM%20Game%20Mode _asgm_base_game_mode))
      (Default|AddNPC _output_get self))
    (:CastFailed
      (Development|PrintString "Incorrect Game Mode Found"))))

(event Collision|EventActorBeginOverlap
  (params (OtherActor :type Actor%20Object%20Reference)))

(event EventTick
  (params (DeltaSeconds :type Float%20%28single-precision%29))
  (bind _pivot (Variables|Default|Getpivot))
  (Utilities|FlowControl|Sequence
    (:then_0
      (if (Variables|FacePlayer|Getalways%20face%20player)
        (Transformation|SetWorldRotation _pivot (Math|Rotator|MakeRotator 0.0 0.0 (.yaw (Math|Rotator|FindLookatRotation (Transformation|GetWorldLocation _pivot) (Transformation|GetActorLocation (Game|Player|GetPlayerPawn 0))))) false false :!label _label)
        (elif (> (Variables|FacePlayer|Getface%20player%20distance) 0.0)
          (if (< (* (Variables|FacePlayer|Getface%20player%20distance) (Variables|FacePlayer|Getface%20player%20distance)) (Class|KismetMathLibrary|VectorDistanceSquared (Transformation|GetActorLocation (Game|Player|GetPlayerPawn 0)) (Transformation|GetWorldLocation (Variables|Default|Getpivot))))
            (goto _label)
            (else
              (Transformation|SetWorldRotation _pivot (Math|Rotator|MakeRotator 0.0 0.0 0.0) false false))))))
    (:then_1
      (if (< (.z (Transformation|GetActorLocation)) -2e+04)
        (Transformation|SetActorLocation (Variables|Default|GetStart%20Location) false false)))))

(event EventInvokeDialogueEvent
  (params (Event%20Name :type Name :default "None"))
  (if (!= Event%20Name "")
    (Development|PrintText (Utilities|Text|FormatText "Called event {0} " Event%20Name))
    (Class|KismetSystemLibrary|SetTimerforNextTick 0 (Utilities|String|ToString(Name) Event%20Name))))

(event EventOnInteract
  (Default|StartDialogue (Variables|Default|GetDialogueComp)))

(fn ConstructionScript
  (|CallParentFunction)
  (Rendering|Components|Sprite|SetSprite (Variables|Default|GetPaperSprite) (Variables|Default|GetCharacter%20Sprite))
  (Variables|/Game/Templates/Defender/Blueprints/Components/DialogueComp.DialogueComp_C|SetDialogueDT (Variables|Default|GetDialogueComp) (Variables|Default|GetDialogue%20DT))
  (Variables|/Game/Templates/Defender/Blueprints/Components/DialogueComp.DialogueComp_C|SetParticipant (Variables|Default|GetDialogueComp) (Variables|Dialogue|GetParticipant)))

(fn RecordDialogueEvent
  (params (event%20name :type Name))
  (bind _output_get (Variables|Default|SetRecorded%20Event event%20name))
  (Default|InvokeWorldEvent (Variables|Default|GetGM%20Game%20Mode) _output_get))

(fn ClearRecordedEvent
  (Variables|Default|SetRecorded%20Event "None"))

(fn InvokeRecordedEvent
  (if (!= (Variables|Default|GetRecorded%20Event) "")
    (Class|KismetSystemLibrary|SetTimerforNextTick 0 (Utilities|String|ToString(Name) (Variables|Default|GetRecorded%20Event)))))

(fn GetNPCSaveData
  (return (Utilities|Struct|MakeS_NPC_SaveData (CallFunction|GetSaveKey) (Transformation|GetActorTransform self) (Variables|/Game/Templates/Defender/Blueprints/Components/DialogueComp.DialogueComp_C|GetContinueFrom (Variables|Default|GetDialogueComp)) (Variables|Default|GetRecorded%20Event))))

(fn LoadNPCSaveData
  (params (Save%20Data :type S%20NPC%20Save%20Data%20Structure))
  (if (== (.actorname Save%20Data) (CallFunction|GetSaveKey))
    (Transformation|SetActorTransform (.tranform Save%20Data) false true)
    (Variables|/Game/Templates/Defender/Blueprints/Components/DialogueComp.DialogueComp_C|SetContinueFrom (Variables|Default|GetDialogueComp) (.continuefrom Save%20Data))
    (CallFunction|RecordDialogueEvent (.recordedevent Save%20Data))
    (CallFunction|InvokeRecordedEvent)
    (else
      (Development|PrintString "Tried to load incorrect npc data"))))

(fn GetSaveKey
  (return (Utilities|String|StringToName (Utilities|GetDisplayName self))))

(fn ChangeDialogue
  (params (new%20dialogue :type Data%20Table%20Object%20Reference))
  (Utilities|IsValid new%20dialogue
    (:Is%20Valid
      (if (Variables|/Game/Templates/Defender/Blueprints/Components/DialogueComp.DialogueComp_C|GetInDialogue (Variables|Default|GetDialogueComp))
        (Development|PrintString "cannot change while in dialogue")
        (else
          (Variables|/Game/Templates/Defender/Blueprints/Components/DialogueComp.DialogueComp_C|SetDialogueDT (Variables|Default|GetDialogueComp) new%20dialogue))))))

(fn ChangeSpeed
  (params (Max%20Walk%20Speed :type Float%20%28single-precision%29))
  (Variables|/Script/Engine.CharacterMovementComponent|SetMaxWalkSpeed (Variables|Character|GetCharacterMovement) Max%20Walk%20Speed))

(fn GetInteractionMessage
  (return "Talk"))

(fn GetInteractVerb
  (return ""))

(fn GetNPCName
  (bind _dialoguecomp (Variables|Default|GetDialogueComp))
  (bind _participant (Variables|/Game/Templates/Defender/Blueprints/Components/DialogueComp.DialogueComp_C|GetParticipant _dialoguecomp))
  (bind _returnvalue (Utilities|GetDataTableRow (.datatable _participant) (.rowname _participant))
    (:then
      (return (.DisplayName (Utilities|Struct|BreakDialogueParticipantStruct _returnvalue))))
    (:RowNotFound
      (return "ERROR NULL VALUE"))))

(fn IsInteractAvailable
  (return (not (Variables|/Game/Templates/Defender/Blueprints/Components/DialogueComp.DialogueComp_C|GetInDialogue (Variables|Default|GetDialogueComp)))))