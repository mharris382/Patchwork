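; HUB game mode that updates the collected-item displays in the level to match world events that have occurred.
; On BeginPlay, if the game instance reports a just-loaded game, a looping timer polls until that flag clears, then stops.
; It then finds every BP_CollectedItemDisplay and sets its collected state from whether its item event ID has occurred; without a fresh load, this runs immediately.
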(event Custom|Check%20if%20done%20loading
  (if (not (Variables|/Game/Patchwork/Blueprints/PatchworkGameInstance.PatchworkGameInstance_C|GetJust%20Loaded%20Game (Variables|Default|GetPatchwork%20Game%20Instance)))
    (Utilities|Time|ClearandInvalidateTimerbyHandle (Variables|Default|Getcheck%20timer))
    (bind _outactors (Actor|GetAllActorsOfClass "/Game/Patchwork/Blueprints/Environment/BP_CollectedItemDisplay.BP_CollectedItemDisplay_C"))
    (for _array_element _outactors
      (bind _event_occured (CallFunction|HasWorldEventOccured (Default|GetItemEventID _array_element)))
      (Default|SetCollected _array_element _event_occured))))

(event EventBeginPlay
  (|CallParentFunction)
  (if (Variables|/Game/Patchwork/Blueprints/PatchworkGameInstance.PatchworkGameInstance_C|GetJust%20Loaded%20Game (Variables|Default|GetPatchwork%20Game%20Instance))
    (bind _returnvalue (Utilities|Time|SetTimerbyEvent (delegate Custom|Check%20if%20done%20loading) 0.1 true))
    (Variables|Default|Setcheck%20timer _returnvalue)
    (else
      (bind _outactors (Actor|GetAllActorsOfClass "/Game/Patchwork/Blueprints/Environment/BP_CollectedItemDisplay.BP_CollectedItemDisplay_C"))
      (for _array_element _outactors
        (bind _event_occured (CallFunction|HasWorldEventOccured (Default|GetItemEventID _array_element)))
        (Default|SetCollected _array_element _event_occured)))))

(fn ConstructionScript)