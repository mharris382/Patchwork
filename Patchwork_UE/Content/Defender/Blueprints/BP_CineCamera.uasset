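; BP_CineCamera is a cine camera that can take over the player's view and track the player character.
; StartTracking sets the camera as player controller 0's view target and enables its built-in look-at tracking on the character.
; StopTracking returns the view target to the character and resets the tracking settings to defaults.
; Both events request a cubic blend and leave triggering to external callers.
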(event Custom|StartTracking
  (Game|Player|SetViewTargetwithBlend (Game|GetPlayerController 0) self 0.0 "VTBlend_Cubic" 0.5 false)
  (Variables|Default|SetLookatTrackingSettings (Utilities|Struct|MakeCameraLookatTrackingSettings true false 0.0 (Utilities|ResolveSoftReference (Game|GetPlayerCharacter 0)))))

(event Custom|StopTracking
  (Game|Player|SetViewTargetwithBlend (Game|GetPlayerController 0) (Game|GetPlayerCharacter 0) 0.0 "VTBlend_Cubic" 0.5 false)
  (Variables|Default|SetLookatTrackingSettings (Utilities|Struct|MakeCameraLookatTrackingSettings false false)))

(fn ConstructionScript)