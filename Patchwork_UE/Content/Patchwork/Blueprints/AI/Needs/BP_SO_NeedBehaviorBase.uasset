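; Base Smart Object behavior that lets a triggered character fulfill a need through its need component.
; Depending on config flags, it marks the need as being fulfilled, then either ends immediately or starts a looping evaluation timer.
; Each tick rolls a per-urgency stop chance, ending on success, missing entry or halted fulfillment.
; On finish it invalidates the timer handle and, when waiting on urgency, sets the fulfilling flag true again rather than clearing it.
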(event Custom|TryFullfillNeed
  (if (Variables|Default|GetSetFullfillingNeed)
    (Variables|/Game/Patchwork/Blueprints/AI/Needs/Need.Need_C|SetIsFulfillingNeed (Variables|Default|GetNeedComponent) true)
    (if (Variables|Default|GetWaitForNeedUrgencyThreshold)
      (bind _returnvalue (Utilities|Time|SetTimerbyEvent (delegate Custom|Evaluate%20Urgency) (Variables|Default|GetEvaluationPeriod) true))
      (Variables|Default|SetEvaluateUrgencyTimerHandle _returnvalue)
      (else
        (GameplayBehavior|EndBehavior (Variables|Default|GetAvatar) :!label _label)))
    (else
      (goto _label))))

(event Custom|Evaluate%20Urgency
  (bind _fuzzystopchancelookup (Variables|Default|GetFuzzyStopChanceLookup))
  (bind _needcomponent (Variables|Default|GetNeedComponent))
  (bind _isurgent (Default|GetNeedUrgency _needcomponent))
  (bind (_value _returnvalue) (Utilities|Map|Find _fuzzystopchancelookup _isurgent))
  (if (Variables|/Game/Patchwork/Blueprints/AI/Needs/Need.Need_C|GetIsFulfillingNeed (Variables|Default|GetNeedComponent))
    (if _returnvalue
      (if (< (Math|Random|RandomFloat) _value)
        (GameplayBehavior|EndBehavior (Variables|Default|GetAvatar)))
      (else
        (Development|PrintText (Variables|Default|GetAvatar) (Utilities|Text|FormatText "{0} has no stop chance for need urgency level {1}" (Utilities|GetClassDisplayName (Utilities|GetClass self)) (Utilities|String|EnumtoString _isurgent)))
        (GameplayBehavior|EndBehavior (Variables|Default|GetAvatar))))
    (else
      (Development|PrintText (Variables|Default|GetAvatar) "Need stopped being fulfilled")
      (GameplayBehavior|EndBehavior (Variables|Default|GetAvatar)))))

(event GameplayBehavior|EventOnTriggeredCharacter
  (params (Avatar :type Character%20Object%20Reference) (Config :type Gameplay%20Behavior%20Config%20Object%20Reference) (SmartObjectOwner :type Actor%20Object%20Reference))
  (bind _output_get (Variables|Default|SetAvatar Avatar))
  (Variables|Default|SetNeedConfig Config)
  (Variables|Default|SetNeedSmartObject SmartObjectOwner)
  (Variables|Default|SetNeedComponent (Actor|GetComponentbyClass _output_get (Variables|Default|GetNeedClass)))
  (CallFunction|TryFullfillNeed))

(event GameplayBehavior|EventOnFinishedCharacter
  (params (Avatar :type Character%20Object%20Reference) (bWasInterrupted :type Boolean)))

(event EventOnFinished
  (params (Avatar :type Actor%20Object%20Reference) (bWasInterrupted :type Boolean))
  (bind _needcomponent (Variables|Default|GetNeedComponent))
  (bind _evaluateurgencytimerhandle (Variables|Default|GetEvaluateUrgencyTimerHandle))
  (Utilities|FlowControl|Sequence
    (:then_0
      (if (Utilities|Time|IsValidTimerHandle _evaluateurgencytimerhandle)
        (Utilities|Time|InvalidateTimerHandle _evaluateurgencytimerhandle)))
    (:then_1
      (if (and (Variables|Default|GetSetFullfillingNeed) (Variables|Default|GetWaitForNeedUrgencyThreshold))
        (Utilities|IsValid _needcomponent
          (:Is%20Valid
            (Variables|/Game/Patchwork/Blueprints/AI/Needs/Need.Need_C|SetIsFulfillingNeed _needcomponent true)))))))