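; CutsceneTester is a debug helper actor that previews a level sequence when play begins, gated by a Test flag.
; After a configurable delay, it plays the assigned sequencer's player, either once or looping indefinitely.
; It can also move the player pawn to the location of an assigned position actor.
; The construction script does nothing; it only holds a disconnected copy of the same logic.
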(event EventBeginPlay
  (if (Variables|Default|GetTest)
    (Utilities|FlowControl|Delay (Variables|Default|GetDelay))
    (Utilities|FlowControl|Sequence
      (:then_0
        (bind _sequencer (Variables|Default|GetSequencer)
          (:then
            (if (Variables|Default|GetLooping)
              (Class|MovieSceneSequencePlayer|PlayLooping (Variables|/Script/LevelSequence.LevelSequenceActor|GetSequencePlayer _sequencer) -1)
              (else
                (Sequencer|Player|Play (Variables|/Script/LevelSequence.LevelSequenceActor|GetSequencePlayer _sequencer) :!class /Script/MovieScene.MovieSceneSequencePlayer))))
          (:else)))
      (:then_1
        (if (Variables|Default|GetTeleportPlayer)
          (bind _teleportplayerposition (Variables|Default|GetTeleportPlayerPosition)
            (:then
              (Transformation|SetActorLocation (Game|Player|GetPlayerPawn 0) (Transformation|GetActorLocation _teleportplayerposition) false false))
            (:else)))))))

(fn ConstructionScript)