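; BP_KeyPart is a collectible key part placed in the paper desert level.
; Its construction script formats PartNumber into a world event name shared by its EventInvoker and EventListener, with overlap handling left to the parent class.
; When the event is received, or has already occurred at BeginPlay, it hides the mesh, spawns a Niagara collection effect and disables invoking on player overlap.
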(event Custom|Key%20Collected
  (Rendering|SetVisibility (Variables|Default|GetStaticMesh) false false)
  (Niagara|SpawnSystematLocation "/Game/Patchwork/Effects/NS_Collection_Effect.NS_Collection_Effect" (Transformation|GetWorldLocation (Variables|Default|GetStaticMesh)))
  (Variables|Default|SetInvoke%20On%20Player%20Overlapped false))

(event EventActorBeginOverlap
  (params (OtherActor :type Actor%20Object%20Reference))
  (|CallParentFunction OtherActor))

(event EventBeginPlay
  (|CallParentFunction)
  (EventDispatchers|BindEventtoOnEventRecieved (Variables|Default|GetEventListener) (delegate Custom|Key%20Collected))
  (bind _occured (Default|HasEventOccured (Variables|Default|GetEventInvoker)))
  (if _occured
    (CallFunction|KeyCollected)))

(fn ConstructionScript
  (bind _part_number (Variables|Default|GetPart%20Number))
  (bind _event_name_format (Variables|Default|GetEvent%20Name%20Format))
  (bind _result (Utilities|Text|FormatText _event_name_format _part_number))
  (bind _returnvalue (Utilities|String|ToString(Text) _result))
  (bind _returnvalue_2 (Utilities|String|StringToName _returnvalue))
  (Variables|Default|SetWorld%20Event%20Name _returnvalue_2)
  (|CallParentFunction)
  (bind _output_get (Variables|/Game/Patchwork/Blueprints/WorldEvents/EventInvoker.EventInvoker_C|SetEvent%20Name (Variables|Default|GetEventInvoker) _returnvalue_2))
  (Variables|/Game/Patchwork/Blueprints/WorldEvents/EventListener.EventListener_C|SetEvent%20Name (Variables|Default|GetEventListener) _output_get))