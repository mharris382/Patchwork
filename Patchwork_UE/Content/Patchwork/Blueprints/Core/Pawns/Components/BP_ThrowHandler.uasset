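; Pawn scene component that throws the object held by the owner's Physics Handle along the component's forward vector.
; StartThrow begins a timer normalized by MaxThrowDuration.
; DoThrowHeldObject ignores that charge, releasing the object, waiting a tick, applying full ThrowForce (mass-independent unless heavy), then notifying the pickup and completion listeners.
; PerformThrow offers a charge-scaled impulse with a debug arrow, but its event-graph call is disconnected.
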(event Custom|Do%20Throw%20Held%20Object
  (params (affect%20by%20mass :type Boolean) (pickup :type Actor%20Object%20Reference))
  (bind _returnvalue (Math|Vector|GetForwardVector))
  (bind _physics_handle (Variables|Default|Getphysics%20handle))
  (bind _throw_force (Variables|Default|Getthrow%20force))
  (bind _returnvalue_2 (Class|PhysicsHandleComponent|GetGrabbedComponent _physics_handle))
  (bind _returnvalue_3 (* _returnvalue _throw_force))
  (bind _aspickup_base (Utilities|Casting|CastToPickupBase pickup))
  (Utilities|IsValid _returnvalue_2
    (:Is%20Valid
      (Variables|Default|Setthrowme _returnvalue_2)
      (Physics|Components|PhysicsHandle|ReleaseComponent _physics_handle)
      (Utilities|FlowControl|DelayUntilNextTick)
      (Physics|AddForce (Variables|Default|Getthrowme) _returnvalue_3 "None" (not (.TreatAsHeavyObject (Utilities|Struct|BreakPickupConfiguration (Variables|/Game/Patchwork/Blueprints/Interactibles/Pickups/PickupBase.PickupBase_C|GetPickup%20Config _aspickup_base)))))
      (Utilities|FlowControl|Sequence
        (:then_0
          (bind _aspickup_base_2 (Utilities|Casting|CastToPickupBase pickup))
          (Default|OnThrown _aspickup_base_2 _returnvalue_3))
        (:then_1
          (Default|CallOnThrowCompleted)
          (Variables|Default|Setthrowing false))))))

(event Custom|Start%20Throw
  (if (not (Variables|Default|Getthrowing))
    (Utilities|IsValid (Class|PhysicsHandleComponent|GetGrabbedComponent (Variables|Default|Getphysics%20handle))
      (:Is%20Valid
        (Variables|Default|Setthrowing true)
        (Variables|Default|Setcurrent%20throw%20t 0.0)))))

(event Input|EnhancedActionEvents|EnhancedInputActionIA_Throw
  (params (ActionValue :type Boolean) (ElapsedSeconds :type Float%20%28double-precision%29) (TriggeredSeconds :type Float%20%28double-precision%29) (InputAction :type Input%20Action%20Object%20Reference :default "/Game/Patchwork/Data/Input/Grabbing/IA_Throw.IA_Throw")))

(event EventBeginPlay
  (Variables|Default|Setphysics%20handle (Actor|GetComponentbyClass (Components|GetOwner) "/Script/Engine.PhysicsHandleComponent")))

(event EventTick
  (params (DeltaSeconds :type Float%20%28single-precision%29))
  (if (Variables|Default|Getthrowing)
    (bind _output_get (Variables|Default|Setcurrent%20throw%20t (+ (/ DeltaSeconds (Variables|Default|Getmax%20throw%20duration)) (Variables|Default|Getcurrent%20throw%20t))))))

(fn PerformThrow
  (params (throw%20target :type Primitive%20Component%20Object%20Reference) (BoneName :type Name))
  (bind _returnvalue (Transformation|GetWorldLocation))
  (bind _current_throw_t (Variables|Default|Getcurrent%20throw%20t))
  (bind _output_get (LocalVariables|Setthrow%20object throw%20target))
  (if (and (Utilities|IsValid _output_get) (Variables|Default|Getthrowing))
    (Physics|AddImpulse (LocalVariables|Getthrow%20object) (* (Math|Vector|GetForwardVector) (* (Math|Float|Lerp (Variables|Default|Getmin%20throw%20force) (Variables|Default|Getthrow%20force) (Math|Float|Clamp(Float) (Variables|Default|Getcurrent%20throw%20t))) (.z (.scale (Transformation|GetRelativeTransform))))) BoneName (not false))
    (Rendering|Debug|DrawDebugArrow _returnvalue (+ (* (Math|Vector|GetForwardVector) (Math|Float|Lerp 1e+02 1e+03 _current_throw_t)) _returnvalue) 1.0 (Math|Color|Lerp(LinearColor) "(R=0.255187,G=1.000000,B=0.000000,A=1.000000)" "(R=1.000000,G=0.000000,B=0.012273,A=1.000000)" _current_throw_t) 5.0 0.0)
    (Default|CallOnThrowCompleted)
    (Variables|Default|Setthrowing false)
    (return true)
    (else
      (return false))))