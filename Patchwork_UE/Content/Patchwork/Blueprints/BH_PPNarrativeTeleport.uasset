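; BH_PPNarrativeTeleport is a trigger actor that teleports the player with a post-process effect, apparently for narrative moments.
; When a player pawn begins overlapping it, it enables a post-process volume, waits for the teleport delay, calls EventTeleportPlayer on that pawn and disables the volume.
; The teleport logic is not in this graph, and the construction script only calls the parent's.
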(event EventBeginPlay)

(event EventTick
  (params (DeltaSeconds :type Float%20%28single-precision%29)))

(event Collision|EventActorBeginOverlap
  (params (OtherActor :type Actor%20Object%20Reference))
  (bind _isplayer (CallFunction|IsPlayerPawn OtherActor))
  (if _isplayer
    (Variables|/Script/Engine.PostProcessVolume|SetbEnabled (Variables|Default|GetPostProcessVolume) true)
    (Utilities|FlowControl|Delay (Variables|Default|GetTeleportDelay))
    (CallFunction|EventTeleportPlayer OtherActor)
    (Variables|/Script/Engine.PostProcessVolume|SetbEnabled (Variables|Default|GetPostProcessVolume) false)))

(fn ConstructionScript
  (|CallParentFunction))