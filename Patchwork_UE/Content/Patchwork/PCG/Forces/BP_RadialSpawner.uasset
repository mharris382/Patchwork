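; Radial PCG spawner that repeatedly triggers FS_MasterField actors found in the level.
; Construction updates its PCG bounds from Radius and height limits, though Min and Max both use positive Radius in X and Y.
; Any actor overlap sets the tick interval to TickRate and appends all world actors of Class that cast to FS_MasterField to Spawned.
; Each tick calls CETrigger on every valid stored field.
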(event EventBeginPlay
  (|CallParentFunction) ; This node is disabled and will not be called.\nDrag off pins to build functionality.
)

(event Collision|EventActorBeginOverlap
  (params (OtherActor :type Actor%20Object%20Reference))
  (|CallParentFunction OtherActor)
  (Actor|Tick|SetActorTickInterval (Variables|Default|GetTickRate))
  (bind _outactors (CallFunction|GetSpawnedActors))
  (for _array_element _outactors
    (bind _asfs_master_field (Utilities|Casting|CastToFS_MasterField _array_element))
    (Utilities|Array|Add (Variables|Default|Getspawned) _asfs_master_field)))

(event EventTick
  (params (DeltaSeconds :type Float%20%28single-precision%29))
  (|CallParentFunction DeltaSeconds)
  (for _array_element (Variables|Default|Getspawned)
    (Utilities|IsValid _array_element
      (:Is%20Valid
        (Default|CETrigger _array_element)))))

(fn ConstructionScript
  (|CallParentFunction)
  (CallFunction|UpdateBoundsforPCG))

(fn GetBoundsMinMax
  (bind _radius (Variables|Default|GetRadius))
  (bind _returnvalue (* _radius 1.0))
  (|CallParentFunction)
  (return (Math|Vector|MakeVector _returnvalue _returnvalue (Variables|Default|GetMinHeight)) (Math|Vector|MakeVector _radius _radius (Variables|Default|GetMaxHeight))))

(fn GetSpawnedActors
  (bind _outactors (Actor|GetAllActorsOfClass (Variables|Default|GetClass)))
  (return _outactors))