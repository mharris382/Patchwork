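; BP_StageManager is a stage manager actor, apparently a base, that tracks a set of collectible fragments for a stage.
; When the stage starts after its transition, it enables every fragment in FragmentSet.
; CanCompleteStage returns true once all fragments are collected, or immediately if the set is empty.
; The begin, complete and completion-callback events are empty stubs.
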(event Custom|On%20Stage%20Started
  (for _array_element (Variables|Default|GetFragment%20Set)
    (Default|SetFragmentEnabled _array_element true)))

(event Custom|On%20Stage%20Complete)

(event Custom|Begin%20Stage)

(event Custom|Complete%20Stage)

(event EventBeginPlay)

(event Collision|EventActorBeginOverlap
  (params (OtherActor :type Actor%20Object%20Reference)))

(event EventTick
  (params (DeltaSeconds :type Float%20%28single-precision%29)))

(fn ConstructionScript)

(fn CanCompleteStage
  (if (> (Utilities|Array|Length (Variables|Default|GetFragment%20Set)) 0)
    (LocalVariables|Setall%20fragments%20collected true)
    (bind _array_element (Utilities|Array|ForEachLoopwithBreak (Variables|Default|GetFragment%20Set) :!label _label)
      (:LoopBody
        (if (not (Variables|/Game/Patchwork/Blueprints/Environment/BP_Collectable.BP_Collectable_C|Getcollected _array_element))
          (LocalVariables|Setall%20fragments%20collected false)
          (goto _label Break)))
      (:Completed
        (return (LocalVariables|Getall%20fragments%20collected))))
    (else
      (return true))))