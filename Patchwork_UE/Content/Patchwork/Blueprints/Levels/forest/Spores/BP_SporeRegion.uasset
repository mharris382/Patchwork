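; Spore zone that shows Niagara particles and attaches a spore effect component to characters entering it.
; A DT_SporeEffects row selects the component class and particle look, applied on construction and on type change.
; Overlap reuses or adds the component and caches it per actor; leaving clears its inside-zone flag.
; SetActive toggles particle visibility and clears that flag on cached components, whether activating or deactivating.
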(event Custom|Change%20Spore%20Type
  (params (spore%20type :type Data%20Table%20Row%20Handle%20Structure))
  (bind _output_get (Variables|SporeSettings|SetEffect%20Type spore%20type))
  (Utilities|FlowControl|Sequence
    (:then_0
      (bind _returnvalue (Utilities|GetDataTableRow "/Game/Patchwork/Data/Datatables/DT_SporeEffects.DT_SporeEffects" (.rowname _output_get))
        (:then
          (Variables|Default|SetPlayer%20Effect%20Class (.PlayerEffectClass (Utilities|Struct|BreakS_SporeEffectData _returnvalue)))
          (CallFunction|SetParticleSettings (.ParticleSettings (Utilities|Struct|BreakS_SporeEffectData _returnvalue))))))
    (:then_1
      (Utilities|Map|Clear (Variables|Default|Getcomponent%20lookup))
      (for _array_element (Variables|Default|Getactors%20inside)
        (CallFunction|UpdateorCreateSporeEffect _array_element)))))

(event Custom|Set%20Active
  (params (active :type Boolean))
  (bind _output_get (Variables|SporeSettings|Setis%20active active))
  (Rendering|SetVisibility (Variables|Default|GetNiagara-Box) _output_get false)
  (bind _values (Utilities|Map|Values (Variables|Default|Getcomponent%20lookup)))
  (for _array_element _values
    (Variables|/Game/Patchwork/Blueprints/Levels/forest/BP_SporeEffectBase.BP_SporeEffectBase_C|SetInside%20Spore%20Zone _array_element false)))

(event EventBeginPlay
  (if (Variables|SporeSettings|Getis%20active)
    (CallFunction|ChangeSporeType (Variables|SporeSettings|GetEffect%20Type))
    (else
      (Rendering|SetVisibility (Variables|Default|GetNiagara-Box) false false))))

(event Collision|EventActorBeginOverlap
  (params (OtherActor :type Actor%20Object%20Reference))
  (bind _ascharacter (Utilities|Casting|CastToCharacter OtherActor))
  (CallFunction|UpdateorCreateSporeEffect _ascharacter))

(event EventTick
  (params (DeltaSeconds :type Float%20%28single-precision%29)))

(event Collision|EventActorEndOverlap
  (params (OtherActor :type Actor%20Object%20Reference))
  (bind _component_lookup (Variables|Default|Getcomponent%20lookup))
  (if (Utilities|Map|Contains _component_lookup OtherActor)
    (Variables|/Game/Patchwork/Blueprints/Levels/forest/BP_SporeEffectBase.BP_SporeEffectBase_C|SetInside%20Spore%20Zone (.Value (Utilities|Map|Find _component_lookup OtherActor)) false)
    (Utilities|Map|Remove _component_lookup OtherActor)))

(fn ConstructionScript
  (for _array_element (Components|GetChildrenComponents (Variables|Default|GetBox) false)
    (bind _asniagara_particle_system_component (Utilities|Casting|CastToNiagaraComponent _array_element))
    (CallFunction|ApplySporeEffecttoSystem _asniagara_particle_system_component)))

(fn UpdateorCreateSporeEffect
  (params (overlapped%20actor :type Actor%20Object%20Reference%20%28by%20ref%29))
  (bind _effect_type (Variables|SporeSettings|GetEffect%20Type))
  (LocalVariables|Setoverlapped%20actoor overlapped%20actor)
  (Utilities|Array|AddUnique (Variables|Default|Getactors%20inside) (LocalVariables|Getoverlapped%20actoor))
  (bind _array_element (Utilities|Array|ForEachLoopwithBreak (Actor|GetComponentsByClass (LocalVariables|Getoverlapped%20actoor) (Variables|Default|GetPlayer%20Effect%20Class)))
    (:LoopBody
      (if (== (Variables|/Game/Patchwork/Blueprints/Levels/forest/BP_SporeEffectBase.BP_SporeEffectBase_C|GetSpore%20Effect%20Name _array_element) (.rowname _effect_type))
        (Utilities|Map|Add (Variables|Default|Getcomponent%20lookup) (LocalVariables|Getoverlapped%20actoor) _array_element)))
    (:Completed
      (if (not (Utilities|Map|Contains (Variables|Default|Getcomponent%20lookup) (LocalVariables|Getoverlapped%20actoor)))
        (bind _returnvalue (Utilities|GetDataTableRow (.datatable _effect_type) (.rowname _effect_type))
          (:then
            (bind _returnvalue_2 (Game|AddComponentbyClass (LocalVariables|Getoverlapped%20actoor) (.PlayerEffectClass (Utilities|Struct|BreakS_SporeEffectData _returnvalue))))
            (Utilities|Map|Add (Variables|Default|Getcomponent%20lookup) (LocalVariables|Getoverlapped%20actoor) _returnvalue_2)
            (Default|OnToxicityChanged _returnvalue_2 0.0)))))))

(fn SetParticleSettings
  (params (settings :type S%20Spore%20Particle%20Settings%20Structure))
  (bind (_color _sizerange _gravity _glitchintensity _trippingintensity) (Utilities|Struct|BreakS_SporeParticleSettings settings))
  (bind (_x _y) (Math|Vector2D|BreakVector2D _sizerange))
  (Effects|Components|ParticleSystem|SetColorParameter (Variables|Default|GetNiagara-Box) "Color" _color)
  (Effects|Components|ParticleSystem|SetFloatParameter (Variables|Default|GetNiagara-Box) "Min Size" _x)
  (Effects|Components|ParticleSystem|SetFloatParameter (Variables|Default|GetNiagara-Box) "Max Size" _y)
  (Effects|Components|ParticleSystem|SetFloatParameter (Variables|Default|GetNiagara-Box) "Gravity" _gravity)
  (Effects|Components|ParticleSystem|SetFloatParameter (Variables|Default|GetNiagara-Box) "Glitch Amount" _glitchintensity)
  (Effects|Components|ParticleSystem|SetFloatParameter (Variables|Default|GetNiagara-Box) "Tripping Offset" _trippingintensity))

(fn GetEffectData
  (bind _effect_type (Variables|SporeSettings|GetEffect%20Type))
  (bind _returnvalue (Utilities|GetDataTableRow (.datatable _effect_type) (.rowname _effect_type))
    (:then
      (return _returnvalue true))
    (:RowNotFound
      (return "" false))))

(fn MatchesSporeType
  (params (SporeName :type Name))
  (return (== SporeName (.rowname (Variables|SporeSettings|GetEffect%20Type)))))

(fn ApplySporeEffecttoSystem
  (params (self2 :type FX%20System%20Component%20Object%20Reference))
  (bind _effect_type (Variables|SporeSettings|GetEffect%20Type))
  (bind _returnvalue (Utilities|GetDataTableRow (.datatable _effect_type) (.rowname _effect_type))
    (:then
      (Variables|Default|SetPlayer%20Effect%20Class (.PlayerEffectClass (Utilities|Struct|BreakS_SporeEffectData _returnvalue)))
      (Effects|Components|ParticleSystem|SetFloatParameter self2 "Spawn Rate" (Variables|VFXSettings|GetSpawn%20Rate))
      (CallFunction|SetParticleSettings (.ParticleSettings (Utilities|Struct|BreakS_SporeEffectData _returnvalue))))))