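; DarknessArea is a configurable box volume that marks actors as inside darkness and can apply its own post-processing.
; When enabled, begin overlap calls SetInsideDarkness(true) on actors implementing BPI_DarknessListener.
; The construction script sizes the box, optionally offsets it to a corner, and sets up the PostProcess component.
; End overlap is empty and the clearing call is unwired, so this volume never resets the darkness state.
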(event EventBeginPlay
  (if (> (Utilities|Array|Length (Collision|GetOverlappingActors (Variables|Default|GetBox) "/Game/Patchwork/Blueprints/Core/Pawns/paperperson.paperperson_C" :!class /Script/Engine.PrimitiveComponent)) 0)
    _))

(event Collision|EventActorBeginOverlap
  (params (OtherActor :type Actor%20Object%20Reference))
  (if (Variables|Default|GetEnabled)
    (bind _asbpi_darkness_listener (Utilities|Casting|CastToBPI_DarknessListener OtherActor))
    (Default|SetInsideDarkness _asbpi_darkness_listener true)))

(event EventTick
  (params (DeltaSeconds :type Float%20%28single-precision%29)))

(event Collision|EventActorEndOverlap
  (params (OtherActor :type Actor%20Object%20Reference)))

(fn ConstructionScript
  (bind _box (Variables|Default|GetBox))
  (bind _postprocess (Variables|Default|GetPostProcess))
  (Utilities|FlowControl|Sequence
    (:then_0
      (Components|Box|SetBoxExtent (Variables|Default|GetBox) (Variables|Default|GetBox%20Size) true)
      (if (Variables|Default|GetOffset%20box%20to%20corner)
        (Transformation|SetRelativeLocation _box (Components|Box|GetScaledBoxExtent _box) false false)))
    (:then_1
      (Variables|/Script/Engine.PostProcessComponent|SetbEnabled _postprocess (and (Variables|Default|GetEnabled) (Variables|Default|GetEnablePostProcessing)))
      (Variables|/Script/Engine.PostProcessComponent|SetSettings _postprocess (Variables|Default|GetPostProcessingSettings)))))