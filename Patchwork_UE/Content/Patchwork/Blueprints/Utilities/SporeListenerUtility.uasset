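; Spore listener component that loads spore effect data for its owning actor.
; On BeginPlay it looks up the configured SporeType data table row and caches it as SporeEffectData, printing an error naming the actor, row and table if missing.
; Applying the effect is unfinished: the WaitForEffect event is empty, its timer is never run, and the lookup of the player's effect component is unused.
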(event Custom|wait%20for%20effect)

(event EventBeginPlay
  (bind _spore_type (Variables|Default|GetSpore%20Type))
  (bind _spore_type_2 (Variables|Default|GetSpore%20Type))
  (bind _returnvalue (Utilities|GetDataTableRow (.datatable _spore_type_2) (.rowname _spore_type_2))
    (:then
      (Variables|Default|Setspore%20effect%20data _returnvalue))
    (:RowNotFound
      (Development|PrintText (Utilities|Text|FormatText "Invalid data table on actor {0}, data table {2} does not have row with name {1} " (Utilities|GetDisplayName (Components|GetOwner)) (.rowname _spore_type) (.datatable _spore_type))))))

(event EventTick
  (params (DeltaSeconds :type Float%20%28single-precision%29)))