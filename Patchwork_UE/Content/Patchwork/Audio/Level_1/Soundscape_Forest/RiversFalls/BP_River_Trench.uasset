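; BP_River_Trench is a river ambience actor for the Level 1 forest soundscape that keeps its sound at the nearest point along a spline to the player.
; BeginPlay caches the player character and starts MoveAudio, which snaps the Audio and Arrow components to that closest point.
; MoveAudio re-arms a half-second timer rather than using Tick.
; StopFollowAudio clears that timer, but nothing in this graph triggers it.
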(event Custom|MoveAudio
  (bind _char_ref (Variables|Default|GetChar%20Ref))
  (bind _spline (Variables|Default|GetSpline))
  (bind _returnvalue (Transformation|GetActorLocation _char_ref))
  (bind _returnvalue_2 (Spline|FindLocationClosesttoWorldLocation _spline _returnvalue "World"))
  (Transformation|SetWorldLocation (Variables|Default|GetArrow) (Math|Vector|MakeVector (.x _returnvalue_2) (.y _returnvalue_2) (.z _returnvalue_2)) false false)
  (bind _returnvalue_3 (Utilities|Time|SetTimerbyEvent (delegate Custom|Move%20Audio) 0.5)))

(event Custom|Move%20Audio
  (CallFunction|MoveAudio))

(event Custom|Stop%20Follow%20Audio
  (Utilities|Time|ClearandInvalidateTimerbyHandle (stale Custom|MoveAudio _returnvalue_3)))

(event EventBeginPlay
  (Variables|Default|SetChar%20Ref (Game|GetPlayerCharacter 0))
  (CallFunction|MoveAudio))

(fn ConstructionScript)