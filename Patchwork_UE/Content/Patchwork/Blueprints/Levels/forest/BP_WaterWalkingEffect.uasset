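; BP_WaterWalkingEffect is an effect component that toggles water walking for its paperperson owner.
; On BeginPlay it caches the owner and its WaterBodyHandler, then binds to the effect gained and lost events.
; Those events switch every WaterBody actor in the world between the water-walking and default collision profiles, updating overlaps.
; The collision change is made on the water itself, so it applies globally rather than per character.
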(event Custom|gained%20water%20walking
  (CallFunction|UpdateWaterBodyCollisions true))

(event Custom|lost%20water%20walking
  (CallFunction|UpdateWaterBodyCollisions false))

(event EventBeginPlay
  (bind _returnvalue (Components|GetOwner))
  (|CallParentFunction)
  (Variables|Default|SetWater%20Body%20Handler (Actor|GetComponentbyClass _returnvalue "/Game/Patchwork/Blueprints/Core/Pawns/Components/WaterBodyHandler.WaterBodyHandler_C"))
  (bind _aspaperperson (Utilities|Casting|CastTopaperperson _returnvalue))
  (Variables|Default|SetPaperperson _aspaperperson)
  (EventDispatchers|BindEventtoOnEffectGained (delegate Custom|gained%20water%20walking))
  (EventDispatchers|BindEventtoOnEffectLost (delegate Custom|lost%20water%20walking)))

(event EventTick
  (params (DeltaSeconds :type Float%20%28single-precision%29))
  (|CallParentFunction DeltaSeconds))

(fn UpdateWaterBodyCollisions
  (params (enable%20collision :type Boolean))
  (LocalVariables|SetCollision%20Profile%20Name (select enable%20collision "WaterBodyCollision_WaterWalking" "WaterBodyCollision"))
  (bind _outactors (Actor|GetAllActorsOfClass "/Script/Water.WaterBody"))
  (for _array_element _outactors
    (Collision|SetCollisionProfileName (Variables|/Script/Water.WaterBody|GetWaterBodyComponent _array_element) (LocalVariables|GetCollision%20Profile%20Name) true :!class /Script/Engine.PrimitiveComponent)))