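; BP_DestructionMarker is a marker actor for procedural city destruction that labels itself through actor tags.
; Its Construction Script clears any Destruct and NoDestruct tags, then re-adds one of them based on the MarkerMode enum, with one mode leaving both off.
; It has no active runtime logic, and this file does not show what reads the tags.
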(event EventBeginPlay
  (|CallParentFunction) ; This node is disabled and will not be called.\nDrag off pins to build functionality.
)

(event Collision|EventActorBeginOverlap
  (params (OtherActor :type Actor%20Object%20Reference))
  (|CallParentFunction OtherActor) ; This node is disabled and will not be called.\nDrag off pins to build functionality.
)

(event EventTick
  (params (DeltaSeconds :type Float%20%28single-precision%29))
  (|CallParentFunction DeltaSeconds) ; This node is disabled and will not be called.\nDrag off pins to build functionality.
)

(fn ConstructionScript
  (|CallParentFunction)
  (Utilities|FlowControl|Sequence
    (:then_0
      (Utilities|Array|RemoveItem (Variables|Default|GetTags) "NoDestruct")
      (Utilities|Array|RemoveItem (Variables|Default|GetTags) "Destruct"))
    (:then_1
      (if (Utilities|Enum|NotEqual(Enum) (Variables|Default|GetMarkerMode) "NewEnumerator2")
        (bind _output_get (LocalVariables|Settmp (Variables|Default|GetTags)))
        (Utilities|Array|AddUnique _output_get (Utilities|String|SelectName "Destruct" "NoDestruct" (Utilities|Enum|NotEqual(Enum) (Variables|Default|GetMarkerMode) "NewEnumerator1")))
        (Variables|Default|SetTags (LocalVariables|Gettmp))))))