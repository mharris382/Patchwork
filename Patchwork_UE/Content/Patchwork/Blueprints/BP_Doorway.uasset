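; BP_Doorway is a doorway effect actor that animates a door material, smoke and lighting shortly after play begins.
; BeginPlay creates a dynamic material instance, resets the vertical offset, smoke spawn rate and lights, then plays the AnimateDoor timeline after a short delay.
; The timeline drives the material's offset, the smoke spawn rate and, through SetLightIntensity, three lights scaled up to a configured intensity.
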(event EventBeginPlay
  (bind _door_effect_door (Variables|Default|Getdoor_effect_Door))
  (bind _returnvalue (Rendering|Material|CreateDynamicMaterialInstance _door_effect_door 0 (Rendering|Material|GetMaterial _door_effect_door 0) "None" :!class /Script/Engine.PrimitiveComponent))
  (bind _output_get (Variables|Default|SetDoor%20Material%20Instance _returnvalue))
  (Rendering|Material|SetMaterial (Variables|Default|Getdoor_effect_Door) 0 _output_get)
  (Rendering|Material|SetScalarParameterValue (Variables|Default|GetDoor%20Material%20Instance) (Variables|Default|GetV%20Offset%20Parameter%20Name) -1.0 :!class /Script/Engine.MaterialInstanceDynamic)
  (Effects|Components|ParticleSystem|SetFloatParameter (Variables|Default|GetSmoke%20Effect) (Variables|Default|GetSpawn%20Rate%20Parameter%20Name) 0.0)
  (Utilities|SetLightIntensity (Math|Float|Lerp 0.0 (Variables|Default|GetLight%20Intensity) 0.0))
  (Utilities|FlowControl|Delay 3.0)
  (bind (_direction _door_height _spawn_rate _light_intensity) (Timeline|Animate%20Door Play)
    (:Update
      (Rendering|Material|SetScalarParameterValue (Variables|Default|GetDoor%20Material%20Instance) (Variables|Default|GetV%20Offset%20Parameter%20Name) _door_height :!class /Script/Engine.MaterialInstanceDynamic)
      (Effects|Components|ParticleSystem|SetFloatParameter (Variables|Default|GetSmoke%20Effect) (Variables|Default|GetSpawn%20Rate%20Parameter%20Name) _spawn_rate)
      (Utilities|SetLightIntensity (Math|Float|Lerp 0.0 (Variables|Default|GetLight%20Intensity) _light_intensity)))))

(event Collision|EventActorBeginOverlap
  (params (OtherActor :type Actor%20Object%20Reference)))

(event EventTick
  (params (DeltaSeconds :type Float%20%28single-precision%29)))

(fn ConstructionScript)