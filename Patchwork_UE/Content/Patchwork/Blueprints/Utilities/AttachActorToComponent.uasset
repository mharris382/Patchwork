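; Utility component that attaches its owning actor to a component on a target actor at BeginPlay.
; It picks the parent by tag (first match, cast to SceneComponent) when a tag is set, otherwise by component class.
; Socket name and location, rotation and scale rules come from variables.
; An Error event prints a generic attach-failure message, ignoring the message passed to it.
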(event Custom|Error
  (params (msg :type Name))
  (Development|PrintText "Error failed to attach"))

(event EventBeginPlay
  (bind _targetactor (Variables|Default|GetTargetActor)
    (:then
      (if (!= (Variables|Default|GetTag) "")
        (bind _asscene_component (Utilities|Casting|CastToSceneComponent (Utilities|Array|Get(acopy) (Actor|GetComponentsbyTag _targetactor "/Script/Engine.ActorComponent" (Variables|Default|GetTag))))
          (:then
            (Variables|Default|Settarget _asscene_component)
            (bind _returnvalue (Transformation|AttachComponentToComponent (Components|GetOwner) (Variables|Default|Gettarget) (Variables|Default|GetSocket%20Name) (Variables|Default|GetLocation%20Rule) (Variables|Default|GetRotation%20Rule) (Variables|Default|GetScale%20Rule) true :!label _label))
            (if _returnvalue
              (CallFunction|Error "None")
              (else
                (Development|PrintText "Error failed to attach"))))
          (:CastFailed
            (CallFunction|Error "None")))
        (else
          (Variables|Default|Settarget (Actor|GetComponentbyClass _targetactor (Variables|Default|GetTargetComponentType)))
          (Utilities|IsValid (Actor|GetComponentbyClass _targetactor (Variables|Default|GetTargetComponentType))
            (:Is%20Valid
              (goto _label))
            (:Is%20Not%20Valid
              (CallFunction|Error "None"))))))
    (:else
      (CallFunction|Error "None"))))

(event EventTick
  (params (DeltaSeconds :type Float%20%28single-precision%29)))