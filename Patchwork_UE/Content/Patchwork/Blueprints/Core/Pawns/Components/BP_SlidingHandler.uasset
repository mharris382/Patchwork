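; Pawn component that manages slide permissions for its paperperson owner.
; After a short delay on BeginPlay it caches the owner and its movement component and enables slide start and stop, with Tick retrying if the movement reference is invalid.
; CanStopSlide traces below the owner and refuses stopping over anything tagged "Slide".
; Helpers set the owner's flags and check walking or sliding state; the walk/slide timing logic is disconnected.
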(event EventBeginPlay
  (Utilities|FlowControl|Delay 0.2)
  (bind _aspaperperson (Utilities|Casting|CastTopaperperson (Components|GetOwner))
    (:then
      (bind _output_get (Variables|Default|SetOwner _aspaperperson))
      (bind _output_get_2 (Variables|Default|SetCharacter%20Movement (Variables|/Script/Engine.Character|GetCharacterMovement _output_get)))
      (Utilities|IsValid _output_get_2
        (:Is%20Valid
          (Variables|/Game/Patchwork/Blueprints/Core/Pawns/paperperson.paperperson_C|Setallow%20start%20slide _output_get true)
          (Variables|/Game/Patchwork/Blueprints/Core/Pawns/paperperson.paperperson_C|Setallow%20stop%20slide _output_get true))))
    (:CastFailed
      (Development|PrintText "Slide Failed"))))

(event EventTick
  (params (DeltaSeconds :type Float%20%28single-precision%29))
  (Variables|Default|GetCharacter%20Movement
    (:then
      (Variables|Default|GetCharacter%20Movement
        (:then)
        (:else)))
    (:else
      (bind _owner (Variables|Default|GetOwner)
        (:then
          (Variables|Default|SetCharacter%20Movement (Variables|/Script/Engine.Character|GetCharacterMovement _owner))
          (Utilities|SetAllowStartStopSlide true true))
        (:else)))))

(fn CanStopSlide
  (params (Reason :type ESlideEndReason%20Enum :default "NewEnumerator0"))
  (bind _owner (Variables|Default|GetOwner))
  (bind _returnvalue (Transformation|GetActorLocation _owner))
  (LocalVariables|Setfound false)
  (bind (_outhits _returnvalue_2) (Class|KismetSystemLibrary|LineTraceMultiforObjects _returnvalue (- _returnvalue (Math|Vector|MakeVector 0.0 0.0 (* (Components|Capsule|GetUnscaledCapsuleHalfHeight (Variables|/Game/Patchwork/Blueprints/Core/Pawns/paperperson.paperperson_C|GetInteractorThird _owner)) 1.25))) (Utilities|Array|MakeArray "ObjectTypeQuery1" "ObjectTypeQuery2") false 0 "ForOneFrame" true))
  (bind _array_element (Utilities|Array|ForEachLoopwithBreak _outhits :!label _label)
    (:LoopBody
      (if _returnvalue_2
        (if (or (Actor|ActorHasTag (.HitActor (Collision|BreakHitResult _array_element)) "Slide") (Components|ComponentHasTag (.HitComponent (Collision|BreakHitResult _array_element)) "Slide"))
          (LocalVariables|Setfound true)
          (goto _label Break))))
    (:Completed
      (return (not (LocalVariables|Getfound))))))