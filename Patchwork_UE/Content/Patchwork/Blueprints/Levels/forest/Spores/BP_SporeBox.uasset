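; BP_SporeBox is a resizable box volume of Niagara spore particles for the forest level, set up entirely in its construction script.
; BoxSize drives both the Box extent and the Niagara "Box Size" parameter.
; Spawn rate scales with the BoxSize product and ParticleDensity, capped at a maximum.
; PositionFromGround optionally raises the box by its Z extent so its base sits at the actor origin.
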(event EventBeginPlay
  (|CallParentFunction) ; This node is disabled and will not be called.\nDrag off pins to build functionality.
)

(event Collision|EventActorBeginOverlap
  (params (OtherActor :type Actor%20Object%20Reference))
  (|CallParentFunction OtherActor) ; This node is disabled and will not be called.\nDrag off pins to build functionality.
)

(event EventTick
  (params (DeltaSeconds :type Float%20%28single-precision%29))
  (|CallParentFunction DeltaSeconds) ; This node is disabled and will not be called.\nDrag off pins to build functionality.
)

(fn ConstructionScript
  (bind _box_size (Variables|Box|GetBox%20Size))
  (bind _niagara_box (Variables|Default|GetNiagara-Box))
  (bind _box_size_2 (Variables|Box|GetBox%20Size))
  (|CallParentFunction)
  (Utilities|FlowControl|Sequence
    (:then_0
      (Components|Box|SetBoxExtent (Variables|Default|GetBox) _box_size true)
      (Effects|Components|ParticleSystem|SetVectorParameter _niagara_box "Box Size" _box_size)
      (Effects|Components|ParticleSystem|SetFloatParameter _niagara_box "Spawn Rate" (Math|Float|Min(Float) (/ (* (.x _box_size_2) (.y _box_size_2) (.z _box_size_2) (Variables|Default|GetParticle%20Density)) 1e+03) 1e+06)))
    (:then_1
      (if (Variables|Box|Getposition%20from%20ground)
        (Transformation|SetRelativeLocation (Variables|Default|GetBox) (Math|Vector|MakeVector 0.0 0.0 (.z (Variables|Box|GetBox%20Size))) false false)))))