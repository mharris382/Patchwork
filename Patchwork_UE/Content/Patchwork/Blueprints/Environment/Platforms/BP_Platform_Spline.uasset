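; BP_Platform_Spline is a platform variant that supplies positions along a spline to movement logic inherited from its parent.
; On BeginPlay it derives a time multiplier from move speed divided by spline length, so speed stays independent of path length.
; GetMoveInterpTime scales and wraps time into a looping 0–1 value.
; GePositionFromInterpTime samples that fraction as a local-space spline location, optionally at constant velocity.
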(event EventBeginPlay
  (|CallParentFunction)
  (Variables|Default|SettimeMultiplier (/ (Variables|Default|GetMoveSpeed) (Spline|GetSplineLength (Variables|Default|GetSpline)))))

(event Collision|EventActorBeginOverlap
  (params (OtherActor :type Actor%20Object%20Reference)))

(event EventTick
  (params (DeltaSeconds :type Float%20%28single-precision%29))
  (|CallParentFunction DeltaSeconds) ; This node is disabled and will not be called.\nDrag off pins to build functionality.
)

(fn ConstructionScript
  (|CallParentFunction))

(fn GePositionfromInterpTime
  (params (percent :type Float%20%28single-precision%29))
  (return (Spline|GetLocationatTime (Variables|Default|GetSpline) percent "Local" (Variables|Default|GetUse%20Constant%20Velocity))))

(fn GetMoveInterpTime
  (params (A :type Float%20%28double-precision%29))
  (return (Math|Float|%(Float) (* A (Variables|Default|GettimeMultiplier)) 1.0)))