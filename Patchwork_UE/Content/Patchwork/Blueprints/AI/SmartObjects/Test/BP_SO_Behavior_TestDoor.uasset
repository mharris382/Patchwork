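; BP_SO_Behavior_TestDoor is a test smart object behavior for characters using a door.
; When triggered, it stores the avatar, casts the owner to BP_DoorBase, waits briefly, then ends the behavior, ending immediately if the cast fails.
; The door-toggling and completion-binding calls are disconnected and their handlers are empty, so it never changes the door's state.
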(event Custom|ExecuteDoorAction
  (params (Character :type Character%20Object%20Reference) (Door :type BP%20Door%20Base%20Object%20Reference)))

(event Custom|OnDoorChangedStateComplete
  (params (IsOpen :type Boolean) (Successful :type Boolean)))

(event GameplayBehavior|EventOnTriggeredCharacter
  (params (Avatar :type Character%20Object%20Reference) (Config :type Gameplay%20Behavior%20Config%20Object%20Reference) (SmartObjectOwner :type Actor%20Object%20Reference))
  (Variables|Default|SetAvatar Avatar)
  (bind _asbp_door_base (Utilities|Casting|CastToBP_DoorBase SmartObjectOwner)
    (:then
      (Variables|Default|SetDoor _asbp_door_base)
      (GameplayTasks|TaskWaitDelay 0 0.1
        (:OnFinish
          (GameplayBehavior|EndBehavior (Variables|Default|GetAvatar)))))
    (:CastFailed
      (GameplayBehavior|EndBehavior (Variables|Default|GetAvatar)))))