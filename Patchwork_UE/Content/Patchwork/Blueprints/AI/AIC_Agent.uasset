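; AI controller that drives an agent pawn from its default state and its needs.
; On possess, it runs the state's behavior tree, then uses path and target resolver components, added if missing, to fill the blackboard.
; Sight perception updates whether the target is visible.
; Relaxation and hunger components start a looping timer, and need updates publish the top need's class, favoring one being fulfilled.
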(event OnPerceptionUpdated(AIPerception)
  (params (UpdatedActors :type Array%20of%20Actor%20Object%20References))
  (CallFunction|AIPerceptionUpdated UpdatedActors))

(event EventBeginPlay)

(event EventTick
  (params (DeltaSeconds :type Float%20%28single-precision%29)))

(event EventPossess
  (params (PossessedPawn :type Pawn%20Object%20Reference))
  (Utilities|FlowControl|Delay 0.2)
  (bind _state (Class|BPIAgent|GetDefaultStateInfo(Message) PossessedPawn))
  (CallFunction|ApplyState _state PossessedPawn)
  (Needs|SetupNeeds PossessedPawn))

(fn ConstructionScript)

(fn ApplyState
  (params (State :type Agent%20State%20Object%20Reference) (Pawn :type Pawn%20Object%20Reference))
  (Utilities|FlowControl|Sequence
    (:then_0
      (Utilities|FlowControl|Sequence
        (:then_0
          (bind _returnvalue (AI|RunBehaviorTree (Variables|/Game/Patchwork/Blueprints/Enemies/Data/AgentState.AgentState_C|GetRootBehavior State)))
          (if (not _returnvalue)
            (Development|PrintString "Failed to start behavior tree")))
        (:then_1
          ;[0.6233 0.6233 0.6233 0.5] Set Path From Path Resolver
          (Utilities|FlowControl|Sequence
            (:then_0
              ;;[0.6233 0.6233 0.6233 0.5] Get Path Resolver For State
              (if (== (Variables|/Game/Patchwork/Blueprints/Enemies/Data/AgentState.AgentState_C|GetTargetResolverTag State) "")
                (Utilities|IsValid (Actor|GetComponentbyClass Pawn (Variables|/Game/Patchwork/Blueprints/Enemies/Data/AgentState.AgentState_C|GetPathResolver State))
                  (:Is%20Valid
                    (Variables|Default|SetPathResolver (Actor|GetComponentbyClass Pawn (Variables|/Game/Patchwork/Blueprints/Enemies/Data/AgentState.AgentState_C|GetPathResolver State))))
                  (:Is%20Not%20Valid
                    (bind _returnvalue_2 (Game|AddComponentbyClass Pawn (Variables|/Game/Patchwork/Blueprints/Enemies/Data/AgentState.AgentState_C|GetPathResolver State)))
                    (Variables|Default|SetPathResolver _returnvalue_2)))
                (else
                  (Development|PrintText "Tags Not Implemented"))))
            (:then_1
              ;;[0.6233 0.6233 0.6233 0.5] Resolve Path
              (bind _path (Default|GetBestPathforAgent (Variables|Default|GetPathResolver) Pawn))
              (bind _output_get (LocalVariables|SetPath _path))
              (Utilities|IsValid _output_get
                (:Is%20Valid
                  (bind _waypointindex (Default|GetNearestWaypoint (LocalVariables|GetPath) (Transformation|GetActorLocation Pawn) Pawn))
                  (LocalVariables|SetPathIndex _waypointindex)
                  (Class|BlackboardComponent|SetValueasInt (AI|GetBlackboard 0) (Variables|BBKeys|GetWaypointKeyName) (LocalVariables|GetPathIndex))
                  (AI|Components|Blackboard|SetValueasObject (AI|GetBlackboard 0) (Variables|BBKeys|GetPathKeyName) (LocalVariables|GetPath)))
                (:Is%20Not%20Valid
                  (Development|PrintString "Error no valid path"))))))
        (:then_2
          ;[0.6233 0.6233 0.6233 0.5] Get Target Resolver
          (Utilities|FlowControl|Sequence
            (:then_0
              ;;[0.6233 0.6233 0.6233 0.5] Get Target Resolver for State
              (if (== (Variables|/Game/Patchwork/Blueprints/Enemies/Data/AgentState.AgentState_C|GetTargetResolverTag State) "")
                (Utilities|IsValid (Actor|GetComponentbyClass Pawn (Variables|/Game/Patchwork/Blueprints/Enemies/Data/AgentState.AgentState_C|GetTargetResolver State))
                  (:Is%20Valid
                    (Variables|Default|SetTargetResolver (Actor|GetComponentbyClass Pawn (Variables|/Game/Patchwork/Blueprints/Enemies/Data/AgentState.AgentState_C|GetTargetResolver State))))
                  (:Is%20Not%20Valid
                    (bind _returnvalue_3 (Game|AddComponentbyClass Pawn (Variables|/Game/Patchwork/Blueprints/Enemies/Data/AgentState.AgentState_C|GetTargetResolver State)))
                    (Variables|Default|SetTargetResolver _returnvalue_3)))
                (else
                  (Development|PrintText "Tags Not Implemented"))))
            (:then_1
              ;;[0.6233 0.6233 0.6233 0.5] Resolve Target
              (bind _target (Default|GetTargetforAgent (Variables|Default|GetTargetResolver) Pawn))
              (Variables|Default|SetTarget _target)
              (Utilities|FlowControl|Sequence
                (:then_0
                  (AI|Components|Blackboard|SetValueasObject (AI|GetBlackboard 0) (Variables|BBKeys|GetTargetKeyName) (Variables|Default|GetTarget)))
                (:then_1
                  (Senses|Sight|UpdateCanSeeTarget))))))))
    (:then_1
      (Utilities|FlowControl|Sequence
        (:then_0
          (Class|BPIAgent|SetInteractAvailable(Message) Pawn (Variables|/Game/Patchwork/Blueprints/Enemies/Data/AgentState.AgentState_C|GetAllowsDialogueWithPlayer State)))))))

(fn CanSenseTarget
  (params (Target :type Actor%20Object%20Reference) (Senses :type EAgentSenses%20Enum :default "NewEnumerator0"))
  (Utilities|IsValid Target
    (:Is%20Valid
      (bind _info (Class|AIPerceptionComponent|GetActorsPerception (Variables|Default|GetAIPerception) Target))
      (for _array_element (.LastSensedStimuli (Utilities|Struct|BreakActorPerceptionBlueprintInfo _info))
        (bind _returnvalue (Class|AIPerceptionSystem|GetSenseClassforStimulus _array_element))
        (if (== _returnvalue (Utilities|Select :Index Senses :NewEnumerator0 "/Script/AIModule.AISense_Sight" :NewEnumerator1 "/Script/AIModule.AISense_Hearing" :NewEnumerator2 "/Script/AIModule.AISense_Touch" :NewEnumerator4 "/Script/AIModule.AISense_Damage"))
          (return (.bSuccessfullySensed (Utilities|Struct|BreakAIStimulus _array_element)) _array_element))))
    (:Is%20Not%20Valid
      (return false ""))))

(fn UpdateCanSeeTarget
  (bind _sensed (Senses|CanSenseTarget (Variables|Default|GetTarget) "NewEnumerator0"))
  (Senses|Sight|SetCanSeeTarget _sensed))

(fn SetCanSeeTarget
  (params (BoolValue :type Boolean))
  (AI|Components|Blackboard|SetValueasBool (AI|GetBlackboard 0) (Variables|BBKeys|GetCanSeeTargetKeyName) BoolValue))

(fn AIPerceptionUpdated
  (params (Array :type Array%20of%20Actor%20Object%20References))
  (bind _returnvalue (AI|GetBlackboard 0))
  (Utilities|IsValid _returnvalue
    (:Is%20Valid
      (for _array_element Array
        (if (== _array_element (AI|Components|Blackboard|GetValueasObject _returnvalue (Variables|BBKeys|GetTargetKeyName)))
          (Utilities|FlowControl|Sequence
            (:then_0
              (bind _sensed (Senses|CanSenseTarget 0 "NewEnumerator0"))
              (Senses|Sight|SetCanSeeTarget _sensed))))))))

(fn SetupNeeds
  (params (Pawn :type Pawn%20Object%20Reference))
  (Utilities|IsValid Pawn
    (:Is%20Valid
      (Utilities|FlowControl|Sequence
        (:then_0
          (Needs|Relaxation|SetupRelaxationNeed (Actor|GetComponentbyClass Pawn "/Game/Patchwork/Blueprints/AI/Needs/RelaxationNeed.RelaxationNeed_C")))
        (:then_1
          (Needs|Relaxation|SetupHungerNeed (Actor|GetComponentbyClass Pawn "/Game/Patchwork/Blueprints/AI/Needs/HungerNeed.HungerNeed_C")))
        (:then_2
          (switch int (Utilities|Array|Length (Variables|Default|GetNeeds))
            (:Default
              (Development|PrintText "TODO implement top need evaluations")
              (AI|Components|Blackboard|SetValueasBool (AI|GetBlackboard 0) (Variables|BBKeys|GetHasNeedsKeyName) true :!label _label)
              (bind _returnvalue (Utilities|Time|SetTimerbyEvent (EventDispatchers|CreateEvent :!event UpdateNeeds) (Variables|Needs|GetNeedUpdateRate) true))
              (Variables|Needs|TimerHandles|SetNeedUpdateTimer _returnvalue))
            (:0
              (AI|Components|Blackboard|SetValueasBool (AI|GetBlackboard 0) (Variables|BBKeys|GetHasNeedsKeyName) false))
            (:1
              (Class|BlackboardComponent|SetValueasClass (AI|GetBlackboard 0) (Variables|BBKeys|GetTopNeedKeyName) (Utilities|GetClass (Utilities|Array|Get(acopy) (Variables|Default|GetNeeds))))
              (goto _label))))))))

(fn SetupRelaxationNeed
  (params (RelaxationNeed :type Relaxation%20Need%20Object%20Reference))
  (Utilities|IsValid RelaxationNeed
    (:Is%20Valid
      (bind _output_get (Variables|Needs|SetRelaxationNeed RelaxationNeed))
      (Utilities|Array|Add (Variables|Default|GetNeeds) _output_get))))

(fn DEPUpdatNeeds
  (Needs|Relaxation|UpdateNeed (Variables|Needs|GetRelaxationNeed) (Variables|Needs|GetNeedUpdateRate)))

(fn UpdateNeed
  (params (Need :type Need%20Object%20Reference) (Rate :type Float%20%28double-precision%29))
  (Default|UpdateNeed Need Rate)
  (AI|Components|Blackboard|SetValueasBool (AI|GetBlackboard 0) (Variables|/Game/Patchwork/Blueprints/AI/Needs/Need.Need_C|GetWantsNeedBBName Need) (Default|WantstoFullfillNeed Need)))

(fn UpdateHungerNeed
  (Needs|Relaxation|UpdateNeed (Variables|Needs|GetRelaxationNeed) (Variables|Needs|GetNeedUpdateRate)))

(fn SetupHungerNeed
  (params (HungerNeed :type Hunger%20Need%20Object%20Reference))
  (Utilities|IsValid HungerNeed
    (:Is%20Valid
      (bind _output_get (Variables|Default|SetHunger%20Need HungerNeed))
      (Utilities|Array|Add (Variables|Default|GetNeeds) _output_get))))

(fn UpdateNeeds
  (LocalVariables|SetTopNeed (Utilities|Array|Get(acopy) (Variables|Default|GetNeeds)))
  (LocalVariables|SetHighestNeed 0.0)
  (LocalVariables|SetSecondBestNeed 0)
  (LocalVariables|SetSecondHighestNeed 0.0)
  (for _array_element (Variables|Default|GetNeeds)
    (Needs|Relaxation|UpdateNeed _array_element (Variables|Needs|GetNeedUpdateRate))
    (if (Variables|/Game/Patchwork/Blueprints/AI/Needs/Need.Need_C|GetIsFulfillingNeed _array_element)
      (LocalVariables|SetHighestNeed 11.0)
      (LocalVariables|SetTopNeed _array_element)
      (elif (>= (Variables|/Game/Patchwork/Blueprints/AI/Needs/Need.Need_C|GetNeedMeter _array_element) (LocalVariables|GetHighestNeed))
        (LocalVariables|SetHighestNeed (Variables|/Game/Patchwork/Blueprints/AI/Needs/Need.Need_C|GetNeedMeter _array_element))
        (LocalVariables|SetTopNeed _array_element)
        (elif (>= (Variables|/Game/Patchwork/Blueprints/AI/Needs/Need.Need_C|GetNeedMeter _array_element) (LocalVariables|GetSecondHighestNeed))
          (LocalVariables|SetSecondHighestNeed (Variables|/Game/Patchwork/Blueprints/AI/Needs/Need.Need_C|GetNeedMeter _array_element))
          (LocalVariables|SetSecondBestNeed _array_element)))))
  (Class|BlackboardComponent|SetValueasClass (AI|GetBlackboard 0) (Variables|BBKeys|GetTopNeedKeyName) (Utilities|GetClass (LocalVariables|GetTopNeed))))