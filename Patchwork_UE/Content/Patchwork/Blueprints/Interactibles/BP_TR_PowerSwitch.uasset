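; BP_TR_PowerSwitch is an interactable switch that disables power for one numbered sector.
; SectorSwitch indexes the Params array for a name that serves as both world event name and material parameter collection scalar.
; Interacting invokes that event through GM_BaseGameMode and zeroes the scalar, with no path to switch power back on.
; LoadEvent restores the scalar to off or on according to whether the event has occurred.
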(event EventBeginPlay
  (bind _asgm_base_game_mode (Utilities|Casting|CastToGM_BaseGameMode (Game|GetGameMode)))
  (Variables|Default|SetAs%20GM%20Base%20Game%20Mode _asgm_base_game_mode))

(event EventLoadEvent
  (params (occured :type Boolean))
  (if occured
    (Utilities|SetPower 0.0)
    (else
      (Utilities|SetPower 1.0))))

(event EventOnInteract
  (bind _event_name (CallFunction|GetEventName))
  (Default|InvokeWorldEvent (Variables|Default|GetAs%20GM%20Base%20Game%20Mode) _event_name)
  (Utilities|SetPower 0.0))

(fn ConstructionScript)

(fn GetInteractMessage
  (return (Utilities|Text|FormatText "Disable Sector {0} power" (+ (Variables|Default|Getsector%20switch) 1))))

(fn GetEventName
  (return (Utilities|Array|Get(acopy) (Variables|Default|Getparams) (Variables|Default|Getsector%20switch))))