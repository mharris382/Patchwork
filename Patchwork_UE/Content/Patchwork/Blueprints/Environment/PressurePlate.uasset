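; Pressure plate that lowers under the player or physics objects above a mass threshold and fires pressed/depressed calls when its movement finishes.
; Box overlap events re-check occupants, counting only gravity-enabled, simulating components; a qualifying player pawn component triggers it regardless of mass.
; A timeline slides the plate, with paired DoOnce gates preventing retriggers.
; Unless StayPressed is set, release waits a delay and reverses only if not re-pressed.
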(event OnComponentBeginOverlap(Box)
  (params (OverlappedComponent :type Primitive%20Component%20Object%20Reference) (OtherActor :type Actor%20Object%20Reference) (OtherComp :type Primitive%20Component%20Object%20Reference) (OtherBodyIndex :type Integer) (bFromSweep :type Boolean) (SweepResult :type Hit%20Result%20Structure%20%28by%20ref%29))
  (CallFunction|CheckforHits))

(event OnComponentEndOverlap(Box)
  (params (OverlappedComponent :type Primitive%20Component%20Object%20Reference) (OtherActor :type Actor%20Object%20Reference) (OtherComp :type Primitive%20Component%20Object%20Reference) (OtherBodyIndex :type Integer))
  (CallFunction|CheckforHits))

(event Custom|Depress%20Plate
  (Utilities|FlowControl|Sequence
    (:then_0
      (Utilities|FlowControl|DoOnce true
        (:Completed
          (if (not (Variables|Default|GetStay%20Pressed))
            (Variables|Default|Setis%20pressed false)
            (Utilities|FlowControl|Delay (Variables|Default|GetDepress%20Delay))
            (if (not (Variables|Default|Getis%20pressed))
              (bind _plate (Timeline|Move%20Plate Reverse)
                (:Update
                  (Transformation|SetRelativeLocation (Variables|Default|GetPlate) (Math|Vector|Lerp(Vector) "0, 0, 0" "0.000000,0.000000,-23.393456" _plate) false false))
                (:Finished
                  (if (Variables|Default|Getis%20pressed)
                    (Default|CallOnPressed)
                    (else
                      (Default|CallOnDepressed))))))))))
    (:then_1
      (Utilities|FlowControl|DoOnce false) ; enters at Reset
    )))

(event Custom|Press%20Plate
  (Utilities|FlowControl|Sequence
    (:then_0
      (Utilities|FlowControl|DoOnce false
        (:Completed
          (Variables|Default|Setis%20pressed true)
          (bind _plate (Timeline|Move%20Plate Play)
            (:Update
              (Transformation|SetRelativeLocation (Variables|Default|GetPlate) (Math|Vector|Lerp(Vector) "0, 0, 0" "0.000000,0.000000,-23.393456" _plate) false false))
            (:Finished
              (if (Variables|Default|Getis%20pressed)
                (Default|CallOnPressed)
                (else
                  (Default|CallOnDepressed))))))))
    (:then_1
      (Utilities|FlowControl|DoOnce true) ; enters at Reset
    )))

(event EventBeginPlay)

(event Collision|EventActorBeginOverlap
  (params (OtherActor :type Actor%20Object%20Reference)))

(event EventTick
  (params (DeltaSeconds :type Float%20%28single-precision%29)))

(fn ConstructionScript)

(fn CheckforHits
  (bind _box (Variables|Default|GetBox))
  (bind _outoverlappingcomponents (Class|PrimitiveComponent|GetOverlappingComponents _box))
  (if (> (Utilities|Array|Length _outoverlappingcomponents) 0)
    (LocalVariables|Settotal%20mass 0.0)
    (for _array_element _outoverlappingcomponents
      (if (and (Class|PrimitiveComponent|IsGravityEnabled _array_element) (Class|SceneComponent|IsAnySimulatingPhysics _array_element))
        (if (== (Components|GetOwner _array_element) (Game|Player|GetPlayerPawn 0))
          (CallFunction|PressPlate :!label _label)
          (return)
          (else
            (LocalVariables|Settotal%20mass (+ (Physics|GetMass _array_element) (LocalVariables|Gettotal%20mass)))
            (if (> (LocalVariables|Gettotal%20mass) (Variables|Default|GetMass%20Threshold))
              (goto _label))))))
    (CallFunction|DepressPlate)
    (else
      (CallFunction|DepressPlate))))