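; BP_PCG_BuildingCutter is a cube gizmo actor that tags itself as a building cutter, judging by its name for PCG buildings.
; Its construction script rebuilds the actor Tags from a floor-removal option and a wall mode of Eraser, Door, Window or Reactive.
; A dynamic material instance colors the cube by wall mode.
; The actor does no cutting itself and has no runtime logic.
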(event EventBeginPlay)

(event Collision|EventActorBeginOverlap
  (params (OtherActor :type Actor%20Object%20Reference)))

(event EventTick
  (params (DeltaSeconds :type Float%20%28single-precision%29)))

(fn ConstructionScript
  (bind _tags (Variables|Actor|GetTags))
  (bind _cube (Variables|Default|GetCube))
  (Utilities|FlowControl|Sequence
    (:then_0
      (bind _returnvalue (Rendering|Material|CreateDynamicMaterialInstance _cube 0 (Rendering|Material|GetMaterial _cube 0) "None" :!class /Script/Engine.PrimitiveComponent))
      (LocalVariables|SetCubeGizmo _returnvalue))
    (:then_1
      (Utilities|FlowControl|Sequence
        (:then_0
          (CallFunction|UpdateTag false "RemoveWalls"))
        (:then_1
          (if (Variables|Default|GetRemoveFloors)
            (Utilities|Array|Add (LocalVariables|Gettmp) (LocalVariables|GetRemoveFloorsTag))))
        (:then_2
          (if (Variables|Default|GetAffectWalls)
            (Utilities|Array|Add (LocalVariables|Gettmp) (Utilities|String|StringToName (Utilities|String|Append "Wall_" (Utilities|Select :Index (Variables|Default|GetWallMode) :NewEnumerator0 "Eraser" :NewEnumerator1 "Door" :NewEnumerator2 "Window" :NewEnumerator3 "Smart"))))))
        (:then_3
          (Utilities|Array|Clear _tags)
          (for _array_element (LocalVariables|Gettmp)
            (Utilities|Array|Add _tags _array_element)))
        (:then_4
          (Rendering|Material|SetVectorParameterValue (LocalVariables|GetCubeGizmo) "Color" (Utilities|Select :Index (Variables|Default|GetWallMode) :NewEnumerator0 "(R=1.000000,G=0.247059,B=0.929412,A=1.000000)" :NewEnumerator1 "(R=0.123627,G=1.000000,B=0.000000,A=1.000000)" :NewEnumerator2 "(R=0.000000,G=1.000000,B=0.950841,A=1.000000)" :NewEnumerator3 "(R=1.000000,G=0.032526,B=0.000000,A=1.000000)") :!class /Script/Engine.MaterialInstanceDynamic))))))

(fn UpdateTag
  (params (HasTag :type Boolean) (TagName :type Name))
  (if HasTag
    (Utilities|Array|AddUnique (Variables|Actor|GetTags) TagName)
    (else
      (Utilities|Array|RemoveItem (Variables|Actor|GetTags) TagName))))